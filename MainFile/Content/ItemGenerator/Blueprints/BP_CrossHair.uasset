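; BP_CrossHair is a HUD that draws a small dot crosshair at the center of the screen.
; Each DrawHUD reads IsLookingAtItems from the player's BP_FirstPersonCharacter to pick the dot's color, green when looking at items and near-white otherwise.
; The dot is a tiny DrawRect placed at half the screen size, and nothing is drawn if the character cast fails.
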(event EventBeginPlay)

(event Collision|EventActorBeginOverlap
  (params (OtherActor :type Actor%20Object%20Reference)))

(event EventTick
  (params (DeltaSeconds :type Float%20%28single-precision%29)))

(event EventDrawHUD
  (params (SizeX :type Integer) (SizeY :type Integer))
  (bind _asbp_first_person_character (Utilities|Casting|CastToBP_FirstPersonCharacter (Game|GetPlayerCharacter 0)))
  (if (Variables|/Game/ItemGenerator/Blueprints/BP_FirstPersonCharacter.BP_FirstPersonCharacter_C|GetIsLookingAtItems _asbp_first_person_character)
    (Variables|Default|SetColor "(R=0.104527,G=1.000000,B=0.000000,A=1.000000)")
    (else
      (Variables|Default|SetColor "(R=0.962442,G=1.000000,B=0.978911,A=1.000000)")))
  (HUD|DrawRect (Variables|Default|GetColor) (Math|Conversions|ToFloat(Integer) (/ SizeX 2)) (Math|Conversions|ToFloat(Integer) (/ SizeY 2)) 3.0 3.0))

(fn ConstructionScript)