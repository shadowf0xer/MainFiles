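; BP_WeaponActor is a dropped weapon item, shown as an item bag, that signals its rarity visually.
; On BeginPlay a timeline scales the capsule up from nearly zero so the bag grows in when it spawns.
; Every Tick switches on WeaponStats.WeaponRarity to recolor the particle system and point light.
; An unconnected node can apply WeaponStats.WeaponModel for unique meshes but never runs, and the overlap event is empty.
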(event EventBeginPlay
  ;[1 1 1] This makes the item bag scale up over time so it's smaller when it spawns.
  (bind _scale (Timeline|Timeline_0 PlayFromStart)
    (:Update
      (Transformation|SetRelativeScale3D (Variables|Default|GetCapsule) (Math|Vector|MakeVector (Math|Float|Lerp 0.01 0.15 _scale) (Math|Float|Lerp 0.01 0.15 _scale) (Math|Float|Lerp 0.01 0.15 _scale))))))

(event Collision|EventActorBeginOverlap
  (params (OtherActor :type Actor%20Object%20Reference)))

(event EventTick
  (params (DeltaSeconds :type Float%20%28single-precision%29))
  ;[1 1 1] Change particle color based on rarity
  (switch Utilities|FlowControl|Switch|SwitchonE_ItemRarity (.weaponrarity (Variables|Default|GetWeaponStats))
    (:NewEnumerator0
      (Effects|Components|ParticleSystem|SetColorParameter (Variables|Default|GetParticleSystem) "InstanceColorScaleOverLife" "(R=0.860914,G=0.880000,B=0.824241,A=1.000000)")
      (Rendering|Components|Light|SetLightColor (Variables|Default|GetPointLight) "(R=1.000000,G=1.000000,B=1.000000,A=1.000000)" true))
    (:NewEnumerator1
      (Effects|Components|ParticleSystem|SetColorParameter (Variables|Default|GetParticleSystem) "InstanceColorScaleOverLife" "(R=0.009350,G=0.935000,B=0.051548,A=1.000000)")
      (Rendering|Components|Light|SetLightColor (Variables|Default|GetPointLight) "(R=0.009350,G=0.935000,B=0.051548,A=1.000000)" true))
    (:NewEnumerator2
      (Effects|Components|ParticleSystem|SetColorParameter (Variables|Default|GetParticleSystem) "InstanceColorScaleOverLife" "(R=0.000000,G=0.276693,B=0.880000,A=1.000000)")
      (Rendering|Components|Light|SetLightColor (Variables|Default|GetPointLight) "(R=0.000000,G=0.276693,B=0.880000,A=1.000000)" true))
    (:NewEnumerator3
      (Effects|Components|ParticleSystem|SetColorParameter (Variables|Default|GetParticleSystem) "InstanceColorScaleOverLife" "(R=0.615000,G=0.043050,B=0.537894,A=1.000000)")
      (Rendering|Components|Light|SetLightColor (Variables|Default|GetPointLight) "(R=0.615000,G=0.043050,B=0.537894,A=1.000000)" true))
    (:NewEnumerator4
      (Effects|Components|ParticleSystem|SetColorParameter (Variables|Default|GetParticleSystem) "InstanceColorScaleOverLife" "(R=0.880000,G=0.209236,B=0.004400,A=1.000000)")
      (Rendering|Components|Light|SetLightColor (Variables|Default|GetPointLight) "(R=0.880000,G=0.209236,B=0.004400,A=1.000000)" true))))

(fn ConstructionScript)