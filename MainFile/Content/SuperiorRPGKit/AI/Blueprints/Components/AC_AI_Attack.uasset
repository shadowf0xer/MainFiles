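; AI component that holds an NPC's combat settings and state for melee, ranged and support actions.
; Initialize copies the general, melee, ranged and support configs into attack radii, tolerances, frequencies, angles and behavior flags.
; Each action type has a timer-based cooldown, with an active cooldown detected by timer handle validity.
; Setters notify on active attack type changes and keep attack and support stances mutually exclusive.
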(event Custom|Initialize
  (params (GeneralConfig :type S%20AI%20Config%20Combat%20General%20Structure) (MeleeConfig :type S%20AI%20Config%20Combat%20Melee%20Structure) (RangedConfig :type S%20AI%20Config%20Combat%20Ranged%20Structure) (SupportConfig :type S%20AI%20Config%20Combat%20Support%20Structure))
  (bind (_combattype _meleetorangedswitchdistance _prioritizesupport _ignorecombat) (Utilities|Struct|BreakS_AI_Config_CombatGeneral GeneralConfig))
  (bind (_attackradius _distancetolerance _attackfrequency _acceptanceangle) (Utilities|Struct|BreakS_AI_Config_CombatMelee MeleeConfig))
  (bind (_attackradius_2 _distancetolerance_2 _attackfrequency_2 _acceptanceangle_2) (Utilities|Struct|BreakS_AI_Config_CombatRanged RangedConfig))
  (bind (_supportradius _distancetolerance_3 _castfrequency _acceptanceangle_3) (Utilities|Struct|BreakS_AI_Config_CombatSupport SupportConfig))
  (Variables|ConfigGeneral|SetCombatType _combattype)
  (Variables|ConfigGeneral|SetMeleeToRangedSwitchDistance _meleetorangedswitchdistance)
  (Variables|ConfigGeneral|SetPrioritizeSupport _prioritizesupport)
  (Variables|ConfigGeneral|SetIgnoreCombat _ignorecombat)
  (Variables|ConfigMelee|SetMeleeAttackRadius _attackradius)
  (Variables|ConfigMelee|SetMeleeAttackDistanceTolerance _distancetolerance)
  (Variables|ConfigMelee|SetMeleeAttackFrequency _attackfrequency)
  (Variables|ConfigMelee|SetMeleeAttackAcceptanceAngle _acceptanceangle)
  (Variables|ConfigRanged|SetRangedAttackRadius _attackradius_2)
  (Variables|ConfigRanged|SetRangedAttackDistanceTolerance _distancetolerance_2)
  (Variables|ConfigRanged|SetRangedAttackFrequency _attackfrequency_2)
  (Variables|ConfigRanged|SetRangedAttackAcceptanceAngle _acceptanceangle_2)
  (Variables|ConfigSupport|SetSupportCastRadius _supportradius)
  (Variables|ConfigSupport|SetSupportDistanceTolerance _distancetolerance_3)
  (Variables|ConfigSupport|SetSupportCastFrequency _castfrequency)
  (Variables|ConfigSupport|SetSupportAcceptanceAngle _acceptanceangle_3))

(event Custom|ActivateRangedCooldown
  (params (CooldownTime :type Float%20%28single-precision%29))
  (bind _returnvalue (Utilities|Time|SetTimerbyEvent (delegate Custom|ResetRangedAttack) CooldownTime))
  (Variables|Default|SetRangedCooldownTimer _returnvalue))

(event Custom|ResetRangedAttack
  (Utilities|Time|ClearandInvalidateTimerbyHandle (Variables|Default|GetRangedCooldownTimer)))

(event Custom|ActivateSupportCooldown
  (params (CooldownTime :type Float%20%28single-precision%29))
  (bind _returnvalue (Utilities|Time|SetTimerbyEvent (delegate Custom|ResetSupportAction) CooldownTime))
  (Variables|Default|SetSupportCooldownTimer _returnvalue))

(event Custom|ResetSupportAction
  (Utilities|Time|ClearandInvalidateTimerbyHandle (Variables|Default|GetSupportCooldownTimer)))

(event Custom|ActivateMeleeCooldown
  (params (CooldownTime :type Float%20%28single-precision%29))
  (bind _returnvalue (Utilities|Time|SetTimerbyEvent (delegate Custom|ResetMeleeAttack) CooldownTime))
  (Variables|Default|SetMeleeCooldownTimer _returnvalue))

(event Custom|ResetMeleeAttack
  (Utilities|Time|ClearandInvalidateTimerbyHandle (Variables|Default|GetMeleeCooldownTimer)))

(fn IsMeleeCooldownActive
  (return (Utilities|Time|IsValidTimerHandle (Variables|Default|GetMeleeCooldownTimer))))

(fn IsRangedCooldownActive
  (return (Utilities|Time|IsValidTimerHandle (Variables|Default|GetRangedCooldownTimer))))

(fn GetActiveAttackType
  (return (Variables|Default|GetActiveAttackType)))

(fn SetActiveAttackType
  (params (NewAttackType :type E_AI_AttackType%20Enum :default "NewEnumerator0"))
  (if (Utilities|Enum|NotEqual(Enum) NewAttackType (Variables|Default|GetActiveAttackType))
    (Variables|Default|SetActiveAttackType NewAttackType)
    (Default|CallOnActiveAttackTypeChanged (Variables|Default|GetActiveAttackType))))

(fn GetCombatType
  (return (Variables|ConfigGeneral|GetCombatType)))

(fn SetCombatType
  (params (CombatType :type E_AI_CombatType%20Enum :default "NewEnumerator0"))
  (if (Utilities|Enum|NotEqual(Enum) CombatType (Variables|ConfigGeneral|GetCombatType))
    (Variables|ConfigGeneral|SetCombatType CombatType)))

(fn GetSwitchDistance
  (return (Variables|ConfigGeneral|GetMeleeToRangedSwitchDistance)))

(fn IsSupportCooldownActive
  (return (Utilities|Time|IsValidTimerHandle (Variables|Default|GetSupportCooldownTimer))))

(fn SetIsinAttackStance
  (params (Active :type Boolean))
  (if Active
    (Variables|Default|SetInAttackStance true)
    (Variables|Default|SetInSupportStance false)
    (else
      (Variables|Default|SetInAttackStance false))))

(fn SetIsinSupportStance
  (params (Active :type Boolean))
  (if Active
    (Variables|Default|SetInSupportStance true)
    (Variables|Default|SetInAttackStance false)
    (else
      (Variables|Default|SetInSupportStance false))))

(fn GetIsinAttackStance
  (return (Variables|Default|GetInAttackStance)))

(fn GetIsinSupportStance
  (return (Variables|Default|GetInSupportStance)))

(fn IsIgnoringCombat
  (return (Variables|ConfigGeneral|GetIgnoreCombat)))