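; AI component in SuperiorRPGKit that tracks an AI's current interaction target and interaction state.
; Setters store a new value and fire a change event only when it differs from the current one, with getters exposing both values.
; IsInteracting reports whether the state matches one specific enum entry, and BeginPlay and Tick are unused.
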(event EventBeginPlay)

(event EventTick
  (params (DeltaSeconds :type Float%20%28single-precision%29)))

(fn GetInteractionTarget
  (return (Variables|Private|GetInteractionTarget)))

(fn SetInteractionTarget
  (params (NewInteractionTarget :type Actor%20Object%20Reference))
  (if (!= NewInteractionTarget (Variables|Private|GetInteractionTarget))
    (Variables|Private|SetInteractionTarget NewInteractionTarget)
    (Default|CallOnInteractionTargetChanged (Variables|Private|GetInteractionTarget))))

(fn GetInteractionState
  (return (Variables|Private|GetInteractionState)))

(fn SetInteractionState
  (params (NewInteractionResult :type E_AI_InteractionState%20Enum :default "NewEnumerator3"))
  (if (Utilities|Enum|NotEqual(Enum) NewInteractionResult (Variables|Private|GetInteractionState))
    (bind _output_get (Variables|Private|SetInteractionState NewInteractionResult))
    (Default|CallOnInteractionResultChanged _output_get)))

(fn IsInteracting
  (return (Utilities|Enum|Equal(Enum) (Variables|Private|GetInteractionState) "NewEnumerator2")))