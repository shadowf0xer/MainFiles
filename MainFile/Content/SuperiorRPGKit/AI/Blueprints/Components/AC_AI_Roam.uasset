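; Actor component that handles AI roaming, storing the radius, break duration range and threshold supplied through a roam config.
; It picks random reachable navigation points around a location or actor, caches the result as the target location and broadcasts the change.
; It also tracks a focus point and focus actor, broadcasting only on change, and notifies the owner's AI controller when the focus actor changes.
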(event Custom|Initialize
  (params (RoamConfig :type S%20AI%20Config%20Roam%20Structure))
  (bind (_radius _breakdurationmin _breakdurationmax _threshold) (Utilities|Struct|BreakS_AI_Config_Roam RoamConfig))
  (Variables|Private|Config|SetRadius _radius)
  (Variables|Private|Config|SetBreakDurationMin _breakdurationmin)
  (Variables|Private|Config|SetBreakDurationMax _breakdurationmax)
  (Variables|Private|Config|SetThreshold _threshold))

(fn FindRandomRoamPoint(AroundLocation)
  (params (Location :type Vector))
  (bind (_success _reachablepoint) (Finders|FindReachablePointinRoamRadius Location))
  (if _success
    (bind _output_get (Variables|Private|SetTargetLocation _reachablepoint))
    (Default|CallOnTargetLocationChanged _output_get)
    (return true (Variables|Private|GetTargetLocation))))

(fn GetRandomBreakDuration
  (return (Math|Random|RandomFloatinRange (Variables|Private|Config|GetBreakDurationMin) (Variables|Private|Config|GetBreakDurationMax))))

(fn GetFocusPoint
  (return (Variables|Private|GetFocusPoint)))

(fn SetFocusPoint
  (params (NewFocusPoint :type Vector))
  (if (Math|Vector|NotEqual(Vector) NewFocusPoint (Variables|Private|GetFocusPoint) 0.0001)
    (Variables|Private|SetFocusPoint NewFocusPoint)
    (Default|CallOnFocusPointChanged (Variables|Private|GetFocusPoint))))

(fn GetFocusActor
  (return (Variables|Private|GetFocusActor)))

(fn SetFocusActor
  (params (NewFocusActor :type Actor%20Object%20Reference))
  (if (!= NewFocusActor (Variables|Private|GetFocusActor))
    (bind _output_get (Variables|Private|SetFocusActor NewFocusActor))
    (Default|CallOnFocusActorChanged _output_get)
    (Class|BPIAIEvents|OnFollowTargetChanged(Message) (AI|GetAIController (Components|GetOwner)) (Getters|GetFocusActor))))

(fn FindRandomRoamPoint(AroundActor)
  (params (Actor :type Actor%20Object%20Reference))
  (Utilities|IsValid Actor
    (:Is%20Valid
      (bind (_success _reachablepoint) (Finders|FindReachablePointinRoamRadius (Transformation|GetActorLocation Actor)))
      (if _success
        (bind _output_get (Variables|Private|SetTargetLocation _reachablepoint))
        (Default|CallOnTargetLocationChanged _output_get)
        (return true (Variables|Private|GetTargetLocation))))))

(fn FindReachablePointinRoamRadius
  (params (Origin :type Vector))
  (bind _radius (Variables|Private|Config|GetRadius))
  (bind (_randomlocation _returnvalue) (AI|Navigation|GetRandomReachablePointinRadius Origin _radius))
  (return _returnvalue _randomlocation))

(fn GetThreshold
  (return (Variables|Private|Config|GetThreshold)))

(fn GetThresholdSquared
  (return (Math|Float|Square (Variables|Private|Config|GetThreshold))))