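; AI targeting component that tracks hostile and friendly actors around its owner and chooses whom to attack or support.
; Sphere-overlap results are filtered by configured classes and diffed against current sets, with a deactivation radius governing removal and the pawn notified of changes.
; A threat map drives enemy targeting, and target changes can alert nearby allies to attack.
; The pawn can override enemy and ally selection, which otherwise defaults to highest threat and nearest ally.
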(event Custom|Initialize
  (params (CombatTriggerConfig :type S%20AI%20Config%20Combat%20Trigger%20Structure))
  (bind (_supportenabled _aggresive _searchradius _deactivationradius _hostileclasses _friendlyclasses _objecttypes _callallies) (Utilities|Struct|BreakS_AI_Config_CombatTrigger CombatTriggerConfig))
  (Variables|Private|Config|SetSupportEnabled _supportenabled)
  (Variables|Private|Config|SetAggresive _aggresive)
  (Variables|Private|Config|SetSearchRadius _searchradius)
  (Variables|Private|Config|SetHostileClasses _hostileclasses)
  (Variables|Private|Config|SetFriendlyClasses _friendlyclasses)
  (Variables|Private|Config|SetObjectTypes _objecttypes)
  (Variables|Private|Config|SetDeactivationRadius _deactivationradius)
  (Variables|Private|Config|SetCallAllies _callallies))

(fn RecalculateThreat
  (bind _keys (Utilities|Map|Keys (Variables|Private|GetThreat)))
  (for _array_element _keys
    (Utilities|IsValid _array_element
      (:Is%20Valid
        (if (> (.Value (Utilities|Map|Find (Variables|Private|GetThreat) _array_element)) (LocalVariables|GetHighestThreatLOCAL))
          (LocalVariables|SetHighestThreatLOCAL (.Value (Utilities|Map|Find (Variables|Private|GetThreat) _array_element)))
          (LocalVariables|SetNewTargetLOCAL _array_element)))))
  (Setters|SetTargetedEnemy (LocalVariables|GetNewTargetLOCAL)))

(fn ModifyThreat
  (params (Actor :type Actor%20Object%20Reference) (Threat :type Float%20%28single-precision%29))
  (Utilities|FlowControl|Sequence
    (:then_0
      (if (Utilities|Map|Contains (Variables|Private|GetThreat) Actor)
        (Utilities|Map|Add (Variables|Private|GetThreat) Actor (Math|Float|Max(Float) (+ (.Value (Utilities|Map|Find (Variables|Private|GetThreat) Actor)) Threat) 0.0))
        (else
          (Utilities|Map|Add (Variables|Private|GetThreat) Actor (Math|Float|Max(Float) Threat 0.0))
          (Utilities|Set|Add (Variables|Private|GetEnemiesInRange) Actor))))
    (:then_1
      (if (== (Getters|GetTargetedEnemy) Actor)
        (if (< Threat 0.0)
          (bind (_success _enemy) (Finders|FindEnemywithHighestThreat))
          (if _success
            (Setters|SetTargetedEnemy _enemy)))
        (elif (> (Getters|GetActorThreat Actor) (Getters|GetActorThreat (Getters|GetTargetedEnemy)))
          (Setters|SetTargetedEnemy Actor))))))

(fn SetTargetedEnemy
  (params (NewTargetedEnemy :type Actor%20Object%20Reference))
  (bind _targetedenemy (Getters|GetTargetedEnemy))
  (if (!= NewTargetedEnemy (Variables|Private|GetTargetedEnemy))
    (Variables|Private|SetTargetedEnemy NewTargetedEnemy)
    (Utilities|FlowControl|Sequence
      (:then_0
        (Variables|Private|SetCurrentTargetCapsuleRadius 0.0)
        (Utilities|IsValid _targetedenemy
          (:Is%20Valid
            (bind _ascapsule_collision (Utilities|Casting|CastToCapsuleComponent (Variables|/Script/Engine.Actor|GetRootComponent _targetedenemy)))
            (Variables|Private|SetCurrentTargetCapsuleRadius (Components|Capsule|GetScaledCapsuleRadius _ascapsule_collision)))))
      (:then_1
        (Class|BPIAIEvents|OnTargetedEnemyChanged(Message) (Pawn|GetControlledPawn (AI|GetAIController (Components|GetOwner))) (Getters|GetTargetedEnemy))
        (CallFunction|CallAlliesinRange (Getters|GetTargetedEnemy))))))

(fn GetTargetedEnemy
  (return (Variables|Private|GetTargetedEnemy)))

(fn GetActorThreat
  (params (Actor :type Actor%20Object%20Reference))
  (bind _threat (Variables|Private|GetThreat))
  (bind (_value _returnvalue) (Utilities|Map|Find _threat Actor))
  (if _returnvalue
    (return _value)
    (else
      (return -1.0))))

(fn GetCurrentTargetCapsuleRadius
  (return (Variables|Private|GetCurrentTargetCapsuleRadius)))

(fn GetSearchRadius
  (return (Variables|Private|Config|GetSearchRadius)))

(fn GetSearchRadiusSquared
  (return (Math|Float|Square (Variables|Private|Config|GetSearchRadius))))

(fn SetSearchRadius
  (params (NewSearchRadius :type Float%20%28single-precision%29))
  (if (!= NewSearchRadius (Variables|Private|Config|GetSearchRadius))
    (bind _output_get (Variables|Private|Config|SetSearchRadius NewSearchRadius))
    (Default|CallOnSearchRadiusChanged _output_get)))

(fn IsActorinSearchRadius
  (params (Actor :type Actor%20Object%20Reference))
  (Utilities|IsValid Actor
    (:Is%20Valid
      (return (< (Transformation|GetSquaredDistanceTo Actor (Components|GetOwner)) (Getters|GetSearchRadiusSquared))))))

(fn FindNearestEnemy
  (LocalVariables|SetNearestDistanceSqLOCAL (Getters|GetSearchRadiusSquared))
  (bind _result (Utilities|Set|ToArray (Variables|Private|GetEnemiesInRange)))
  (for _array_element _result
    (bind _output_get (LocalVariables|SetDistanceToTargetSqLOCAL (Transformation|GetSquaredDistanceTo _array_element (Components|GetOwner))))
    (if (< _output_get (LocalVariables|GetNearestDistanceSqLOCAL))
      (LocalVariables|SetNearestDistanceSqLOCAL (LocalVariables|GetDistanceToTargetSqLOCAL))
      (LocalVariables|SetSuccessLOCAL true)
      (LocalVariables|SetTargetLOCAL _array_element)))
  (return (LocalVariables|GetSuccessLOCAL) (LocalVariables|GetTargetLOCAL)))

(fn FindNearestAlly
  (LocalVariables|SetNearestDistanceSqLOCAL (Getters|GetSearchRadiusSquared))
  (bind _result (Utilities|Set|ToArray (Variables|Private|GetAlliesInRange)))
  (for _array_element _result
    (bind _output_get (LocalVariables|SetDistanceToTargetSqLOCAL (Transformation|GetSquaredDistanceTo _array_element (Components|GetOwner))))
    (if (< _output_get (LocalVariables|GetNearestDistanceSqLOCAL))
      (LocalVariables|SetNearestDistanceSqLOCAL (LocalVariables|GetDistanceToTargetSqLOCAL))
      (LocalVariables|SetSuccessLOCAL true)
      (LocalVariables|SetTargetLOCAL _array_element)))
  (return (LocalVariables|GetSuccessLOCAL) (LocalVariables|GetTargetLOCAL)))

(fn FindRandomEnemy
  (if (> (Utilities|Set|Length (Variables|Private|GetEnemiesInRange)) 0)
    (bind _result (Utilities|Set|ToArray (Variables|Private|GetEnemiesInRange)))
    (return true (Utilities|Array|Get(acopy) _result (Math|Random|RandomIntegerinRange 0 (Utilities|Array|LastIndex _result))))
    (else
      (return false 0))))

(fn FindRandomAlly
  (if (> (Utilities|Set|Length (Variables|Private|GetAlliesInRange)) 0)
    (bind _result (Utilities|Set|ToArray (Variables|Private|GetAlliesInRange)))
    (return true (Utilities|Array|Get(acopy) _result (Math|Random|RandomIntegerinRange 0 (Utilities|Array|LastIndex _result))))
    (else
      (return false 0))))

(fn FindEnemywithHighestThreat
  (bind _keys (Utilities|Map|Keys (Variables|Private|GetThreat)))
  (for _array_element _keys
    (if (>= (.Value (Utilities|Map|Find (Variables|Private|GetThreat) _array_element)) (LocalVariables|GetCurrentHighestThreatLOCAL))
      (LocalVariables|SetCurrentHighestThreatLOCAL (.Value (Utilities|Map|Find (Variables|Private|GetThreat) _array_element)))
      (LocalVariables|SetEnemyWithHighestThreatLOCAL _array_element)
      (LocalVariables|SetSuccessLOCAL true)))
  (return (LocalVariables|GetSuccessLOCAL) (LocalVariables|GetEnemyWithHighestThreatLOCAL)))

(fn GetDeactivationRadius
  (return (Variables|Private|Config|GetDeactivationRadius)))

(fn GetDeactivationRadiusSquared
  (return (Math|Float|Square (Variables|Private|Config|GetDeactivationRadius))))

(fn SetDeactivationRadius
  (params (NewDeactivationRadius :type Float%20%28single-precision%29))
  (if (!= NewDeactivationRadius (Variables|Private|Config|GetDeactivationRadius))
    (bind _output_get (Variables|Private|Config|SetDeactivationRadius NewDeactivationRadius))
    (Default|CallOnDeactivationRadiusChanged _output_get)))

(fn IsActorinDeactivationRadius
  (params (Actor :type Actor%20Object%20Reference))
  (Utilities|IsValid Actor
    (:Is%20Valid
      (return (< (Transformation|GetSquaredDistanceTo Actor (Components|GetOwner)) (Getters|GetDeactivationRadiusSquared))))))

(fn UpdateEnemiesinRange
  (params (ActorsToCheck :type Array%20of%20Actor%20Object%20References))
  (Utilities|FlowControl|Sequence
    (:then_0
      (for _array_element ActorsToCheck
        (if (Conditions|IsActorHostile _array_element)
          (bind _result (Class|BPIRPGCombat|CanbeTargeted(Message) _array_element))
          (if _result
            (Utilities|Set|Add (LocalVariables|GetNewHostileActorsInRangeLOCAL) _array_element)))))
    (:then_1
      (bind _result_2 (Utilities|Set|Intersection (LocalVariables|GetNewHostileActorsInRangeLOCAL) (Variables|Private|GetEnemiesInRange))) ; Returns hostile actors that haven't change.
      (bind _result_3 (Utilities|Set|Difference (Variables|Private|GetEnemiesInRange) _result_2)) ; Returns hostile actors that are no longer in the range.
      (bind _result_4 (Utilities|Set|Difference (LocalVariables|GetNewHostileActorsInRangeLOCAL) _result_2)) ; Returns new hostile actors that are in the range.
      (bind _result_5 (Utilities|Set|Union (Variables|Private|GetEnemiesInRange) (LocalVariables|GetNewHostileActorsInRangeLOCAL)))
      (Variables|Private|SetEnemiesInRange _result_5)
      (Utilities|FlowControl|Sequence
        (:then_0
          (bind _result_6 (Utilities|Set|ToArray _result_3))
          (for _array_element_2 _result_6
            (Utilities|IsValid _array_element_2
              (:Is%20Valid
                (bind _result_7 (Class|BPIRPGCombat|CanbeTargeted(Message) _array_element_2))
                (if (or (not _result_7) (not (Conditions|IsActorinDeactivationRadius _array_element_2)))
                  (Utilities|Map|Remove (Variables|Private|GetThreat) _array_element_2)
                  (Utilities|Set|Remove (Variables|Private|GetEnemiesInRange) _array_element_2)
                  (Class|BPIAIEvents|OnEnemyBeyondRange(Message) (Pawn|GetControlledPawn (AI|GetAIController (Components|GetOwner))) _array_element_2)))
              (:Is%20Not%20Valid
                (Utilities|Map|Remove (Variables|Private|GetThreat) _array_element_2)
                (Utilities|Set|Remove (Variables|Private|GetEnemiesInRange) _array_element_2)))))
        (:then_1
          (bind _result_8 (Utilities|Set|ToArray _result_4))
          (for _array_element_3 _result_8
            (Utilities|Map|Add (Variables|Private|GetThreat) _array_element_3 0.0)
            (Class|BPIAIEvents|OnEnemyinRange(Message) (Pawn|GetControlledPawn (AI|GetAIController (Components|GetOwner))) _array_element_3)))))))

(fn GetActorsinSearchRadius
  (bind (_outactors _returnvalue) (Collision|SphereOverlapActors (Transformation|GetActorLocation (Components|GetOwner)) (Getters|GetSearchRadius) (Variables|Private|Config|GetObjectTypes) 0 (Variables|Private|Config|GetIgnoredActors)))
  (return _returnvalue _outactors))

(fn UpdateAlliesinRange
  (params (ActorsToCheck :type Array%20of%20Actor%20Object%20References))
  (Utilities|FlowControl|Sequence
    (:then_0
      (for _array_element ActorsToCheck
        (if (Conditions|IsActorFriendly _array_element)
          (bind _result (Class|BPIRPGCombat|CanbeTargeted(Message) _array_element))
          (if _result
            (Utilities|Set|Add (LocalVariables|GetNewFriendlyActorsInRangeLOCAL) _array_element)))))
    (:then_1
      (bind _result_2 (Utilities|Set|Intersection (LocalVariables|GetNewFriendlyActorsInRangeLOCAL) (Variables|Private|GetAlliesInRange))) ; Returns friendly actors that haven't change.
      (bind _result_3 (Utilities|Set|Difference (Variables|Private|GetAlliesInRange) _result_2)) ; Returns friendly actors that are no longer in the range.
      (bind _result_4 (Utilities|Set|Difference (LocalVariables|GetNewFriendlyActorsInRangeLOCAL) _result_2)) ; Returns new friendly actors that are in the range.
      (bind _result_5 (Utilities|Set|Union (Variables|Private|GetAlliesInRange) (LocalVariables|GetNewFriendlyActorsInRangeLOCAL)))
      (Variables|Private|SetAlliesInRange _result_5)
      (Utilities|FlowControl|Sequence
        (:then_0
          (bind _result_6 (Utilities|Set|ToArray _result_3))
          (for _array_element_2 _result_6
            (Utilities|IsValid _array_element_2
              (:Is%20Valid
                (bind _result_7 (Class|BPIRPGCombat|CanbeTargeted(Message) _array_element_2))
                (if (or (not _result_7) (not (Conditions|IsActorinDeactivationRadius _array_element_2)))
                  (Utilities|Set|Remove (Variables|Private|GetAlliesInRange) _array_element_2)
                  (Class|BPIAIEvents|OnAllyBeyondRange(Message) (Pawn|GetControlledPawn (AI|GetAIController (Components|GetOwner))) _array_element_2)))
              (:Is%20Not%20Valid
                (Utilities|Set|Remove (Variables|Private|GetAlliesInRange) _array_element_2)))))
        (:then_1
          (bind _result_8 (Utilities|Set|ToArray _result_4))
          (for _array_element_3 _result_8
            (Class|BPIAIEvents|OnAllyinRange(Message) (Pawn|GetControlledPawn (AI|GetAIController (Components|GetOwner))) _array_element_3)))))))

(fn GetTargetedAlly
  (return (Variables|Private|GetTargetedAlly)))

(fn SetTargetedAlly
  (params (NewTargetedAlly :type Actor%20Object%20Reference))
  (bind _targetedally (Getters|GetTargetedAlly))
  (bind _targetedally_2 (Getters|GetTargetedAlly))
  (if (!= NewTargetedAlly (Variables|Private|GetTargetedAlly))
    (Variables|Private|SetTargetedAlly NewTargetedAlly)
    (Utilities|FlowControl|Sequence
      (:then_0
        (Variables|Private|SetCurrentTargetCapsuleRadius 0.0)
        (Utilities|IsValid _targetedally_2
          (:Is%20Valid
            (bind _ascapsule_collision (Utilities|Casting|CastToCapsuleComponent (Variables|/Script/Engine.Actor|GetRootComponent _targetedally_2)))
            (Variables|Private|SetCurrentTargetCapsuleRadius (Components|Capsule|GetScaledCapsuleRadius _ascapsule_collision)))))
      (:then_1
        (Class|BPIAIEvents|OnTargetedAllyChanged(Message) (Pawn|GetControlledPawn (AI|GetAIController (Components|GetOwner))) (Getters|GetTargetedAlly))
        (Utilities|IsValid _targetedally
          (:Is%20Valid
            (Utilities|Set|Add (Variables|Private|GetAlliesInRange) _targetedally)))))))

(fn GetIsinCombat
  (return (Variables|Default|GetInCombat)))

(fn SetIsinCombat
  (params (InCombat :type Boolean))
  (Variables|Default|SetInCombat InCombat))

(fn GetEnemiesinRange
  (return (Variables|Private|GetEnemiesInRange)))

(fn GetAlliesinRange
  (return (Variables|Private|GetAlliesInRange)))

(fn FindAllytoSupport
  (if (Variables|Private|Config|GetSupportEnabled)
    (bind (_overridden _success _allytosupport) (Class|BPIAIActions|GenerateAllytoSupport(Message) (Pawn|GetControlledPawn (AI|GetAIController (Components|GetOwner))) (Variables|Private|GetAlliesInRange)))
    (if _overridden
      (return _success _allytosupport)
      (else
        (bind (_success_2 _nearestally) (Finders|FindNearestAlly))
        (return _success_2 _nearestally)))))

(fn FindEnemytoAttack
  (bind (_overridden _success _enemytoattack) (Class|BPIAIActions|GenerateEnemytoAttack(Message) (Pawn|GetControlledPawn (AI|GetAIController (Components|GetOwner))) (Variables|Private|GetEnemiesInRange)))
  (if _overridden
    (return _success _enemytoattack)
    (else
      (bind (_success_2 _enemy) (Finders|FindEnemywithHighestThreat))
      (return _success_2 _enemy))))

(fn CallAlliesinRange
  (params (AttackTarget :type Actor%20Object%20Reference))
  (if (Variables|Private|Config|GetCallAllies)
    (bind _result (Utilities|Set|ToArray (Variables|Private|GetAlliesInRange)))
    (for _array_element _result
      (Class|BPIAICommands|Attack(Message) (AI|GetAIController _array_element) AttackTarget false))))

(fn IsActorHostile
  (params (Actor :type Actor%20Object%20Reference))
  (bind _returnvalue (Utilities|GetClass Actor))
  (bind _array_element (Utilities|Array|ForEachLoopwithBreak (Variables|Private|Config|GetHostileClasses) :!label _label)
    (:LoopBody
      (if (.IncludeChildrenClasses (Utilities|Struct|BreakS_AI_ClassConfig _array_element))
        (if (Utilities|ClassIsChildOf _returnvalue (.Class (Utilities|Struct|BreakS_AI_ClassConfig _array_element)))
          (LocalVariables|SetResultLOCAL true)
          (goto _label Break))
        (elif (== (.Class (Utilities|Struct|BreakS_AI_ClassConfig _array_element)) _returnvalue)
          (LocalVariables|SetResultLOCAL true)
          (goto _label Break))))
    (:Completed
      (return (LocalVariables|GetResultLOCAL)))))

(fn IsActorFriendly
  (params (Actor :type Actor%20Object%20Reference))
  (bind _returnvalue (Utilities|GetClass Actor))
  (bind _array_element (Utilities|Array|ForEachLoopwithBreak (Variables|Private|Config|GetFriendlyClasses) :!label _label)
    (:LoopBody
      (if (.IncludeChildrenClasses (Utilities|Struct|BreakS_AI_ClassConfig _array_element))
        (if (Utilities|ClassIsChildOf _returnvalue (.Class (Utilities|Struct|BreakS_AI_ClassConfig _array_element)))
          (LocalVariables|SetResultLOCAL true)
          (goto _label Break))
        (elif (== (.Class (Utilities|Struct|BreakS_AI_ClassConfig _array_element)) _returnvalue)
          (LocalVariables|SetResultLOCAL true)
          (goto _label Break))))
    (:Completed
      (return (LocalVariables|GetResultLOCAL)))))