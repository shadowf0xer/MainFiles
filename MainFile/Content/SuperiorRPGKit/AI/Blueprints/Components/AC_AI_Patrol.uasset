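; AI patrol component that stores a route of locations, the target point and a configurable random break duration for its owner.
; Setting a route targets the point nearest the owner, which is also the fallback when the target leaves the route.
; Next-point selection supports Loop, Back and Forth, and Random (excluding current) modes without changing the target.
; Setters fire change events, but Back and Forth flips direction directly, skipping its event.
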(event Custom|Initialize
  (params (PatrolConfig :type S%20AI%20Config%20Patrol%20Structure))
  (bind (_breakdurationmin _breakdurationmax) (Utilities|Struct|BreakS_AI_Config_Patrol PatrolConfig))
  (Variables|Private|Config|SetBreakDurationMin _breakdurationmin)
  (Variables|Private|Config|SetBreakDurationMax _breakdurationmax))

(event EventBeginPlay)

(event EventTick
  (params (DeltaSeconds :type Float%20%28single-precision%29)))

(fn SetPatrolRoute
  (params (NewPatrolRoute :type Array%20of%20Vectors))
  (bind _output_get (Variables|Private|SetPatrolRoute NewPatrolRoute))
  (Default|CallOnPatrolRouteChanged _output_get)
  (bind (_success _nearestpatrolpoint) (Finders|FindNearestPatrolPoint (Transformation|GetActorLocation (Components|GetOwner))))
  (if _success
    (Setters|SetTargetPatrolPoint _nearestpatrolpoint)))

(fn GetNextPatrolPoint
  (bind _patrolroute (Variables|Private|GetPatrolRoute))
  (bind _targetpatrolpoint (Variables|Private|GetTargetPatrolPoint))
  (bind _patrolroute_2 (Variables|Private|GetPatrolRoute))
  (bind _targetpatrolpoint_2 (Variables|Private|GetTargetPatrolPoint))
  (bind _patrolroute_3 (Variables|Private|GetPatrolRoute))
  (bind _patrolroute_4 (Variables|Private|GetPatrolRoute))
  (bind _targetpatrolpoint_3 (Variables|Private|GetTargetPatrolPoint))
  (bind _patrolroute_5 (Variables|Private|GetPatrolRoute))
  (bind _targetpatrolpoint_4 (Variables|Private|GetTargetPatrolPoint))
  (bind _returnvalue (Utilities|Array|FindItem _patrolroute _targetpatrolpoint_4))
  (bind _returnvalue_2 (Utilities|Array|FindItem _patrolroute_2 _targetpatrolpoint))
  (bind _returnvalue_3 (Utilities|Array|FindItem _patrolroute_3 _targetpatrolpoint_2))
  (bind _returnvalue_4 (Utilities|Array|FindItem _patrolroute_5 _targetpatrolpoint_3))
  (bind _returnvalue_5 (- _returnvalue_4 1))
  (bind _returnvalue_6 (- _returnvalue_2 1))
  (bind _returnvalue_7 (+ _returnvalue 1))
  (bind _returnvalue_8 (+ _returnvalue_3 1))
  (if (>= (Utilities|Array|Length (Variables|Private|GetPatrolRoute)) 2) ; Patrol route needs to consist of\nat least to patrol points.
    (if (Utilities|Array|ContainsItem (Variables|Private|GetPatrolRoute) (Variables|Private|GetTargetPatrolPoint)) ; Does patrol route still contains\nthe active patrol point.
      (switch Utilities|FlowControl|Switch|SwitchonE_AI_PatrolType (Variables|Private|Config|GetPatrolType)
        (:NewEnumerator0
          (switch Utilities|FlowControl|Switch|SwitchonE_AI_PatrolDirection (Variables|Private|Config|GetDirection)
            (:NewEnumerator0
              (if (Utilities|Array|IsValidIndex (Variables|Private|GetPatrolRoute) _returnvalue_8)
                (return (Utilities|Array|Get(acopy) (Variables|Private|GetPatrolRoute) _returnvalue_8))
                (else
                  (return (Utilities|Array|Get(acopy) (Variables|Private|GetPatrolRoute))))))
            (:NewEnumerator1
              (if (Utilities|Array|IsValidIndex (Variables|Private|GetPatrolRoute) _returnvalue_6)
                (return (Utilities|Array|Get(acopy) (Variables|Private|GetPatrolRoute) _returnvalue_6))
                (else
                  (return (Utilities|Array|Get(acopy) _patrolroute_4 (Utilities|Array|LastIndex _patrolroute_4))))))))
        (:NewEnumerator1
          (switch Utilities|FlowControl|Switch|SwitchonE_AI_PatrolDirection (Variables|Private|Config|GetDirection)
            (:NewEnumerator0
              (if (Utilities|Array|IsValidIndex (Variables|Private|GetPatrolRoute) _returnvalue_7)
                (return (Utilities|Array|Get(acopy) (Variables|Private|GetPatrolRoute) _returnvalue_7))
                (else
                  (Variables|Private|Config|SetDirection "NewEnumerator1")
                  (return (Utilities|Array|Get(acopy) (Variables|Private|GetPatrolRoute) (- (Utilities|Array|FindItem (Variables|Private|GetPatrolRoute) (Variables|Private|GetTargetPatrolPoint)) 1))))))
            (:NewEnumerator1
              (if (Utilities|Array|IsValidIndex (Variables|Private|GetPatrolRoute) _returnvalue_5)
                (return (Utilities|Array|Get(acopy) (Variables|Private|GetPatrolRoute) _returnvalue_5))
                (else
                  (Variables|Private|Config|SetDirection "NewEnumerator0")
                  (return (Utilities|Array|Get(acopy) (Variables|Private|GetPatrolRoute) (+ (Utilities|Array|FindItem (Variables|Private|GetPatrolRoute) (Variables|Private|GetTargetPatrolPoint)) 1))))))))
        (:NewEnumerator2
          (LocalVariables|SetAvailableRandomPatrolPointsLOCAL (Variables|Private|GetPatrolRoute))
          (Utilities|Array|RemoveItem (LocalVariables|GetAvailableRandomPatrolPointsLOCAL) (Variables|Private|GetTargetPatrolPoint))
          (return (Utilities|Array|Get(acopy) (LocalVariables|GetAvailableRandomPatrolPointsLOCAL) (Math|Random|RandomIntegerinRange 0 (Utilities|Array|LastIndex (LocalVariables|GetAvailableRandomPatrolPointsLOCAL)))))))
      (else
        (bind (_success _nearestpatrolpoint) (Finders|FindNearestPatrolPoint (Transformation|GetActorLocation (Components|GetOwner))))
        (if _success
          (return _nearestpatrolpoint))))))

(fn GetTargetPatrolPoint
  (return (Variables|Private|GetTargetPatrolPoint)))

(fn SetTargetPatrolPoint
  (params (NewTargetPatrolPoint :type Vector))
  (if (Math|Vector|NotEqual(Vector) NewTargetPatrolPoint (Variables|Private|GetTargetPatrolPoint) 0.0001)
    (Variables|Private|SetTargetPatrolPoint NewTargetPatrolPoint)
    (Default|CallOnTargetPatrolPointChanged (Variables|Private|GetTargetPatrolPoint))))

(fn FindNearestPatrolPoint
  (params (FromLocation :type Vector))
  (for (_array_element _array_index) (Variables|Private|GetPatrolRoute)
    (if (== _array_index 0)
      (LocalVariables|SetSuccessLOCAL true)
      (LocalVariables|SetCurrentDistanceSquaredLOCAL (Math|Vector|VectorLengthSquared (- _array_element FromLocation)))
      (LocalVariables|SetNearestPatrolPointLOCAL _array_element)
      (elif (< (Math|Vector|VectorLengthSquared (- _array_element FromLocation)) (LocalVariables|GetCurrentDistanceSquaredLOCAL))
        (LocalVariables|SetSuccessLOCAL true)
        (LocalVariables|SetCurrentDistanceSquaredLOCAL (Math|Vector|VectorLengthSquared (- _array_element FromLocation)))
        (LocalVariables|SetNearestPatrolPointLOCAL _array_element))))
  (return (LocalVariables|GetSuccessLOCAL) (LocalVariables|GetNearestPatrolPointLOCAL)))

(fn GetPatrolRoute
  (return (Variables|Private|GetPatrolRoute)))

(fn GetRandomBreakDuration
  (return (Math|Random|RandomFloatinRange (Variables|Private|Config|GetBreakDurationMin) (Variables|Private|Config|GetBreakDurationMax))))

(fn GetDirection
  (return (Variables|Private|Config|GetDirection)))

(fn SetDirection
  (params (NewDirectionDirection :type E_AI_PatrolDirection%20Enum :default "NewEnumerator0"))
  (if (Utilities|Enum|NotEqual(Enum) NewDirectionDirection (Variables|Private|Config|GetDirection))
    (bind _output_get (Variables|Private|Config|SetDirection NewDirectionDirection))
    (Default|CallOnDirectionChanged _output_get)))

(fn GetPatrolType
  (return (Variables|Private|Config|GetPatrolType)))

(fn SetPatrolType
  (params (NewPatrolType :type E_AI_PatrolType%20Enum :default "NewEnumerator0"))
  (if (Utilities|Enum|NotEqual(Enum) NewPatrolType (Variables|Private|Config|GetPatrolType))
    (bind _output_get (Variables|Private|Config|SetPatrolType NewPatrolType))
    (Default|CallOnPatrolTypeChanged _output_get)))