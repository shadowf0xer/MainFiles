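; AI follow component that stores a follow target, follow threshold and distance tolerance for an AI-controlled character.
; An Initialize event seeds threshold and tolerance from a follow config, with squared getters available for both values.
; Setters fire change notifications only when values differ, and a target change also sends an OnFollowTargetChanged message to the controlled pawn via the owner's AI controller.
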(event Custom|Initialize
  (params (FollowConfig :type S%20AI%20Config%20Follow%20Structure))
  (bind (_distancetolerance _threshold) (Utilities|Struct|BreakS_AI_Config_Follow FollowConfig))
  (Variables|Private|Config|SetDistanceTolerance _distancetolerance)
  (Variables|Private|Config|SetThreshold _threshold))

(fn GetTarget
  (return (Variables|Private|GetCurrentTarget)))

(fn SetTarget
  (params (NewTarget :type Actor%20Object%20Reference))
  (if (!= NewTarget (Variables|Private|GetCurrentTarget))
    (bind _output_get (Variables|Private|SetCurrentTarget NewTarget))
    (Default|CallOnTargetChanged _output_get)
    (Class|BPIAIEvents|OnFollowTargetChanged(Message) (Pawn|GetControlledPawn (AI|GetAIController (Components|GetOwner))) (Getters|GetTarget))))

(fn SetThreshold
  (params (NewRadius :type Float%20%28single-precision%29))
  (if (!= NewRadius (Variables|Private|Config|GetThreshold))
    (Variables|Private|Config|SetThreshold NewRadius)
    (Default|CallOnThresholdChanged (Variables|Private|Config|GetThreshold))))

(fn GetThreshold
  (return (Variables|Private|Config|GetThreshold)))

(fn GetThresholdSquared
  (return (Math|Float|Square (Variables|Private|Config|GetThreshold))))

(fn GetDistanceToleranceSquared
  (return (Math|Float|Square (Variables|Private|Config|GetDistanceTolerance))))

(fn SetDistanceTolerance
  (params (NewDistanceTolerance :type Float%20%28single-precision%29))
  (if (!= NewDistanceTolerance (Variables|Private|Config|GetDistanceTolerance))
    (Variables|Private|Config|SetDistanceTolerance NewDistanceTolerance)
    (Default|CallOnDistanceToleranceChanged (Variables|Private|Config|GetDistanceTolerance))))

(fn GetDistanceTolerance
  (return (Variables|Private|Config|GetDistanceTolerance)))