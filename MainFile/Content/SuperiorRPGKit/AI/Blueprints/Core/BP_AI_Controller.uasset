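; AI controller for SuperiorRPGKit pawns that runs a main behavior tree and exposes commands for idle, move, roam, follow, patrol, attack, support and interaction.
; Roam, follow, patrol, attack and target components are initialized from one data table row.
; Commands set ActiveBehavior and feed components, usually clearing combat targets; Move issues MoveTo directly, while Attack registers threat and can force a target.
; Movement completion and attack-effect resolution are forwarded to the pawn as messages.
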(event Custom|OnReceiveMoveCompleted
  (params (RequestID :type AI%20Request%20ID%20Structure) (Result :type EPathFollowingResult%20Enum :default "Success"))
  (Class|BPIAIEvents|OnMovementFinished(Message) (Pawn|GetControlledPawn) Result (Variables|Default|GetActiveBehavior)))

(event EventBeginPlay
  (Utilities|Array|Add (Variables|/Game/SuperiorRPGKit/AI/Blueprints/Components/AC_AI_Target.AC_AI_Target_C|GetIgnoredActors (Variables|Default|GetAC_AI_Target)) (Pawn|GetControlledPawn))
  (AI|RunBehaviorTree "/Game/SuperiorRPGKit/AI/Blueprints/Core/Main_BT.Main_BT")
  (EventDispatchers|AssignReceiveMoveCompleted (delegate Custom|OnReceiveMoveCompleted)))

(fn ConstructionScript)

(fn Initialize
  (params (Configuration :type Data%20Table%20Row%20Handle%20Structure))
  (bind (_datatable _rowname) (Utilities|Struct|BreakDataTableRowHandle Configuration))
  (bind _returnvalue (Utilities|GetDataTableRow _datatable _rowname)
    (:then
      (Default|Initialize (Variables|Default|GetAC_AI_Roam) (.Roam (Utilities|Struct|BreakS_AI_Config _returnvalue)))
      (Default|Initialize (Variables|Default|GetAC_AI_Follow) (.Follow (Utilities|Struct|BreakS_AI_Config _returnvalue)))
      (Default|Initialize (Variables|Default|GetAC_AI_Patrol) (.Patrol (Utilities|Struct|BreakS_AI_Config _returnvalue)))
      (Default|Initialize (Variables|Default|GetAC_AI_Attack) (.Combat_General (Utilities|Struct|BreakS_AI_Config _returnvalue)) (.Combat_Melee (Utilities|Struct|BreakS_AI_Config _returnvalue)) (.Combat_Ranged (Utilities|Struct|BreakS_AI_Config _returnvalue)) (.Combat_Support (Utilities|Struct|BreakS_AI_Config _returnvalue)))
      (Default|Initialize (Variables|Default|GetAC_AI_Target) (.Combat_Activation (Utilities|Struct|BreakS_AI_Config _returnvalue))))))

(fn Attack
  (params (AttackTarget :type Actor%20Object%20Reference) (Forced :type Boolean))
  (if (not (Default|IsIgnoringCombat (Variables|Default|GetAC_AI_Attack)))
    (Variables|/Game/SuperiorRPGKit/AI/Blueprints/Components/AC_AI_Target.AC_AI_Target_C|SetForcedAttack (Variables|Default|GetAC_AI_Target) Forced)
    (Utilities|FlowControl|Sequence
      (:then_0
        (if (Variables|/Game/SuperiorRPGKit/AI/Blueprints/Components/AC_AI_Target.AC_AI_Target_C|GetForcedAttack (Variables|Default|GetAC_AI_Target))
          (Utilities|IsValid AttackTarget
            (:Is%20Valid
              (Default|SetTargetedEnemy (Variables|Default|GetAC_AI_Target) AttackTarget)))))
      (:then_1
        (Default|ModifyThreat (Variables|Default|GetAC_AI_Target) AttackTarget 0.0)
        (Default|SetTargetedAlly (Variables|Default|GetAC_AI_Target))
        (Variables|Default|SetActiveBehavior "NewEnumerator4")
        (return true)))))

(fn EndInteraction
  (params (Reason :type E_AI_InteractionEndReason%20Enum :default "NewEnumerator0"))
  (bind _ac_ai_interact (Variables|Default|GetAC_AI_Interact))
  (Variables|/Game/SuperiorRPGKit/AI/Blueprints/Components/AC_AI_Interact.AC_AI_Interact_C|SetLastInteractionEndReason _ac_ai_interact Reason)
  (Default|SetInteractionState _ac_ai_interact "NewEnumerator3")
  (return true))

(fn Follow
  (params (FollowTarget :type Actor%20Object%20Reference))
  (bind _ac_ai_target (Variables|Default|GetAC_AI_Target))
  (Default|SetTarget (Variables|Default|GetAC_AI_Follow) FollowTarget)
  (Variables|Default|SetActiveBehavior "NewEnumerator2")
  (Default|SetTargetedAlly _ac_ai_target)
  (Default|SetTargetedEnemy _ac_ai_target)
  (return true))

(fn Idle
  (bind _ac_ai_target (Variables|Default|GetAC_AI_Target))
  (Variables|Default|SetActiveBehavior "NewEnumerator0")
  (Default|SetTargetedAlly _ac_ai_target)
  (Default|SetTargetedEnemy _ac_ai_target)
  (return true))

(fn Move
  (params (Destination :type Vector :default "0, 0, 0") (TargetActor :type Actor%20Object%20Reference) (AcceptanceRadius :type Float%20%28single-precision%29) (StopOnOverlap :type Boolean))
  (bind _ac_ai_target (Variables|Default|GetAC_AI_Target))
  (Variables|Default|SetActiveBehavior "NewEnumerator0")
  (Default|SetTargetedAlly _ac_ai_target)
  (Default|SetTargetedEnemy _ac_ai_target)
  (Utilities|IsValid TargetActor
    (:Is%20Valid
      (AI|Navigation|MovetoActor TargetActor AcceptanceRadius StopOnOverlap true)
      (return true))
    (:Is%20Not%20Valid
      (AI|Navigation|MovetoLocation Destination AcceptanceRadius StopOnOverlap true false)
      (return true))))

(fn Patrol
  (params (PatrolRoute :type Array%20of%20Vectors) (Type :type E_AI_PatrolType%20Enum :default "NewEnumerator0") (Direction :type E_AI_PatrolDirection%20Enum :default "NewEnumerator0"))
  (bind _ac_ai_target (Variables|Default|GetAC_AI_Target))
  (Default|SetPatrolRoute (Variables|Default|GetAC_AI_Patrol) PatrolRoute)
  (Default|SetPatrolType (Variables|Default|GetAC_AI_Patrol) Type)
  (Default|SetDirection (Variables|Default|GetAC_AI_Patrol) Direction)
  (Variables|Default|SetActiveBehavior "NewEnumerator3")
  (Default|SetTargetedAlly _ac_ai_target)
  (Default|SetTargetedEnemy _ac_ai_target)
  (return true))

(fn ResolveAttackEffect
  (Class|BPIAIEvents|OnAttackEffectResolved(Message) (Pawn|GetControlledPawn) (Variables|/Game/SuperiorRPGKit/AI/Blueprints/Components/AC_AI_Attack.AC_AI_Attack_C|GetAttackID (Variables|Default|GetAC_AI_Attack)))
  (return true))

(fn RoamAroundActor
  (params (RoamTarget :type Actor%20Object%20Reference))
  (bind _ac_ai_roam (Variables|Default|GetAC_AI_Roam))
  (bind _ac_ai_target (Variables|Default|GetAC_AI_Target))
  (Default|SetFocusActor _ac_ai_roam RoamTarget)
  (Default|SetFocusPoint _ac_ai_roam "0, 0, 0")
  (Variables|Default|SetActiveBehavior "NewEnumerator1")
  (Default|SetTargetedAlly _ac_ai_target)
  (Default|SetTargetedEnemy _ac_ai_target)
  (return true))

(fn RoamAroundPoint
  (params (Point :type Vector :default "0, 0, 0"))
  (bind _ac_ai_roam (Variables|Default|GetAC_AI_Roam))
  (bind _ac_ai_target (Variables|Default|GetAC_AI_Target))
  (Default|SetFocusPoint _ac_ai_roam Point)
  (Default|SetFocusActor _ac_ai_roam)
  (Variables|Default|SetActiveBehavior "NewEnumerator1")
  (Default|SetTargetedAlly _ac_ai_target)
  (Default|SetTargetedEnemy _ac_ai_target)
  (return true))

(fn StartInteraction
  (params (InteractionTarget :type Actor%20Object%20Reference))
  (bind _ac_ai_target (Variables|Default|GetAC_AI_Target))
  (Utilities|IsValid InteractionTarget
    (:Is%20Valid
      (bind _result (Class|BPIRPGInteractable|IsInteractable(Message) InteractionTarget (Pawn|GetControlledPawn)))
      (if _result
        (Default|SetInteractionTarget (Variables|Default|GetAC_AI_Interact) InteractionTarget)
        (Variables|Default|SetActiveBehavior "NewEnumerator5")
        (Default|SetTargetedAlly _ac_ai_target)
        (Default|SetTargetedEnemy _ac_ai_target)
        (return true)))))

(fn Support
  (params (SupportTarget :type Actor%20Object%20Reference))
  (if (not (Default|IsIgnoringCombat (Variables|Default|GetAC_AI_Attack)))
    (if (Default|IsActorinDeactivationRadius (Variables|Default|GetAC_AI_Target) SupportTarget)
      (Default|SetTargetedAlly (Variables|Default|GetAC_AI_Target) SupportTarget)
      (Default|SetTargetedEnemy (Variables|Default|GetAC_AI_Target))
      (Variables|Default|SetActiveBehavior "NewEnumerator6")
      (return true))))