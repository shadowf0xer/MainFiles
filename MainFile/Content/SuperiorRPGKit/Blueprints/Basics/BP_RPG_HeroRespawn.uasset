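; Interactable hero respawn point that a player activates to set where they respawn, exposing its RespawnPoint's location and rotation as the respawn transform.
; Interaction passes the actor to the interacting owner's AC_RPG_SavesManager through ActivateRespawnSERVER, and interactability is checked against that manager's active respawn.
; Activate and Deactivate tint the mesh through dynamic materials, and children can override them for custom effects.
; An InvisibleInGame option hides the mesh and disables its collision.
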(event EventBeginPlay)

(event Collision|EventActorBeginOverlap
  (params (OtherActor :type Actor%20Object%20Reference)))

(event EventTick
  (params (DeltaSeconds :type Float%20%28single-precision%29)))

(event Custom|Activate
  (bind _mesh (Variables|Default|GetMesh))
  ;[0.1 0.1 0.1 1 14] On Activation/Deactivation change spawner color. Can be overridden by children blueprints to implement your own effects. IE. "fountain" respawn could glow and play some vfx when it is activated.
  (if (not (Variables|Default|GetInvisibleInGame))
    (bind _returnvalue (Rendering|Material|CreateDynamicMaterialInstance _mesh 0 (Rendering|Material|GetMaterial _mesh 0) :!class /Script/Engine.PrimitiveComponent))
    (Rendering|Material|SetVectorParameterValue _returnvalue "Color" "(R=0.000000,G=1.000000,B=0.000000,A=1.000000)" :!class /Script/Engine.MaterialInstanceDynamic)))

(event Custom|Deactivate
  (bind _mesh (Variables|Default|GetMesh))
  ;[0.1 0.1 0.1 1 14] On Activation/Deactivation change spawner color. Can be overridden by children blueprints to implement your own effects. IE. "fountain" respawn could glow and play some vfx when it is activated.
  (if (not (Variables|Default|GetInvisibleInGame))
    (bind _returnvalue (Rendering|Material|CreateDynamicMaterialInstance _mesh 0 (Rendering|Material|GetMaterial _mesh 0) :!class /Script/Engine.PrimitiveComponent))
    (Rendering|Material|SetVectorParameterValue _returnvalue "Color" "(R=1.000000,G=1.000000,B=1.000000,A=1.000000)" :!class /Script/Engine.MaterialInstanceDynamic)))

(event EventOnBeginInteract
  (params (InteractingActor :type Actor%20Object%20Reference) (InteractionManager :type AC%20RPG%20Interaction%20Manager%20Object%20Reference))
  (bind _returnvalue (Components|GetOwner InteractionManager))
  (bind _returnvalue_2 (Actor|GetComponentbyClass _returnvalue "/Game/SuperiorRPGKit/Blueprints/Components/AC_RPG_SavesManager.AC_RPG_SavesManager_C"))
  ;[0.1 0.1 0.1 1 14] Activate respawn on interaction.
  (Utilities|IsValid InteractionManager
    (:Is%20Valid
      (Utilities|IsValid _returnvalue_2
        (:Is%20Valid
          (Default|ActivateRespawnSERVER _returnvalue_2 self))))))

(fn ConstructionScript
  (bind _mesh (Variables|Default|GetMesh))
  (if (Variables|Default|GetInvisibleInGame)
    (Collision|SetCollisionEnabled _mesh "NoCollision")
    (Development|SetHiddeninGame _mesh true false)))

(fn GetRespawnTransform
  (bind _respawnpoint (Variables|Default|GetRespawnPoint))
  (bind _returnvalue (Transformation|GetWorldTransform _respawnpoint))
  (return (Math|Transform|MakeTransform (.location _returnvalue) (.rotation _returnvalue) "1,1,1")))

(fn GetInteractionAction
  (params (InteractingActor :type Actor%20Object%20Reference))
  (return "NewEnumerator3"))

(fn GetInteractionRadius
  (params (InteractingActor :type Actor%20Object%20Reference))
  (return 3e+02))

(fn GetInteractionText
  (return "Activate Respawn Fountain"))

(fn GetInteractionTime
  (params (InteractingActor :type Actor%20Object%20Reference))
  (return 0.0))

(fn GetInteractionType
  (return "NewEnumerator3"))

(fn IsInteractable
  (params (InteractingActor :type Actor%20Object%20Reference) (InteractionManager :type AC%20RPG%20Interaction%20Manager%20Object%20Reference))
  (Utilities|IsValid InteractionManager
    (:Is%20Valid
      (return (!= (Variables|/Game/SuperiorRPGKit/Blueprints/Components/AC_RPG_SavesManager.AC_RPG_SavesManager_C|GetActiveRespawn (Actor|GetComponentbyClass (Components|GetOwner InteractionManager) "/Game/SuperiorRPGKit/Blueprints/Components/AC_RPG_SavesManager.AC_RPG_SavesManager_C")) (Variables|Default|GetRespawnPoint))))))