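; BP_RPG_Stash is an interactable storage chest that opens a player's personal stash.
; It answers interaction queries with fixed prompt, radius and type, is always interactable, and takes no hold time.
; On interact, it points the interacting owner's AC_RPG_ItemsManager StashContainer at its PersonalStashContainer and requests stash access on the server.
; Interacting again while open finishes the interaction, which clears InteractedActor and leaves the stash.
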(event EventOnBeginInteract
  (params (InteractingActor :type Actor%20Object%20Reference) (InteractionManager :type AC%20RPG%20Interaction%20Manager%20Object%20Reference))
  (bind _returnvalue (Components|GetOwner InteractionManager))
  (bind _returnvalue_2 (Actor|GetComponentbyClass _returnvalue "/Game/SuperiorRPGKit/Blueprints/Components/AC_RPG_ItemsManager.AC_RPG_ItemsManager_C"))
  ;[0.1 0.1 0.1 1 14] Open Stash when player interacts with it. Also finishes interaction (closes Stash) if player attempts to interact with it again while it is open.
  (Utilities|IsValid InteractionManager
    (:Is%20Valid
      (if (== (Variables|/Game/SuperiorRPGKit/Blueprints/Components/AC_RPG_InteractionManager.AC_RPG_InteractionManager_C|GetInteractedActor InteractionManager) self) ; Are we already interacting with this actor.
        (Default|FinishActorInteractionSERVER InteractionManager)
        (else
          (Utilities|IsValid _returnvalue_2
            (:Is%20Valid
              (Variables|/Game/SuperiorRPGKit/Blueprints/Components/AC_RPG_InteractionManager.AC_RPG_InteractionManager_C|SetInteractedActor InteractionManager self)
              (Variables|/Game/SuperiorRPGKit/Blueprints/Components/AC_RPG_ItemsManager.AC_RPG_ItemsManager_C|SetStashContainer _returnvalue_2 (Variables|/Game/SuperiorRPGKit/Blueprints/Components/AC_RPG_ItemsManager.AC_RPG_ItemsManager_C|GetPersonalStashContainer _returnvalue_2))
              (Default|AccessStashSERVER _returnvalue_2))))))))

(event EventOnFinishInteract
  (params (InteractingActor :type Actor%20Object%20Reference) (InteractionManager :type AC%20RPG%20Interaction%20Manager%20Object%20Reference))
  (bind _returnvalue (Components|GetOwner InteractionManager))
  (bind _returnvalue_2 (Actor|GetComponentbyClass _returnvalue "/Game/SuperiorRPGKit/Blueprints/Components/AC_RPG_ItemsManager.AC_RPG_ItemsManager_C"))
  ;[0.1 0.1 0.1 1 14] Close Stash.
  (Utilities|IsValid InteractionManager
    (:Is%20Valid
      (Variables|/Game/SuperiorRPGKit/Blueprints/Components/AC_RPG_InteractionManager.AC_RPG_InteractionManager_C|SetInteractedActor InteractionManager 0)
      (Utilities|IsValid _returnvalue_2
        (:Is%20Valid
          (Default|LeaveStashSERVER _returnvalue_2))))))

(fn ConstructionScript)

(fn GetInteractionAction
  (params (InteractingActor :type Actor%20Object%20Reference))
  (return "NewEnumerator3"))

(fn GetInteractionRadius
  (params (InteractingActor :type Actor%20Object%20Reference))
  (return 2.5e+02))

(fn GetInteractionText
  (return "Open storage chest"))

(fn GetInteractionTime
  (params (InteractingActor :type Actor%20Object%20Reference))
  (return 0.0))

(fn GetInteractionType
  (return "NewEnumerator3"))

(fn IsInteractable
  (params (InteractingActor :type Actor%20Object%20Reference) (InteractionManager :type AC%20RPG%20Interaction%20Manager%20Object%20Reference))
  (return true))