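; Base in-game player controller for the RPG kit, parent of top-down and third-person controllers, handling the player's hero from spawn to save and quit.
; A client/server chain reads the last-played save, spawns the hero at a saved or global respawn, initializes HUD and manager components, then loads hero data.
; It also routes input to windows and quick slots, reacts to manager events, auto-respawns dead heroes, and saves on leaving.
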(event EventBeginPlay
  (Input|SetInputModeGameandUI self 0 "DoNotLock" false) ; Set proper input mode.
  (Utilities|FlowControl|Delay 2.0)
  (Networking|SwitchHasAuthority
    (:Authority
      (CallFunction|LoadPlayerHeroCLIENT))))

(event EventEndPlay
  (params (EndPlayReason :type EEndPlayReason%20Enum :default "Destroyed"))
  ;[0.1 0.1 0.1 1 14] Saves game automatically when host ends the session.
  (switch Utilities|FlowControl|Switch|SwitchonEEndPlayReason EndPlayReason
    (:LevelTransition
      (CallFunction|SavePlayerDataCLIENT))))

(event OnLoadFinished(AC_RPG_SavesManager)
  ;[0.1 0.1 0.1 1 14] Reset hero collision when load finishes so it will update all NPC quest availability (these signs displayed over their heads)
  (Collision|SetActorEnableCollision (Variables|Default|GetPlayerHero) false)
  (Collision|SetActorEnableCollision (Variables|Default|GetPlayerHero) true))

(event Custom|Initialization_CLIENT
  (params (PlayerHero :type BP%20RPG%20Hero%20Object%20Reference))
  (Utilities|FlowControl|DoOnce false
    (:Completed
      (bind _output_get (Variables|Default|SetPlayerHero PlayerHero))
      (Game|Player|SetViewTargetwithBlend _output_get 0.0 "VTBlend_Linear" 0.0 false) ; Use hero camera in case player doesn't possess hero.\n(ie. in top down mode, where hero is possessed by AI)
      (Variables|/Game/SuperiorRPGKit/Blueprints/Basics/BP_RPG_Hero.BP_RPG_Hero_C|SetPlayerController (Variables|Default|GetPlayerHero) self)
      (Variables|/Game/SuperiorRPGKit/Blueprints/Components/AC_RPG_StatsManager.AC_RPG_StatsManager_C|SetCharacterID (Variables|Default|GetAC_RPG_StatsManager) (Variables|/Game/SuperiorRPGKit/Blueprints/Basics/BP_RPG_Hero.BP_RPG_Hero_C|GetHeroID (Variables|Default|GetPlayerHero)))
      (bind _asbp_rpg_hud (Utilities|Casting|CastToBP_RPG_HUD (HUD|GetHUD)))
      (Variables|Default|SetPlayerHUD _asbp_rpg_hud)
      ;[0.1 0.1 0.1 1 14] Create HUD windows.
      (Default|CreateWidgets (Variables|Default|GetPlayerHUD))
      ;[0.1 0.1 0.1 1 14] Initialize stats related widgets.
      (Default|AddWidgetstoRefresh (Variables|Default|GetAC_RPG_StatsManager) (Utilities|Array|MakeArray (Variables|/Game/SuperiorRPGKit/Blueprints/Basics/BP_RPG_HUD.BP_RPG_HUD_C|GetStatsWindow (Variables|Default|GetPlayerHUD)) (Variables|/Game/SuperiorRPGKit/Blueprints/Basics/BP_RPG_HUD.BP_RPG_HUD_C|GetHeroSmallWindow (Variables|Default|GetPlayerHUD))))
      (Default|InitializeStatsWindow (Variables|Default|GetAC_RPG_StatsManager) (Variables|/Game/SuperiorRPGKit/Blueprints/Basics/BP_RPG_HUD.BP_RPG_HUD_C|GetStatsWindow (Variables|Default|GetPlayerHUD)))
      (Default|SetBuffsandEffectsContainer (Variables|Default|GetAC_RPG_StatsManager) (Variables|/Game/SuperiorRPGKit/Widgets/Player/WBP_RPG_InGameHUD.WBP_RPG_InGameHUD_C|GetContainer_BuffsAndEffects (Variables|/Game/SuperiorRPGKit/Blueprints/Basics/BP_RPG_HUD.BP_RPG_HUD_C|GetInGameHUD (Variables|Default|GetPlayerHUD))))
      ;[0.1 0.1 0.1 1 14] Initialize items related widgets.
      (Default|AddWidgetstoRefresh (Variables|Default|GetAC_RPG_ItemsManager) (Utilities|Array|MakeArray (Variables|/Game/SuperiorRPGKit/Blueprints/Basics/BP_RPG_HUD.BP_RPG_HUD_C|GetInventoryWindow (Variables|Default|GetPlayerHUD))))
      (Default|InitializeInventoryWindow (Variables|Default|GetAC_RPG_ItemsManager) (Variables|/Game/SuperiorRPGKit/Blueprints/Basics/BP_RPG_Hero.BP_RPG_Hero_C|GetAC_RPG_Container%28Inventory%29 (Variables|Default|GetPlayerHero)) (Variables|/Game/SuperiorRPGKit/Widgets/Player/WBP_RPG_InventoryWindow.WBP_RPG_InventoryWindow_C|GetWBP_UIC_InventoryContainer (Variables|/Game/SuperiorRPGKit/Blueprints/Basics/BP_RPG_HUD.BP_RPG_HUD_C|GetInventoryWindow (Variables|Default|GetPlayerHUD))))
      (Default|InitializeStashWindow (Variables|Default|GetAC_RPG_ItemsManager) (Variables|/Game/SuperiorRPGKit/Widgets/Player/WBP_RPG_StorageWindow.WBP_RPG_StorageWindow_C|GetWBP_UIC_StorageContainer (Variables|/Game/SuperiorRPGKit/Blueprints/Basics/BP_RPG_HUD.BP_RPG_HUD_C|GetStorageWindow (Variables|Default|GetPlayerHUD))))
      (Default|InitializeVendorWindow (Variables|Default|GetAC_RPG_ItemsManager) (Variables|/Game/SuperiorRPGKit/Widgets/Player/WBP_RPG_VendorWindow.WBP_RPG_VendorWindow_C|GetWBP_UIC_VendorContainer (Variables|/Game/SuperiorRPGKit/Blueprints/Basics/BP_RPG_HUD.BP_RPG_HUD_C|GetVendorWindow (Variables|Default|GetPlayerHUD))))
      (Default|InitializeEquipmentWindow (Variables|Default|GetAC_RPG_ItemsManager) (Variables|/Game/SuperiorRPGKit/Blueprints/Basics/BP_RPG_Hero.BP_RPG_Hero_C|GetAC_RPG_Equipment (Variables|Default|GetPlayerHero)))
      (Default|InitializeCraftingWindow (Variables|Default|GetAC_RPG_CraftingManager) (Variables|Default|GetAC_RPG_ItemsManager))
      ;[0.1 0.1 0.1 1 14] Initialize quests and achievements related widgets.
      (Default|AddWidgetstoRefresh (Variables|Default|GetAC_RPG_QuestsManager) (Utilities|Array|MakeArray (Variables|/Game/SuperiorRPGKit/Blueprints/Basics/BP_RPG_HUD.BP_RPG_HUD_C|GetQuestLogWindow (Variables|Default|GetPlayerHUD)) (Variables|/Game/SuperiorRPGKit/Blueprints/Basics/BP_RPG_HUD.BP_RPG_HUD_C|GetQuestPopUpWindow (Variables|Default|GetPlayerHUD)) (Variables|/Game/SuperiorRPGKit/Blueprints/Basics/BP_RPG_HUD.BP_RPG_HUD_C|GetTrackerWindow (Variables|Default|GetPlayerHUD))))
      (Default|AddWidgetstoRefresh (Variables|Default|GetAC_RPG_AchievementsManager) (Utilities|Array|MakeArray (Variables|/Game/SuperiorRPGKit/Blueprints/Basics/BP_RPG_HUD.BP_RPG_HUD_C|GetAchievementsWindow (Variables|Default|GetPlayerHUD))))
      ;[0.1 0.1 0.1 1 14] Initialize skills related widgets. Also create skill tree widget for specific hero.
      (bind _returnvalue (UserInterface|CreateWidget (Variables|/Game/SuperiorRPGKit/Blueprints/Basics/BP_RPG_Hero.BP_RPG_Hero_C|GetSkillTreeWidget (Variables|Default|GetPlayerHero))))
      (Default|InitializeSkillsWindow (Variables|Default|GetAC_RPG_SkillsManager) (Variables|/Game/SuperiorRPGKit/Blueprints/Basics/BP_RPG_Hero.BP_RPG_Hero_C|GetSkillsDatatable (Variables|Default|GetPlayerHero)) _returnvalue (Variables|/Game/SuperiorRPGKit/Blueprints/Basics/BP_RPG_HUD.BP_RPG_HUD_C|GetSkillsWindow (Variables|Default|GetPlayerHUD)))
      ;[0.1 0.1 0.1 1 14] Initialize Quick Access Bar(s)
      (Default|InitializeQuickAccessBars (Variables|Default|GetAC_RPG_QuickAccessManager))
      ;[0.1 0.1 0.1 1 14] Initialize Options Manager
      (Default|InitializeOptionsManager (Variables|Default|GetAC_RPG_OptionsManager) (Variables|/Game/SuperiorRPGKit/Blueprints/Basics/BP_RPG_Hero.BP_RPG_Hero_C|GetCamera (Variables|Default|GetPlayerHero)) true)
      ;[0.1 0.1 0.1 1 14] Initialize dialogue window.
      (Default|InitializeDialogueWindow (Variables|Default|GetAC_RPG_InteractionManager) (Variables|/Game/SuperiorRPGKit/Blueprints/Basics/BP_RPG_HUD.BP_RPG_HUD_C|GetDialogueWindow (Variables|Default|GetPlayerHUD)))
      ;[0.1 0.1 0.1 1 14] Initialize Notifications containers.
      (Default|InitializeNotificationsContainer (Variables|Default|GetAC_RPG_NotificationsManager%28Center%29) (Variables|/Game/SuperiorRPGKit/Blueprints/Basics/BP_RPG_HUD.BP_RPG_HUD_C|GetNotificationContainer (Variables|Default|GetPlayerHUD)))
      (Default|InitializeNotificationsContainer (Variables|Default|GetAC_RPG_NotificationsManager%28Corner%29) (Variables|/Game/SuperiorRPGKit/Blueprints/Basics/BP_RPG_HUD.BP_RPG_HUD_C|GetNotificationContainer (Variables|Default|GetPlayerHUD)))
      ;[0.1 0.1 0.1 1 14] Hide loading screen
      (Default|FadeOut (Variables|/Game/SuperiorRPGKit/Blueprints/Basics/BP_RPG_HUD.BP_RPG_HUD_C|GetLoadingScreen (Variables|Default|GetPlayerHUD)))
      (CallFunction|InitializationSERVER))))

(event Custom|LoadPlayerData_CLIENT
  (if (not (Variables|Development|GetSkipHeroLoad))
    (bind _returnvalue (SaveGame|LoadGamefromSlot "General"))
    (bind _asbp_rpg_save_general (Utilities|Casting|CastToBP_RPG_SAVE_General _returnvalue))
    (Default|LoadHero (Variables|Default|GetAC_RPG_SavesManager) (Variables|/Game/SuperiorRPGKit/Blueprints/Saves/BP_RPG_SAVE_General.BP_RPG_SAVE_General_C|GetLastPlayedHeroSave _asbp_rpg_save_general))))

(event Custom|Initialization_SERVER
  (bind _playerhero (Variables|Default|GetPlayerHero))
  (bind _ac_rpg_statsmanager (Variables|Default|GetAC_RPG_StatsManager))
  (Utilities|FlowControl|DoOnce false
    (:Completed
      ;[0.1 0.1 0.1 1 14] Initialize player components.
      (Default|InitializeAttributesandStats(Hero) (Variables|Default|GetAC_RPG_StatsManager))
      (Default|InitializeItemsManager (Variables|Default|GetAC_RPG_ItemsManager) (Variables|/Game/SuperiorRPGKit/Blueprints/Basics/BP_RPG_Hero.BP_RPG_Hero_C|GetAC_RPG_Container%28Inventory%29 _playerhero) (Variables|/Game/SuperiorRPGKit/Blueprints/Basics/BP_RPG_Hero.BP_RPG_Hero_C|GetAC_RPG_Equipment _playerhero) (Variables|/Game/SuperiorRPGKit/Blueprints/Basics/BP_RPG_Hero.BP_RPG_Hero_C|GetAC_RPG_Container%28PersonalStash%29 _playerhero))
      (Default|InitializeCraftingManager (Variables|Default|GetAC_RPG_CraftingManager) (Variables|Default|GetAC_RPG_ItemsManager))
      (Default|InitializeQuestsManager (Variables|Default|GetAC_RPG_QuestsManager))
      (Default|InitializeAchievementsManager (Variables|Default|GetAC_RPG_AchievementsManager))
      (Default|InitializeSkillsManager (Variables|Default|GetAC_RPG_SkillsManager) (Variables|/Game/SuperiorRPGKit/Blueprints/Basics/BP_RPG_Hero.BP_RPG_Hero_C|GetSkillsDatatable (Variables|Default|GetPlayerHero)))
      ;[0.1 0.1 0.1 1 14] Recalculate stats and initially set health and mana to max values.
      (Default|RecalculatePerLevelBonuses (Variables|Default|GetAC_RPG_StatsManager))
      (Default|PerformFullAttributesandStatsRecalculation (Variables|Default|GetAC_RPG_StatsManager))
      (Default|SetStatCurrentValuetoMax _ac_rpg_statsmanager "NewEnumerator1")
      (Default|SetStatCurrentValuetoMax _ac_rpg_statsmanager "NewEnumerator2")
      (CallFunction|LoadPlayerDataCLIENT))))

(event Custom|SpawnPlayerHero_SERVER
  (params (HeroID :type Name) (SpawnPointID :type Name) (MapName :type Name))
  (Utilities|FlowControl|DoOnce false
    (:Completed
      ;[0.1 0.1 0.1 1 14] Check if player last map is the same as host map.
      (bind _returnvalue (Game|GetCurrentLevelName true))
      (if (Utilities|Name|Equal(Name) (Utilities|String|StringToName _returnvalue) MapName)
        ;[0.1 0.1 0.1 1 14] If player and host maps were the same just use player last spawn.
        (bind (_success _respawn) (Default|FindRespawnwithID (Variables|Default|GetAC_RPG_SavesManager) SpawnPointID))
        (if _success
          (Default|ActivateRespawnSERVER (Variables|Default|GetAC_RPG_SavesManager) _respawn)
          ;[0.1 0.1 0.1 1 14] Spawn player hero at respawn.
          (bind _returnvalue_2 (Utilities|GetDataTableRow "/Game/SuperiorRPGKit/Datatables/DT_RPG_Heroes.DT_RPG_Heroes" HeroID :!label _label)
            (:then
              (bind _transform (Default|GetRespawnTransform (Variables|/Game/SuperiorRPGKit/Blueprints/Components/AC_RPG_SavesManager.AC_RPG_SavesManager_C|GetActiveRespawn (Variables|Default|GetAC_RPG_SavesManager))))
              (bind _returnvalue_3 (Game|SpawnActorfromClass (.ActorClass (Utilities|Struct|BreakS_RPG_Hero_Static _returnvalue_2)) _transform "AdjustIfPossibleButAlwaysSpawn" 0 0))
              (bind _output_get (Variables|Default|SetPlayerHero _returnvalue_3))
              (Variables|/Game/SuperiorRPGKit/Blueprints/Basics/BP_RPG_Hero.BP_RPG_Hero_C|SetPlayerController _output_get self)
              (Variables|/Game/SuperiorRPGKit/Blueprints/Components/AC_RPG_StatsManager.AC_RPG_StatsManager_C|SetCharacterID (Variables|Default|GetAC_RPG_StatsManager) (Variables|/Game/SuperiorRPGKit/Blueprints/Basics/BP_RPG_Hero.BP_RPG_Hero_C|GetHeroID (Variables|Default|GetPlayerHero)))
              (Utilities|FlowControl|Sequence
                (:then_0
                  (if (Variables|Default|GetThirdPersonMode)
                    (Pawn|Possess (Variables|Default|GetPlayerHero))))
                (:then_1
                  (Utilities|FlowControl|Delay 1.0)
                  (CallFunction|InitializationCLIENT (Variables|Default|GetPlayerHero))))))
          (else
            (Development|PrintString "ERROR. Respawn does not exist. Hero won't spawn." true true "(R=1.000000,G=0.000000,B=0.000000,A=1.000000)" :!label _label_2)))
        (else
          ;[0.1 0.1 0.1 1 14] If player and host maps were different use global spawn point (which usually is last spawn point activated by players on given map).
          (bind (_success_2 _respawn_2) (Default|FindRespawnwithID (Variables|Default|GetAC_RPG_SavesManager) (Variables|/Game/SuperiorRPGKit/Blueprints/Basics/BP_RPG_GameInstance.BP_RPG_GameInstance_C|GetGlobalSpawnPointID (.AsBP%20RPG%20Game%20Instance (Utilities|Casting|CastToBP_RPG_GameInstance (Game|GetGameInstance))))))
          (if _success_2
            (Default|ActivateRespawnSERVER (Variables|Default|GetAC_RPG_SavesManager) _respawn_2)
            (goto _label)
            (else
              (goto _label_2))))))))

(event Custom|LoadPlayerHero_CLIENT
  (Utilities|FlowControl|DoOnce false
    (:Completed
      (if (not (Variables|Development|GetSkipHeroLoad))
        (bind _returnvalue (SaveGame|LoadGamefromSlot "General"))
        (bind _asbp_rpg_save_general (Utilities|Casting|CastToBP_RPG_SAVE_General _returnvalue)
          (:then
            (bind _returnvalue_2 (SaveGame|LoadGamefromSlot (Variables|/Game/SuperiorRPGKit/Blueprints/Saves/BP_RPG_SAVE_General.BP_RPG_SAVE_General_C|GetLastPlayedHeroSave _asbp_rpg_save_general)))
            (bind _asbp_rpg_save_hero (Utilities|Casting|CastToBP_RPG_SAVE_Hero _returnvalue_2)
              (:then
                (CallFunction|SpawnPlayerHeroSERVER (Variables|/Game/SuperiorRPGKit/Blueprints/Saves/BP_RPG_SAVE_Hero.BP_RPG_SAVE_Hero_C|GetHeroID _asbp_rpg_save_hero) (Variables|/Game/SuperiorRPGKit/Blueprints/Saves/BP_RPG_SAVE_Hero.BP_RPG_SAVE_Hero_C|GetSpawnID _asbp_rpg_save_hero) (Variables|/Game/SuperiorRPGKit/Blueprints/Saves/BP_RPG_SAVE_Hero.BP_RPG_SAVE_Hero_C|GetMapName _asbp_rpg_save_hero)))
              (:CastFailed
                (bind _returnvalue_3 (Game|GetCurrentLevelName true :!label _label))
                (CallFunction|SpawnPlayerHeroSERVER (Variables|Development|GetTestHeroID) "Default" (Utilities|String|StringToName _returnvalue_3)) ; Spawn default hero if failed to load
              )))
          (:CastFailed
            (Development|PrintString "ERROR: Attempted to load hero that doesn't exist. Try loading character from main menu level or check in \"SkipHeroLoad\" variable in player controller blueprint." true true "(R=1.000000,G=0.000000,B=0.000000,A=1.000000)" 5.0)))
        (else
          (goto _label))))))

(event Custom|SavePlayerData_CLIENT
  (bind _returnvalue (SaveGame|LoadGamefromSlot "General"))
  (bind _asbp_rpg_save_general (Utilities|Casting|CastToBP_RPG_SAVE_General _returnvalue))
  (Default|SaveHero (Variables|Default|GetAC_RPG_SavesManager) (Variables|/Game/SuperiorRPGKit/Blueprints/Saves/BP_RPG_SAVE_General.BP_RPG_SAVE_General_C|GetLastPlayedHeroSave _asbp_rpg_save_general)))

(event Custom|CancelAllDraggingEvents
  (bind _ac_rpg_quickaccessmanager (Variables|Default|GetAC_RPG_QuickAccessManager))
  (bind _ac_rpg_skillsmanager (Variables|Default|GetAC_RPG_SkillsManager))
  (bind _ac_rpg_itemsmanager (Variables|Default|GetAC_RPG_ItemsManager))
  ;[0.1 0.1 0.1 1 12] Cancel all dragging events when right mouse button is pressed.
  (Utilities|FlowControl|Sequence
    (:then_0
      (if (Variables|/Game/SuperiorRPGKit/Blueprints/Components/AC_RPG_ItemsManager.AC_RPG_ItemsManager_C|GetDraggingItem _ac_rpg_itemsmanager)
        (Default|CancelItemDraggingSERVER _ac_rpg_itemsmanager)))
    (:then_1
      (if (Variables|/Game/SuperiorRPGKit/Blueprints/Components/AC_RPG_SkillsManager.AC_RPG_SkillsManager_C|GetDraggingSkill _ac_rpg_skillsmanager)
        (Default|CancelSkillDragging _ac_rpg_skillsmanager)))
    (:then_2
      (if (Variables|/Game/SuperiorRPGKit/Blueprints/Components/AC_RPG_QuickAccessManager.AC_RPG_QuickAccessManager_C|GetDraggingQuickSlot _ac_rpg_quickaccessmanager)
        (Default|CancelDraggingCLIENT _ac_rpg_quickaccessmanager)))))

(event Input|MouseEvents|RightMouseButton
  (params (Key :type Key%20Structure))
  ;[0.1 0.1 0.1 1 12] Cancel all dragging events when right mouse button is pressed.
  (:Pressed
    (CallFunction|CancelAllDraggingEvents)))

(event Input|KeyboardEvents|Escape
  (params (Key :type Key%20Structure))
  ;[0.1 0.1 0.1 1 12] Cancel key rebinding.
  (:Pressed
    (Default|StopListeningforKeyRebinding (Variables|Default|GetAC_RPG_OptionsManager))))

(event Input|KeyboardEvents|ScrollLock
  (params (Key :type Key%20Structure))
  ;[0.1 0.1 0.1 1 12] Cancel key rebinding.
  (:Pressed
    (Default|StopListeningforKeyRebinding (Variables|Default|GetAC_RPG_OptionsManager))))

(event Input|KeyboardEvents|AnyKey
  (params (Key :type Key%20Structure))
  ;[0.1 0.1 0.1 1 12] Input for key rebinding.
  (:Pressed
    (Default|RebindKey (Variables|Default|GetAC_RPG_OptionsManager) Key)))

(event Input|KeyboardEvents|LeftShift
  (params (Key :type Key%20Structure))
  ;[0.1 0.1 0.1 1 12] Activate Stacks Splitting when left shift is pressed (and hold) also activate Quick Access Bar Registration (shift + right click).
  (:Pressed
    (Default|ToggleStackSplitingOperation (Variables|Default|GetAC_RPG_ItemsManager) true))
  (:Released
    (if (not (Class|KismetInputLibrary|PointerEventIsMouseButtonDown (Utilities|Struct|MakePointerEvent) "LeftMouseButton")) ; Prevents from executing "released" Left Shift button \nwhen left mouse button is pressed
      (Default|ToggleStackSplitingOperation (Variables|Default|GetAC_RPG_ItemsManager) false))))

(event Input|KeyboardEvents|LeftCtrl
  (params (Key :type Key%20Structure))
  ;[0.1 0.1 0.1 1 12] Activate Quick Actions (one click to buy/sell/store/withdraw/equip/unequip)
  ; when left control is pressed (and hold).
  (:Pressed
    (Default|ToggleQuickActionOperations (Variables|Default|GetAC_RPG_ItemsManager) true))
  (:Released
    (if (not (Class|KismetInputLibrary|PointerEventIsMouseButtonDown (Utilities|Struct|MakePointerEvent) "LeftMouseButton")) ; Prevents from executing "released" Left Ctrl button \nwhen left mouse button is pressed
      (Default|ToggleQuickActionOperations (Variables|Default|GetAC_RPG_ItemsManager) false))))

(event Input|MouseEvents|MouseWheelUp
  (params (Key :type Key%20Structure))
  ;[0.1 0.1 0.1 1 14] Zoom in/out skill tree.
  (:Pressed
    (bind _playerhud (Variables|Default|GetPlayerHUD)
      (:then
        (Class|BPIRPGSkillsUpdater|ZoominSkillTree(Message) (Class|PanelWidget|GetChildat (Variables|/Game/SuperiorRPGKit/Widgets/Player/WBP_RPG_SkillsWindow.WBP_RPG_SkillsWindow_C|GetContainer_SkillTree (Variables|/Game/SuperiorRPGKit/Blueprints/Basics/BP_RPG_HUD.BP_RPG_HUD_C|GetSkillsWindow _playerhud)))))
      (:else))))

(event Input|MouseEvents|MouseWheelDown
  (params (Key :type Key%20Structure))
  ;[0.1 0.1 0.1 1 14] Zoom in/out skill tree.
  (:Pressed
    (bind _playerhud (Variables|Default|GetPlayerHUD)
      (:then
        (Class|BPIRPGSkillsUpdater|ZoomOutSkillTree(Message) (Class|PanelWidget|GetChildat (Variables|/Game/SuperiorRPGKit/Widgets/Player/WBP_RPG_SkillsWindow.WBP_RPG_SkillsWindow_C|GetContainer_SkillTree (Variables|/Game/SuperiorRPGKit/Blueprints/Basics/BP_RPG_HUD.BP_RPG_HUD_C|GetSkillsWindow _playerhud)))))
      (:else))))

(event Input|ActionEvents|InputActionToggleCraftingWindow
  (params (Key :type Key%20Structure))
  (:Pressed
    (if (not (Default|IsPauseMenuOpen (Variables|Default|GetPlayerHUD)))
      (Default|ToggleCraftingWindow (Variables|Default|GetPlayerHUD)))))

(event Input|ActionEvents|InputActionToggleInventory
  (params (Key :type Key%20Structure))
  (bind _ac_rpg_itemsmanager (Variables|Default|GetAC_RPG_ItemsManager))
  (:Pressed
    (if (not (Default|IsPauseMenuOpen (Variables|Default|GetPlayerHUD)))
      (Default|ToggleInventoryWindow (Variables|Default|GetPlayerHUD))
      ;[0.1 0.1 0.1 1 12] When we toggle inventory we should leave vendor and stash as well.
      (Default|LeaveStashSERVER _ac_rpg_itemsmanager)
      (Default|LeaveVendorSERVER _ac_rpg_itemsmanager))))

(event Input|ActionEvents|InputActionToggleCharacterInfo
  (params (Key :type Key%20Structure))
  (:Pressed
    (if (not (Default|IsPauseMenuOpen (Variables|Default|GetPlayerHUD)))
      (Default|ToggleStatsWindow (Variables|Default|GetPlayerHUD)))))

(event Input|ActionEvents|InputActionToggleQuestLog
  (params (Key :type Key%20Structure))
  (:Pressed
    (if (not (Default|IsPauseMenuOpen (Variables|Default|GetPlayerHUD)))
      (Default|ToggleQuestLogWindow (Variables|Default|GetPlayerHUD)))))

(event Input|ActionEvents|InputActionToggleAchievementsInfo
  (params (Key :type Key%20Structure))
  (:Pressed
    (if (not (Default|IsPauseMenuOpen (Variables|Default|GetPlayerHUD)))
      (Default|ToggleAchievementsWindow (Variables|Default|GetPlayerHUD)))))

(event Input|ActionEvents|InputActionToggleSkillTree
  (params (Key :type Key%20Structure))
  (:Pressed
    (if (not (Default|IsPauseMenuOpen (Variables|Default|GetPlayerHUD)))
      (Default|ToggleSkillsWindow (Variables|Default|GetPlayerHUD)))))

(event Input|ActionEvents|InputActionTogglePauseMenu
  (params (Key :type Key%20Structure))
  (:Pressed
    (bind _closedanywindow (Default|CloseAllOpenWindows (Variables|Default|GetPlayerHUD)))
    (if (not _closedanywindow) ; do not bring up pause menu if\nany of windows got closed
      (Default|TogglePauseMenu (Variables|Default|GetPlayerHUD))
      (else
        (Default|FinishActorInteractionSERVER (Variables|Default|GetAC_RPG_InteractionManager)) ; Additionally, when windows are getting closed we also finish interaction\n(ie. vendor window is closed so we do not interact with NPC anymore).
      ))))

(event Custom|OnQuickSlotPressed
  (params (QuickSlotIndex :type Integer))
  (bind _result (Default|CanUseSkill (Variables|Default|GetPlayerHero)))
  (if _result
    (Default|ActivateQuickSlotSERVER (Variables|Default|GetAC_RPG_QuickAccessManager) QuickSlotIndex)))

(event Input|ActionEvents|InputActionQuickSlot_2
  (params (Key :type Key%20Structure))
  ;[0.1 0.1 0.1 1 14] Quickslots
  (:Pressed
    (CallFunction|OnQuickSlotPressed 2)))

(event Input|ActionEvents|InputActionQuickSlot_3
  (params (Key :type Key%20Structure))
  ;[0.1 0.1 0.1 1 14] Quickslots
  (:Pressed
    (CallFunction|OnQuickSlotPressed 3)))

(event Input|ActionEvents|InputActionQuickSlot_4
  (params (Key :type Key%20Structure))
  ;[0.1 0.1 0.1 1 14] Quickslots
  (:Pressed
    (CallFunction|OnQuickSlotPressed 4)))

(event Input|ActionEvents|InputActionQuickSlot_1
  (params (Key :type Key%20Structure))
  ;[0.1 0.1 0.1 1 14] Quickslots
  (:Pressed
    (CallFunction|OnQuickSlotPressed 1)))

(event Input|ActionEvents|InputActionQuickSlot_5
  (params (Key :type Key%20Structure))
  ;[0.1 0.1 0.1 1 14] Quickslots
  (:Pressed
    (CallFunction|OnQuickSlotPressed 5)))

(event Input|ActionEvents|InputActionQuickSlot_6
  (params (Key :type Key%20Structure))
  ;[0.1 0.1 0.1 1 14] Quickslots
  (:Pressed
    (CallFunction|OnQuickSlotPressed 6)))

(event Input|ActionEvents|InputActionQuickSlot_7
  (params (Key :type Key%20Structure))
  ;[0.1 0.1 0.1 1 14] Quickslots
  (:Pressed
    (CallFunction|OnQuickSlotPressed 7)))

(event Input|ActionEvents|InputActionQuickSlot_8
  (params (Key :type Key%20Structure))
  ;[0.1 0.1 0.1 1 14] Quickslots
  (:Pressed
    (CallFunction|OnQuickSlotPressed 8)))

(event Input|ActionEvents|InputActionQuickSlot_9
  (params (Key :type Key%20Structure))
  ;[0.1 0.1 0.1 1 14] Quickslots
  (:Pressed
    (CallFunction|OnQuickSlotPressed 9)))

(event Input|ActionEvents|InputActionQuickSlot_10
  (params (Key :type Key%20Structure))
  ;[0.1 0.1 0.1 1 14] Quickslots
  (:Pressed
    (CallFunction|OnQuickSlotPressed 10)))

(event OnItemUsed(AC_RPG_ItemsManager)
  (params (ItemID :type Name :default "None"))
  (bind _result (Default|CanUseItem (Variables|Default|GetPlayerHero)))
  (if _result
    (Default|ActivateItem (Variables|Default|GetPlayerHero) ItemID (Variables|Default|GetAC_RPG_ItemsManager))
    (else
      (Variables|/Game/SuperiorRPGKit/Blueprints/Components/AC_RPG_ItemsManager.AC_RPG_ItemsManager_C|SetUsingItem (Variables|Default|GetAC_RPG_ItemsManager) false))))

(event OnVendorAccessed(AC_RPG_ItemsManager)
  (params (VendorContainer :type AC%20RPG%20Container%20Object%20Reference))
  (Default|SetInventoryWindowVisibility (Variables|Default|GetPlayerHUD) true)
  (Default|SetVendorWindowVisibility (Variables|Default|GetPlayerHUD) true)
  (Default|SetDialogueWindowVisibility (Variables|Default|GetPlayerHUD) false))

(event OnStashLeft(AC_RPG_ItemsManager)
  (Default|SetStorageWindowVisibility (Variables|Default|GetPlayerHUD) false)
  (Default|SetInventoryWindowVisibility (Variables|Default|GetPlayerHUD) false))

(event OnStashAccessed(AC_RPG_ItemsManager)
  (params (StashContainer :type AC%20RPG%20Container%20Object%20Reference))
  (Default|SetInventoryWindowVisibility (Variables|Default|GetPlayerHUD) true)
  (Default|SetStorageWindowVisibility (Variables|Default|GetPlayerHUD) true))

(event OnVendorLeft(AC_RPG_ItemsManager)
  (Default|SetVendorWindowVisibility (Variables|Default|GetPlayerHUD) false)
  (Default|SetInventoryWindowVisibility (Variables|Default|GetPlayerHUD) false))

(event OnDialogueStarted(AC_RPG_InteractionManager)
  (Default|SetDialogueWindowVisibility (Variables|Default|GetPlayerHUD) true))

(event OnDialogueEnded(AC_RPG_InteractionManager)
  (Default|SetDialogueWindowVisibility (Variables|Default|GetPlayerHUD) false))

(event OnSkillCastRequested(AC_RPG_SkillsManager)
  (params (SkillID :type Name :default "None") (SkillLevel :type Integer))
  (Default|QueueSkill (Variables|Default|GetPlayerHero) SkillID))

(event OnKilled(AC_RPG_StatsManager)
  (params (Killer :type Actor%20Object%20Reference))
  (Utilities|FlowControl|Sequence
    (:then_0
      ;[0.1 0.1 0.1 1 14] Disable any hero movement.
      (Pawn|Components|CharacterMovement|DisableMovement (Variables|/Script/Engine.Character|GetCharacterMovement (Variables|Default|GetPlayerHero)))
      ;[0.1 0.1 0.1 1 14] If was hero was controlled by AI, it unpossess the hero.
      ; Non-possessed character doesn't affect navigation grid.
      (bind _aicontroller (Variables|/Game/SuperiorRPGKit/Blueprints/Basics/BP_RPG_Hero.BP_RPG_Hero_C|GetAIController (Variables|Default|GetPlayerHero))
        (:then
          (Pawn|UnPossess _aicontroller))
        (:else)))
    (:then_1
      ;[0.1 0.1 0.1 1 14] Play death effect on all clients.
      (Default|DeathEffectMULTICAST (Variables|Default|GetPlayerHero))
      ;[0.1 0.1 0.1 1 14] For third person additionalyl turn off targeting if it was active.
      (if (Variables|Default|GetThirdPersonMode)
        (bind _asbp_rpg_pc_in_game_third_person (Utilities|Casting|CastToBP_RPG_PC_InGame_ThirdPerson self))
        (if (Variables|/Game/SuperiorRPGKit/Blueprints/Basics/ThirdPerson/BP_RPG_PC_InGame_ThirdPerson.BP_RPG_PC_InGame_ThirdPerson_C|GetLockOnActive _asbp_rpg_pc_in_game_third_person)
          (Default|ToggleTargetingSERVER _asbp_rpg_pc_in_game_third_person))))
    (:then_2
      ;[0.1 0.1 0.1 1 14] Respawn automatically after small delay.
      (Utilities|FlowControl|Delay 5.0)
      (CallFunction|Respawn))))

(event OnDamageReceived(AC_RPG_StatsManager)
  (params (Damage :type Float%20%28single-precision%29) (CriticalHit :type Boolean) (DamageDealer :type Actor%20Object%20Reference))
  (Default|DisplayDamagePopUpCLIENT (Variables|Default|GetAC_RPG_FloatingTextManager) Damage (Transformation|GetActorLocation (Variables|Default|GetPlayerHero)) CriticalHit)
  (Default|FinishActorInteractionSERVER (Variables|Default|GetAC_RPG_InteractionManager)))

(event Custom|Respawn
  (bind _playerhero (Variables|Default|GetPlayerHero))
  (Utilities|FlowControl|Sequence
    (:then_0
      ;[0.1 0.1 0.1 1 14] Restore hero movement capabilities.
      (Pawn|Components|CharacterMovement|SetMovementMode (Variables|/Script/Engine.Character|GetCharacterMovement (Variables|Default|GetPlayerHero)) "MOVE_Walking" 0)
      ;[0.1 0.1 0.1 1 14] Re-possess hero by AI if it was controlled by AI before death.
      (bind _aicontroller (Variables|/Game/SuperiorRPGKit/Blueprints/Basics/BP_RPG_Hero.BP_RPG_Hero_C|GetAIController _playerhero)
        (:then
          (Pawn|Possess _aicontroller _playerhero))
        (:else)))
    (:then_1
      ;[0.1 0.1 0.1 1 14] Set current health to max value.
      (Default|SetStatCurrentValuetoMax (Variables|Default|GetAC_RPG_StatsManager) "NewEnumerator1"))
    (:then_2
      ;[0.1 0.1 0.1 1 14] Move hero to respawn point.
      (bind _transform (Default|GetRespawnTransform (Variables|/Game/SuperiorRPGKit/Blueprints/Components/AC_RPG_SavesManager.AC_RPG_SavesManager_C|GetActiveRespawn (Variables|Default|GetAC_RPG_SavesManager))))
      (Transformation|SetActorTransform (Variables|Default|GetPlayerHero) _transform))
    (:then_3
      ;[0.1 0.1 0.1 1 14] Play resurrection effect on all clients.
      (Default|ResurrectionEffectMULTICAST (Variables|Default|GetPlayerHero)))))

(event Custom|ReturnToMainMenu
  (Utilities|FlowControl|DoOnce false
    (:Completed
      (Default|Fadein (Variables|/Game/SuperiorRPGKit/Blueprints/Basics/BP_RPG_HUD.BP_RPG_HUD_C|GetLoadingScreen (Variables|Default|GetPlayerHUD)))
      (CallFunction|SavePlayerDataCLIENT)
      (Utilities|FlowControl|Delay 1.0)
      (Game|OpenLevel(byName) (Variables|Default|GetMainMenuMap)))))

(event Custom|QuitToDesktop
  (Utilities|FlowControl|DoOnce false
    (:Completed
      (CallFunction|SavePlayerDataCLIENT)
      (Utilities|FlowControl|Delay 0.2)
      (Game|QuitGame 0 "Quit"))))

(fn ConstructionScript)