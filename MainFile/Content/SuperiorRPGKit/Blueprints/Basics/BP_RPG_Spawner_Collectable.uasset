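; Spawner actor that populates a radius around itself with collectables of a configurable class, up to a maximum count.
; On the authority, it can spawn at BeginPlay, placing one or all missing collectables at random navigable points with random yaw.
; Each collectable receives the spawner as its AssociatedSpawner; RemoveCollectable untracks and destroys one.
; Spawning and removal both start a random-delay respawn timer, skipped when already running or at capacity.
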(event Custom|StartRespawnTimer
  (if (> (- (Variables|Config|GetMaxNumberOfCollectables) (Utilities|Array|Length (Variables|Default|GetSpawnedCollectables))) 0) ; Spawn collectables only if their \nmax number hasn't been reached.
    (if (not (Utilities|Time|IsTimerActivebyHandle (stale _returnvalue))) ; Do nto restart timer if it is already counting.
      (bind _returnvalue (Utilities|Time|SetTimerbyEvent (EventDispatchers|CreateEvent :!event SpawnCollectables) (Math|Random|RandomFloatinRange (Variables|Config|GetMinRespawnTime) (Variables|Config|GetMaxRespawnTime)))))))

(event EventBeginPlay
  (Networking|SwitchHasAuthority
    (:Authority
      (if (Variables|Config|GetSpawnOnBeginPlay)
        (CallFunction|SpawnCollectables)))))

(fn ConstructionScript
  (Components|Sphere|SetSphereRadius (Variables|Default|GetSphere_SpawnRadius) (Variables|Config|GetSpawnRadius) true))

(fn GetRandomLocationinSpawnRadius
  (bind _returnvalue (Transformation|GetActorLocation))
  (bind _spawnradius (Variables|Config|GetSpawnRadius))
  (bind (_randomlocation _returnvalue_2) (Class|NavigationSystem|GetRandomPointinNavigableRadius _returnvalue _spawnradius))
  (return _returnvalue_2 _randomlocation))

(fn SpawnCollectables
  (bind _output_get (LocalVariables|SetTotalNumberOfMissingCollectablesLOCAL (- (Variables|Config|GetMaxNumberOfCollectables) (Utilities|Array|Length (Variables|Default|GetSpawnedCollectables)))))
  (if (> _output_get 0)
    (Utilities|FlowControl|Sequence
      (:then_0
        ;[0.1 0.1 0.1 1 14] Spawn collectable(s) in spawner radius.
        (for _index (range 1 (Math|Integer|SelectInt (LocalVariables|GetTotalNumberOfMissingCollectablesLOCAL) 1 (Variables|Config|GetSpawnAllAtOnce)))
          (bind (_result _spawnlocation) (Getters|GetRandomLocationinSpawnRadius))
          (if _result
            (bind _returnvalue (Game|SpawnActorfromClass (Variables|Config|GetCollectableToSpawn) (Math|Transform|MakeTransform _spawnlocation (Math|Rotator|MakeRotator 0.0 0.0 (Math|Random|RandomFloatinRange 0.0 359.0)) "1,1,1") "AdjustIfPossibleButDontSpawnIfColliding" 0 self 0))
            (Utilities|IsValid _returnvalue
              (:Is%20Valid
                (Utilities|Array|Add (Variables|Default|GetSpawnedCollectables) _returnvalue))))))
      (:then_1
        (CallFunction|StartRespawnTimer)))))

(fn RemoveCollectable
  (params (Collectable :type BP%20RPG%20Quest%20Collectable%20Object%20Reference))
  (Utilities|FlowControl|Sequence
    (:then_0
      (Utilities|Array|RemoveItem (Variables|Default|GetSpawnedCollectables) Collectable))
    (:then_1
      (Actor|DestroyActor Collectable))
    (:then_2
      (CallFunction|StartRespawnTimer))))