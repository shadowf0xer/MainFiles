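; Base replicated enemy character for the RPG kit, with stubbed AI events and combat functions for child Blueprints to extend.
; Stats come from the StatsManager component, whose damage events feed threat to the AI controller and whose health mirrors into a replicated percentage driving floating and hover health bars.
; On death it grants XP, quest and achievement progress to nearby players, spawns rolled loot, and unpossesses, re-possessing before delayed destruction to clean up the controller.
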(event OnStatCurrentPercentageValueChanged(AC_RPG_StatsManager)
  (params (Stat :type E_RPG_StatType%20Enum :default "NewEnumerator0") (PercentageValue :type Float%20%28single-precision%29))
  ;[0.1 0.1 0.1 1 14] Whenever current health value changes on server (in StatsManager) we reflects its in replicated variable so health value is always up to date on clients.
  ; (So we see proper value in various widgets).
  (if (Utilities|Enum|Equal(Enum) Stat "NewEnumerator1")
    (Variables|Replication|SetHealthPercentage PercentageValue)))

(event OnBeginCursorOver(CapsuleComponent)
  (params (TouchedComponent :type Primitive%20Component%20Object%20Reference))
  ;[0.1 0.1 0.1 1 14] Handles cursor over begin/end behavior.
  (bind _result (CallFunction|IsInteractable))
  (if _result
    (Variables|Default|SetHoveredOver true)
    (bind _asbp_rpg_pc_in_game (Utilities|Casting|CastToBP_RPG_PC_InGame (Game|GetPlayerController 0)))
    (Widget|SetVisibility (Variables|/Game/SuperiorRPGKit/Widgets/Player/WBP_RPG_InGameHUD.WBP_RPG_InGameHUD_C|GetWBP_RPG_EnemyInfo (Variables|/Game/SuperiorRPGKit/Blueprints/Basics/BP_RPG_HUD.BP_RPG_HUD_C|GetInGameHUD (Variables|/Game/SuperiorRPGKit/Blueprints/Basics/BP_RPG_PC_InGame.BP_RPG_PC_InGame_C|GetPlayerHUD _asbp_rpg_pc_in_game))) "HitTestInvisible")
    (bind _returnvalue (Utilities|GetDataTableRow "/Game/SuperiorRPGKit/Datatables/DT_RPG_Enemies.DT_RPG_Enemies" (Variables|Config|GetEnemyID))
      (:then
        (Rendering|Components|TextRender|SetText (Variables|/Game/SuperiorRPGKit/Widgets/Player/WBP_RPG_EnemyInfo.WBP_RPG_EnemyInfo_C|GetTextBlock_EnemyName (Variables|/Game/SuperiorRPGKit/Widgets/Player/WBP_RPG_InGameHUD.WBP_RPG_InGameHUD_C|GetWBP_RPG_EnemyInfo (Variables|/Game/SuperiorRPGKit/Blueprints/Basics/BP_RPG_HUD.BP_RPG_HUD_C|GetInGameHUD (Variables|/Game/SuperiorRPGKit/Blueprints/Basics/BP_RPG_PC_InGame.BP_RPG_PC_InGame_C|GetPlayerHUD _asbp_rpg_pc_in_game)))) (.DisplayName (Utilities|Struct|BreakS_RPG_Enemy_Static _returnvalue)))
        (Progress|SetPercent (Variables|/Game/SuperiorRPGKit/Widgets/Player/WBP_RPG_EnemyInfo.WBP_RPG_EnemyInfo_C|GetProgressBar_Stat (Variables|/Game/SuperiorRPGKit/Widgets/Player/WBP_RPG_InGameHUD.WBP_RPG_InGameHUD_C|GetWBP_RPG_EnemyInfo (Variables|/Game/SuperiorRPGKit/Blueprints/Basics/BP_RPG_HUD.BP_RPG_HUD_C|GetInGameHUD (Variables|/Game/SuperiorRPGKit/Blueprints/Basics/BP_RPG_PC_InGame.BP_RPG_PC_InGame_C|GetPlayerHUD _asbp_rpg_pc_in_game)))) (Variables|Replication|GetHealthPercentage))))))

(event OnEndCursorOver(CapsuleComponent)
  (params (TouchedComponent :type Primitive%20Component%20Object%20Reference))
  ;[0.1 0.1 0.1 1 14] Handles cursor over begin/end behavior.
  (Variables|Default|SetHoveredOver false)
  (bind _asbp_rpg_pc_in_game (Utilities|Casting|CastToBP_RPG_PC_InGame (Game|GetPlayerController 0)))
  (Widget|SetVisibility (Variables|/Game/SuperiorRPGKit/Widgets/Player/WBP_RPG_InGameHUD.WBP_RPG_InGameHUD_C|GetWBP_RPG_EnemyInfo (Variables|/Game/SuperiorRPGKit/Blueprints/Basics/BP_RPG_HUD.BP_RPG_HUD_C|GetInGameHUD (Variables|/Game/SuperiorRPGKit/Blueprints/Basics/BP_RPG_PC_InGame.BP_RPG_PC_InGame_C|GetPlayerHUD _asbp_rpg_pc_in_game))) "Collapsed"))

(event Custom|Initialize
  (bind _ac_rpg_statsmanager (Variables|Components|GetAC_RPG_StatsManager))
  (Variables|AI|SetInitialSpawnLocation (Transformation|GetActorLocation)) ; Store location where enemy was spawned.
  ;[0.1 0.1 0.1 1 14] Initialize enemy stats.
  (Default|InitializeStats(Enemy) _ac_rpg_statsmanager)
  (Default|PerformFullAttributesandStatsRecalculation _ac_rpg_statsmanager)
  (Default|SetStatCurrentValuetoMax (Variables|Components|GetAC_RPG_StatsManager) "NewEnumerator1")
  ;[0.1 0.1 0.1 1 14] Initialize AI Controller.
  (bind _asbp_ai_controller (Utilities|Casting|CastToBP_AI_Controller (AI|GetAIController self)))
  (bind _output_get (Variables|References|SetAIController _asbp_ai_controller))
  (Default|Initialize _output_get (Variables|Config|GetAIConfiguration)))

(event OnDamageReceived(AC_RPG_StatsManager)
  (params (Damage :type Float%20%28single-precision%29) (CriticalHit :type Boolean) (DamageDealer :type Actor%20Object%20Reference))
  (Utilities|IsValid DamageDealer
    (:Is%20Valid
      (Default|ModifyThreat (Variables|/Game/SuperiorRPGKit/AI/Blueprints/Core/BP_AI_Controller.BP_AI_Controller_C|GetAC_AI_Target (Variables|References|GetAIController)) DamageDealer Damage))))

(event OnKilled(AC_RPG_StatsManager)
  (params (Killer :type Actor%20Object%20Reference))
  (bind _self self)
  (bind _self_2 self)
  (bind _returnvalue (AI|GetAIController _self))
  (bind _returnvalue_2 (AI|GetAIController _self_2))
  (Utilities|FlowControl|Sequence
    (:then_0
      (DeathRewards|AllocateRewards) ; Give rewards to players in radius.
      (DeathRewards|SpawnLoot) ; Spawn loot on the ground.
    )
    (:then_1
      (Pawn|Components|CharacterMovement|DisableMovement (Variables|Character|GetCharacterMovement)) ; Disable any movement.
      ;[0.1 0.1 0.1 1 14] AI unpossesses dead enemy so it doesn't affect navigation grid while it lies dead on the ground.
      ; IMPORTANT: In the moment you want to remove enemy from the game (ie. after 5 seconds) you HAVE TO re-possess that enemy by its AI so upon deleting the enemy, its AI will be deleted as well.
      (Utilities|IsValid _returnvalue
        (:Is%20Valid
          (Pawn|UnPossess _returnvalue))))
    (:then_2
      (Utilities|FlowControl|Delay 5.0)
      ;[0.1 0.1 0.1 1 14] AI (if exists) repossesses dead enemy so it got destroyed together with controlled pawn.
      (Utilities|IsValid _returnvalue_2
        (:Is%20Valid
          (Pawn|Possess _returnvalue_2 self))
        (:Is%20Not%20Valid
          _))
      (Actor|DestroyActor))
    (:then_3
      (CallFunction|DeathEffectMULTICAST))
    (:then_4
      (Variables|Replication|SetDead true))))

(event Custom|DeathEffect_MULTICAST
  ;[0.1 0.1 0.1 1 14] General set up for death event, usually extended in children blueprints.
  (Variables|/Game/SuperiorRPGKit/Blueprints/Components/AC_RPG_StatsManager.AC_RPG_StatsManager_C|SetDead (Variables|Components|GetAC_RPG_StatsManager) true)
  (Collision|SetCollisionEnabled (Variables|Collision|GetCapsuleComponent) "NoCollision")
  (bind _returnvalue (Animation|GetCurrentMontage :!class /Script/Engine.Character))
  (Animation|StopAnimMontage _returnvalue))

(event Custom|PlayMontage_MULTICAST
  (params (AnimMontage :type Anim%20Montage%20Object%20Reference) (InPlayRate :type Float%20%28single-precision%29) (StartSectionName :type Name))
  ;[0.1 0.1 0.1 1 14] Used to play and stop montages on all clients.
  (Animation|PlayAnimMontage AnimMontage InPlayRate StartSectionName))

(event Custom|StopCurrentMontage_MULTICAST
  ;[0.1 0.1 0.1 1 14] Used to play and stop montages on all clients.
  (bind _returnvalue (Animation|GetCurrentMontage :!class /Script/Engine.Character))
  (Animation|StopAnimMontage _returnvalue))

(event OnEffectTickExecuted(AC_RPG_StatsManager)
  (params (EffectType :type E_RPG_EffectType%20Enum :default "NewEnumerator0") (EffectStruct :type S%20RPG%20Effect%20Dynamic%20Structure))
  (switch Utilities|FlowControl|Switch|SwitchonE_RPG_EffectType EffectType
    (:NewEnumerator5
      (Default|ReceiveDamage (Variables|Components|GetAC_RPG_StatsManager) (Utilities|Struct|BreakS_RPG_Effect_Dynamic EffectStruct) 0.0 0.0))))

(event EventOnCombatDisengaged
  (params (AttackType :type E_AI_AttackType%20Enum :default "NewEnumerator0"))
  ;[0.1 0.1 0.1] Engage/disengage combat.
)

(event EventOnAttackEffectResolved
  (params (AttackID :type Name :default "None"))
  ;[0.1 0.1 0.1] Attack
)

(event EventOnAttackInterrupted
  (params (AttackType :type E_AI_AttackType%20Enum :default "NewEnumerator0"))
  ;[0.1 0.1 0.1] Attack
)

(event EventOnFollowTargetChanged
  (params (FollowTarget :type Actor%20Object%20Reference))
  ;[0.1 0.1 0.1] Follow
)

(event EventOnSwitchedtoSupport
  (params (SwitchedFrom :type E_AI_AttackType%20Enum :default "NewEnumerator0"))
  ;[0.1 0.1 0.1] Switch weapon/stance
)

(event EventOnInteractionStarted
  (params (InteractedActor :type Actor%20Object%20Reference))
  ;[0.1 0.1 0.1] Interact
)

(event EventOnInteractionEnded
  (params (InteractedActor :type Actor%20Object%20Reference) (Reason :type E_AI_InteractionEndReason%20Enum :default "NewEnumerator0"))
  ;[0.1 0.1 0.1] Interact
)

(event EventOnSwitchedtoMelee
  (params (SwitchedFrom :type E_AI_AttackType%20Enum :default "NewEnumerator0"))
  ;[0.1 0.1 0.1] Switch weapon/stance
)

(event EventOnSwitchingInterrupted
  ;[0.1 0.1 0.1] Switch weapon/stance
)

(event EventOnSwitchedtoRanged
  (params (SwitchedFrom :type E_AI_AttackType%20Enum :default "NewEnumerator0"))
  ;[0.1 0.1 0.1] Switch weapon/stance
)

(event EventOnRoamBreakStarted
  (params (BreakDuration :type Float%20%28single-precision%29))
  ;[0.1 0.1 0.1] Roam
)

(event EventOnPatrolBreakStarted
  (params (BreakDuration :type Float%20%28single-precision%29))
  ;[0.1 0.1 0.1] Patrol
)

(event EventOnPatrolBreakEnded
  (params (TimeElapsed :type Float%20%28single-precision%29))
  ;[0.1 0.1 0.1] Patrol
)

(event EventOnRoamBreakEnded
  (params (TimeElapsed :type Float%20%28single-precision%29))
  ;[0.1 0.1 0.1] Roam
)

(event EventOnRoamTargetChanged
  (params (RoamTarget :type Actor%20Object%20Reference))
  ;[0.1 0.1 0.1] Roam
)

(event EventOnMovementFinished
  (params (Result :type EPathFollowingResult%20Enum :default "Success") (Behavior :type E_AI_BehaviorType%20Enum :default "NewEnumerator0"))
  ;[0.1 0.1 0.1] Move
)

(event EventOnCombatEngaged
  (params (AttackType :type E_AI_AttackType%20Enum :default "NewEnumerator0"))
  ;[0.1 0.1 0.1] Engage/disengage combat.
)

(fn ConstructionScript
  (Variables|/Game/SuperiorRPGKit/Blueprints/Components/AC_RPG_StatsManager.AC_RPG_StatsManager_C|SetCharacterID (Variables|Components|GetAC_RPG_StatsManager) (Variables|Config|GetEnemyID)))

(fn OnRepCurrentHealth
  (bind _healthpercentage (Variables|Replication|GetHealthPercentage))
  (bind _healthpercentage_2 (Variables|Replication|GetHealthPercentage))
  (bind _asbp_rpg_pc_in_game (Utilities|Casting|CastToBP_RPG_PC_InGame (Game|GetPlayerController 0)))
  (if (not (Variables|/Game/SuperiorRPGKit/Blueprints/Basics/BP_RPG_PC_InGame.BP_RPG_PC_InGame_C|GetThirdPersonMode _asbp_rpg_pc_in_game))
    (Utilities|FlowControl|Sequence
      (:then_0
        ;[0.1 0.1 0.1 1 14] Update floating health bar value.
        (bind _aswbp_rpg_floating_stat_bar (Utilities|Casting|CastToWBP_RPG_FloatingStatBar (UserInterface|GetUserWidgetObject (Variables|Components|GetHealthBar))))
        (Default|SetBarPercent _aswbp_rpg_floating_stat_bar _healthpercentage)
        (Development|SetHiddeninGame (Variables|Components|GetHealthBar) (or (== _healthpercentage 1.0) (== _healthpercentage 0.0)) false))
      (:then_1
        ;[0.1 0.1 0.1 1 14] Update top EnemyInfo widget health bar value if cursor is hovered over this enemy.
        (if (Variables|Default|GetHoveredOver)
          (Progress|SetPercent (Variables|/Game/SuperiorRPGKit/Widgets/Player/WBP_RPG_EnemyInfo.WBP_RPG_EnemyInfo_C|GetProgressBar_Stat (Variables|/Game/SuperiorRPGKit/Widgets/Player/WBP_RPG_InGameHUD.WBP_RPG_InGameHUD_C|GetWBP_RPG_EnemyInfo (Variables|/Game/SuperiorRPGKit/Blueprints/Basics/BP_RPG_HUD.BP_RPG_HUD_C|GetInGameHUD (Variables|/Game/SuperiorRPGKit/Blueprints/Basics/BP_RPG_PC_InGame.BP_RPG_PC_InGame_C|GetPlayerHUD _asbp_rpg_pc_in_game)))) _healthpercentage_2)
          (if (== _healthpercentage_2 0.0) ; Hide enemy info when killed.
            (Widget|SetVisibility (Variables|/Game/SuperiorRPGKit/Widgets/Player/WBP_RPG_InGameHUD.WBP_RPG_InGameHUD_C|GetWBP_RPG_EnemyInfo (Variables|/Game/SuperiorRPGKit/Blueprints/Basics/BP_RPG_HUD.BP_RPG_HUD_C|GetInGameHUD (Variables|/Game/SuperiorRPGKit/Blueprints/Basics/BP_RPG_PC_InGame.BP_RPG_PC_InGame_C|GetPlayerHUD _asbp_rpg_pc_in_game))) "Collapsed")))))))

(fn AllocateRewards
  (LocalVariables|SetRadiusSquaredLOCAL (Math|Float|Square (Variables|Config|GetRewardRadius)))
  (bind _returnvalue (Utilities|GetDataTableRow "/Game/SuperiorRPGKit/Datatables/DT_RPG_Enemies.DT_RPG_Enemies" (Variables|Config|GetEnemyID))
    (:then
      (LocalVariables|SetXPRewardLOCAL (* (Variables|/Game/SuperiorRPGKit/Blueprints/Components/AC_RPG_StatsManager.AC_RPG_StatsManager_C|GetCurrentLevel (Variables|Components|GetAC_RPG_StatsManager)) (.PerLevelXP (Utilities|Struct|BreakS_RPG_Enemy_Static _returnvalue))))
      (LocalVariables|SetAchievementsObjectivesLOCAL (.AchievementsObjectives (Utilities|Struct|BreakS_RPG_Enemy_Static _returnvalue)))
      (LocalVariables|SetQuestObjectivesLOCAL (.QuestObjectives (Utilities|Struct|BreakS_RPG_Enemy_Static _returnvalue)))
      (bind _asbp_rpg_gm_in_game (Utilities|Casting|CastToBP_RPG_GM_InGame (Game|GetGameMode)))
      (for _array_element (Variables|/Game/SuperiorRPGKit/Blueprints/Basics/BP_RPG_GM_InGame.BP_RPG_GM_InGame_C|GetConnectedPlayers _asbp_rpg_gm_in_game)
        (LocalVariables|SetPlayerLOCAL _array_element)
        (bind _playerhero (Variables|/Game/SuperiorRPGKit/Blueprints/Basics/BP_RPG_PC_InGame.BP_RPG_PC_InGame_C|GetPlayerHero (LocalVariables|GetPlayerLOCAL))
          (:then
            ;[0.1 0.1 0.1 1 14] Check if player can receive reward for killed enemy.
            (bind _result (Default|CanReceiveKillReward _playerhero))
            (if _result
              (if (< (Transformation|GetSquaredDistanceTo _playerhero) (LocalVariables|GetRadiusSquaredLOCAL))
                (Utilities|FlowControl|Sequence
                  (:then_0
                    ;[0.1 0.1 0.1 1 14] Give XP to player.
                    (Default|ReceiveExperience (Actor|GetComponentbyClass (LocalVariables|GetPlayerLOCAL) "/Game/SuperiorRPGKit/Blueprints/Components/AC_RPG_StatsManager.AC_RPG_StatsManager_C") (LocalVariables|GetXPRewardLOCAL)))
                  (:then_1
                    ;[0.1 0.1 0.1 1 14] Add achievements progress to player.
                    (for _array_element_2 (LocalVariables|GetAchievementsObjectivesLOCAL)
                      (Default|AddAchievementsProgress (Actor|GetComponentbyClass (LocalVariables|GetPlayerLOCAL) "/Game/SuperiorRPGKit/Blueprints/Components/AC_RPG_AchievementsManager.AC_RPG_AchievementsManager_C") _array_element_2 1)))
                  (:then_2
                    ;[0.1 0.1 0.1 1 14] Add quest objective progress to player.
                    (for _array_element_3 (LocalVariables|GetQuestObjectivesLOCAL)
                      (Default|AddQuestObjectiveProgress (Actor|GetComponentbyClass (LocalVariables|GetPlayerLOCAL) "/Game/SuperiorRPGKit/Blueprints/Components/AC_RPG_QuestsManager.AC_RPG_QuestsManager_C") _array_element_3 1)))))))
          (:else))))))

(fn OnRepDead
  (if (not (Variables|/Game/SuperiorRPGKit/Blueprints/Components/AC_RPG_StatsManager.AC_RPG_StatsManager_C|GetDead (Variables|Components|GetAC_RPG_StatsManager)))
    (Variables|/Game/SuperiorRPGKit/Blueprints/Components/AC_RPG_StatsManager.AC_RPG_StatsManager_C|SetDead (Variables|Components|GetAC_RPG_StatsManager) true)
    (Collision|SetCollisionEnabled (Variables|Collision|GetCapsuleComponent) "NoCollision")
    (Rendering|SetActorHiddenInGame true)))

(fn SpawnLoot
  (bind _returnvalue (Utilities|GetDataTableRow "/Game/SuperiorRPGKit/Datatables/DT_RPG_Enemies.DT_RPG_Enemies" (Variables|Config|GetEnemyID))
    (:then
      (for _index (range 1 (Math|Random|RandomIntegerinRange 3 3))
        (LocalVariables|SetRolledItemLOCAL (Utilities|Array|Get(acopy) (.LootableItems (Utilities|Struct|BreakS_RPG_Enemy_Static _returnvalue)) (Math|Random|RandomIntegerinRange 0 (- (Utilities|Array|Length (.LootableItems (Utilities|Struct|BreakS_RPG_Enemy_Static _returnvalue))) 1))))
        (LocalVariables|SetRolledItemQualityLOCAL (CallFunction|RollItemQuality (LocalVariables|GetRolledItemLOCAL)))
        (Game|SpawnActorfromClass "/Game/SuperiorRPGKit/Blueprints/Basics/BP_RPG_Item.BP_RPG_Item_C" (Math|Transform|MakeTransform (.RandomLocation (Class|NavigationSystem|GetRandomPointinNavigableRadius (Transformation|GetActorLocation) 3e+02)) "0, 0, 0" "1,1,1") "AdjustIfPossibleButDontSpawnIfColliding" 0 (Utilities|Struct|MakeS_RPG_Item_Dynamic (LocalVariables|GetRolledItemLOCAL) 1 (LocalVariables|GetRolledItemQualityLOCAL) (CallFunction|RollItemBonuses (LocalVariables|GetRolledItemLOCAL) (LocalVariables|GetRolledItemQualityLOCAL) false)) false 0)))))

(fn CanAttack
  (params (AttackType :type E_AI_AttackType%20Enum :default "NewEnumerator0"))
  (return (not (Variables|/Game/SuperiorRPGKit/Blueprints/Components/AC_RPG_StatsManager.AC_RPG_StatsManager_C|GetDead (Variables|Components|GetAC_RPG_StatsManager)))))

(fn CanbeTargeted
  (return (not (Variables|/Game/SuperiorRPGKit/Blueprints/Components/AC_RPG_StatsManager.AC_RPG_StatsManager_C|GetDead (Variables|Components|GetAC_RPG_StatsManager)))))

(fn CanInteract
  (return (not (Variables|/Game/SuperiorRPGKit/Blueprints/Components/AC_RPG_StatsManager.AC_RPG_StatsManager_C|GetDead (Variables|Components|GetAC_RPG_StatsManager)))))

(fn CanMove
  (return (not (Variables|/Game/SuperiorRPGKit/Blueprints/Components/AC_RPG_StatsManager.AC_RPG_StatsManager_C|GetDead (Variables|Components|GetAC_RPG_StatsManager)))))

(fn CanReceiveKillReward
  (return false))

(fn CanSupport
  (return (not (Variables|/Game/SuperiorRPGKit/Blueprints/Components/AC_RPG_StatsManager.AC_RPG_StatsManager_C|GetDead (Variables|Components|GetAC_RPG_StatsManager)))))

(fn CanSwitchWeapon
  (return (not (Variables|/Game/SuperiorRPGKit/Blueprints/Components/AC_RPG_StatsManager.AC_RPG_StatsManager_C|GetDead (Variables|Components|GetAC_RPG_StatsManager)))))

(fn CanUseItem
  (return (not (Variables|/Game/SuperiorRPGKit/Blueprints/Components/AC_RPG_StatsManager.AC_RPG_StatsManager_C|GetDead (Variables|Components|GetAC_RPG_StatsManager)))))

(fn CanUseSkill
  (return (not (Variables|/Game/SuperiorRPGKit/Blueprints/Components/AC_RPG_StatsManager.AC_RPG_StatsManager_C|GetDead (Variables|Components|GetAC_RPG_StatsManager)))))

(fn DisengageCombat
  (params (AttackType :type E_AI_AttackType%20Enum :default "NewEnumerator0"))
  (return true 0.0))

(fn EngageCombat
  (params (AttackType :type E_AI_AttackType%20Enum :default "NewEnumerator0"))
  (return true 0.0))

(fn GenerateAllytoSupport
  (params (AlliesInRange :type Set%20of%20Actor%20Object%20References))
  (return false false 0))

(fn GenerateEnemytoAttack
  (params (EnemiesInRange :type Set%20of%20Actor%20Object%20References))
  (return false false 0))

(fn GetInteractionAction
  (params (InteractingActor :type Actor%20Object%20Reference))
  (return "NewEnumerator3"))

(fn GetInteractionRadius
  (params (InteractingActor :type Actor%20Object%20Reference))
  (return 0.0))

(fn GetInteractionText
  (return ""))

(fn GetInteractionTime
  (params (InteractingActor :type Actor%20Object%20Reference))
  (return 0.0))

(fn GetInteractionType
  (return "NewEnumerator5"))

(fn IsInteractable
  (params (InteractingActor :type Actor%20Object%20Reference) (InteractionManager :type AC%20RPG%20Interaction%20Manager%20Object%20Reference))
  (return (> (Variables|Replication|GetHealthPercentage) 0.0)))

(fn StartInteracting
  (params (InteractedActor :type Actor%20Object%20Reference))
  (return false 0.0))

(fn StopInteracting
  (params (InteractedActor :type Actor%20Object%20Reference) (Reason :type E_AI_InteractionEndReason%20Enum :default "NewEnumerator0"))
  (return false))

(fn SwitchtoMelee
  (params (SwitchingFrom :type E_AI_AttackType%20Enum :default "NewEnumerator0"))
  (return true 0.0))

(fn SwitchtoRanged
  (params (SwitchingFrom :type E_AI_AttackType%20Enum :default "NewEnumerator0"))
  (return true 0.0))

(fn SwitchtoSupport
  (params (SwitchingFrom :type E_AI_AttackType%20Enum :default "NewEnumerator0"))
  (return false 0.0))

(fn UseMeleeAttack
  (params (TargetActor :type Actor%20Object%20Reference))
  (return false 0.0))

(fn UseRangedAttack
  (params (TargetActor :type Actor%20Object%20Reference))
  (return false 0.0))

(fn UseSupportAction
  (params (TargetActor :type Actor%20Object%20Reference))
  (return false 0.0))