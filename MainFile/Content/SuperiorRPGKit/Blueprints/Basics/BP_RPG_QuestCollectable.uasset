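; BP_RPG_QuestCollectable is an interactable world item that advances a quest objective when the player collects it.
; It implements the kit's interaction functions, showing a "Collect" prompt with its display name, and is interactable only while the interactor's quest manager needs its objective.
; On interaction, a DoOnce adds one progress to that objective through the quest manager, then asks any associated spawner to remove the collectable.
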(event EventBeginPlay)

(event Collision|EventActorBeginOverlap
  (params (OtherActor :type Actor%20Object%20Reference)))

(event EventTick
  (params (DeltaSeconds :type Float%20%28single-precision%29)))

(event EventOnBeginInteract
  (params (InteractingActor :type Actor%20Object%20Reference) (InteractionManager :type AC%20RPG%20Interaction%20Manager%20Object%20Reference))
  (bind _returnvalue (Components|GetOwner InteractionManager))
  (bind _returnvalue_2 (Actor|GetComponentbyClass _returnvalue "/Game/SuperiorRPGKit/Blueprints/Components/AC_RPG_QuestsManager.AC_RPG_QuestsManager_C"))
  ;[0.1 0.1 0.1 1 14] On interaction add progress to quest objective specified by colelctable.
  (Utilities|IsValid _returnvalue_2
    (:Is%20Valid
      (Utilities|FlowControl|DoOnce false
        (:Completed
          (Default|AddQuestObjectiveProgress _returnvalue_2 (Variables|Config|GetQuestObjective) 1)
          (bind _associatedspawner (Variables|Runtime|GetAssociatedSpawner)
            (:then
              (Default|RemoveCollectable _associatedspawner self))
            (:else)))))))

(event EventOnFinishInteract
  (params (InteractingActor :type Actor%20Object%20Reference) (InteractionManager :type AC%20RPG%20Interaction%20Manager%20Object%20Reference)))

(fn ConstructionScript)

(fn GetInteractionAction
  (params (InteractingActor :type Actor%20Object%20Reference))
  (return "NewEnumerator3"))

(fn GetInteractionRadius
  (params (InteractingActor :type Actor%20Object%20Reference))
  (return 2e+02))

(fn GetInteractionText
  (return (Utilities|Text|FormatText "Collect {display name}" (Variables|Config|GetDisplayName))))

(fn GetInteractionTime
  (params (InteractingActor :type Actor%20Object%20Reference))
  (return 0.0))

(fn GetInteractionType
  (return "NewEnumerator1"))

(fn IsInteractable
  (params (InteractingActor :type Actor%20Object%20Reference) (InteractionManager :type AC%20RPG%20Interaction%20Manager%20Object%20Reference))
  (return (Default|DoesAnyQuestNeedObjective (Actor|GetComponentbyClass (Components|GetOwner InteractionManager) "/Game/SuperiorRPGKit/Blueprints/Components/AC_RPG_QuestsManager.AC_RPG_QuestsManager_C") (Variables|Config|GetQuestObjective))))