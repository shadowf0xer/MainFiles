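; RPG HUD that creates and owns the game's UI: loading screen, in-game HUD windows, dialogue window, pause menu and notifications.
; Toggle and Set functions show or collapse each window, closing conflicting ones; storage and vendor share a widget switcher.
; Dialogue hides the in-game HUD, and inventory hides the tracker.
; SwitchUIMode checks for open windows, dialogue or pause menu to toggle interaction info and signal UI mode changes.
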(event Custom|CreateWidgets
  (Utilities|FlowControl|Sequence
    (:then_0
      ;[0.1 0.1 0.1 1 14] Create main in-game HUD and store references to all main player windows (characters stats, inventory, quest log etc.)
      (bind _returnvalue (UserInterface|CreateWidget "/Game/SuperiorRPGKit/Widgets/Player/WBP_RPG_InGameHUD.WBP_RPG_InGameHUD_C"))
      (bind _output_get (Variables|HUD|SetInGameHUD _returnvalue))
      (UserInterface|Viewport|AddtoViewport _output_get 0)
      (Variables|PlayerWindows|SetStatsWindow (Variables|/Game/SuperiorRPGKit/Widgets/Player/WBP_RPG_InGameHUD.WBP_RPG_InGameHUD_C|GetWBP_RPG_StatsWindow _returnvalue))
      (Variables|PlayerWindows|SetInventoryWindow (Variables|/Game/SuperiorRPGKit/Widgets/Player/WBP_RPG_InGameHUD.WBP_RPG_InGameHUD_C|GetWBP_RPG_InventoryWindow _returnvalue))
      (Variables|PlayerWindows|SetStorageWindow (Variables|/Game/SuperiorRPGKit/Widgets/Player/WBP_RPG_InGameHUD.WBP_RPG_InGameHUD_C|GetWBP_RPG_StorageWindow _returnvalue))
      (Variables|PlayerWindows|SetVendorWindow (Variables|/Game/SuperiorRPGKit/Widgets/Player/WBP_RPG_InGameHUD.WBP_RPG_InGameHUD_C|GetWBP_RPG_VendorWindow _returnvalue))
      (Variables|PlayerWindows|SetQuestLogWindow (Variables|/Game/SuperiorRPGKit/Widgets/Player/WBP_RPG_InGameHUD.WBP_RPG_InGameHUD_C|GetWBP_RPG_QuestLogWindow _returnvalue))
      (Variables|PlayerWindows|SetQuestPopUpWindow (Variables|/Game/SuperiorRPGKit/Widgets/Player/WBP_RPG_InGameHUD.WBP_RPG_InGameHUD_C|GetWBP_RPG_QuestPopUpWindow _returnvalue))
      (Variables|PlayerWindows|SetTrackerWindow (Variables|/Game/SuperiorRPGKit/Widgets/Player/WBP_RPG_InGameHUD.WBP_RPG_InGameHUD_C|GetWBP_RPG_TrackerWindow _returnvalue))
      (Variables|PlayerWindows|SetAchievementsWindow (Variables|/Game/SuperiorRPGKit/Widgets/Player/WBP_RPG_InGameHUD.WBP_RPG_InGameHUD_C|GetWBP_RPG_AchievementWindow _returnvalue))
      (Variables|PlayerWindows|SetSkillsWindow (Variables|/Game/SuperiorRPGKit/Widgets/Player/WBP_RPG_InGameHUD.WBP_RPG_InGameHUD_C|GetWBP_RPG_SkillsWindow _returnvalue))
      (Variables|PlayerWindows|SetCraftingWindow (Variables|/Game/SuperiorRPGKit/Widgets/Player/WBP_RPG_InGameHUD.WBP_RPG_InGameHUD_C|GetWBP_RPG_CraftingWindow _returnvalue))
      (Variables|Default|SetInteractionInfo (Variables|/Game/SuperiorRPGKit/Widgets/Player/WBP_RPG_InGameHUD.WBP_RPG_InGameHUD_C|GetWBP_RPG_InteractionInfo _returnvalue))
      (Variables|PlayerWindows|SetHeroSmallWindow (Variables|/Game/SuperiorRPGKit/Widgets/Player/WBP_RPG_InGameHUD.WBP_RPG_InGameHUD_C|GetWBP_RPG_Hero_SmallWindow _returnvalue)))
    (:then_1
      ;[0.1 0.1 0.1 1 14] Create dialogue window.
      (bind _returnvalue_2 (UserInterface|CreateWidget "/Game/SuperiorRPGKit/Widgets/Interaction/WBP_RPG_DialogueWindow.WBP_RPG_DialogueWindow_C"))
      (bind _output_get_2 (Variables|DialogWindow|SetDialogueWindow _returnvalue_2))
      (UserInterface|Viewport|AddtoViewport _output_get_2 0)
      (Widget|SetVisibility _output_get_2 "Collapsed"))
    (:then_2
      ;[0.1 0.1 0.1 1 14] Create pause menu.
      (bind _returnvalue_3 (UserInterface|CreateWidget "/Game/SuperiorRPGKit/Widgets/PauseMenu/WBP_RPG_PauseMenu.WBP_RPG_PauseMenu_C" 0 self))
      (bind _output_get_3 (Variables|PauseMenu|SetPauseMenu _returnvalue_3))
      (UserInterface|Viewport|AddtoViewport _output_get_3 1)
      (Widget|SetVisibility _output_get_3 "Collapsed"))
    (:then_3
      ;[0.1 0.1 0.1 1 14] Create notifications container.
      (bind _returnvalue_4 (UserInterface|CreateWidget "/Game/SuperiorRPGKit/Widgets/Notifications/WBP_RPG_NotificationContainer.WBP_RPG_NotificationContainer_C"))
      (bind _output_get_4 (Variables|HUD|SetNotificationContainer _returnvalue_4))
      (UserInterface|Viewport|AddtoViewport _output_get_4 5))))

(event EventBeginPlay
  ;[0.1 0.1 0.1 1 14] Create Loading Screen on top of everything.
  (if (not (Utilities|IsValid (Variables|HUD|GetLoadingScreen)))
    (bind _returnvalue (UserInterface|CreateWidget "/Game/SuperiorRPGKit/Widgets/LoadingScreen/WBP_RPG_LoadingScreen.WBP_RPG_LoadingScreen_C"))
    (bind _output_get (Variables|HUD|SetLoadingScreen _returnvalue))
    (UserInterface|Viewport|AddtoViewport _output_get 10)))

(fn ConstructionScript)

(fn ToggleInventoryWindow
  (switch Utilities|FlowControl|Switch|SwitchonESlateVisibility (Widget|GetVisibility (Variables|PlayerWindows|GetInventoryWindow))
    (:Visible
      (Widget|SetVisibility (Variables|PlayerWindows|GetInventoryWindow) "Collapsed" :!label _label)
      (PlayerWindows|SetStorageWindowVisibility false)
      (PlayerWindows|SetVendorWindowVisibility false)
      (PlayerWindows|SetTrackerWindowVisibility true)
      (HUD|SwitchUIMode))
    (:Collapsed
      (Widget|SetVisibility (Variables|PlayerWindows|GetInventoryWindow) "SelfHitTestInvisible" :!label _label_2)
      (PlayerWindows|SetTrackerWindowVisibility false)
      (HUD|SwitchUIMode))
    (:Hidden
      (goto _label_2))
    (:HitTestInvisible
      (goto _label))
    (:SelfHitTestInvisible
      (goto _label))))

(fn SetInventoryWindowVisibility
  (params (Visible :type Boolean))
  (if Visible
    (Widget|SetVisibility (Variables|PlayerWindows|GetInventoryWindow) "SelfHitTestInvisible")
    (PlayerWindows|SetTrackerWindowVisibility false)
    (HUD|SwitchUIMode)
    (else
      (Widget|SetVisibility (Variables|PlayerWindows|GetInventoryWindow) "Collapsed")
      (PlayerWindows|SetStorageWindowVisibility false)
      (PlayerWindows|SetTrackerWindowVisibility true)
      (HUD|SwitchUIMode))))

(fn ToggleStatsWindow
  (switch Utilities|FlowControl|Switch|SwitchonESlateVisibility (Widget|GetVisibility (Variables|PlayerWindows|GetStatsWindow))
    (:Visible
      (Widget|SetVisibility (Variables|PlayerWindows|GetStatsWindow) "Collapsed" :!label _label)
      (HUD|SwitchUIMode))
    (:Collapsed
      (Widget|SetVisibility (Variables|PlayerWindows|GetStatsWindow) "SelfHitTestInvisible" :!label _label_2)
      (PlayerWindows|SetQuestLogWindowVisibility false)
      (PlayerWindows|SetAchievementsWindowVisibility false)
      (PlayerWindows|SetCraftingWindowVisibility false)
      (HUD|SwitchUIMode))
    (:Hidden
      (goto _label_2))
    (:HitTestInvisible
      (goto _label))
    (:SelfHitTestInvisible
      (goto _label))))

(fn SetStatsWindowVisibility
  (params (Visible :type Boolean))
  (if Visible
    (Widget|SetVisibility (Variables|PlayerWindows|GetStatsWindow) "SelfHitTestInvisible")
    (PlayerWindows|SetQuestLogWindowVisibility false)
    (PlayerWindows|SetAchievementsWindowVisibility false)
    (PlayerWindows|SetCraftingWindowVisibility false)
    (else
      (Widget|SetVisibility (Variables|PlayerWindows|GetStatsWindow) "Collapsed"))))

(fn ToggleStorageWindow
  (bind _storagewindow (Variables|PlayerWindows|GetStorageWindow))
  (switch Utilities|FlowControl|Switch|SwitchonESlateVisibility (Widget|GetVisibility (Variables|PlayerWindows|GetStorageWindow))
    (:Visible
      (Widget|SetVisibility (Variables|PlayerWindows|GetStorageWindow) "Collapsed" :!label _label))
    (:Collapsed
      (Widget|SetVisibility _storagewindow "SelfHitTestInvisible" :!label _label_2)
      (Class|WidgetSwitcher|SetActiveWidget (Variables|/Game/SuperiorRPGKit/Widgets/Player/WBP_RPG_InGameHUD.WBP_RPG_InGameHUD_C|GetWidgetSwitcher_StorageVendor (Variables|HUD|GetInGameHUD)) _storagewindow)
      (PlayerWindows|SetSkillsWindowVisibility false)
      (PlayerWindows|SetCraftingWindowVisibility false)
      (PlayerWindows|SetQuestLogWindowVisibility false))
    (:Hidden
      (goto _label_2))
    (:HitTestInvisible
      (goto _label))
    (:SelfHitTestInvisible
      (goto _label))))

(fn SetStorageWindowVisibility
  (params (Visible :type Boolean))
  (bind _storagewindow (Variables|PlayerWindows|GetStorageWindow))
  (if Visible
    (Widget|SetVisibility _storagewindow "SelfHitTestInvisible")
    (Class|WidgetSwitcher|SetActiveWidget (Variables|/Game/SuperiorRPGKit/Widgets/Player/WBP_RPG_InGameHUD.WBP_RPG_InGameHUD_C|GetWidgetSwitcher_StorageVendor (Variables|HUD|GetInGameHUD)) _storagewindow)
    (PlayerWindows|SetSkillsWindowVisibility false)
    (PlayerWindows|SetCraftingWindowVisibility false)
    (PlayerWindows|SetQuestLogWindowVisibility false)
    (else
      (Widget|SetVisibility (Variables|PlayerWindows|GetStorageWindow) "Collapsed"))))

(fn ToggleVendorWindow
  (bind _vendorwindow (Variables|PlayerWindows|GetVendorWindow))
  (switch Utilities|FlowControl|Switch|SwitchonESlateVisibility (Widget|GetVisibility (Variables|PlayerWindows|GetVendorWindow))
    (:Visible
      (Widget|SetVisibility (Variables|PlayerWindows|GetVendorWindow) "Collapsed" :!label _label))
    (:Collapsed
      (Widget|SetVisibility _vendorwindow "SelfHitTestInvisible" :!label _label_2)
      (Class|WidgetSwitcher|SetActiveWidget (Variables|/Game/SuperiorRPGKit/Widgets/Player/WBP_RPG_InGameHUD.WBP_RPG_InGameHUD_C|GetWidgetSwitcher_StorageVendor (Variables|HUD|GetInGameHUD)) _vendorwindow)
      (PlayerWindows|SetSkillsWindowVisibility false)
      (PlayerWindows|SetCraftingWindowVisibility false)
      (PlayerWindows|SetQuestLogWindowVisibility false))
    (:Hidden
      (goto _label_2))
    (:HitTestInvisible
      (goto _label))
    (:SelfHitTestInvisible
      (goto _label))))

(fn SetVendorWindowVisibility
  (params (Visible :type Boolean))
  (bind _vendorwindow (Variables|PlayerWindows|GetVendorWindow))
  (if Visible
    (Widget|SetVisibility _vendorwindow "SelfHitTestInvisible")
    (Class|WidgetSwitcher|SetActiveWidget (Variables|/Game/SuperiorRPGKit/Widgets/Player/WBP_RPG_InGameHUD.WBP_RPG_InGameHUD_C|GetWidgetSwitcher_StorageVendor (Variables|HUD|GetInGameHUD)) _vendorwindow)
    (PlayerWindows|SetSkillsWindowVisibility false)
    (PlayerWindows|SetCraftingWindowVisibility false)
    (PlayerWindows|SetQuestLogWindowVisibility false)
    (else
      (Widget|SetVisibility (Variables|PlayerWindows|GetVendorWindow) "Collapsed"))))

(fn ToggleQuestLogWindow
  (switch Utilities|FlowControl|Switch|SwitchonESlateVisibility (Widget|GetVisibility (Variables|PlayerWindows|GetQuestLogWindow))
    (:Visible
      (Widget|SetVisibility (Variables|PlayerWindows|GetQuestLogWindow) "Collapsed" :!label _label)
      (HUD|SwitchUIMode))
    (:Collapsed
      (Widget|SetVisibility (Variables|PlayerWindows|GetQuestLogWindow) "SelfHitTestInvisible" :!label _label_2)
      (PlayerWindows|SetStatsWindowVisibility false)
      (PlayerWindows|SetAchievementsWindowVisibility false)
      (PlayerWindows|SetSkillsWindowVisibility false)
      (PlayerWindows|SetCraftingWindowVisibility false)
      (PlayerWindows|SetStorageWindowVisibility false)
      (PlayerWindows|SetVendorWindowVisibility false)
      (HUD|SwitchUIMode))
    (:Hidden
      (goto _label_2))
    (:HitTestInvisible
      (goto _label))
    (:SelfHitTestInvisible
      (goto _label))))

(fn SetQuestLogWindowVisibility
  (params (Visible :type Boolean))
  (if Visible
    (Widget|SetVisibility (Variables|PlayerWindows|GetQuestLogWindow) "SelfHitTestInvisible")
    (PlayerWindows|SetStatsWindowVisibility false)
    (PlayerWindows|SetAchievementsWindowVisibility false)
    (PlayerWindows|SetSkillsWindowVisibility false)
    (PlayerWindows|SetCraftingWindowVisibility false)
    (PlayerWindows|SetStorageWindowVisibility false)
    (PlayerWindows|SetVendorWindowVisibility false)
    (else
      (Widget|SetVisibility (Variables|PlayerWindows|GetQuestLogWindow) "Collapsed"))))

(fn ToggleQuestPopUpWindow
  (switch Utilities|FlowControl|Switch|SwitchonESlateVisibility (Widget|GetVisibility (Variables|PlayerWindows|GetQuestPopUpWindow))
    (:Visible
      (Widget|SetVisibility (Variables|PlayerWindows|GetQuestPopUpWindow) "Collapsed" :!label _label))
    (:Collapsed
      (Widget|SetVisibility (Variables|PlayerWindows|GetQuestPopUpWindow) "SelfHitTestInvisible" :!label _label_2)
      (PlayerWindows|SetQuestLogWindowVisibility false)
      (PlayerWindows|SetSkillsWindowVisibility false)
      (PlayerWindows|SetCraftingWindowVisibility false))
    (:Hidden
      (goto _label_2))
    (:HitTestInvisible
      (goto _label))
    (:SelfHitTestInvisible
      (goto _label))))

(fn SetQuestPopUpWindowVisibility
  (params (Visible :type Boolean))
  (if Visible
    (Widget|SetVisibility (Variables|PlayerWindows|GetQuestPopUpWindow) "SelfHitTestInvisible")
    (PlayerWindows|SetQuestLogWindowVisibility false)
    (PlayerWindows|SetSkillsWindowVisibility false)
    (PlayerWindows|SetCraftingWindowVisibility false)
    (else
      (Widget|SetVisibility (Variables|PlayerWindows|GetQuestPopUpWindow) "Collapsed"))))

(fn ToggleinGameHUD
  (switch Utilities|FlowControl|Switch|SwitchonESlateVisibility (Widget|GetVisibility (Variables|HUD|GetInGameHUD))
    (:Visible
      (Widget|SetVisibility (Variables|HUD|GetInGameHUD) "Collapsed" :!label _label))
    (:Collapsed
      (Widget|SetVisibility (Variables|HUD|GetInGameHUD) "SelfHitTestInvisible" :!label _label_2))
    (:Hidden
      (goto _label_2))
    (:HitTestInvisible
      (goto _label))
    (:SelfHitTestInvisible
      (goto _label))))

(fn SetinGameHUDVisibility
  (params (Visible :type Boolean))
  (if Visible
    (Widget|SetVisibility (Variables|HUD|GetInGameHUD) "SelfHitTestInvisible")
    (else
      (Widget|SetVisibility (Variables|HUD|GetInGameHUD) "Collapsed"))))

(fn ToggleDialogueWindow
  (switch Utilities|FlowControl|Switch|SwitchonESlateVisibility (Widget|GetVisibility (Variables|DialogWindow|GetDialogueWindow))
    (:Visible
      (Widget|SetVisibility (Variables|DialogWindow|GetDialogueWindow) "Collapsed" :!label _label)
      (HUD|SetinGameHUDVisibility true))
    (:Collapsed
      (Widget|SetVisibility (Variables|DialogWindow|GetDialogueWindow) "SelfHitTestInvisible" :!label _label_2)
      (HUD|SetinGameHUDVisibility false))
    (:Hidden
      (goto _label_2))
    (:HitTestInvisible
      (goto _label))
    (:SelfHitTestInvisible
      (goto _label))))

(fn SetDialogueWindowVisibility
  (params (Visible :type Boolean))
  (if Visible
    (Widget|SetVisibility (Variables|DialogWindow|GetDialogueWindow) "SelfHitTestInvisible")
    (HUD|SetinGameHUDVisibility false)
    (else
      (Widget|SetVisibility (Variables|DialogWindow|GetDialogueWindow) "Collapsed")
      (HUD|SetinGameHUDVisibility true))))

(fn ToggleTracker
  (switch Utilities|FlowControl|Switch|SwitchonESlateVisibility (Widget|GetVisibility (Variables|PlayerWindows|GetTrackerWindow))
    (:Visible
      (Widget|SetVisibility (Variables|PlayerWindows|GetTrackerWindow) "Collapsed" :!label _label))
    (:Collapsed
      (Widget|SetVisibility (Variables|PlayerWindows|GetTrackerWindow) "HitTestInvisible" :!label _label_2))
    (:Hidden
      (goto _label_2))
    (:HitTestInvisible
      (goto _label))
    (:SelfHitTestInvisible
      (goto _label))))

(fn SetTrackerWindowVisibility
  (params (Visible :type Boolean))
  (if Visible
    (Widget|SetVisibility (Variables|PlayerWindows|GetTrackerWindow) "HitTestInvisible")
    (else
      (Widget|SetVisibility (Variables|PlayerWindows|GetTrackerWindow) "Collapsed"))))

(fn ToggleAchievementsWindow
  (switch Utilities|FlowControl|Switch|SwitchonESlateVisibility (Widget|GetVisibility (Variables|PlayerWindows|GetAchievementsWindow))
    (:Visible
      (Widget|SetVisibility (Variables|PlayerWindows|GetAchievementsWindow) "Collapsed" :!label _label)
      (HUD|SwitchUIMode))
    (:Collapsed
      (Widget|SetVisibility (Variables|PlayerWindows|GetAchievementsWindow) "SelfHitTestInvisible" :!label _label_2)
      (PlayerWindows|SetStatsWindowVisibility false)
      (PlayerWindows|SetQuestLogWindowVisibility false)
      (PlayerWindows|SetCraftingWindowVisibility false)
      (HUD|SwitchUIMode))
    (:Hidden
      (goto _label_2))
    (:HitTestInvisible
      (goto _label))
    (:SelfHitTestInvisible
      (goto _label))))

(fn SetAchievementsWindowVisibility
  (params (Visible :type Boolean))
  (if Visible
    (Widget|SetVisibility (Variables|PlayerWindows|GetAchievementsWindow) "SelfHitTestInvisible")
    (PlayerWindows|SetStatsWindowVisibility false)
    (PlayerWindows|SetQuestLogWindowVisibility false)
    (PlayerWindows|SetCraftingWindowVisibility false)
    (else
      (Widget|SetVisibility (Variables|PlayerWindows|GetAchievementsWindow) "Collapsed"))))

(fn ToggleSkillsWindow
  (switch Utilities|FlowControl|Switch|SwitchonESlateVisibility (Widget|GetVisibility (Variables|PlayerWindows|GetSkillsWindow))
    (:Visible
      (Widget|SetVisibility (Variables|PlayerWindows|GetSkillsWindow) "Collapsed" :!label _label)
      (HUD|SwitchUIMode))
    (:Collapsed
      (Widget|SetVisibility (Variables|PlayerWindows|GetSkillsWindow) "SelfHitTestInvisible" :!label _label_2)
      (PlayerWindows|SetQuestPopUpWindowVisibility false)
      (PlayerWindows|SetQuestLogWindowVisibility false)
      (PlayerWindows|SetStorageWindowVisibility false)
      (PlayerWindows|SetVendorWindowVisibility false)
      (PlayerWindows|SetCraftingWindowVisibility false)
      (HUD|SwitchUIMode))
    (:Hidden
      (goto _label_2))
    (:HitTestInvisible
      (goto _label))
    (:SelfHitTestInvisible
      (goto _label))))

(fn SetSkillsWindowVisibility
  (params (Visible :type Boolean))
  (if Visible
    (Widget|SetVisibility (Variables|PlayerWindows|GetSkillsWindow) "SelfHitTestInvisible")
    (PlayerWindows|SetQuestPopUpWindowVisibility false)
    (PlayerWindows|SetQuestLogWindowVisibility false)
    (PlayerWindows|SetStorageWindowVisibility false)
    (PlayerWindows|SetVendorWindowVisibility false)
    (PlayerWindows|SetCraftingWindowVisibility false)
    (else
      (Widget|SetVisibility (Variables|PlayerWindows|GetSkillsWindow) "Collapsed"))))

(fn TogglePauseMenu
  (bind _pausemenu (Variables|PauseMenu|GetPauseMenu))
  (switch Utilities|FlowControl|Switch|SwitchonESlateVisibility (Widget|GetVisibility (Variables|PauseMenu|GetPauseMenu))
    (:Visible
      (Widget|SetVisibility (Variables|PauseMenu|GetPauseMenu) "Collapsed" :!label _label)
      (HUD|SwitchUIMode))
    (:Collapsed
      (Widget|SetVisibility _pausemenu "SelfHitTestInvisible" :!label _label_2)
      (Class|WidgetSwitcher|SetActiveWidgetIndex (Variables|/Game/SuperiorRPGKit/Widgets/PauseMenu/WBP_RPG_PauseMenu.WBP_RPG_PauseMenu_C|GetWidgetSwitcher_Main _pausemenu))
      (HUD|SwitchUIMode))
    (:Hidden
      (goto _label_2))
    (:HitTestInvisible
      (goto _label))
    (:SelfHitTestInvisible
      (goto _label))))

(fn IsAnyWindowOpen
  (return (Math|Boolean|ORBoolean (Widget|IsVisible (Variables|PlayerWindows|GetStatsWindow)) (Widget|IsVisible (Variables|PlayerWindows|GetInventoryWindow)) (Widget|IsVisible (Variables|PlayerWindows|GetStorageWindow)) (Widget|IsVisible (Variables|PlayerWindows|GetVendorWindow)) (Widget|IsVisible (Variables|PlayerWindows|GetQuestLogWindow)) (Widget|IsVisible (Variables|PlayerWindows|GetSkillsWindow)) (Widget|IsVisible (Variables|PlayerWindows|GetAchievementsWindow)) (Widget|IsVisible (Variables|PlayerWindows|GetCraftingWindow)))))

(fn SwitchUIMode
  (if (Math|Boolean|ANDBoolean (not (Conditions|IsAnyWindowOpen)) (not (Conditions|IsPauseMenuOpen)) (not (Conditions|IsDialogueWindowOpen)))
    (Widget|SetVisibility (Variables|Default|GetInteractionInfo) "SelfHitTestInvisible")
    (Default|CallUIModeDisabled)
    (else
      (Widget|SetVisibility (Variables|Default|GetInteractionInfo) "Collapsed")
      (Default|CallUIModeEnabled))))

(fn IsPauseMenuOpen
  (return (Widget|IsVisible (Variables|PauseMenu|GetPauseMenu))))

(fn CloseAllOpenWindows
  (if (Conditions|IsAnyWindowOpen)
    ;[0.1 0.1 0.1 1 14] Hide all player window.
    (PlayerWindows|SetStatsWindowVisibility false)
    (PlayerWindows|SetInventoryWindowVisibility false)
    (PlayerWindows|SetStorageWindowVisibility false)
    (PlayerWindows|SetVendorWindowVisibility false)
    (PlayerWindows|SetQuestLogWindowVisibility false)
    (PlayerWindows|SetQuestPopUpWindowVisibility false)
    (PlayerWindows|SetAchievementsWindowVisibility false)
    (PlayerWindows|SetSkillsWindowVisibility false)
    (PlayerWindows|SetCraftingWindowVisibility false)
    (HUD|SwitchUIMode)
    (return true)
    (else
      (return false))))

(fn ToggleCraftingWindow
  (switch Utilities|FlowControl|Switch|SwitchonESlateVisibility (Widget|GetVisibility (Variables|PlayerWindows|GetCraftingWindow))
    (:Visible
      (Widget|SetVisibility (Variables|PlayerWindows|GetCraftingWindow) "Collapsed" :!label _label)
      (HUD|SwitchUIMode))
    (:Collapsed
      (Widget|SetVisibility (Variables|PlayerWindows|GetCraftingWindow) "SelfHitTestInvisible" :!label _label_2)
      (PlayerWindows|SetStatsWindowVisibility false)
      (PlayerWindows|SetAchievementsWindowVisibility false)
      (PlayerWindows|SetSkillsWindowVisibility false)
      (PlayerWindows|SetQuestLogWindowVisibility false)
      (PlayerWindows|SetStorageWindowVisibility false)
      (PlayerWindows|SetVendorWindowVisibility false)
      (HUD|SwitchUIMode))
    (:Hidden
      (goto _label_2))
    (:HitTestInvisible
      (goto _label))
    (:SelfHitTestInvisible
      (goto _label))))

(fn SetCraftingWindowVisibility
  (params (Visible :type Boolean))
  (if Visible
    (Widget|SetVisibility (Variables|PlayerWindows|GetCraftingWindow) "SelfHitTestInvisible")
    (PlayerWindows|SetStatsWindowVisibility false)
    (PlayerWindows|SetAchievementsWindowVisibility false)
    (PlayerWindows|SetSkillsWindowVisibility false)
    (PlayerWindows|SetQuestLogWindowVisibility false)
    (PlayerWindows|SetStorageWindowVisibility false)
    (PlayerWindows|SetVendorWindowVisibility false)
    (else
      (Widget|SetVisibility (Variables|PlayerWindows|GetCraftingWindow) "Collapsed"))))

(fn IsDialogueWindowOpen
  (return (Widget|IsVisible (Variables|DialogWindow|GetDialogueWindow))))