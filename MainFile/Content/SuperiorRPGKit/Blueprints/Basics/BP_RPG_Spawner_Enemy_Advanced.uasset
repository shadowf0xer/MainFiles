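; Server-authoritative enemy spawner that activates when heroes enter its radius and spawns a list of guaranteed plus probability-weighted bonus enemies.
; GenerateSpawnPoints traces a diamond grid onto navigable ground, and SpawnEnemies shuffles these points, then initializes enemies at the set level.
; With no heroes nearby, it despawns out-of-combat enemies within 60% of the radius, re-queuing living ones.
; A random startup delay staggers spawner ticks.
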(event EventBeginPlay
  (Networking|SwitchHasAuthority
    (:Authority
      (Components|DestroyComponent (Variables|Default|GetSphere_ActivationRadius)) ; Destroy components as they are\nonly for editor preview reasons.
      (Config|GenerateEnemiestoSpawn)
      (Utilities|FlowControl|Delay (Math|Random|RandomFloatinRange 0.0 1.0)) ; Spawners will activate after random time\nso they won't tick all at once.
      (Actor|Tick|SetActorTickEnabled true))))

(event EventTick
  (params (DeltaSeconds :type Float%20%28single-precision%29))
  (Networking|SwitchHasAuthority
    (:Authority
      (if (Variables|Runtime|GetActive)
        (if (== (Utilities|Array|Length (Getters|GetPlayersinActivationRadius)) 0)
          (if (Variables|Runtime|GetActive)
            (Variables|Runtime|SetActive false)))
        (elif (> (Utilities|Array|Length (Getters|GetPlayersinActivationRadius)) 0)
          (if (not (Variables|Runtime|GetActive))
            (Variables|Runtime|SetActive true)
            (CallFunction|SpawnEnemies))
          (elif (> (Utilities|Array|Length (Variables|Runtime|GetSpawnedEnemies)) 0)
            (CallFunction|DespawnEnemies)))))))

(fn ConstructionScript
  (Components|Sphere|SetSphereRadius (Variables|Default|GetSphere_SpawnRadius) (Variables|Config|Spawning|GetSpawnRadius) true)
  (Components|Sphere|SetSphereRadius (Variables|Default|GetSphere_ActivationRadius) (Variables|Config|Activation|GetActivationRadius) true)
  (Rendering|SetVisibility (Variables|Default|GetSphere_SpawnRadius) (Variables|Config|EditorOnly|GetShowSpawnRadius) false)
  (Rendering|SetVisibility (Variables|Default|GetSphere_ActivationRadius) (Variables|Config|EditorOnly|GetShowActivationRadius) false))

(fn SpawnEnemies
  (Utilities|Array|Shuffle (Variables|Config|Spawning|GetSpawnPoints))
  (bind (_arrayindex _arrayelement) (Utilities|Array|ReverseforEachLoop (Variables|Runtime|GetEnemiesToSpawn))
    (:LoopBody
      (bind _returnvalue (Game|SpawnActorfromClass _arrayelement (Math|Transform|MakeTransform (+ (Utilities|Array|Get(acopy) (Variables|Config|Spawning|GetSpawnPoints) _arrayindex) (Transformation|GetActorLocation)) (Math|Rotator|MakeRotator 0.0 0.0 (Math|Random|RandomFloatinRange 0.0 359.0)) "1,1,1") "AdjustIfPossibleButDontSpawnIfColliding" 0 0))
      (Utilities|IsValid _returnvalue
        (:Is%20Valid
          (LocalVariables|SetSpawnedEnemyLOCAL _returnvalue)
          (Utilities|Array|RemoveIndex (Variables|Runtime|GetEnemiesToSpawn) _arrayindex)
          (Utilities|Array|Add (Variables|Runtime|GetSpawnedEnemies) (LocalVariables|GetSpawnedEnemyLOCAL))
          (Variables|/Game/SuperiorRPGKit/Blueprints/Components/AC_RPG_StatsManager.AC_RPG_StatsManager_C|SetCurrentLevel (Variables|/Game/SuperiorRPGKit/Blueprints/Basics/BP_RPG_Enemy.BP_RPG_Enemy_C|GetAC_RPG_StatsManager (LocalVariables|GetSpawnedEnemyLOCAL)) (Variables|Config|Enemies|GetLevel))
          (Default|Initialize (LocalVariables|GetSpawnedEnemyLOCAL)))))))

(fn GetPlayersinActivationRadius
  (bind _outactors (Collision|SphereOverlapActors (Transformation|GetActorLocation) (Variables|Config|Activation|GetActivationRadius) (Utilities|Array|MakeArray "ObjectTypeQuery3") "/Game/SuperiorRPGKit/Blueprints/Basics/BP_RPG_Hero.BP_RPG_Hero_C"))
  (return _outactors))

(fn DespawnEnemies
  (bind _enemies (Getters|GetSpawnedEnemiesinActivationRadius))
  (bind _arrayelement (Utilities|Array|ReverseforEachLoop _enemies)
    (:LoopBody
      (Utilities|IsValid _arrayelement
        (:Is%20Valid
          (if (not (Default|GetIsinCombat (Variables|/Game/SuperiorRPGKit/AI/Blueprints/Core/BP_AI_Controller.BP_AI_Controller_C|GetAC_AI_Target (Variables|/Game/SuperiorRPGKit/Blueprints/Basics/BP_RPG_Enemy.BP_RPG_Enemy_C|GetAIController _arrayelement))))
            (Utilities|FlowControl|Sequence
              (:then_0
                (if (not (Variables|/Game/SuperiorRPGKit/Blueprints/Components/AC_RPG_StatsManager.AC_RPG_StatsManager_C|GetDead (Variables|/Game/SuperiorRPGKit/Blueprints/Basics/BP_RPG_Enemy.BP_RPG_Enemy_C|GetAC_RPG_StatsManager _arrayelement)))
                  (Utilities|Array|Add (Variables|Runtime|GetEnemiesToSpawn) (Utilities|GetClass _arrayelement))))
              (:then_1
                (Actor|DestroyActor _arrayelement)
                (Utilities|Array|RemoveItem (Variables|Runtime|GetSpawnedEnemies) _arrayelement)))))
        (:Is%20Not%20Valid
          (Utilities|Array|RemoveItem (Variables|Runtime|GetSpawnedEnemies) _arrayelement))))))

(fn GenerateEnemiestoSpawn
  (Variables|Runtime|SetEnemiesToSpawn (Variables|Config|Enemies|GetGuaranteedEnemies))
  (LocalVariables|SetNumberOfBonusEnemiesLOCAL (Math|Random|RandomIntegerinRange (Variables|Config|Enemies|GetMinBonusEnemies) (Variables|Config|Enemies|GetMaxBonusEnemies)))
  (for _index (range 1 (LocalVariables|GetNumberOfBonusEnemiesLOCAL))
    (bind _rolledenemy (Getters|GetRandomBonusEnemy))
    (if (Utilities|IsValidClass _rolledenemy)
      (Utilities|Array|Add (Variables|Runtime|GetEnemiesToSpawn) _rolledenemy))))

(fn GetRandomBonusEnemy
  (bind _keys (Utilities|Map|Keys (Variables|Config|Enemies|GetBonusEnemies)))
  (for _array_element _keys
    (LocalVariables|SetTotalProbabilityLOCAL (+ (.Value (Utilities|Map|Find (Variables|Config|Enemies|GetBonusEnemies) _array_element)) (LocalVariables|GetTotalProbabilityLOCAL))))
  (LocalVariables|SetRolledProbabilityLOCAL (Math|Random|RandomFloatinRange 0.0 (LocalVariables|GetTotalProbabilityLOCAL)))
  (bind _keys_2 (Utilities|Map|Keys (Variables|Config|Enemies|GetBonusEnemies)))
  (bind _array_element_2 (Utilities|Array|ForEachLoopwithBreak _keys_2 :!label _label)
    (:LoopBody
      (LocalVariables|SetCurrentProbabilityLOCAL (+ (.Value (Utilities|Map|Find (Variables|Config|Enemies|GetBonusEnemies) _array_element_2)) (LocalVariables|GetCurrentProbabilityLOCAL)))
      (if (<= (LocalVariables|GetRolledProbabilityLOCAL) (LocalVariables|GetCurrentProbabilityLOCAL))
        (LocalVariables|SetEnemyLOCAL _array_element_2)
        (goto _label Break)))
    (:Completed
      (return (LocalVariables|GetEnemyLOCAL)))))

(fn GenerateSpawnPoints
  (bind _distancebetweenspawnpoints (Variables|Config|Spawning|GetDistanceBetweenSpawnPoints))
  (bind _spawnradius (Variables|Config|Spawning|GetSpawnRadius))
  (LocalVariables|SetGridDimensionsLOCAL (.ReturnValue (Math|Float|Division(WholeandRemainder) (Variables|Config|Spawning|GetSpawnRadius) (Variables|Config|Spawning|GetDistanceBetweenSpawnPoints))))
  (Utilities|Array|Clear (Variables|Config|Spawning|GetSpawnPoints))
  (for _index (range (* (LocalVariables|GetGridDimensionsLOCAL) -1) (LocalVariables|GetGridDimensionsLOCAL))
    (LocalVariables|SetXLOCAL _index)
    (for _index_2 (range (* (LocalVariables|GetGridDimensionsLOCAL) -1) (LocalVariables|GetGridDimensionsLOCAL))
      (LocalVariables|SetYLOCAL _index_2)
      (if (<= (+ (Math|Integer|Absolute(Integer) (LocalVariables|GetXLOCAL)) (Math|Integer|Absolute(Integer) (LocalVariables|GetYLOCAL))) (LocalVariables|GetGridDimensionsLOCAL))
        (bind (_outhit _returnvalue) (Collision|LineTraceByChannel (+ (+ (Math|Vector|MakeVector (* (LocalVariables|GetXLOCAL) _distancebetweenspawnpoints) (* (LocalVariables|GetYLOCAL) _distancebetweenspawnpoints) 0.0) (Transformation|GetActorLocation)) (Math|Vector|MakeVector 0.0 0.0 _spawnradius)) (- (+ (Math|Vector|MakeVector (* (LocalVariables|GetXLOCAL) _distancebetweenspawnpoints) (* (LocalVariables|GetYLOCAL) _distancebetweenspawnpoints) 0.0) (Transformation|GetActorLocation)) (Math|Vector|MakeVector 0.0 0.0 _spawnradius)) "TraceTypeQuery1" false 0 "ForDuration"))
        (if _returnvalue
          (if (Math|Vector|NotEqual(Vector) (.ImpactPoint (Collision|BreakHitResult _outhit)) (.TraceStart (Collision|BreakHitResult _outhit)) 1.0)
            (Utilities|Array|Add (Variables|Config|Spawning|GetSpawnPoints) (- (.RandomLocation (Class|NavigationSystem|GetRandomPointinNavigableRadius (.ImpactPoint (Collision|BreakHitResult _outhit)) (* (Variables|Config|Spawning|GetDistanceBetweenSpawnPoints) 0.1))) (Transformation|GetActorLocation)))))))))

(fn GetSpawnedEnemiesinActivationRadius
  (bind (_outactors _returnvalue) (Collision|SphereOverlapActors (Transformation|GetActorLocation) (* (Variables|Config|Activation|GetActivationRadius) 0.6) (Utilities|Array|MakeArray "ObjectTypeQuery8") "/Game/SuperiorRPGKit/Blueprints/Basics/BP_RPG_Enemy.BP_RPG_Enemy_C"))
  (if _returnvalue
    (for _array_element (Variables|Runtime|GetSpawnedEnemies)
      (if (Utilities|Array|ContainsItem _outactors _array_element)
        (Utilities|Array|Add (LocalVariables|GetEnemiesLOCAL) _array_element)))
    (return (LocalVariables|GetEnemiesLOCAL))))