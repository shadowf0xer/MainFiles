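; RPG game instance that looks up the display names of keys bound to input actions and axes.
; Two functions search the ActionKeymappings and AxisKeymappings maps by name, each map entry holding an array of key mappings.
; The first two array entries become the main and secondary key names, each guarded by an index validity check.
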(fn GetActionInputKeyName
  (params (Action :type Name))
  (bind _actionkeymappings (Variables|Default|GetActionKeymappings))
  (bind (_value _returnvalue) (Utilities|Map|Find _actionkeymappings Action))
  (bind _arrayofactionkeymappings (Utilities|Struct|BreakS_RPG_ArrayOfActionKeymappings _value))
  ;[0.1 0.1 0.1 1 14] Returns name of the key bound to given action.
  (if _returnvalue
    (Utilities|FlowControl|Sequence
      (:then_0
        (if (Utilities|Array|IsValidIndex _arrayofactionkeymappings)
          (LocalVariables|SetMainKeyLOCAL (Class|KismetInputLibrary|KeyGetDisplayName (.Key (Utilities|Struct|BreakInputActionKeyMapping (Utilities|Array|Get(acopy) _arrayofactionkeymappings)))))))
      (:then_1
        (if (Utilities|Array|IsValidIndex _arrayofactionkeymappings 1)
          (LocalVariables|SetSecondaryKeyLOCAL (Class|KismetInputLibrary|KeyGetDisplayName (.Key (Utilities|Struct|BreakInputActionKeyMapping (Utilities|Array|Get(acopy) _arrayofactionkeymappings 1)))))))
      (:then_2
        (return (LocalVariables|GetMainKeyLOCAL) (LocalVariables|GetSecondaryKeyLOCAL))))
    (else
      (return (LocalVariables|GetMainKeyLOCAL) (LocalVariables|GetSecondaryKeyLOCAL)))))

(fn GetAxisInputKeyName
  (params (Action :type Name%20%28by%20ref%29))
  (bind _axiskeymappings (Variables|Default|GetAxisKeymappings))
  (bind (_value _returnvalue) (Utilities|Map|Find _axiskeymappings Action))
  (bind _arrayofaxiskeymappings (Utilities|Struct|BreakS_RPG_ArrayOfAxisKeymappings _value))
  ;[0.1 0.1 0.1 1 14] Returns name of the key bound to given action.
  (if _returnvalue
    (Utilities|FlowControl|Sequence
      (:then_0
        (if (Utilities|Array|IsValidIndex _arrayofaxiskeymappings)
          (LocalVariables|SetMainKeyLOCAL (Class|KismetInputLibrary|KeyGetDisplayName (.Key (Utilities|Struct|BreakInputAxisKeyMapping (Utilities|Array|Get(acopy) _arrayofaxiskeymappings)))))))
      (:then_1
        (if (Utilities|Array|IsValidIndex _arrayofaxiskeymappings 1)
          (LocalVariables|SetSecondaryKeyLOCAL (Class|KismetInputLibrary|KeyGetDisplayName (.Key (Utilities|Struct|BreakInputAxisKeyMapping (Utilities|Array|Get(acopy) _arrayofaxiskeymappings 1)))))))
      (:then_2
        (return (LocalVariables|GetMainKeyLOCAL) (LocalVariables|GetSecondaryKeyLOCAL))))
    (else
      (return (LocalVariables|GetMainKeyLOCAL) (LocalVariables|GetSecondaryKeyLOCAL)))))