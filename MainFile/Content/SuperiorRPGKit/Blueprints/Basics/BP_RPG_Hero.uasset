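; Base hero character for the RPG kit, providing shared combat, death and state-check logic that child hero blueprints override or extend.
; Resolve events fire attack and skill dispatchers on authority then unbind them, while item effects go to the controller's items manager.
; Multicast events replicate montages, death and resurrection, toggling the Dead flag and capsule collision.
; Can* functions gate actions mainly on controller state such as death, open UI and item use.
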(event EventBeginPlay)

(event Custom|ActivateQueuedAction
  (bind _queuedattack (Variables|Combat|GetQueuedAttack))
  (if (Utilities|Name|NotEqual(Name) _queuedattack "None")
    (CallFunction|ActivateSkill _queuedattack)
    (else
      (CallFunction|ActivateAttack))))

(event Custom|ActivateSkill
  (params (SkillID :type Name)))

(event Custom|ActivateAttack)

(event Custom|ResolveItemEffect
  ;[0.1 0.1 0.1 1 14] General set up to execute items effects (these are executed directly in itemsmanager).
  (Networking|SwitchHasAuthority
    (:Authority
      (bind _playercontroller (Variables|References|GetPlayerController)
        (:then
          (Default|ExecuteItemEffect (Variables|/Game/SuperiorRPGKit/Blueprints/Basics/BP_RPG_PC_InGame.BP_RPG_PC_InGame_C|GetAC_RPG_ItemsManager _playercontroller)))
        (:else)))))

(event Custom|ResolveAttackEffect
  ;[0.1 0.1 0.1 1 14] General set up to execute attacks effects.
  (Networking|SwitchHasAuthority
    (:Authority
      (Default|CallAttackEffectResolved)
      (EventDispatchers|UnbindallEventsfromAttackEffectResolved))))

(event Custom|QueueSkill
  (params (SkillID :type Name)))

(event Custom|ResetCombatState)

(event Custom|SaveAttackCombo)

(event Custom|ResolveSkillEffect
  ;[0.1 0.1 0.1 1 14] General set up to execute skills effects.
  (Networking|SwitchHasAuthority
    (:Authority
      (Default|CallSkillEffectResolved)
      (EventDispatchers|UnbindallEventsfromSkillEffectResolved))))

(event Custom|ActivateItem
  (params (ItemID :type Name) (ItemsManager :type AC%20RPG%20Items%20Manager%20Object%20Reference)))

(event Custom|PlayMontage_MULTICAST
  (params (AnimMontage :type Anim%20Montage%20Object%20Reference) (InPlayRate :type Float%20%28single-precision%29) (StartSectionName :type Name))
  ;[0.1 0.1 0.1 1 14] Used to play and stop montages on all clients.
  (Animation|PlayAnimMontage AnimMontage InPlayRate StartSectionName))

(event Custom|StopCurrentMontage_MULTICAST
  ;[0.1 0.1 0.1 1 14] Used to play and stop montages on all clients.
  (bind _returnvalue (Animation|GetCurrentMontage :!class /Script/Engine.Character))
  (Animation|StopAnimMontage _returnvalue))

(event Custom|DeathEffect_MULTICAST
  ;[0.1 0.1 0.1 1 14] General death set up, usually extended in specific hero blueprints. (Each hero will usually have some unique part of the death event, like animation, vfx or sfx).
  ;;[0.1 0.1 0.1 1 14] Clear planned events in case hero died during attacking, casting skill or using item.
  (EventDispatchers|UnbindallEventsfromAttackEffectResolved)
  (EventDispatchers|UnbindallEventsfromSkillEffectResolved)
  (CallFunction|ResetCombatState)
  (Utilities|FlowControl|Sequence
    (:then_0
      (bind _playercontroller (Variables|References|GetPlayerController)
        (:then
          (Variables|/Game/SuperiorRPGKit/Blueprints/Components/AC_RPG_StatsManager.AC_RPG_StatsManager_C|SetDead (Variables|/Game/SuperiorRPGKit/Blueprints/Basics/BP_RPG_PC_InGame.BP_RPG_PC_InGame_C|GetAC_RPG_StatsManager _playercontroller) true))
        (:else)))
    (:then_1
      (Collision|SetCollisionEnabled (Variables|Collision|GetCapsuleComponent) "NoCollision"))))

(event Custom|ResurrectionEffect_MULTICAST
  ;[0.1 0.1 0.1 1 14] General resurrection set up, usually extended in specific hero blueprints. (Each hero will usually have some unique part of the resurrection event, like animation, vfx or sfx).
  (Utilities|FlowControl|Sequence
    (:then_0
      (bind _playercontroller (Variables|References|GetPlayerController)
        (:then
          (Variables|/Game/SuperiorRPGKit/Blueprints/Components/AC_RPG_StatsManager.AC_RPG_StatsManager_C|SetDead (Variables|/Game/SuperiorRPGKit/Blueprints/Basics/BP_RPG_PC_InGame.BP_RPG_PC_InGame_C|GetAC_RPG_StatsManager _playercontroller) false))
        (:else)))
    (:then_1
      (Collision|SetCollisionEnabled (Variables|Collision|GetCapsuleComponent) "QueryAndPhysics"))))

(event Custom|MainMenuSpawnEffect
  ;[0.1 0.1 0.1 1 14] Overridden by children blueprints. Mainly to play spawn animation in main menu during character selection.
)

(fn ConstructionScript)

(fn CanAttack
  (params (AttackType :type E_AI_AttackType%20Enum :default "NewEnumerator0"))
  (Utilities|IsValid (Variables|References|GetPlayerController)
    (:Is%20Valid
      (return (Math|Boolean|ANDBoolean (not (Variables|/Game/SuperiorRPGKit/Blueprints/Components/AC_RPG_StatsManager.AC_RPG_StatsManager_C|GetDead (Variables|/Game/SuperiorRPGKit/Blueprints/Basics/BP_RPG_PC_InGame.BP_RPG_PC_InGame_C|GetAC_RPG_StatsManager (Variables|References|GetPlayerController)))) (not (Variables|/Game/SuperiorRPGKit/Blueprints/Basics/BP_RPG_PC_InGame.BP_RPG_PC_InGame_C|GetUIOpen (Variables|References|GetPlayerController))) (not (Variables|/Game/SuperiorRPGKit/Blueprints/Components/AC_RPG_ItemsManager.AC_RPG_ItemsManager_C|GetUsingItem (Variables|/Game/SuperiorRPGKit/Blueprints/Basics/BP_RPG_PC_InGame.BP_RPG_PC_InGame_C|GetAC_RPG_ItemsManager (Variables|References|GetPlayerController)))))))
    (:Is%20Not%20Valid
      (return false))))

(fn CanbeTargeted
  (Utilities|IsValid (Variables|References|GetPlayerController)
    (:Is%20Valid
      (return (not (Variables|/Game/SuperiorRPGKit/Blueprints/Components/AC_RPG_StatsManager.AC_RPG_StatsManager_C|GetDead (Variables|/Game/SuperiorRPGKit/Blueprints/Basics/BP_RPG_PC_InGame.BP_RPG_PC_InGame_C|GetAC_RPG_StatsManager (Variables|References|GetPlayerController))))))
    (:Is%20Not%20Valid
      (return false))))

(fn CanInteract
  (return false))

(fn CanMove
  (Utilities|IsValid (Variables|References|GetPlayerController)
    (:Is%20Valid
      (return (and (not (Variables|/Game/SuperiorRPGKit/Blueprints/Components/AC_RPG_StatsManager.AC_RPG_StatsManager_C|GetDead (Variables|/Game/SuperiorRPGKit/Blueprints/Basics/BP_RPG_PC_InGame.BP_RPG_PC_InGame_C|GetAC_RPG_StatsManager (Variables|References|GetPlayerController)))) (not (Variables|/Game/SuperiorRPGKit/Blueprints/Basics/BP_RPG_PC_InGame.BP_RPG_PC_InGame_C|GetUIOpen (Variables|References|GetPlayerController))))))
    (:Is%20Not%20Valid
      (return false))))

(fn CanReceiveKillReward
  (Utilities|IsValid (Variables|References|GetPlayerController)
    (:Is%20Valid
      (return (not (Variables|/Game/SuperiorRPGKit/Blueprints/Components/AC_RPG_StatsManager.AC_RPG_StatsManager_C|GetDead (Variables|/Game/SuperiorRPGKit/Blueprints/Basics/BP_RPG_PC_InGame.BP_RPG_PC_InGame_C|GetAC_RPG_StatsManager (Variables|References|GetPlayerController))))))
    (:Is%20Not%20Valid
      (return false))))

(fn CanSupport
  (return false))

(fn CanSwitchWeapon
  (return false))

(fn CanUseItem
  (return (Math|Boolean|ANDBoolean (not (Variables|/Game/SuperiorRPGKit/Blueprints/Components/AC_RPG_StatsManager.AC_RPG_StatsManager_C|GetDead (Variables|/Game/SuperiorRPGKit/Blueprints/Basics/BP_RPG_PC_InGame.BP_RPG_PC_InGame_C|GetAC_RPG_StatsManager (Variables|References|GetPlayerController)))) (Utilities|Name|Equal(Name) (Variables|Combat|GetQueuedAttack) "None") (not (Variables|Combat|GetIsAttacking)))))

(fn CanUseSkill
  (Utilities|IsValid (Variables|References|GetPlayerController)
    (:Is%20Valid
      (return (Math|Boolean|ANDBoolean (not (Variables|/Game/SuperiorRPGKit/Blueprints/Components/AC_RPG_StatsManager.AC_RPG_StatsManager_C|GetDead (Variables|/Game/SuperiorRPGKit/Blueprints/Basics/BP_RPG_PC_InGame.BP_RPG_PC_InGame_C|GetAC_RPG_StatsManager (Variables|References|GetPlayerController)))) (not (Variables|/Game/SuperiorRPGKit/Blueprints/Basics/BP_RPG_PC_InGame.BP_RPG_PC_InGame_C|GetUIOpen (Variables|References|GetPlayerController))) (not (Variables|/Game/SuperiorRPGKit/Blueprints/Components/AC_RPG_ItemsManager.AC_RPG_ItemsManager_C|GetUsingItem (Variables|/Game/SuperiorRPGKit/Blueprints/Basics/BP_RPG_PC_InGame.BP_RPG_PC_InGame_C|GetAC_RPG_ItemsManager (Variables|References|GetPlayerController)))))))
    (:Is%20Not%20Valid
      (return false))))