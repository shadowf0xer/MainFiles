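; Server-authoritative RPG enemy spawner that creates random amounts of configured enemy classes at random navigable points within a spawn radius.
; It triggers once, on BeginPlay or when a hero enters the activation sphere, optionally gated by an ongoing quest, which blocks BeginPlay spawning.
; Spawned enemies receive the spawner's level and are initialized.
; Each qualifying hero overlap also adds that hero to their threat pools.
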(event OnComponentBeginOverlap(Sphere_ActivationRadius)
  (params (OverlappedComponent :type Primitive%20Component%20Object%20Reference) (OtherActor :type Actor%20Object%20Reference) (OtherComp :type Primitive%20Component%20Object%20Reference) (OtherBodyIndex :type Integer) (bFromSweep :type Boolean) (SweepResult :type Hit%20Result%20Structure%20%28by%20ref%29))
  (Networking|SwitchHasAuthority
    (:Authority
      (bind _asbp_rpg_hero (Utilities|Casting|CastToBP_RPG_Hero OtherActor))
      (bind _result (Condition|CanTriggerSpawner (Variables|/Game/SuperiorRPGKit/Blueprints/Basics/BP_RPG_Hero.BP_RPG_Hero_C|GetPlayerController _asbp_rpg_hero))) ; Check fi player can trigger spawner\n(ie. has required quest).
      (if _result
        (if (not (Variables|Default|GetActivated)) ; Do not trigger spawner\nif it is already active.\n(to avoid infinite enemies spawning)
          (Variables|Default|SetActivated true)
          (CallFunction|SpawnEnemies))
        ;[0.1 0.1 0.1 1 14] Whenever player enters radius of the spawner add him to
        ; all enemies threat pool, so they can attack him.
        (for _array_element (Variables|Default|GetSpawnedEnemies)
          (Default|ModifyThreat (Variables|/Game/SuperiorRPGKit/AI/Blueprints/Core/BP_AI_Controller.BP_AI_Controller_C|GetAC_AI_Target (Variables|/Game/SuperiorRPGKit/Blueprints/Basics/BP_RPG_Enemy.BP_RPG_Enemy_C|GetAIController _array_element)) OtherActor 0.0))))))

(event EventBeginPlay
  (Networking|SwitchHasAuthority
    (:Authority
      (if (Variables|Config|GetSpawnOnBeginPlay)
        (bind _result (Condition|CanTriggerSpawner))
        (if _result
          (Variables|Default|SetActivated true)
          (CallFunction|SpawnEnemies))))))

(event Collision|EventActorBeginOverlap
  (params (OtherActor :type Actor%20Object%20Reference)))

(event EventTick
  (params (DeltaSeconds :type Float%20%28single-precision%29)))

(fn ConstructionScript
  (Components|Sphere|SetSphereRadius (Variables|Default|GetSphere_SpawnRadius) (Variables|Config|GetSpawnRadius) true)
  (Components|Sphere|SetSphereRadius (Variables|Default|GetSphere_ActivationRadius) (Variables|Config|GetActivationRadius) true))

(fn SpawnEnemies
  (for _array_element (Variables|Config|GetEnemiesToSpawn)
    (LocalVariables|SetAmountToSpawnLOCAL (Math|Random|RandomIntegerinRange (.MinSpawnAmount (Utilities|Struct|BreakS_RPG_EnemySpawn _array_element)) (.MaxSpawnAmount (Utilities|Struct|BreakS_RPG_EnemySpawn _array_element)))) ; Roll random number of enemies to spawn.
    (for _index (range 1 (LocalVariables|GetAmountToSpawnLOCAL))
      ;[0.1 0.1 0.1 1 14] Spawn enemy at random location in spawner radius.
      ; NOTE: Spawn Location is chosen randomly in NAVIGABLE radius. It is possible that if spawn radius is small and there is many enemies some of them won't spawn.
      ; Take number of enemies to spawn more as approximate value than guaranteed.
      (bind (_result _spawnlocation) (Getters|GetRandomLocationinSpawnRadius))
      (if _result
        (bind _returnvalue (Game|SpawnActorfromClass (.EnemyActorClass (Utilities|Struct|BreakS_RPG_EnemySpawn _array_element)) (Math|Transform|MakeTransform _spawnlocation (Math|Rotator|MakeRotator 0.0 0.0 (Math|Random|RandomFloatinRange 0.0 359.0)) "1,1,1") "AdjustIfPossibleButDontSpawnIfColliding" 0 0))
        (Utilities|IsValid _returnvalue
          (:Is%20Valid
            (LocalVariables|SetSpawnedEnemyLOCAL _returnvalue)
            (Utilities|Array|Add (Variables|Default|GetSpawnedEnemies) (LocalVariables|GetSpawnedEnemyLOCAL))
            (Variables|/Game/SuperiorRPGKit/Blueprints/Components/AC_RPG_StatsManager.AC_RPG_StatsManager_C|SetCurrentLevel (Variables|/Game/SuperiorRPGKit/Blueprints/Basics/BP_RPG_Enemy.BP_RPG_Enemy_C|GetAC_RPG_StatsManager (LocalVariables|GetSpawnedEnemyLOCAL)) (Variables|Config|GetLevel))
            (Default|Initialize (LocalVariables|GetSpawnedEnemyLOCAL))))))))

(fn GetRandomLocationinSpawnRadius
  (bind _returnvalue (Transformation|GetActorLocation))
  (bind _spawnradius (Variables|Config|GetSpawnRadius))
  (bind (_randomlocation _returnvalue_2) (Class|NavigationSystem|GetRandomPointinNavigableRadius _returnvalue _spawnradius))
  (return _returnvalue_2 _randomlocation))

(fn CanTriggerSpawner
  (params (PlayerController :type BP%20RPG%20PC%20in%20Game%20Object%20Reference))
  (bind _requiredquest (Variables|Config|GetRequiredQuest))
  (if (Utilities|Name|NotEqual(Name) _requiredquest "None")
    (Utilities|IsValid PlayerController
      (:Is%20Valid
        ;[0.1 0.1 0.1 1 14] Check if player has quest if it is required to trigger spawner.
        (return (Utilities|Map|Contains (Variables|/Game/SuperiorRPGKit/Blueprints/Components/AC_RPG_QuestsManager.AC_RPG_QuestsManager_C|GetOngoingQuests (Variables|/Game/SuperiorRPGKit/Blueprints/Basics/BP_RPG_PC_InGame.BP_RPG_PC_InGame_C|GetAC_RPG_QuestsManager PlayerController)) _requiredquest)))
      (:Is%20Not%20Valid
        (return false)))
    (else
      (return true))))