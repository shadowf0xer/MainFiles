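; Interactable actor for the RPG kit that supplies interaction text, type, action, radius and time, and accepts limited simultaneous users until one interaction succeeds.
; Begin events track interacting actors, with the first starting a fixed auto-finish timer.
; Finish and cancel events remove the actor, clear the timer as appropriate, and can end other participants' interactions through flag-controlled messages to their AI controllers.
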(event EventBeginPlay)

(event Collision|EventActorBeginOverlap
  (params (OtherActor :type Actor%20Object%20Reference)))

(event EventTick
  (params (DeltaSeconds :type Float%20%28single-precision%29)))

(event Custom|InteractionAutofinish
  (Class|BPIAICommands|EndInteraction(Message) (AI|GetAIController (Utilities|Array|Get(acopy) (Variables|Runtime|GetInteractingActors))) "NewEnumerator0"))

(event EventOnBeginInteract
  (params (InteractingActor :type Actor%20Object%20Reference) (InteractionManager :type AC%20RPG%20Interaction%20Manager%20Object%20Reference))
  (Utilities|IsValid InteractingActor
    (:Is%20Valid
      (Utilities|Array|AddUnique (Variables|Runtime|GetInteractingActors) InteractingActor)
      (if (== (Utilities|Array|Length (Variables|Runtime|GetInteractingActors)) 1) ; First interacting actor starts the timer.
        (bind _returnvalue (Utilities|Time|SetTimerbyEvent (EventDispatchers|CreateEvent :!event Custom|InteractionAutofinish) 5.0)) ; Consider interaction finished after 5 seconds.
        (Variables|Runtime|SetInteractionTimer _returnvalue)))))

(event EventOnFinishInteract
  (params (InteractingActor :type Actor%20Object%20Reference) (InteractionManager :type AC%20RPG%20Interaction%20Manager%20Object%20Reference))
  (Variables|Runtime|SetInteractionSucceeded true)
  (Utilities|FlowControl|Sequence
    (:then_0
      (Utilities|IsValid InteractingActor
        (:Is%20Valid
          (Utilities|Array|RemoveItem (Variables|Runtime|GetInteractingActors) InteractingActor))))
    (:then_1
      (if (Variables|Config|GetFinishOnOtherActorsWhenFinished)
        (for _array_element (Variables|Runtime|GetInteractingActors)
          (Class|BPIAICommands|EndInteraction(Message) (AI|GetAIController _array_element) "NewEnumerator0"))
        (Utilities|Array|Clear (Variables|Runtime|GetInteractingActors))
        (elif (Variables|Config|GetCancelOnOtherActorsWhenFinished)
          (for _array_element_2 (Variables|Runtime|GetInteractingActors)
            (Class|BPIAICommands|EndInteraction(Message) (AI|GetAIController _array_element_2) "NewEnumerator1"))
          (Utilities|Array|Clear (Variables|Runtime|GetInteractingActors)))))
    (:then_2
      (Utilities|Time|ClearandInvalidateTimerbyHandle (Variables|Runtime|GetInteractionTimer)))))

(event EventOnCancelInteract
  (params (InteractingActor :type Actor%20Object%20Reference) (InteractionManager :type AC%20RPG%20Interaction%20Manager%20Object%20Reference))
  (bind _interactingactors (Variables|Runtime|GetInteractingActors))
  (Utilities|FlowControl|Sequence
    (:then_0
      (Utilities|IsValid InteractingActor
        (:Is%20Valid
          (Utilities|Array|RemoveItem (Variables|Runtime|GetInteractingActors) InteractingActor))))
    (:then_1
      (if (Variables|Config|GetCancelOnOtherActorsWhenCanceled)
        (Utilities|Time|ClearandInvalidateTimerbyHandle (Variables|Runtime|GetInteractionTimer))
        (if (> (Utilities|Array|Length _interactingactors) 0)
          (for _array_element _interactingactors
            (Class|BPIAICommands|EndInteraction(Message) (AI|GetAIController _array_element) "NewEnumerator1"))
          (Utilities|Array|Clear (Variables|Runtime|GetInteractingActors)))
        (elif (== (Utilities|Array|Length (Variables|Runtime|GetInteractingActors)) 0)
          (Utilities|Time|ClearandInvalidateTimerbyHandle (Variables|Runtime|GetInteractionTimer)))))))

(fn ConstructionScript)

(fn GetInteractionAction
  (params (InteractingActor :type Actor%20Object%20Reference))
  (return "NewEnumerator0"))

(fn GetInteractionRadius
  (params (InteractingActor :type Actor%20Object%20Reference))
  (return 2e+02))

(fn GetInteractionText
  (return (Utilities|Text|FormatText "Interact with {display name}" (Variables|Config|GetDisplayName))))

(fn GetInteractionTime
  (params (InteractingActor :type Actor%20Object%20Reference))
  (return 5.0))

(fn GetInteractionType
  (return "NewEnumerator3"))

(fn IsInteractable
  (params (InteractingActor :type Actor%20Object%20Reference) (InteractionManager :type AC%20RPG%20Interaction%20Manager%20Object%20Reference))
  (bind _interactingactors (Variables|Runtime|GetInteractingActors))
  (bind _returnvalue (Utilities|Array|Length _interactingactors))
  (return (and (< (Math|Integer|SelectInt (- _returnvalue 1) _returnvalue (Utilities|Array|ContainsItem (Variables|Runtime|GetInteractingActors) InteractingActor)) (Variables|Config|GetMaxInteractingActors)) (not (Variables|Runtime|GetInteractionSucceeded)))))