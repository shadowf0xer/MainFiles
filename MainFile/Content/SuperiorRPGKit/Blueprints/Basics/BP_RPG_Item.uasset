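; World item pickup for the RPG kit that hands itself to the interactor's items manager component through a server pickup call.
; On BeginPlay the server optionally rolls a random item, quality and bonuses from the items data table.
; To save bandwidth it replicates only name and quality, not the whole item struct.
; OnReps update the floating name tooltip, shown on cursor hover, and tint the box by quality.
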(event OnBeginCursorOver(Cube)
  (params (TouchedComponent :type Primitive%20Component%20Object%20Reference))
  ;[0.1 0.1 0.1 1 14] Show/Hide item name on cursor over. (Top-Down mode only)
  (Development|SetHiddeninGame (Variables|Default|GetFloatingName) false false))

(event OnEndCursorOver(Cube)
  (params (TouchedComponent :type Primitive%20Component%20Object%20Reference))
  ;[0.1 0.1 0.1 1 14] Show/Hide item name on cursor over. (Top-Down mode only)
  (Development|SetHiddeninGame (Variables|Default|GetFloatingName) true false))

(event EventBeginPlay
  (Networking|SwitchHasAuthority
    (:Authority
      (if (Variables|Config|GetGenerateRandomItem)
        ;[0.1 0.1 0.1 1 14] Roll random item from data table.
        (bind _itemid (Randomization|GetRandomItemfromDatatable))
        (Variables|Config|SetItemData (Utilities|Struct|MakeS_RPG_Item_Dynamic _itemid 1 (CallFunction|RollItemQuality _itemid) (CallFunction|RollItemBonuses _itemid (CallFunction|RollItemQuality _itemid) false)))
        (CallFunction|UpdateReplicatedData)
        (else
          ;[0.1 0.1 0.1 1 14] Update name of item and its quality displayed to players.
          (CallFunction|UpdateReplicatedData))))
    (:Remote
      ;[0.1 0.1 0.1] Update displayed item name on client. (In case it doesn't manage to create widget when name variable is repliacted)
      (bind _aswbp_rpg_world_item_tooltip (Utilities|Casting|CastToWBP_RPG_WorldItemTooltip (UserInterface|GetUserWidgetObject (Variables|Default|GetFloatingName))))
      (Rendering|Components|TextRender|SetText (Variables|/Game/SuperiorRPGKit/Widgets/Items/WBP_RPG_WorldItemTooltip.WBP_RPG_WorldItemTooltip_C|GetTextBlock_ItemName _aswbp_rpg_world_item_tooltip) (Variables|Replicated|GetItemName)))))

(event EventOnBeginInteract
  (params (InteractingActor :type Actor%20Object%20Reference) (InteractionManager :type AC%20RPG%20Interaction%20Manager%20Object%20Reference))
  (bind _returnvalue (Components|GetOwner InteractionManager))
  (bind _returnvalue_2 (Actor|GetComponentbyClass _returnvalue "/Game/SuperiorRPGKit/Blueprints/Components/AC_RPG_ItemsManager.AC_RPG_ItemsManager_C"))
  (Utilities|IsValid _returnvalue_2
    (:Is%20Valid
      (Default|PickUpItemSERVER _returnvalue_2 self))))

(fn ConstructionScript)

(fn UpdateReplicatedData
  (bind _itemdata (Variables|Config|GetItemData))
  (bind (_id _rolledquality) (Utilities|Struct|BreakS_RPG_Item_Dynamic _itemdata))
  ;[0.1 0.1 0.1 1 14] Read data from Item Structure and assign its parts to replicated variables.
  ; (Generally we won't need whole structure to be replicated so we save bandwidth usage replicating only specific variables).
  (bind _returnvalue (Utilities|GetDataTableRow "/Game/SuperiorRPGKit/Datatables/DT_RPG_Items.DT_RPG_Items" _id)
    (:then
      (Variables|Replicated|SetItemName (Utilities|Struct|BreakS_RPG_Item_Static _returnvalue))
      (Variables|Replicated|SetItemQuality _rolledquality))))

(fn OnRepItemName
  ;[0.1 0.1 0.1 1 14] Update name displayed in "floating" widget.
  (bind _aswbp_rpg_world_item_tooltip (Utilities|Casting|CastToWBP_RPG_WorldItemTooltip (UserInterface|GetUserWidgetObject (Variables|Default|GetFloatingName))))
  (Rendering|Components|TextRender|SetText (Variables|/Game/SuperiorRPGKit/Widgets/Items/WBP_RPG_WorldItemTooltip.WBP_RPG_WorldItemTooltip_C|GetTextBlock_ItemName _aswbp_rpg_world_item_tooltip) (Variables|Replicated|GetItemName)))

(fn OnRepItemQuality
  ;[0.1 0.1 0.1 1 14] Change dropped item box color depending on quality. (can be replaced with color streak vfx or something if you want to make it fancy)
  (bind _returnvalue (Rendering|Material|CreateDynamicMaterialInstance (Variables|Default|GetCube) 0 "/Game/SuperiorRPGKit/Demo/Meshes/Items/Equipment/Materials/M_FlatColor.M_FlatColor" :!class /Script/Engine.PrimitiveComponent))
  (Rendering|Material|SetVectorParameterValue _returnvalue "Color" (CallFunction|ItemQualitytoColor (Variables|Replicated|GetItemQuality)) :!class /Script/Engine.MaterialInstanceDynamic))

(fn GetRandomItemfromDatatable
  (bind _outrownames (DataTable|GetDataTableRowNames "/Game/SuperiorRPGKit/Datatables/DT_RPG_Items.DT_RPG_Items"))
  (return (Utilities|Array|Get(acopy) _outrownames (Math|Random|RandomIntegerinRange 0 (- (Utilities|Array|Length _outrownames) 1)))))

(fn GetInteractionAction
  (params (InteractingActor :type Actor%20Object%20Reference))
  (return "NewEnumerator3"))

(fn GetInteractionRadius
  (params (InteractingActor :type Actor%20Object%20Reference))
  (return 2e+02))

(fn GetInteractionText
  (return (Utilities|Text|FormatText "Pick up {item name}" (Variables|Replicated|GetItemName))))

(fn GetInteractionTime
  (params (InteractingActor :type Actor%20Object%20Reference))
  (return 0.0))

(fn GetInteractionType
  (return "NewEnumerator1"))

(fn IsInteractable
  (params (InteractingActor :type Actor%20Object%20Reference) (InteractionManager :type AC%20RPG%20Interaction%20Manager%20Object%20Reference))
  (return true))