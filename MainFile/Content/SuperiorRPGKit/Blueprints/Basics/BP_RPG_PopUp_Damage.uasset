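; Pooled floating damage number actor that shows damage text at a given world location through a widget component.
; DisplayText sets the text, tints it red for damage dealt to the player or white otherwise, plays the pop-up animation with the critical flag and moves the actor into place.
; After a short delay it hides the widget and returns itself to the FloatingTextManager's free pool for reuse instead of respawning.
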(event Custom|DisplayText
  (params (Text :type Text) (Location :type Vector) (Critical :type Boolean) (DealtToPlayer :type Boolean))
  (Development|SetHiddeninGame (Variables|Default|GetDamagePopUpText) false false) ; make pop up visible
  (bind _damagepopupwidget (Variables|References|GetDamagePopUpWidget)
    (:then
      (Rendering|Components|TextRender|SetText (Variables|/Game/SuperiorRPGKit/Widgets/PopUp/WBP_RPG_DamagePopUp.WBP_RPG_DamagePopUp_C|GetTextBlock_Damage _damagepopupwidget) Text) ; update pop up text
      (Appearance|SetColorandOpacity (Variables|/Game/SuperiorRPGKit/Widgets/PopUp/WBP_RPG_DamagePopUp.WBP_RPG_DamagePopUp_C|GetTextBlock_Damage _damagepopupwidget) (Utilities|Struct|MakeSlateColor (select DealtToPlayer "(R=0.750000,G=0.000000,B=0.000000,A=1.000000)" "(R=1.000000,G=1.000000,B=1.000000,A=1.000000)")) :!class /Script/UMG.TextBlock) ; update pop up color
      (Default|PlayPopUpAnimation (Variables|References|GetDamagePopUpWidget) Critical) ; play pop up animation
      (Transformation|SetActorLocation Location false false) ; set initial pop up location
      (Utilities|FlowControl|Delay 1.0)
      (Development|SetHiddeninGame (Variables|Default|GetDamagePopUpText) true false) ; after short delay hide pop up
      (Utilities|Array|Add (Variables|/Game/SuperiorRPGKit/Blueprints/Components/AC_RPG_FloatingTextManager.AC_RPG_FloatingTextManager_C|GetFreeDamagePopUps (Variables|References|GetFloatingTextManager)) self) ; once pop up hides add it to\npool of available pop ups\n(so we can reuse it instead of \nspawning new one everytime)
    )
    (:else)))

(event EventBeginPlay
  ;[0.1 0.1 0.1 1 14] Set reference to widget.
  (bind _aswbp_rpg_damage_pop_up (Utilities|Casting|CastToWBP_RPG_DamagePopUp (UserInterface|GetUserWidgetObject (Variables|Default|GetDamagePopUpText))))
  (Variables|References|SetDamagePopUpWidget _aswbp_rpg_damage_pop_up))

(fn ConstructionScript)