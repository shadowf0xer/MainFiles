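; Main menu PlayerController that handles hero creation, selection and deletion, then launches offline, listen-server host or join-by-IP play.
; A "General" save indexes per-hero save slots and remembers the last played hero.
; Heroes from DT_RPG_Heroes spawn at the first PlayerStart as previews, with saved equipment for existing ones.
; It also creates the menu and loading screen, initializes options and forwards key-rebinding input to ACRPGOptionsManager.
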(event Custom|InitialLoad
  ;[0.1 0.1 0.1 1 14] Loads general save (or creates it if game is played first time). If loaded successfully additionally loads last player hero, so it can be displayed in menu level.
  (bind _returnvalue (SaveGame|DoesSaveGameExist "General"))
  (if _returnvalue
    (bind _returnvalue_2 (SaveGame|LoadGamefromSlot "General"))
    (bind _asbp_rpg_save_general (Utilities|Casting|CastToBP_RPG_SAVE_General _returnvalue_2))
    (bind _returnvalue_3 (SaveGame|LoadGamefromSlot (Variables|/Game/SuperiorRPGKit/Blueprints/Saves/BP_RPG_SAVE_General.BP_RPG_SAVE_General_C|GetLastPlayedHeroSave _asbp_rpg_save_general)))
    (bind _asbp_rpg_save_hero (Utilities|Casting|CastToBP_RPG_SAVE_Hero _returnvalue_3))
    (Variables|HeroSelection|SetSelectedHeroSave (Variables|/Game/SuperiorRPGKit/Blueprints/Saves/BP_RPG_SAVE_General.BP_RPG_SAVE_General_C|GetLastPlayedHeroSave _asbp_rpg_save_general))
    (HeroSelection|SpawnExistingHero (Variables|/Game/SuperiorRPGKit/Blueprints/Saves/BP_RPG_SAVE_Hero.BP_RPG_SAVE_Hero_C|GetHeroID _asbp_rpg_save_hero))
    (else
      (bind _returnvalue_4 (SaveGame|CreateSaveGameObject "/Game/SuperiorRPGKit/Blueprints/Saves/BP_RPG_SAVE_General.BP_RPG_SAVE_General_C"))
      (SaveGame|SaveGametoSlot _returnvalue_4 "General"))))

(event EventBeginPlay
  ;[0.1 0.1 0.1 1 14] Add Loading screen on top of everything.
  (bind _returnvalue (UserInterface|CreateWidget "/Game/SuperiorRPGKit/Widgets/LoadingScreen/WBP_RPG_LoadingScreen.WBP_RPG_LoadingScreen_C"))
  (bind _output_get (Variables|Widgets|SetLoadingScreen _returnvalue))
  (UserInterface|Viewport|AddtoViewport _output_get 10)
  (Input|SetInputModeGameandUI self 0 "DoNotLock" false) ; Set proper input mode.
  (CallFunction|InitialLoad) ; Initial load to get last player hero.
  ;[0.1 0.1 0.1 1 14] Create main menu widget.
  (bind _returnvalue_2 (UserInterface|CreateWidget "/Game/SuperiorRPGKit/Widgets/MainMenu/WBP_RPG_MainMenu.WBP_RPG_MainMenu_C" 0 self))
  (bind _output_get_2 (Variables|Widgets|SetMainMenu _returnvalue_2))
  (UserInterface|Viewport|AddtoViewport _output_get_2 0)
  ;[0.1 0.1 0.1 1 14] After slight delay Initialize OptionsManager which will load player settings.
  ; Slight delay is needed because loaded settings will also set proper values in settings widgets so we just make sure that widget has got time to initialize itself.
  (Utilities|FlowControl|Delay 0.1)
  (Default|InitializeOptionsManager (Variables|Default|GetAC_RPG_OptionsManager) 0 true)
  ;[0.1 0.1 0.1 1 14] After another delay we can hide loading screen.
  (Utilities|FlowControl|Delay 1.0)
  (Default|FadeOut (Variables|Widgets|GetLoadingScreen)))

(event Custom|HostGame
  (params (GameName :type String))
  ;[0.1 0.1 0.1 1 14] HOST. Load selected hero map and open level in listen mode.
  (Utilities|FlowControl|DoOnce false
    (:Completed
      (bind _returnvalue (SaveGame|LoadGamefromSlot (Variables|HeroSelection|GetSelectedHeroSave)))
      (bind _asbp_rpg_save_hero (Utilities|Casting|CastToBP_RPG_SAVE_Hero _returnvalue))
      (Default|Fadein (Variables|Widgets|GetLoadingScreen)) ; Show loading screen
      (Utilities|FlowControl|Delay 1.0) ; Short delay to imitate "loading" behavior.
      (Game|OpenLevel(byName) (Variables|/Game/SuperiorRPGKit/Blueprints/Saves/BP_RPG_SAVE_Hero.BP_RPG_SAVE_Hero_C|GetMapName _asbp_rpg_save_hero) true "listen"))))

(event Custom|JoinGame
  (params (IP :type String))
  ;[0.1 0.1 0.1 1 14] JOIN. Connects to the hosted game with given IP.
  (Utilities|FlowControl|DoOnce false
    (:Completed
      (Default|Fadein (Variables|Widgets|GetLoadingScreen)) ; Show loading screen
      (Utilities|FlowControl|Delay 1.0) ; Short delay to imitate "loading" behavior.
      (Game|OpenLevel(byName) (Utilities|String|StringToName IP)))))

(event Custom|PlayOffline
  ;[0.1 0.1 0.1 1 14] OFFLINE. Load selected hero map.
  (Utilities|FlowControl|DoOnce false
    (:Completed
      (bind _returnvalue (SaveGame|LoadGamefromSlot (Variables|HeroSelection|GetSelectedHeroSave)))
      (bind _asbp_rpg_save_hero (Utilities|Casting|CastToBP_RPG_SAVE_Hero _returnvalue))
      (Default|Fadein (Variables|Widgets|GetLoadingScreen)) ; Show loading screen
      (Utilities|FlowControl|Delay 1.0) ; Short delay to imitate "loading" behavior.
      (Game|OpenLevel(byName) (Variables|/Game/SuperiorRPGKit/Blueprints/Saves/BP_RPG_SAVE_Hero.BP_RPG_SAVE_Hero_C|GetMapName _asbp_rpg_save_hero)))))

(event Input|KeyboardEvents|Escape
  (params (Key :type Key%20Structure))
  ;[0.1 0.1 0.1 1 12] Cancel key rebinding.
  (:Pressed
    (Default|StopListeningforKeyRebinding (Variables|Default|GetAC_RPG_OptionsManager))))

(event Input|KeyboardEvents|ScrollLock
  (params (Key :type Key%20Structure))
  ;[0.1 0.1 0.1 1 12] Cancel key rebinding.
  (:Pressed
    (Default|StopListeningforKeyRebinding (Variables|Default|GetAC_RPG_OptionsManager))))

(event Input|KeyboardEvents|AnyKey
  (params (Key :type Key%20Structure))
  ;[0.1 0.1 0.1 1 12] Input for key rebinding.
  (:Pressed
    (Default|RebindKey (Variables|Default|GetAC_RPG_OptionsManager) Key)))

(fn ConstructionScript)

(fn StartHeroCreation
  ;[0.1 0.1 0.1 1 14] Spawn first available hero.
  (bind _output_get (Variables|HeroCreation|SetSelectedHero (Utilities|Array|Get(acopy) (Variables|HeroCreation|GetAvailableHeroes))))
  (HeroCreation|SpawnNewHero _output_get))

(fn SpawnNewHero
  (params (HeroClass :type Name))
  (Default|UpdateHeroAttributes (Variables|Widgets|GetMainMenu) HeroClass (not (Utilities|Array|ContainsItem (Variables|HeroCreation|GetLockedHeroes) HeroClass))) ; Update hero data displayed to player.
  ;[0.1 0.1 0.1 1 14] If there is another hero spawned - destroy it.
  (bind _displayedcharacter (Variables|Default|GetDisplayedCharacter)
    (:then
      (Actor|DestroyActor _displayedcharacter))
    (:else
      _))
  (bind _outactors (Actor|GetAllActorsOfClass "/Script/Engine.PlayerStart"))
  (Utilities|IsValid (Utilities|Array|Get(acopy) _outactors)
    (:Is%20Valid
      (bind _returnvalue (Utilities|GetDataTableRow "/Game/SuperiorRPGKit/Datatables/DT_RPG_Heroes.DT_RPG_Heroes" HeroClass)
        (:then
          (Rendering|Components|TextRender|SetText (Variables|/Game/SuperiorRPGKit/Widgets/MainMenu/WBP_RPG_MainMenu.WBP_RPG_MainMenu_C|GetTextBlock_HeroClass (Variables|Widgets|GetMainMenu)) (.DisplayName (Utilities|Struct|BreakS_RPG_Hero_Static _returnvalue)))
          ;[0.1 0.1 0.1 1 14] Spawn hero at PlayerStart transform.
          (bind _returnvalue_2 (Game|SpawnActorfromClass (.ActorClass (Utilities|Struct|BreakS_RPG_Hero_Static _returnvalue)) (Transformation|GetActorTransform (Utilities|Array|Get(acopy) _outactors)) "AlwaysSpawn" 0 0))
          (bind _output_get (Variables|Default|SetDisplayedCharacter _returnvalue_2))
          (Default|MainMenuSpawnEffect _output_get) ; Play hero spawn effect (ie. animation + vfx)
          (return _output_get))))))

(fn SelectNextHeroClass
  ;[0.1 0.1 0.1 1 14] Cycle to the next available hero.
  (bind _output_get (Variables|HeroCreation|SetSelectedHero (Utilities|Array|Get(acopy) (Variables|HeroCreation|GetAvailableHeroes) (Math|Integer|SelectInt (+ (Utilities|Array|FindItem (Variables|HeroCreation|GetAvailableHeroes) (Variables|HeroCreation|GetSelectedHero)) 1) 0 (< (+ (Utilities|Array|FindItem (Variables|HeroCreation|GetAvailableHeroes) (Variables|HeroCreation|GetSelectedHero)) 1) (Utilities|Array|Length (Variables|HeroCreation|GetAvailableHeroes)))))))
  (HeroCreation|SpawnNewHero _output_get))

(fn SelectPreviousHeroClass
  ;[0.1 0.1 0.1 1 14] Cycle to previous available hero.
  (bind _output_get (Variables|HeroCreation|SetSelectedHero (Utilities|Array|Get(acopy) (Variables|HeroCreation|GetAvailableHeroes) (Math|Integer|SelectInt (- (Utilities|Array|FindItem (Variables|HeroCreation|GetAvailableHeroes) (Variables|HeroCreation|GetSelectedHero)) 1) (- (Utilities|Array|Length (Variables|HeroCreation|GetAvailableHeroes)) 1) (>= (- (Utilities|Array|FindItem (Variables|HeroCreation|GetAvailableHeroes) (Variables|HeroCreation|GetSelectedHero)) 1) 0)))))
  (HeroCreation|SpawnNewHero _output_get))

(fn ShowAvailableHeroes
  (Widget|Panel|ClearChildren (Variables|/Game/SuperiorRPGKit/Widgets/MainMenu/WBP_RPG_MainMenu.WBP_RPG_MainMenu_C|GetContainer_HeroSlots (Variables|Widgets|GetMainMenu))) ; Clear hero slots.
  (bind _returnvalue (SaveGame|LoadGamefromSlot "General"))
  (bind _asbp_rpg_save_general (Utilities|Casting|CastToBP_RPG_SAVE_General _returnvalue))
  ;[0.1 0.1 0.1 1 14] For each hero save create hero slot widget and populate it with necessary data.
  (for _array_element (Variables|/Game/SuperiorRPGKit/Blueprints/Saves/BP_RPG_SAVE_General.BP_RPG_SAVE_General_C|GetPlayerHeroesSaves _asbp_rpg_save_general)
    (bind _returnvalue_2 (SaveGame|LoadGamefromSlot _array_element))
    (bind _asbp_rpg_save_hero (Utilities|Casting|CastToBP_RPG_SAVE_Hero _returnvalue_2))
    (bind _returnvalue_3 (UserInterface|CreateWidget "/Game/SuperiorRPGKit/Widgets/MainMenu/WBP_RPG_HeroSelectionSlot.WBP_RPG_HeroSelectionSlot_C" 0 self))
    (Utilities|Array|Add (Variables|Widgets|GetHeroSelectionSlots) _returnvalue_3)
    (Default|SetSlotData _returnvalue_3 _asbp_rpg_save_hero)
    (Default|ToggleHighlight _returnvalue_3 (Utilities|Enum|Equal(Enum) (Variables|/Game/SuperiorRPGKit/Widgets/MainMenu/WBP_RPG_HeroSelectionSlot.WBP_RPG_HeroSelectionSlot_C|GetAssignedHeroSaveName _returnvalue_3) (Variables|/Game/SuperiorRPGKit/Blueprints/Saves/BP_RPG_SAVE_General.BP_RPG_SAVE_General_C|GetLastPlayedHeroSave _asbp_rpg_save_general)))
    (Class|VerticalBox|AddChildtoVerticalBox (Variables|/Game/SuperiorRPGKit/Widgets/MainMenu/WBP_RPG_MainMenu.WBP_RPG_MainMenu_C|GetContainer_HeroSlots (Variables|Widgets|GetMainMenu)) _returnvalue_3)
    (Layout|BorderSlot|SetPadding _returnvalue_3 (Utilities|Struct|MakeMargin 0.0 0.0 0.0 16.0) :!class /Script/UMG.UserWidget))
  (Widget|SetVisibility (Variables|/Game/SuperiorRPGKit/Widgets/MainMenu/WBP_RPG_MainMenu.WBP_RPG_MainMenu_C|GetContainer_OnHeroSelected (Variables|Widgets|GetMainMenu)) (select (Utilities|Array|ContainsItem (Variables|/Game/SuperiorRPGKit/Blueprints/Saves/BP_RPG_SAVE_General.BP_RPG_SAVE_General_C|GetPlayerHeroesSaves _asbp_rpg_save_general) (Variables|/Game/SuperiorRPGKit/Blueprints/Saves/BP_RPG_SAVE_General.BP_RPG_SAVE_General_C|GetLastPlayedHeroSave _asbp_rpg_save_general)) "SelfHitTestInvisible" "Hidden")))

(fn CreateNewHero
  (params (HeroName :type String))
  ;[0.2 0.2 0.2] Check hero name length.
  (if (and (>= (Utilities|String|Len HeroName) 3) (<= (Utilities|String|Len HeroName) 12))
    ;[0.2 0.2 0.2] Check whether hero name is unique, if so add it to the pool of player heroes.
    (bind _returnvalue (SaveGame|LoadGamefromSlot "General"))
    (bind _asbp_rpg_save_general (Utilities|Casting|CastToBP_RPG_SAVE_General _returnvalue))
    (if (not (Utilities|Array|ContainsItem (Variables|/Game/SuperiorRPGKit/Blueprints/Saves/BP_RPG_SAVE_General.BP_RPG_SAVE_General_C|GetPlayerHeroesSaves _asbp_rpg_save_general) (Utilities|String|Append "Hero_" HeroName)))
      (Utilities|Array|Add (Variables|/Game/SuperiorRPGKit/Blueprints/Saves/BP_RPG_SAVE_General.BP_RPG_SAVE_General_C|GetPlayerHeroesSaves _asbp_rpg_save_general) (Utilities|String|Append "Hero_" HeroName))
      (Variables|/Game/SuperiorRPGKit/Blueprints/Saves/BP_RPG_SAVE_General.BP_RPG_SAVE_General_C|SetLastPlayedHeroSave _asbp_rpg_save_general (Utilities|String|Append "Hero_" HeroName))
      (SaveGame|SaveGametoSlot _asbp_rpg_save_general "General")
      ;[0.2 0.2 0.2] Create hero save slot and populate it with default data.
      (bind _returnvalue_2 (SaveGame|CreateSaveGameObject "/Game/SuperiorRPGKit/Blueprints/Saves/BP_RPG_SAVE_Hero.BP_RPG_SAVE_Hero_C"))
      (LocalVariables|SetSaveLOCAL _returnvalue_2)
      (bind _returnvalue_3 (Utilities|GetDataTableRow "/Game/SuperiorRPGKit/Datatables/DT_RPG_Heroes.DT_RPG_Heroes" (Variables|HeroCreation|GetSelectedHero))
        (:then
          (LocalVariables|SetHeroDefaultDataLOCAL _returnvalue_3)
          (Variables|/Game/SuperiorRPGKit/Blueprints/Saves/BP_RPG_SAVE_Hero.BP_RPG_SAVE_Hero_C|SetHeroName (LocalVariables|GetSaveLOCAL) HeroName)
          (Variables|/Game/SuperiorRPGKit/Blueprints/Saves/BP_RPG_SAVE_Hero.BP_RPG_SAVE_Hero_C|SetHeroID (LocalVariables|GetSaveLOCAL) (Variables|HeroCreation|GetSelectedHero))
          (Variables|/Game/SuperiorRPGKit/Blueprints/Saves/BP_RPG_SAVE_Hero.BP_RPG_SAVE_Hero_C|SetMapName (LocalVariables|GetSaveLOCAL) (Variables|NewGameSettings|GetDefaultMap))
          (Variables|/Game/SuperiorRPGKit/Blueprints/Saves/BP_RPG_SAVE_Hero.BP_RPG_SAVE_Hero_C|SetSpawnID (LocalVariables|GetSaveLOCAL) (Variables|NewGameSettings|GetDefaultSpawnPoint))
          (Variables|/Game/SuperiorRPGKit/Blueprints/Saves/BP_RPG_SAVE_Hero.BP_RPG_SAVE_Hero_C|SetAddStarterStuff (LocalVariables|GetSaveLOCAL) true)
          (SaveGame|SaveGametoSlot (LocalVariables|GetSaveLOCAL) (Utilities|String|Append "Hero_" HeroName))
          (Variables|HeroSelection|SetSelectedHeroSave (Utilities|String|Append "Hero_" HeroName))
          (return true)))
      (else
        (Development|PrintString "Hero with this name already exists." true true "(R=1.000000,G=0.500000,B=0.000000,A=1.000000)")
        (return false)))
    (else
      (Development|PrintString "Hero name must be between 3 and 12 characters." true true "(R=1.000000,G=0.500000,B=0.000000,A=1.000000)")
      (return false))))

(fn SelectHero
  (params (HeroSaveName :type String))
  (Variables|HeroSelection|SetSelectedHeroSave HeroSaveName)
  (Utilities|FlowControl|Sequence
    (:then_0
      ;[0.1 0.1 0.1 1 14] Toggle highlight under the hero slot widget that is associated to selected hero.
      (for _array_element (Variables|Widgets|GetHeroSelectionSlots)
        (Default|ToggleHighlight _array_element (Utilities|Enum|Equal(Enum) (Variables|/Game/SuperiorRPGKit/Widgets/MainMenu/WBP_RPG_HeroSelectionSlot.WBP_RPG_HeroSelectionSlot_C|GetAssignedHeroSaveName _array_element) HeroSaveName))))
    (:then_1
      ;[0.1 0.1 0.1 1 14] Spawn selected hero actor.
      (bind _returnvalue (SaveGame|LoadGamefromSlot HeroSaveName))
      (bind _asbp_rpg_save_hero (Utilities|Casting|CastToBP_RPG_SAVE_Hero _returnvalue)
        (:then
          (HeroSelection|SpawnExistingHero (Variables|/Game/SuperiorRPGKit/Blueprints/Saves/BP_RPG_SAVE_Hero.BP_RPG_SAVE_Hero_C|GetHeroID _asbp_rpg_save_hero)))
        (:CastFailed
          (bind _displayedcharacter (Variables|Default|GetDisplayedCharacter)
            (:then
              (Actor|DestroyActor _displayedcharacter))
            (:else)))))
    (:then_2
      ;[0.1 0.1 0.1] Save selected hero to general save.
      (bind _returnvalue_2 (SaveGame|LoadGamefromSlot "General"))
      (bind _asbp_rpg_save_general (Utilities|Casting|CastToBP_RPG_SAVE_General _returnvalue_2))
      (Variables|/Game/SuperiorRPGKit/Blueprints/Saves/BP_RPG_SAVE_General.BP_RPG_SAVE_General_C|SetLastPlayedHeroSave _asbp_rpg_save_general HeroSaveName)
      (SaveGame|SaveGametoSlot _asbp_rpg_save_general "General"))))

(fn SpawnExistingHero
  (params (HeroID :type Name))
  ;[0.1 0.1 0.1 1 14] If there is another hero spawned - destroy it.
  (bind _displayedcharacter (Variables|Default|GetDisplayedCharacter)
    (:then
      (Actor|DestroyActor _displayedcharacter))
    (:else
      _))
  ;[0.1 0.1 0.1 1 14] Spawn hero at PlayerStart transform.
  (bind _outactors (Actor|GetAllActorsOfClass "/Script/Engine.PlayerStart"))
  (Utilities|IsValid (Utilities|Array|Get(acopy) _outactors)
    (:Is%20Valid
      (bind _returnvalue (Utilities|GetDataTableRow "/Game/SuperiorRPGKit/Datatables/DT_RPG_Heroes.DT_RPG_Heroes" HeroID)
        (:then
          (bind _returnvalue_2 (Game|SpawnActorfromClass (.ActorClass (Utilities|Struct|BreakS_RPG_Hero_Static _returnvalue)) (Transformation|GetActorTransform (Utilities|Array|Get(acopy) _outactors)) "AlwaysSpawn" 0 0))
          (bind _output_get (Variables|Default|SetDisplayedCharacter _returnvalue_2))
          (HeroSelection|UpdateHeroEquipment _output_get) ; Update its current equipment.
          (Default|MainMenuSpawnEffect _output_get) ; Play hero spawn effect (ie. animation + vfx)
          (return _output_get))))))

(fn DeleteHero
  (params (HeroSaveName :type String))
  (bind _returnvalue (SaveGame|LoadGamefromSlot "General"))
  (bind _asbp_rpg_save_general (Utilities|Casting|CastToBP_RPG_SAVE_General _returnvalue))
  (LocalVariables|SetSaveLOCAL _asbp_rpg_save_general)
  ;[0.1 0.1 0.1] Remove hero from the pool of player heroes.
  (Utilities|Array|RemoveItem (Variables|/Game/SuperiorRPGKit/Blueprints/Saves/BP_RPG_SAVE_General.BP_RPG_SAVE_General_C|GetPlayerHeroesSaves (LocalVariables|GetSaveLOCAL)) HeroSaveName)
  ;[0.1 0.1 0.1] If deleted hero was the one that we played last, assign first hero from the pool as new "selected" hero. (so it will be displayed to player)
  (bind _output_get (Variables|/Game/SuperiorRPGKit/Blueprints/Saves/BP_RPG_SAVE_General.BP_RPG_SAVE_General_C|SetLastPlayedHeroSave (LocalVariables|GetSaveLOCAL) (Utilities|String|SelectString (Utilities|Array|Get(acopy) (Variables|/Game/SuperiorRPGKit/Blueprints/Saves/BP_RPG_SAVE_General.BP_RPG_SAVE_General_C|GetPlayerHeroesSaves (LocalVariables|GetSaveLOCAL))) (Variables|/Game/SuperiorRPGKit/Blueprints/Saves/BP_RPG_SAVE_General.BP_RPG_SAVE_General_C|GetLastPlayedHeroSave (LocalVariables|GetSaveLOCAL)) (Utilities|Enum|Equal(Enum) (Variables|/Game/SuperiorRPGKit/Blueprints/Saves/BP_RPG_SAVE_General.BP_RPG_SAVE_General_C|GetLastPlayedHeroSave (LocalVariables|GetSaveLOCAL)) HeroSaveName))))
  (Variables|HeroSelection|SetSelectedHeroSave _output_get)
  (SaveGame|SaveGametoSlot (LocalVariables|GetSaveLOCAL) "General")
  (SaveGame|DeleteGameinSlot HeroSaveName)
  (HeroSelection|ShowAvailableHeroes)
  (HeroSelection|SelectHero (Variables|HeroSelection|GetSelectedHeroSave)))

(fn UpdateHeroEquipment
  (params (Hero :type BP%20RPG%20Hero%20Object%20Reference))
  (bind _ac_rpg_equipment (Variables|/Game/SuperiorRPGKit/Blueprints/Basics/BP_RPG_Hero.BP_RPG_Hero_C|GetAC_RPG_Equipment Hero))
  ;[0.1 0.1 0.1 1 14] Read hero equipment from save file and attach all equipment parts to hero actor.
  (bind _returnvalue (SaveGame|LoadGamefromSlot (Variables|HeroSelection|GetSelectedHeroSave)))
  (bind _asbp_rpg_save_hero (Utilities|Casting|CastToBP_RPG_SAVE_Hero _returnvalue))
  (for (_array_element _array_index) (Variables|/Game/SuperiorRPGKit/Blueprints/Saves/BP_RPG_SAVE_Hero.BP_RPG_SAVE_Hero_C|GetEquippedItemSlots _asbp_rpg_save_hero)
    (Utilities|Map|Add (Variables|/Game/SuperiorRPGKit/Blueprints/Components/AC_RPG_Equipment.AC_RPG_Equipment_C|GetEquippedItems _ac_rpg_equipment) _array_element (Utilities|Array|Get(acopy) (Variables|/Game/SuperiorRPGKit/Blueprints/Saves/BP_RPG_SAVE_Hero.BP_RPG_SAVE_Hero_C|GetEquippedItemsData _asbp_rpg_save_hero) _array_index))
    (Default|ChangeEquipmentMeshMULTICAST _ac_rpg_equipment _array_element (Utilities|Struct|BreakS_RPG_Item_Dynamic (Utilities|Array|Get(acopy) (Variables|/Game/SuperiorRPGKit/Blueprints/Saves/BP_RPG_SAVE_Hero.BP_RPG_SAVE_Hero_C|GetEquippedItemsData _asbp_rpg_save_hero) _array_index)))))