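; Quest function library for the RPG kit that formats a time in seconds as hours:minutes:seconds text.
; TimeToText splits the value with chained whole-and-remainder divisions, rounding only the leftover seconds, so that field can read 60.
; Each field passes through ConvertIntToDoubleDigit, which prepends a zero to single-character values.
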(fn TimetoText
  (params (Time%28InSeconds%29 :type Float%20%28single-precision%29))
  (bind (_remainder _returnvalue) (Math|Float|Division(WholeandRemainder) Time%28InSeconds%29 3.6e+03))
  (bind (_remainder_2 _returnvalue_2) (Math|Float|Division(WholeandRemainder) _remainder 6e+01))
  (return (Utilities|Text|FormatText "{hours}:{minutes}:{seconds}" (Utilities|Text|ToText(String) (CallFunction|ConvertInttoDoubleDigit (Math|Float|Round _remainder_2))) (Utilities|Text|ToText(String) (CallFunction|ConvertInttoDoubleDigit _returnvalue_2)) (Utilities|Text|ToText(String) (CallFunction|ConvertInttoDoubleDigit _returnvalue)))))

(fn ConvertInttoDoubleDigit
  (params (Value :type Integer))
  (bind _returnvalue (Utilities|String|ToString(Integer) Value))
  (if (> (Utilities|String|Len _returnvalue) 1)
    (return (Utilities|String|ToString(Integer) Value))
    (else
      (return (Utilities|String|Append "0" _returnvalue)))))