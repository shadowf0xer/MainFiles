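; Blueprint function library of helpers for the RPG kit's stats, buffs and effects.
; Converts attribute and stat enums to display names and formats durations as minutes and zero-padded seconds.
; Math helpers sum int or float modifier arrays, or apply them as successive, compounding fractions of a base value, clamped at zero.
; Lookup helpers fetch buff and effect static data from their DataTables, using the enum's string as row name.
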(fn AttributeTypetoText
  (params (AttributeType :type E_RPG_AttributeType%20Enum :default "NewEnumerator4"))
  (return (Utilities|Select :Index AttributeType :NewEnumerator4 "Non Available" :NewEnumerator0 "Strength" :NewEnumerator1 "Dexterity" :NewEnumerator2 "Endurance" :NewEnumerator3 "Wisdom")))

(fn StatTypetoText
  (params (StatType :type E_RPG_StatType%20Enum :default "NewEnumerator0"))
  (return (Utilities|Select :Index StatType :NewEnumerator0 "Non Available" :NewEnumerator1 "Health" :NewEnumerator2 "Mana" :NewEnumerator3 "Power" :NewEnumerator4 "Movement Speed" :NewEnumerator5 "Critical Rate" :NewEnumerator6 "Critical Power" :NewEnumerator7 "Defence" :NewEnumerator11 "")))

(fn DurationTimetoText
  (params (Duration :type Float%20%28single-precision%29))
  (bind (_remainder _returnvalue) (Math|Float|Division(WholeandRemainder) Duration 6e+01))
  (return (Utilities|Text|FormatText "{minutes}:{seconds}" _returnvalue (NumbersConversion|SingleDigittoDoubleNumber (Math|Float|Truncate _remainder)))))

(fn SingleDigittoDoubleNumber
  (params (Number :type Integer))
  (bind _returnvalue (Utilities|String|ToString(Integer) Number))
  (return (select (> (Utilities|String|Len _returnvalue) 1) (Utilities|Text|ToText(String) _returnvalue) (Utilities|Text|ToText(String) (Utilities|String|Append "0" _returnvalue)))))

(fn AddUpAllArrayIntegers
  (params (Array :type Array%20of%20Integers))
  (for _array_element Array
    (LocalVariables|SetResultLOCAL (+ _array_element (LocalVariables|GetResultLOCAL))))
  (return (LocalVariables|GetResultLOCAL)))

(fn AddUpAllArrayFloats
  (params (Array :type Array%20of%20Floats%20%28single-precision%29))
  (for _array_element Array
    (LocalVariables|SetResultLOCAL (+ _array_element (LocalVariables|GetResultLOCAL))))
  (return (LocalVariables|GetResultLOCAL)))

(fn MultiplyAllArrayIntegersbyBaseValue
  (params (BaseValue :type Integer) (Array :type Array%20of%20Integers) (Divisor :type Integer))
  (LocalVariables|SetResultLOCAL BaseValue)
  (for _array_element Array
    (LocalVariables|SetResultLOCAL (+ (/ (* _array_element (LocalVariables|GetResultLOCAL)) Divisor) (LocalVariables|GetResultLOCAL))))
  (return (Math|Integer|Max(Integer) (LocalVariables|GetResultLOCAL))))

(fn MultiplyAllArrayFloatbyBaseValue
  (params (BaseValue :type Float%20%28single-precision%29) (Array :type Array%20of%20Floats%20%28single-precision%29) (Divisor :type Float%20%28single-precision%29))
  (LocalVariables|SetResultLOCAL BaseValue)
  (for _array_element Array
    (LocalVariables|SetResultLOCAL (+ (* (/ _array_element Divisor) (LocalVariables|GetResultLOCAL)) (LocalVariables|GetResultLOCAL))))
  (return (Math|Float|Max(Float) (LocalVariables|GetResultLOCAL) 0.0)))

(fn GetBuffStaticDatafromDatatable
  (params (BuffType :type E_RPG_BuffType%20Enum :default "NewEnumerator0"))
  (bind _returnvalue (Utilities|GetDataTableRow "/Game/SuperiorRPGKit/Datatables/DT_RPG_Buffs.DT_RPG_Buffs" (Utilities|String|StringToName (Utilities|String|EnumtoString BuffType)))
    (:then
      (return _returnvalue))))

(fn GetEffectStaticDatafromDatatable
  (params (EffectType :type E_RPG_EffectType%20Enum :default "NewEnumerator0"))
  (bind _returnvalue (Utilities|GetDataTableRow "/Game/SuperiorRPGKit/Datatables/DT_RPG_Effects.DT_RPG_Effects" (Utilities|String|StringToName (Utilities|String|EnumtoString EffectType)))
    (:then
      (return _returnvalue))))