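; Function library for RPG items: rolls quality and bonuses, converts quality, type and bonus enums to display data, and applies or removes bonuses.
; Bonus count scales with quality; stored 0–1 weights later map to data-table min/max ranges, truncated by flat or percentage type.
; Apply and Remove route each bonus to the target's AC_RPG_StatsManager.
; Quality rolling uses a uniform demo pick; the weighted rarity cascade is disconnected.
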(fn ItemQualitytoColor
  (params (ItemQuality :type E_RPG_ItemQuality%20Enum :default "NewEnumerator0"))
  (return (Utilities|Select :Index ItemQuality :NewEnumerator0 "(R=1.000000,G=1.000000,B=1.000000,A=1.000000)" :NewEnumerator1 "(R=0.000000,G=0.200000,B=1.000000,A=1.000000)" :NewEnumerator2 "(R=0.800000,G=0.000000,B=1.000000,A=1.000000)" :NewEnumerator3 "(R=1.000000,G=0.500000,B=0.000000,A=1.000000)")))

(fn RollItemQuality
  (params (ItemID :type Name))
  (bind _returnvalue (Utilities|GetDataTableRow "/Game/SuperiorRPGKit/Datatables/DT_RPG_Items.DT_RPG_Items" ItemID)
    (:then
      ;[1 1 1] Connect these two nodes to have more advanced quality roll.
      (LocalVariables|SetAvailableQualitiesLOCAL (.AvailableQuality (Utilities|Struct|BreakS_RPG_Item_Static _returnvalue)))
      ;[1 1 1] DELETE - simplified version - demo only.
      (return (Utilities|Array|Get(acopy) (LocalVariables|GetAvailableQualitiesLOCAL) (Math|Random|RandomIntegerinRange 0 (- (Utilities|Array|Length (LocalVariables|GetAvailableQualitiesLOCAL)) 1)))) ; If only one quality was set, use it.
    )))

(fn ItemQualitytoText
  (params (ItemQuality :type E_RPG_ItemQuality%20Enum :default "NewEnumerator0"))
  (return (Utilities|Select :Index ItemQuality :NewEnumerator0 "Common" :NewEnumerator1 "Rare" :NewEnumerator2 "Epic" :NewEnumerator3 "Legendary")))

(fn ItemTypetoText
  (params (ItemType :type E_RPG_ItemType%20Enum :default "NewEnumerator4"))
  (return (Utilities|Select :Index ItemType :NewEnumerator4 "" :NewEnumerator0 "Weapon" :NewEnumerator1 "Armor" :NewEnumerator2 "Accessory" :NewEnumerator3 "Consumable" :NewEnumerator5 "Offhand" :NewEnumerator6 "Material")))

(fn RollItemBonuses
  (params (ItemID :type Name) (ItemQuality :type E_RPG_ItemQuality%20Enum :default "NewEnumerator0") (AllowDuplicates :type Boolean))
  (bind _returnvalue (Utilities|GetDataTableRow "/Game/SuperiorRPGKit/Datatables/DT_RPG_Items.DT_RPG_Items" ItemID)
    (:then
      (bind _returnvalue_2 (Utilities|GetDataTableRow "/Game/SuperiorRPGKit/Datatables/DT_RPG_ItemBonuses.DT_RPG_ItemBonuses" (Utilities|Struct|BreakS_RPG_Item_Static _returnvalue))
        (:then
          (bind _keys (Utilities|Map|Keys (Utilities|Struct|BreakS_RPG_ItemBonus _returnvalue_2)))
          (LocalVariables|SetAvailableBonusesLOCAL _keys)
          (LocalVariables|SetBonusesCountLOCAL (Utilities|Select :Index ItemQuality :NewEnumerator0 1 :NewEnumerator1 2 :NewEnumerator2 3 :NewEnumerator3 4))
          (for _index (range 1 (LocalVariables|GetBonusesCountLOCAL))
            ;[0.1 0.1 0.1 1 14] Roll random bonus at random weight (from 0 to 1)
            (LocalVariables|SetRolledBonusIndexLOCAL (Math|Random|RandomIntegerinRange 0 (- (Utilities|Array|Length (LocalVariables|GetAvailableBonusesLOCAL)) 1)))
            (Utilities|Array|Add (LocalVariables|GetRolledBonusesLOCAL) (Utilities|Struct|MakeS_RPG_BonusValue (Utilities|Array|Get(acopy) (LocalVariables|GetAvailableBonusesLOCAL) (LocalVariables|GetRolledBonusIndexLOCAL)) (Math|Random|RandomFloatinRange 0.0 1.0)))
            ;[0.1 0.1 0.1 1 14] If duplicates are not allowed remove rolled bonus from pool of available bonuses.
            (if (not AllowDuplicates)
              (Utilities|Array|RemoveIndex (LocalVariables|GetAvailableBonusesLOCAL) (LocalVariables|GetRolledBonusIndexLOCAL))))
          (return (LocalVariables|GetRolledBonusesLOCAL)))))))

(fn CalculateItemBonusesValues
  (params (Item :type S%20RPG%20Item%20Dynamic%20Structure))
  (bind (_id _occupiedspaceincontainer _currentamountinstack _rolledquality _rolledbonusesweights) (Utilities|Struct|BreakS_RPG_Item_Dynamic Item))
  (bind _returnvalue (Utilities|GetDataTableRow "/Game/SuperiorRPGKit/Datatables/DT_RPG_Items.DT_RPG_Items" _id)
    (:then
      (bind _returnvalue_2 (Utilities|GetDataTableRow "/Game/SuperiorRPGKit/Datatables/DT_RPG_ItemBonuses.DT_RPG_ItemBonuses" (Utilities|Struct|BreakS_RPG_Item_Static _returnvalue))
        (:then
          ;[1 1 1] Calculate values of all weighted item bonuses.
          (for _array_element _rolledbonusesweights
            (Utilities|Map|Add (LocalVariables|GetBonusesValuesLOCAL) (.BonusType (Utilities|Struct|BreakS_RPG_BonusValue _array_element)) (* (Math|Float|Truncate (* (Math|Float|MapRangeClamped (.Value (Utilities|Struct|BreakS_RPG_BonusValue _array_element)) 0.0 1.0 (.MinValue (Utilities|Struct|BreakS_RPG_BonusRange (.Value (Utilities|Map|Find (Utilities|Struct|BreakS_RPG_ItemBonus _returnvalue_2) (.BonusType (Utilities|Struct|BreakS_RPG_BonusValue _array_element)))))) (.MaxValue (Utilities|Struct|BreakS_RPG_BonusRange (.Value (Utilities|Map|Find (Utilities|Struct|BreakS_RPG_ItemBonus _returnvalue_2) (.BonusType (Utilities|Struct|BreakS_RPG_BonusValue _array_element))))))) (Math|Float|SelectFloat 1e+01 1.0 (.Percentage (Conversion|BonusTypetoText (.BonusType (Utilities|Struct|BreakS_RPG_BonusValue _array_element))))))) (/ 1.0 (Math|Float|SelectFloat 1e+01 1.0 (.Percentage (Conversion|BonusTypetoText (.BonusType (Utilities|Struct|BreakS_RPG_BonusValue _array_element)))))))))
          (return (LocalVariables|GetBonusesValuesLOCAL)))))))

(fn ApplyBonuses
  (params (Target :type Actor%20Object%20Reference) (Bonuses :type Map%20of%20E_RPG_BonusType%20Enums%20to%20Float%20%28single-precision%29s :default "NewEnumerator0"))
  (LocalVariables|SetTargetLOCAL Target)
  (bind _keys (Utilities|Map|Keys Bonuses))
  (for _array_element _keys
    (LocalVariables|SetBonusValueLOCAL (.Value (Utilities|Map|Find Bonuses _array_element)))
    (switch Utilities|FlowControl|Switch|SwitchonE_RPG_BonusType _array_element
      (:NewEnumerator0
        (Default|AddAttributeFlatBonus (Actor|GetComponentbyClass (LocalVariables|GetTargetLOCAL) "/Game/SuperiorRPGKit/Blueprints/Components/AC_RPG_StatsManager.AC_RPG_StatsManager_C") "NewEnumerator0" (Math|Float|Truncate (LocalVariables|GetBonusValueLOCAL))))
      (:NewEnumerator1
        (Default|AddAttributePercentageBonus (Actor|GetComponentbyClass (LocalVariables|GetTargetLOCAL) "/Game/SuperiorRPGKit/Blueprints/Components/AC_RPG_StatsManager.AC_RPG_StatsManager_C") "NewEnumerator0" (Math|Float|Truncate (LocalVariables|GetBonusValueLOCAL))))
      (:NewEnumerator2
        (Default|AddAttributeFlatBonus (Actor|GetComponentbyClass (LocalVariables|GetTargetLOCAL) "/Game/SuperiorRPGKit/Blueprints/Components/AC_RPG_StatsManager.AC_RPG_StatsManager_C") "NewEnumerator1" (Math|Float|Truncate (LocalVariables|GetBonusValueLOCAL))))
      (:NewEnumerator3
        (Default|AddAttributePercentageBonus (Actor|GetComponentbyClass (LocalVariables|GetTargetLOCAL) "/Game/SuperiorRPGKit/Blueprints/Components/AC_RPG_StatsManager.AC_RPG_StatsManager_C") "NewEnumerator1" (Math|Float|Truncate (LocalVariables|GetBonusValueLOCAL))))
      (:NewEnumerator4
        (Default|AddAttributeFlatBonus (Actor|GetComponentbyClass (LocalVariables|GetTargetLOCAL) "/Game/SuperiorRPGKit/Blueprints/Components/AC_RPG_StatsManager.AC_RPG_StatsManager_C") "NewEnumerator2" (Math|Float|Truncate (LocalVariables|GetBonusValueLOCAL))))
      (:NewEnumerator5
        (Default|AddAttributePercentageBonus (Actor|GetComponentbyClass (LocalVariables|GetTargetLOCAL) "/Game/SuperiorRPGKit/Blueprints/Components/AC_RPG_StatsManager.AC_RPG_StatsManager_C") "NewEnumerator2" (Math|Float|Truncate (LocalVariables|GetBonusValueLOCAL))))
      (:NewEnumerator6
        (Default|AddAttributeFlatBonus (Actor|GetComponentbyClass (LocalVariables|GetTargetLOCAL) "/Game/SuperiorRPGKit/Blueprints/Components/AC_RPG_StatsManager.AC_RPG_StatsManager_C") "NewEnumerator3" (Math|Float|Truncate (LocalVariables|GetBonusValueLOCAL))))
      (:NewEnumerator7
        (Default|AddAttributePercentageBonus (Actor|GetComponentbyClass (LocalVariables|GetTargetLOCAL) "/Game/SuperiorRPGKit/Blueprints/Components/AC_RPG_StatsManager.AC_RPG_StatsManager_C") "NewEnumerator3" (Math|Float|Truncate (LocalVariables|GetBonusValueLOCAL))))
      (:NewEnumerator8
        (Default|AddStatFlatBonus (Actor|GetComponentbyClass (LocalVariables|GetTargetLOCAL) "/Game/SuperiorRPGKit/Blueprints/Components/AC_RPG_StatsManager.AC_RPG_StatsManager_C") "NewEnumerator1" (LocalVariables|GetBonusValueLOCAL)))
      (:NewEnumerator9
        (Default|AddStatPercentageBonus (Actor|GetComponentbyClass (LocalVariables|GetTargetLOCAL) "/Game/SuperiorRPGKit/Blueprints/Components/AC_RPG_StatsManager.AC_RPG_StatsManager_C") "NewEnumerator1" (LocalVariables|GetBonusValueLOCAL)))
      (:NewEnumerator10
        (Default|AddStatFlatBonus (Actor|GetComponentbyClass (LocalVariables|GetTargetLOCAL) "/Game/SuperiorRPGKit/Blueprints/Components/AC_RPG_StatsManager.AC_RPG_StatsManager_C") "NewEnumerator2" (LocalVariables|GetBonusValueLOCAL)))
      (:NewEnumerator11
        (Default|AddStatPercentageBonus (Actor|GetComponentbyClass (LocalVariables|GetTargetLOCAL) "/Game/SuperiorRPGKit/Blueprints/Components/AC_RPG_StatsManager.AC_RPG_StatsManager_C") "NewEnumerator2" (LocalVariables|GetBonusValueLOCAL)))
      (:NewEnumerator12
        (Default|AddStatFlatBonus (Actor|GetComponentbyClass (LocalVariables|GetTargetLOCAL) "/Game/SuperiorRPGKit/Blueprints/Components/AC_RPG_StatsManager.AC_RPG_StatsManager_C") "NewEnumerator3" (LocalVariables|GetBonusValueLOCAL)))
      (:NewEnumerator13
        (Default|AddStatPercentageBonus (Actor|GetComponentbyClass (LocalVariables|GetTargetLOCAL) "/Game/SuperiorRPGKit/Blueprints/Components/AC_RPG_StatsManager.AC_RPG_StatsManager_C") "NewEnumerator3" (LocalVariables|GetBonusValueLOCAL)))
      (:NewEnumerator14
        (Default|AddStatFlatBonus (Actor|GetComponentbyClass (LocalVariables|GetTargetLOCAL) "/Game/SuperiorRPGKit/Blueprints/Components/AC_RPG_StatsManager.AC_RPG_StatsManager_C") "NewEnumerator7" (LocalVariables|GetBonusValueLOCAL)))
      (:NewEnumerator15
        (Default|AddStatPercentageBonus (Actor|GetComponentbyClass (LocalVariables|GetTargetLOCAL) "/Game/SuperiorRPGKit/Blueprints/Components/AC_RPG_StatsManager.AC_RPG_StatsManager_C") "NewEnumerator7" (LocalVariables|GetBonusValueLOCAL)))
      (:NewEnumerator16
        (Default|AddStatFlatBonus (Actor|GetComponentbyClass (LocalVariables|GetTargetLOCAL) "/Game/SuperiorRPGKit/Blueprints/Components/AC_RPG_StatsManager.AC_RPG_StatsManager_C") "NewEnumerator4" (LocalVariables|GetBonusValueLOCAL)))
      (:NewEnumerator17
        (Default|AddStatFlatBonus (Actor|GetComponentbyClass (LocalVariables|GetTargetLOCAL) "/Game/SuperiorRPGKit/Blueprints/Components/AC_RPG_StatsManager.AC_RPG_StatsManager_C") "NewEnumerator5" (LocalVariables|GetBonusValueLOCAL)))
      (:NewEnumerator18
        (Default|AddStatFlatBonus (Actor|GetComponentbyClass (LocalVariables|GetTargetLOCAL) "/Game/SuperiorRPGKit/Blueprints/Components/AC_RPG_StatsManager.AC_RPG_StatsManager_C") "NewEnumerator6" (LocalVariables|GetBonusValueLOCAL))))))

(fn RemoveBonuses
  (params (Target :type Actor%20Object%20Reference) (Bonuses :type Map%20of%20E_RPG_BonusType%20Enums%20to%20Float%20%28single-precision%29s :default "NewEnumerator0"))
  (LocalVariables|SetTargetLOCAL Target)
  (bind _keys (Utilities|Map|Keys Bonuses))
  (for _array_element _keys
    (LocalVariables|SetBonusValueLOCAL (.Value (Utilities|Map|Find Bonuses _array_element)))
    (switch Utilities|FlowControl|Switch|SwitchonE_RPG_BonusType _array_element
      (:NewEnumerator0
        (Default|RemoveAttributeFlatBonus (Actor|GetComponentbyClass (LocalVariables|GetTargetLOCAL) "/Game/SuperiorRPGKit/Blueprints/Components/AC_RPG_StatsManager.AC_RPG_StatsManager_C") "NewEnumerator0" (Math|Float|Truncate (LocalVariables|GetBonusValueLOCAL))))
      (:NewEnumerator1
        (Default|RemoveAttributePercentageBonus (Actor|GetComponentbyClass (LocalVariables|GetTargetLOCAL) "/Game/SuperiorRPGKit/Blueprints/Components/AC_RPG_StatsManager.AC_RPG_StatsManager_C") "NewEnumerator0" (Math|Float|Truncate (LocalVariables|GetBonusValueLOCAL))))
      (:NewEnumerator2
        (Default|RemoveAttributeFlatBonus (Actor|GetComponentbyClass (LocalVariables|GetTargetLOCAL) "/Game/SuperiorRPGKit/Blueprints/Components/AC_RPG_StatsManager.AC_RPG_StatsManager_C") "NewEnumerator1" (Math|Float|Truncate (LocalVariables|GetBonusValueLOCAL))))
      (:NewEnumerator3
        (Default|RemoveAttributePercentageBonus (Actor|GetComponentbyClass (LocalVariables|GetTargetLOCAL) "/Game/SuperiorRPGKit/Blueprints/Components/AC_RPG_StatsManager.AC_RPG_StatsManager_C") "NewEnumerator1" (Math|Float|Truncate (LocalVariables|GetBonusValueLOCAL))))
      (:NewEnumerator4
        (Default|RemoveAttributeFlatBonus (Actor|GetComponentbyClass (LocalVariables|GetTargetLOCAL) "/Game/SuperiorRPGKit/Blueprints/Components/AC_RPG_StatsManager.AC_RPG_StatsManager_C") "NewEnumerator2" (Math|Float|Truncate (LocalVariables|GetBonusValueLOCAL))))
      (:NewEnumerator5
        (Default|RemoveAttributePercentageBonus (Actor|GetComponentbyClass (LocalVariables|GetTargetLOCAL) "/Game/SuperiorRPGKit/Blueprints/Components/AC_RPG_StatsManager.AC_RPG_StatsManager_C") "NewEnumerator2" (Math|Float|Truncate (LocalVariables|GetBonusValueLOCAL))))
      (:NewEnumerator6
        (Default|RemoveAttributeFlatBonus (Actor|GetComponentbyClass (LocalVariables|GetTargetLOCAL) "/Game/SuperiorRPGKit/Blueprints/Components/AC_RPG_StatsManager.AC_RPG_StatsManager_C") "NewEnumerator3" (Math|Float|Truncate (LocalVariables|GetBonusValueLOCAL))))
      (:NewEnumerator7
        (Default|RemoveAttributePercentageBonus (Actor|GetComponentbyClass (LocalVariables|GetTargetLOCAL) "/Game/SuperiorRPGKit/Blueprints/Components/AC_RPG_StatsManager.AC_RPG_StatsManager_C") "NewEnumerator3" (Math|Float|Truncate (LocalVariables|GetBonusValueLOCAL))))
      (:NewEnumerator8
        (Default|RemoveStatFlatBonus (Actor|GetComponentbyClass (LocalVariables|GetTargetLOCAL) "/Game/SuperiorRPGKit/Blueprints/Components/AC_RPG_StatsManager.AC_RPG_StatsManager_C") "NewEnumerator1" (LocalVariables|GetBonusValueLOCAL)))
      (:NewEnumerator9
        (Default|RemoveStatPercentageBonus (Actor|GetComponentbyClass (LocalVariables|GetTargetLOCAL) "/Game/SuperiorRPGKit/Blueprints/Components/AC_RPG_StatsManager.AC_RPG_StatsManager_C") "NewEnumerator1" (LocalVariables|GetBonusValueLOCAL)))
      (:NewEnumerator10
        (Default|RemoveStatFlatBonus (Actor|GetComponentbyClass (LocalVariables|GetTargetLOCAL) "/Game/SuperiorRPGKit/Blueprints/Components/AC_RPG_StatsManager.AC_RPG_StatsManager_C") "NewEnumerator2" (LocalVariables|GetBonusValueLOCAL)))
      (:NewEnumerator11
        (Default|RemoveStatPercentageBonus (Actor|GetComponentbyClass (LocalVariables|GetTargetLOCAL) "/Game/SuperiorRPGKit/Blueprints/Components/AC_RPG_StatsManager.AC_RPG_StatsManager_C") "NewEnumerator2" (LocalVariables|GetBonusValueLOCAL)))
      (:NewEnumerator12
        (Default|RemoveStatFlatBonus (Actor|GetComponentbyClass (LocalVariables|GetTargetLOCAL) "/Game/SuperiorRPGKit/Blueprints/Components/AC_RPG_StatsManager.AC_RPG_StatsManager_C") "NewEnumerator3" (LocalVariables|GetBonusValueLOCAL)))
      (:NewEnumerator13
        (Default|RemoveStatPercentageBonus (Actor|GetComponentbyClass (LocalVariables|GetTargetLOCAL) "/Game/SuperiorRPGKit/Blueprints/Components/AC_RPG_StatsManager.AC_RPG_StatsManager_C") "NewEnumerator3" (LocalVariables|GetBonusValueLOCAL)))
      (:NewEnumerator14
        (Default|RemoveStatFlatBonus (Actor|GetComponentbyClass (LocalVariables|GetTargetLOCAL) "/Game/SuperiorRPGKit/Blueprints/Components/AC_RPG_StatsManager.AC_RPG_StatsManager_C") "NewEnumerator7" (LocalVariables|GetBonusValueLOCAL)))
      (:NewEnumerator15
        (Default|RemoveStatPercentageBonus (Actor|GetComponentbyClass (LocalVariables|GetTargetLOCAL) "/Game/SuperiorRPGKit/Blueprints/Components/AC_RPG_StatsManager.AC_RPG_StatsManager_C") "NewEnumerator7" (LocalVariables|GetBonusValueLOCAL)))
      (:NewEnumerator16
        (Default|RemoveStatFlatBonus (Actor|GetComponentbyClass (LocalVariables|GetTargetLOCAL) "/Game/SuperiorRPGKit/Blueprints/Components/AC_RPG_StatsManager.AC_RPG_StatsManager_C") "NewEnumerator4" (LocalVariables|GetBonusValueLOCAL)))
      (:NewEnumerator17
        (Default|RemoveStatFlatBonus (Actor|GetComponentbyClass (LocalVariables|GetTargetLOCAL) "/Game/SuperiorRPGKit/Blueprints/Components/AC_RPG_StatsManager.AC_RPG_StatsManager_C") "NewEnumerator5" (LocalVariables|GetBonusValueLOCAL)))
      (:NewEnumerator18
        (Default|RemoveStatFlatBonus (Actor|GetComponentbyClass (LocalVariables|GetTargetLOCAL) "/Game/SuperiorRPGKit/Blueprints/Components/AC_RPG_StatsManager.AC_RPG_StatsManager_C") "NewEnumerator6" (LocalVariables|GetBonusValueLOCAL))))))

(fn BonusTypetoText
  (params (BonusType :type E_RPG_BonusType%20Enum :default "NewEnumerator0"))
  (switch Utilities|FlowControl|Switch|SwitchonE_RPG_BonusType BonusType
    (:NewEnumerator0
      (return "Strength" false))
    (:NewEnumerator1
      (return "Strength" true))
    (:NewEnumerator2
      (return "Dexterity" false))
    (:NewEnumerator3
      (return "Dexterity" true))
    (:NewEnumerator4
      (return "Endurance" false))
    (:NewEnumerator5
      (return "Endurance" true))
    (:NewEnumerator6
      (return "Wisdom" false))
    (:NewEnumerator7
      (return "Wisdom" true))
    (:NewEnumerator8
      (return "Health" false))
    (:NewEnumerator9
      (return "Health" true))
    (:NewEnumerator10
      (return "Mana" false))
    (:NewEnumerator11
      (return "Mana" true))
    (:NewEnumerator12
      (return "Power" false))
    (:NewEnumerator13
      (return "Power" true))
    (:NewEnumerator14
      (return "Defence" false))
    (:NewEnumerator15
      (return "Defence" true))
    (:NewEnumerator16
      (return "Movement Speed" true))
    (:NewEnumerator17
      (return "Critical Rate" true))
    (:NewEnumerator18
      (return "Critical Power" true))))