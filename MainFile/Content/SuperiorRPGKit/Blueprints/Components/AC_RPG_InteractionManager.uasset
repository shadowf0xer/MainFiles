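; Player controller component that manages actor interaction and NPC dialogue in the RPG kit.
; Server events send begin and finish interaction messages to actors, passing the player's hero and this component.
; Client events show or hide dialogue and fire start and end notifications.
; Dialogue construction reads hero and NPC data tables, plays or skips the greeting, and fills pooled choice slots with vendor, quest, objective and farewell options.
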(event EventBeginPlay
  (bind _asbp_rpg_pc_in_game (Utilities|Casting|CastToBP_RPG_PC_InGame (Components|GetOwner) :!label _label)
    (:then
      (Variables|References|SetPlayerController _asbp_rpg_pc_in_game))
    (:CastFailed
      (Utilities|FlowControl|Delay 0.2)
      (goto _label))))

(event Custom|FinishActorInteraction_SERVER
  (Class|BPIRPGInteractable|OnFinishInteract(Message) (Variables|References|GetInteractedActor) (Variables|/Game/SuperiorRPGKit/Blueprints/Basics/BP_RPG_PC_InGame.BP_RPG_PC_InGame_C|GetPlayerHero (Variables|References|GetPlayerController)) self)
  (Variables|Dialogue|SetSkipGreetingNPC false))

(event Custom|StartActorInteraction_SERVER
  (params (Actor :type Actor%20Object%20Reference))
  (Class|BPIRPGInteractable|OnBeginInteract(Message) Actor (Variables|/Game/SuperiorRPGKit/Blueprints/Basics/BP_RPG_PC_InGame.BP_RPG_PC_InGame_C|GetPlayerHero (Variables|References|GetPlayerController)) self))

(event Custom|HideDialogueWindow_CLIENT
  (Default|CallOnDialogueEnded))

(event Custom|ShowDialogueWindow_CLIENT
  (params (NPC%20ID :type Name) (AcceptableQuests :type Array%20of%20Names) (FinishableQuests :type Array%20of%20Names) (ProgressableObjectives :type Array%20of%20Names) (Vendor :type Boolean) (SkipGreeting :type Boolean))
  (CallFunction|ConstructDialogueWindow NPC%20ID AcceptableQuests FinishableQuests ProgressableObjectives Vendor SkipGreeting)
  (Default|CallOnDialogueStarted))

(fn ConstructDialogueWindow
  (params (NPC%20ID :type Name) (AcceptableQuests :type Array%20of%20Names) (FinishableQuests :type Array%20of%20Names) (ProgressableObjectives :type Array%20of%20Names) (Vendor :type Boolean) (SkipGreeting :type Boolean))
  ;[0.1 0.1 0.1 1 14] Set player portrait.
  (bind _returnvalue (Utilities|GetDataTableRow "/Game/SuperiorRPGKit/Datatables/DT_RPG_Heroes.DT_RPG_Heroes" (Variables|/Game/SuperiorRPGKit/Blueprints/Components/AC_RPG_StatsManager.AC_RPG_StatsManager_C|GetCharacterID (Actor|GetComponentbyClass (Components|GetOwner) "/Game/SuperiorRPGKit/Blueprints/Components/AC_RPG_StatsManager.AC_RPG_StatsManager_C")))
    (:then
      (Appearance|SetBrushfromTexture (Variables|/Game/SuperiorRPGKit/Widgets/Interaction/WBP_RPG_DialogueWindow.WBP_RPG_DialogueWindow_C|GetImage_PortraitPlayer (Variables|References|GetDialogueWindow)) (.Portrait (Utilities|Struct|BreakS_RPG_Hero_Static _returnvalue)) false)
      (bind _returnvalue_2 (Utilities|GetDataTableRow "/Game/SuperiorRPGKit/Datatables/DT_RPG_NPC.DT_RPG_NPC" NPC%20ID)
        (:then
          (LocalVariables|SetNPCStructLOCAL _returnvalue_2)
          ;[0.1 0.1 0.1 1 14] Set NPC name and portrait.
          (Rendering|Components|TextRender|SetText (Variables|/Game/SuperiorRPGKit/Widgets/Interaction/WBP_RPG_DialogueWindow.WBP_RPG_DialogueWindow_C|GetTextBlock_NPCName (Variables|References|GetDialogueWindow)) (.DisplayName (Utilities|Struct|BreakS_RPG_NPC_Static (LocalVariables|GetNPCStructLOCAL))))
          (Appearance|SetBrushfromTexture (Variables|/Game/SuperiorRPGKit/Widgets/Interaction/WBP_RPG_DialogueWindow.WBP_RPG_DialogueWindow_C|GetImage_PortraitNPC (Variables|References|GetDialogueWindow)) (.Portrait (Utilities|Struct|BreakS_RPG_NPC_Static (LocalVariables|GetNPCStructLOCAL))) false)
          (for _array_element (Variables|/Game/SuperiorRPGKit/Widgets/Interaction/WBP_RPG_DialogueWindow.WBP_RPG_DialogueWindow_C|GetChoiceSlots (Variables|References|GetDialogueWindow))
            (Widget|SetVisibility _array_element "Collapsed"))
          (Utilities|FlowControl|Sequence
            (:then_0
              ;[0.1 0.1 0.1 1 14] Display player greeting as initial text or skip it and display dialogue options.
              (if SkipGreeting
                (Default|SwitchPortraittoPlayer (Variables|References|GetDialogueWindow))
                (Class|WidgetSwitcher|SetActiveWidgetIndex (Variables|/Game/SuperiorRPGKit/Widgets/Interaction/WBP_RPG_DialogueWindow.WBP_RPG_DialogueWindow_C|GetWidgetSwitcher_DialogueSelection (Variables|References|GetDialogueWindow)) 1)
                (else
                  (Default|StartGreetingDialogueSequence (Variables|/Game/SuperiorRPGKit/Widgets/Interaction/WBP_RPG_DialogueWindow.WBP_RPG_DialogueWindow_C|GetWBP_RPG_DialogueSlot (Variables|References|GetDialogueWindow)) (.InitialPlayerText (Utilities|Struct|BreakS_RPG_NPC_Dialogue (.GreetingDialogue (Utilities|Struct|BreakS_RPG_NPC_Static (LocalVariables|GetNPCStructLOCAL))))) (.Dialogues (Utilities|Struct|BreakS_RPG_NPC_Dialogue (.GreetingDialogue (Utilities|Struct|BreakS_RPG_NPC_Static (LocalVariables|GetNPCStructLOCAL)))))))))
            (:then_1
              ;[0.1 0.1 0.1 1 14] If NPC is vendor make its first dialogue option to trigger vendor event (basically display shop window).
              (if Vendor
                (bind _choiceslot (Default|GetChoiceSlotfromPool (Variables|References|GetDialogueWindow) (LocalVariables|GetSlotIndexLOCAL)))
                (Variables|/Game/SuperiorRPGKit/Widgets/Interaction/WBP_RPG_ChoiceSlot.WBP_RPG_ChoiceSlot_C|SetDialogueOption _choiceslot "NewEnumerator1")
                (Default|SetDialogueData _choiceslot (.VendorDialogue (Utilities|Struct|BreakS_RPG_NPC_Static (LocalVariables|GetNPCStructLOCAL))) "None")
                (Widget|SetVisibility _choiceslot "Visible")
                (Math|Integer|IncrementInt (LocalVariables|GetSlotIndexLOCAL))))
            (:then_2
              ;[0.1 0.1 0.1 1 14] Display dialogue options for all currently acceptable quests.
              (for _array_element_2 AcceptableQuests
                (if (.ReturnValue (Utilities|Map|Find (Utilities|Struct|BreakS_RPG_NPC_Static (LocalVariables|GetNPCStructLOCAL)) _array_element_2))
                  (bind _choiceslot_2 (Default|GetChoiceSlotfromPool (Variables|References|GetDialogueWindow) (LocalVariables|GetSlotIndexLOCAL)))
                  (Variables|/Game/SuperiorRPGKit/Widgets/Interaction/WBP_RPG_ChoiceSlot.WBP_RPG_ChoiceSlot_C|SetDialogueOption _choiceslot_2 "NewEnumerator2")
                  (Default|SetDialogueData _choiceslot_2 (.Value (Utilities|Map|Find (Utilities|Struct|BreakS_RPG_NPC_Static (LocalVariables|GetNPCStructLOCAL)) _array_element_2)) _array_element_2)
                  (Widget|SetVisibility _choiceslot_2 "Visible")
                  (Math|Integer|IncrementInt (LocalVariables|GetSlotIndexLOCAL)))))
            (:then_3
              ;[0.1 0.1 0.1 1 14] Display dialogue options for all currently finishable quests.
              (for _array_element_3 FinishableQuests
                (if (.ReturnValue (Utilities|Map|Find (Utilities|Struct|BreakS_RPG_NPC_Static (LocalVariables|GetNPCStructLOCAL)) _array_element_3))
                  (bind _choiceslot_3 (Default|GetChoiceSlotfromPool (Variables|References|GetDialogueWindow) (LocalVariables|GetSlotIndexLOCAL)))
                  (Variables|/Game/SuperiorRPGKit/Widgets/Interaction/WBP_RPG_ChoiceSlot.WBP_RPG_ChoiceSlot_C|SetDialogueOption _choiceslot_3 "NewEnumerator3")
                  (Default|SetDialogueData _choiceslot_3 (.Value (Utilities|Map|Find (Utilities|Struct|BreakS_RPG_NPC_Static (LocalVariables|GetNPCStructLOCAL)) _array_element_3)) _array_element_3)
                  (Widget|SetVisibility _choiceslot_3 "Visible")
                  (Math|Integer|IncrementInt (LocalVariables|GetSlotIndexLOCAL)))))
            (:then_4
              ;[0.1 0.1 0.1 1 14] Display dialogue options for all currently progressable objectives.
              (for _array_element_4 ProgressableObjectives
                (if (.ReturnValue (Utilities|Map|Find (Utilities|Struct|BreakS_RPG_NPC_Static (LocalVariables|GetNPCStructLOCAL)) _array_element_4))
                  (bind _choiceslot_4 (Default|GetChoiceSlotfromPool (Variables|References|GetDialogueWindow) (LocalVariables|GetSlotIndexLOCAL)))
                  (Variables|/Game/SuperiorRPGKit/Widgets/Interaction/WBP_RPG_ChoiceSlot.WBP_RPG_ChoiceSlot_C|SetDialogueOption _choiceslot_4 "NewEnumerator4")
                  (Default|SetDialogueData _choiceslot_4 (.Value (Utilities|Map|Find (Utilities|Struct|BreakS_RPG_NPC_Static (LocalVariables|GetNPCStructLOCAL)) _array_element_4)) _array_element_4)
                  (Widget|SetVisibility _choiceslot_4 "Visible")
                  (Math|Integer|IncrementInt (LocalVariables|GetSlotIndexLOCAL)))))
            (:then_5
              ;[0.1 0.1 0.1 1 14] Add one last dialogue option for farewell dialogue (to leave npc).
              (bind _choiceslot_5 (Default|GetChoiceSlotfromPool (Variables|References|GetDialogueWindow) (LocalVariables|GetSlotIndexLOCAL)))
              (Variables|/Game/SuperiorRPGKit/Widgets/Interaction/WBP_RPG_ChoiceSlot.WBP_RPG_ChoiceSlot_C|SetDialogueOption _choiceslot_5 "NewEnumerator0")
              (Default|SetDialogueData _choiceslot_5 (Utilities|Struct|BreakS_RPG_NPC_Static (LocalVariables|GetNPCStructLOCAL)) "None")
              (Widget|SetVisibility _choiceslot_5 "Visible")
              (Math|Integer|IncrementInt (LocalVariables|GetSlotIndexLOCAL)))))))))

(fn InitializeDialogueWindow
  (params (DialogueWindow :type WBP%20RPG%20Dialogue%20Window%20Object%20Reference))
  (Variables|References|SetDialogueWindow DialogueWindow))