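; Actor component that manages the RPG quick access bar, binding skills and items to slots and activating them through the owner's skills and items managers.
; Server events register, swap, remove and use entries in a slot map, then client events mirror it to slot widgets with cooldowns and item counts.
; Slot grids are built per bar widget, and drag-and-drop uses a cursor-following widget updated on Tick.
; It also exports and reloads slot data for saving.
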(event EventTick
  (params (DeltaSeconds :type Float%20%28single-precision%29))
  (if (not (Networking|IsDedicatedServer))
    ;[0.1 0.1 0.1 1 12] Adjusts DraggedQuickSlot widget position in viewport. (so it follows the cursor)
    (if (Variables|Management|GetDraggingQuickSlot)
      (bind _quickslotdragwidget (Utilities|GetDraggedQuickSlotWidget))
      (bind _returnvalue (Class|WidgetLayoutLibrary|GetMousePositiononViewport))
      (Class|UserWidget|SetPositioninViewport _quickslotdragwidget _returnvalue false))))

(event Custom|ActivateQuickSlot_SERVER
  (params (QuickSlotIndex :type Integer))
  (bind _quickaccess (Variables|Management|GetQuickAccess))
  (bind (_value _returnvalue) (Utilities|Map|Find _quickaccess QuickSlotIndex))
  (bind (_registeredid _quickaccesstype) (Utilities|Struct|BreakS_RPG_QuickSlot _value))
  (if _returnvalue
    (if (Utilities|Name|NotEqual(Name) _registeredid "None")
      (switch Utilities|FlowControl|Switch|SwitchonE_RPG_QuickAccessType _quickaccesstype
        (:NewEnumerator0
          ;[0.1 0.1 0.1 1 14] use skill
          (Default|UseSkillSERVER (Actor|GetComponentbyClass (Components|GetOwner) "/Game/SuperiorRPGKit/Blueprints/Components/AC_RPG_SkillsManager.AC_RPG_SkillsManager_C") _registeredid))
        (:NewEnumerator2
          ;[0.1 0.1 0.1 1 14] use item
          (Default|UseItemSERVER (Actor|GetComponentbyClass (Components|GetOwner) "/Game/SuperiorRPGKit/Blueprints/Components/AC_RPG_ItemsManager.AC_RPG_ItemsManager_C") _registeredid))))))

(event Custom|DropObjectToQuickSlot_SERVER
  (params (QuickSlotIndex :type Integer) (QuickSlotData :type S%20RPG%20Quick%20Slot%20Structure))
  (bind (_registeredid _quickaccesstype) (Utilities|Struct|BreakS_RPG_QuickSlot QuickSlotData))
  (bind (_result _quickslotdata) (Getters|GetObjectRegisteredinQuickSlot QuickSlotIndex))
  (if _result
    (CallFunction|StartDraggingCLIENT QuickSlotIndex _quickslotdata) ; Swap with another object that was in slot we dropped dragged object to.
    (else
      (CallFunction|CancelDraggingCLIENT) ; Finish dragging.
    ))
  ;[0.1 0.1 0.1 1 14] Drop dragged object to slot.
  (switch Utilities|FlowControl|Switch|SwitchonE_RPG_QuickAccessType _quickaccesstype
    (:NewEnumerator0
      (Management|RegisterSkill QuickSlotIndex _registeredid))
    (:NewEnumerator2
      (Management|RegisterItem QuickSlotIndex _registeredid))))

(event Custom|DragObjectFromQuickSlot_SERVER
  (params (QuickSlotIndex :type Integer))
  ;[0.1 0.1 0.1 1 14] Drag object from quick slot.
  (CallFunction|StartDraggingCLIENT QuickSlotIndex (.Value (Utilities|Map|Find (Variables|Management|GetQuickAccess) QuickSlotIndex)))
  ;[0.1 0.1 0.1 1 14] Remove dragged object from quick slot.
  (Utilities|Map|Remove (Variables|Management|GetQuickAccess) QuickSlotIndex)
  (CallFunction|UpdateQuickAccessSlotCLIENT QuickSlotIndex))

(event Custom|RegisterObjectInQuickSlot_SERVER
  (params (QuickSlotIndex :type Integer) (QuickSlotData :type S%20RPG%20Quick%20Slot%20Structure))
  (bind (_registeredid _quickaccesstype) (Utilities|Struct|BreakS_RPG_QuickSlot QuickSlotData))
  ;[0.1 0.1 0.1 1 14] Register object to quick slot.
  (switch Utilities|FlowControl|Switch|SwitchonE_RPG_QuickAccessType _quickaccesstype
    (:NewEnumerator0
      (Management|RegisterSkill QuickSlotIndex _registeredid))
    (:NewEnumerator2
      (Management|RegisterItem QuickSlotIndex _registeredid))))

(event Custom|UnregisterObjectFromQuickSlot_SERVER
  (params (QuickSlotIndex :type Integer))
  ;[0.1 0.1 0.1 1 14] Unregister object from quick slot.
  (Utilities|Map|Remove (Variables|Management|GetQuickAccess) QuickSlotIndex)
  (CallFunction|UpdateQuickAccessSlotCLIENT QuickSlotIndex))

(event Custom|UpdateSlotCooldown_CLIENT
  (params (ID :type Name) (TimeLeft :type Float%20%28single-precision%29) (InitialTime :type Float%20%28single-precision%29))
  ;[0.1 0.1 0.1 1 14] Update displayed cooldown time.
  (for _array_element (Variables|References|GetQuickAccessSlots)
    (if (Utilities|Name|Equal(Name) (Variables|/Game/SuperiorRPGKit/Widgets/QuickAccess/WBP_RPG_QuickAccessSlot.WBP_RPG_QuickAccessSlot_C|GetAssignedID _array_element) ID)
      (Default|DisplayCooldown _array_element TimeLeft InitialTime))))

(event Custom|UpdateQuickAccessSlot_CLIENT
  (params (SlotIndex :type Integer) (QuickSlotData :type S%20RPG%20Quick%20Slot%20Structure))
  (bind (_registeredid _quickaccesstype) (Utilities|Struct|BreakS_RPG_QuickSlot QuickSlotData))
  (bind _returnvalue (Components|GetOwner))
  (bind _returnvalue_2 (Actor|GetComponentbyClass _returnvalue "/Game/SuperiorRPGKit/Blueprints/Components/AC_RPG_ItemsManager.AC_RPG_ItemsManager_C"))
  (if (Utilities|Name|Equal(Name) (.RegisteredID (Utilities|Struct|BreakS_RPG_QuickSlot QuickSlotData)) "None")
    (Utilities|Map|Remove (Variables|Management|GetQuickAccess) SlotIndex)
    (else
      (Utilities|Map|Add (Variables|Management|GetQuickAccess) SlotIndex QuickSlotData)))
  ;[0.1 0.1 0.1 1 14] Update data in quick access slot.
  (bind _quickaccessslot (Getters|GetQuickAccessSlot SlotIndex))
  (Utilities|IsValid _quickaccessslot
    (:Is%20Valid
      (Default|AssignData _quickaccessslot QuickSlotData)
      (switch Utilities|FlowControl|Switch|SwitchonE_RPG_QuickAccessType _quickaccesstype
        (:NewEnumerator0
          (Default|CancelSkillDragging (Actor|GetComponentbyClass (Components|GetOwner) "/Game/SuperiorRPGKit/Blueprints/Components/AC_RPG_SkillsManager.AC_RPG_SkillsManager_C")))
        (:NewEnumerator2
          ;[0.1 0.1 0.1 1 14] Update number of available items in displayed in quick access slot.
          (bind _totalamount (Default|GetTotalAmountOfIteminContainer _returnvalue_2 (Variables|/Game/SuperiorRPGKit/Blueprints/Components/AC_RPG_ItemsManager.AC_RPG_ItemsManager_C|GetInventoryContainer _returnvalue_2) _registeredid))
          (Management|SetItemAmountinQuickSlots _registeredid _totalamount))))))

(event Custom|UpdateQuickAccessBar_CLIENT
  (params (SlotIndexes :type Array%20of%20Integers) (IDs :type Array%20of%20S%20RPG%20Quick%20Slot%20Structures))
  ;[0.1 0.1 0.1 1 14] Update all slots in quick access bar.
  (for (_array_element _array_index) IDs
    (CallFunction|UpdateQuickAccessSlotCLIENT (Utilities|Array|Get(acopy) SlotIndexes _array_index) _array_element)))

(event Custom|StartDragging_CLIENT
  (params (QuickSlotIndex :type Integer) (QuickSlotData :type S%20RPG%20Quick%20Slot%20Structure))
  (bind _quickaccess (Variables|Management|GetQuickAccess))
  (bind (_value _returnvalue) (Utilities|Map|Find _quickaccess QuickSlotIndex))
  ;[0.1 0.1 0.1 1 14] Start dragging
  (if _returnvalue
    (if (Utilities|Name|NotEqual(Name) (.RegisteredID (Utilities|Struct|BreakS_RPG_QuickSlot _value)) "None")
      (Variables|Management|SetDraggingQuickSlot true)
      (bind _quickslotdragwidget (Utilities|GetDraggedQuickSlotWidget))
      (Widget|SetVisibility _quickslotdragwidget "HitTestInvisible")
      (Variables|/Game/SuperiorRPGKit/Widgets/QuickAccess/WBP_RPG_QuickSlotDragging.WBP_RPG_QuickSlotDragging_C|SetDraggedQuickSlot _quickslotdragwidget QuickSlotData)
      (bind _quickaccessslot (Getters|GetQuickAccessSlot QuickSlotIndex))
      (Class|Image|SetBrush (Variables|/Game/SuperiorRPGKit/Widgets/QuickAccess/WBP_RPG_QuickSlotDragging.WBP_RPG_QuickSlotDragging_C|GetImage_Icon _quickslotdragwidget) (Variables|/Script/UMG.Image|GetBrush (Variables|/Game/SuperiorRPGKit/Widgets/QuickAccess/WBP_RPG_QuickAccessSlot.WBP_RPG_QuickAccessSlot_C|GetImage_RegisteredObjectIcon _quickaccessslot))))))

(event Custom|CancelDragging_CLIENT
  ;[0.1 0.1 0.1 1 14] Stop Dragging
  (if (Variables|Management|GetDraggingQuickSlot)
    (Variables|Management|SetDraggingQuickSlot false)
    (bind _quickslotdragwidget (Utilities|GetDraggedQuickSlotWidget))
    (Widget|SetVisibility _quickslotdragwidget "Collapsed")))

(fn InitializeQuickAccessBars
  (bind _returnvalue (Components|GetOwner))
  (bind _quickslotsperrow (Variables|Config|GetQuickSlotsPerRow))
  (if (not (Networking|IsDedicatedServer))
    (Utilities|Array|Clear (Variables|References|GetQuickAccessSlots))
    ;[0.1 0.1 0.1 1 14] Get all quick access bars.
    (bind _foundwidgets (Widget|GetAllWidgetsOfClass "/Game/SuperiorRPGKit/Widgets/QuickAccess/WBP_RPG_QuickAccessBar.WBP_RPG_QuickAccessBar_C" false))
    (for _array_element _foundwidgets
      ;[0.1 0.1 0.1 1 14] Fill each quick access bar with desired number of quick slots.
      (Widget|Panel|ClearChildren (Variables|/Game/SuperiorRPGKit/Widgets/QuickAccess/WBP_RPG_QuickAccessBar.WBP_RPG_QuickAccessBar_C|GetUniformGridPanel_QuickSlots _array_element))
      (for _index (range 0 (- (Variables|Config|GetQuickSlotsAmount) 1))
        (bind _result (Math|Integer|IncrementInt (LocalVariables|GetSlotIndexLOCAL))
          (:%20%20
            (bind _returnvalue_2 (UserInterface|CreateWidget "/Game/SuperiorRPGKit/Widgets/QuickAccess/WBP_RPG_QuickAccessSlot.WBP_RPG_QuickAccessSlot_C" 0 _result (Actor|GetComponentbyClass _returnvalue "/Game/SuperiorRPGKit/Blueprints/Components/AC_RPG_ItemsManager.AC_RPG_ItemsManager_C") (Actor|GetComponentbyClass _returnvalue "/Game/SuperiorRPGKit/Blueprints/Components/AC_RPG_SkillsManager.AC_RPG_SkillsManager_C") self))
            (Utilities|Array|Add (Variables|References|GetQuickAccessSlots) _returnvalue_2)
            (bind _returnvalue_3 (Class|UniformGridPanel|AddChildtoUniformGrid (Variables|/Game/SuperiorRPGKit/Widgets/QuickAccess/WBP_RPG_QuickAccessBar.WBP_RPG_QuickAccessBar_C|GetUniformGridPanel_QuickSlots _array_element) _returnvalue_2))
            (Class|UniformGridSlot|SetColumn _returnvalue_3 (Math|Integer|%(Integer) _index _quickslotsperrow))
            (Class|UniformGridSlot|SetRow _returnvalue_3 (/ _index _quickslotsperrow))))))))

(fn GetQuickAccessSlot
  (params (SlotIndex :type Integer))
  (bind _array_element (Utilities|Array|ForEachLoopwithBreak (Variables|References|GetQuickAccessSlots) :!label _label)
    (:LoopBody
      (if (== (Variables|/Game/SuperiorRPGKit/Widgets/QuickAccess/WBP_RPG_QuickAccessSlot.WBP_RPG_QuickAccessSlot_C|GetSlotIndex _array_element) SlotIndex)
        (LocalVariables|SetSlotLOCAL _array_element)
        (goto _label Break)))
    (:Completed
      (return (LocalVariables|GetSlotLOCAL)))))

(fn SetItemAmountinQuickSlots
  (params (ItemID :type Name) (Amount :type Integer))
  (bind _quickaccess (Variables|Management|GetQuickAccess))
  ;[0.1 0.1 0.1 1 14] Update number of specific item available displayed in quick slots.
  (bind _keys (Utilities|Map|Keys _quickaccess))
  (for _array_element _keys
    (if (Utilities|Name|Equal(Name) (.RegisteredID (Utilities|Struct|BreakS_RPG_QuickSlot (.Value (Utilities|Map|Find _quickaccess _array_element)))) ItemID)
      (bind _quickaccessslot (Getters|GetQuickAccessSlot _array_element))
      (Utilities|IsValid _quickaccessslot
        (:Is%20Valid
          (Default|SetItemAmount _quickaccessslot Amount))))))

(fn UnregisterObjectfromAllQuickSlots
  (params (ID :type Name))
  (bind _quickaccess (Variables|Management|GetQuickAccess))
  ;[0.1 0.1 0.1 1 14] Remove object from all quick slots that it has been registered in.
  (bind _keys (Utilities|Map|Keys _quickaccess))
  (for _array_element _keys
    (if (Utilities|Name|Equal(Name) (.RegisteredID (Utilities|Struct|BreakS_RPG_QuickSlot (.Value (Utilities|Map|Find _quickaccess _array_element)))) ID)
      (CallFunction|UnregisterObjectfromQuickSlotSERVER _array_element))))

(fn GetObjectRegisteredinQuickSlot
  (params (QuickSlotIndex :type Integer))
  (bind _quickaccess (Variables|Management|GetQuickAccess))
  (bind (_value _returnvalue) (Utilities|Map|Find _quickaccess QuickSlotIndex))
  (if _returnvalue
    (if (Utilities|Name|Equal(Name) (.RegisteredID (Utilities|Struct|BreakS_RPG_QuickSlot _value)) "None")
      (return false "")
      (else
        (return true _value)))
    (else
      (return false ""))))

(fn RegisterSkill
  (params (QuickSlotIndex :type Integer) (SkillID :type Name))
  (bind _returnvalue (Components|GetOwner))
  (bind _s_rpg_quickslot (Utilities|Struct|MakeS_RPG_QuickSlot SkillID "NewEnumerator0"))
  (bind _returnvalue_2 (Actor|GetComponentbyClass _returnvalue "/Game/SuperiorRPGKit/Blueprints/Components/AC_RPG_SkillsManager.AC_RPG_SkillsManager_C"))
  (bind _skillsoncooldown (Variables|/Game/SuperiorRPGKit/Blueprints/Components/AC_RPG_SkillsManager.AC_RPG_SkillsManager_C|GetSkillsOnCooldown _returnvalue_2))
  (bind _value (Utilities|Map|Find _skillsoncooldown SkillID))
  (bind (_remainingtime _initialtime) (Utilities|Struct|BreakS_RPG_Cooldown _value))
  ;[0.1 0.1 0.1 1 14] Assign skill to quick slot.
  (if (Utilities|Enum|NotEqual(Enum) (Default|GetSkillType (Actor|GetComponentbyClass (Components|GetOwner) "/Game/SuperiorRPGKit/Blueprints/Components/AC_RPG_SkillsManager.AC_RPG_SkillsManager_C") SkillID) "NewEnumerator1")
    (Utilities|Map|Add (Variables|Management|GetQuickAccess) QuickSlotIndex _s_rpg_quickslot)
    (CallFunction|UpdateQuickAccessSlotCLIENT QuickSlotIndex _s_rpg_quickslot)
    ;[0.1 0.1 0.1 1 14] Also update its cooldown value if skill is on cooldown.
    (if (Default|IsSkillonCooldown _returnvalue_2 SkillID)
      (CallFunction|UpdateSlotCooldownCLIENT SkillID (- _remainingtime (Class|KismetSystemLibrary|GetTimerElapsedTimeHandle (Variables|/Game/SuperiorRPGKit/Blueprints/Components/AC_RPG_SkillsManager.AC_RPG_SkillsManager_C|GetCooldownTimerHandle _returnvalue_2))) _initialtime))))

(fn RegisterItem
  (params (QuickSlotIndex :type Integer) (ItemID :type Name))
  (bind _s_rpg_quickslot (Utilities|Struct|MakeS_RPG_QuickSlot ItemID "NewEnumerator2"))
  (bind _returnvalue (Utilities|GetDataTableRow "/Game/SuperiorRPGKit/Datatables/DT_RPG_Items.DT_RPG_Items" ItemID)
    (:then
      (if (.RegistrableInQuickBar (Utilities|Struct|BreakS_RPG_Item_Static _returnvalue)) ; Is item registrable?
        (Utilities|Map|Add (Variables|Management|GetQuickAccess) QuickSlotIndex _s_rpg_quickslot)
        (Default|CancelItemDragging (Actor|GetComponentbyClass (Components|GetOwner) "/Game/SuperiorRPGKit/Blueprints/Components/AC_RPG_ItemsManager.AC_RPG_ItemsManager_C"))
        (CallFunction|UpdateQuickAccessSlotCLIENT QuickSlotIndex _s_rpg_quickslot)))))

(fn IsObjectAssignedtoAnyQuickSlot
  (params (ID :type Name))
  (bind _values (Utilities|Map|Values (Variables|Management|GetQuickAccess)))
  (bind _array_element (Utilities|Array|ForEachLoopwithBreak _values :!label _label)
    (:LoopBody
      (if (Utilities|Name|Equal(Name) (.RegisteredID (Utilities|Struct|BreakS_RPG_QuickSlot _array_element)) ID)
        (LocalVariables|SetResultLOCAL true)
        (goto _label Break)))
    (:Completed
      (return (LocalVariables|GetResultLOCAL)))))

(fn GetQuickAccessDatatoSave
  (bind _quickaccess (Variables|Management|GetQuickAccess))
  (bind _values (Utilities|Map|Values _quickaccess))
  (bind _keys (Utilities|Map|Keys _quickaccess))
  (return _keys _values))

(fn LoadQuickAccessData
  (params (QuickAccessSlots :type Array%20of%20Integers) (QuickAccessSlotsData :type Array%20of%20S%20RPG%20Quick%20Slot%20Structures))
  (for (_array_element _array_index) QuickAccessSlots
    (Utilities|Map|Add (Variables|Management|GetQuickAccess) _array_element (Utilities|Array|Get(acopy) QuickAccessSlotsData _array_index)))
  (CallFunction|UpdateQuickAccessBarCLIENT QuickAccessSlots QuickAccessSlotsData))