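; Actor component that decides which quest indicator its owner shows for a player, based on quests it can give, finish or progress objectives for.
; Helpers check its quest and objective sets against a passed QuestsManager, returning either the first match or all matches.
; UpdateIndicatorState walks a display priority list and sends the first valid state and quest ID to the manager's client refresh call.
; GetHighestPriorityAvailableAction uses the same priority walk to return just the state.
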(fn HasAnyAcceptableQuests
  (params (QuestsManager :type AC%20RPG%20Quests%20Manager%20Object%20Reference))
  (bind _output_get (LocalVariables|SetQuestsManagerLOCAL QuestsManager))
  (Utilities|IsValid _output_get
    (:Is%20Valid
      (bind _result (Utilities|Set|ToArray (Variables|Default|GetQuestsToAccept)))
      (bind _array_element (Utilities|Array|ForEachLoopwithBreak _result :!label _label)
        (:LoopBody
          (bind _canbedisplayed (Default|CanQuestbeDisplayedtoAccept (LocalVariables|GetQuestsManagerLOCAL) _array_element))
          (if _canbedisplayed
            (LocalVariables|SetGotAcceptableQuestsLOCAL true)
            (LocalVariables|SetAcceptableQuestLOCAL _array_element)
            (goto _label Break)))
        (:Completed
          (return (LocalVariables|GetGotAcceptableQuestsLOCAL) (LocalVariables|GetAcceptableQuestLOCAL)))))))

(fn UpdateIndicatorState
  (params (QuestsManager :type AC%20RPG%20Quests%20Manager%20Object%20Reference))
  (LocalVariables|SetQuestManagerLOCAL QuestsManager)
  (bind _array_element (Utilities|Array|ForEachLoopwithBreak (Variables|Default|GetQuestIndicatorDisplayPriority) :!label _label)
    (:LoopBody
      (switch Utilities|FlowControl|Switch|SwitchonE_RPG_QuestIndicatorState _array_element
        (:NewEnumerator1
          (bind (_hasfinishablequests _indicatedquestid) (Conditions|HasAnyFinishableQuests (LocalVariables|GetQuestManagerLOCAL)))
          (if _hasfinishablequests
            (Default|RefreshDisplayedQuestInfoStateCLIENT (LocalVariables|GetQuestManagerLOCAL) (Components|GetOwner self) "NewEnumerator1" _indicatedquestid)
            (goto _label Break)))
        (:NewEnumerator2
          (bind (_hasobjectivestoprogress _indicatedquestid_2) (Conditions|HasAnyObjectivetoProgress (LocalVariables|GetQuestManagerLOCAL)))
          (if _hasobjectivestoprogress
            (Default|RefreshDisplayedQuestInfoStateCLIENT (LocalVariables|GetQuestManagerLOCAL) (Components|GetOwner self) "NewEnumerator2" _indicatedquestid_2)
            (goto _label Break)))
        (:NewEnumerator0
          (bind (_hasacceptablequests _indicatedquestid_3) (Conditions|HasAnyAcceptableQuests (LocalVariables|GetQuestManagerLOCAL)))
          (if _hasacceptablequests
            (Default|RefreshDisplayedQuestInfoStateCLIENT (LocalVariables|GetQuestManagerLOCAL) (Components|GetOwner self) "NewEnumerator0" _indicatedquestid_3)
            (goto _label Break)))
        (:NewEnumerator3
          (Default|RefreshDisplayedQuestInfoStateCLIENT (LocalVariables|GetQuestManagerLOCAL) (Components|GetOwner self) "NewEnumerator3" "None")
          (goto _label Break))))))

(fn HasAnyObjectivetoProgress
  (params (QuestsManager :type AC%20RPG%20Quests%20Manager%20Object%20Reference))
  (bind _output_get (LocalVariables|SetQuestsManagerLOCAL QuestsManager))
  (Utilities|IsValid _output_get
    (:Is%20Valid
      (bind _result (Utilities|Set|ToArray (Variables|Default|GetObjectivesToProgress)))
      (bind _array_element (Utilities|Array|ForEachLoopwithBreak _result :!label _label)
        (:LoopBody
          (if (Utilities|Array|ContainsItem (Variables|/Game/SuperiorRPGKit/Blueprints/Components/AC_RPG_QuestsManager.AC_RPG_QuestsManager_C|GetOngoingObjectives (LocalVariables|GetQuestsManagerLOCAL)) _array_element)
            (LocalVariables|SetHasObjectivesToProgressLOCAL true)
            (bind _questid (Default|GetOngoingQuestwithObjective (LocalVariables|GetQuestsManagerLOCAL) _array_element))
            (LocalVariables|SetObjectiveOfQuestLOCAL _questid)
            (goto _label Break)))
        (:Completed
          (return (LocalVariables|GetHasObjectivesToProgressLOCAL) (LocalVariables|GetObjectiveOfQuestLOCAL)))))))

(fn GetAcceptableQuests
  (params (QuestsManager :type AC%20RPG%20Quests%20Manager%20Object%20Reference))
  (bind _output_get (LocalVariables|SetQuestsManagerLOCAL QuestsManager))
  (Utilities|IsValid _output_get
    (:Is%20Valid
      (bind _result (Utilities|Set|ToArray (Variables|Default|GetQuestsToAccept)))
      (for _array_element _result
        (bind _canbedisplayed (Default|CanQuestbeDisplayedtoAccept (LocalVariables|GetQuestsManagerLOCAL) _array_element))
        (if _canbedisplayed
          (Utilities|Array|Add (LocalVariables|GetAcceptableQuestsLOCAL) _array_element)))
      (return (LocalVariables|GetAcceptableQuestsLOCAL)))))

(fn GettProgressableObjectives
  (params (QuestsManager :type AC%20RPG%20Quests%20Manager%20Object%20Reference))
  (bind _output_get (LocalVariables|SetQuestsManagerLOCAL QuestsManager))
  (Utilities|IsValid _output_get
    (:Is%20Valid
      (bind _result (Utilities|Set|ToArray (Variables|Default|GetObjectivesToProgress)))
      (for _array_element _result
        (if (Utilities|Array|ContainsItem (Variables|/Game/SuperiorRPGKit/Blueprints/Components/AC_RPG_QuestsManager.AC_RPG_QuestsManager_C|GetOngoingObjectives (LocalVariables|GetQuestsManagerLOCAL)) _array_element)
          (Utilities|Array|Add (LocalVariables|GetProgressableObjectivesLOCAL) _array_element)))
      (return (LocalVariables|GetProgressableObjectivesLOCAL)))))

(fn HasAnyFinishableQuests
  (params (QuestsManager :type AC%20RPG%20Quests%20Manager%20Object%20Reference))
  (bind _output_get (LocalVariables|SetQuestsManagerLOCAL QuestsManager))
  (Utilities|IsValid _output_get
    (:Is%20Valid
      (bind _result (Utilities|Set|ToArray (Variables|Default|GetQuestsToFinish)))
      (bind _array_element (Utilities|Array|ForEachLoopwithBreak _result :!label _label)
        (:LoopBody
          (bind _canbedisplayed (Default|CanQuestbeDisplayedtoFinish (LocalVariables|GetQuestsManagerLOCAL) _array_element))
          (if _canbedisplayed
            (LocalVariables|SetHasFinishableQuestsLOCAL true)
            (LocalVariables|SetFinishableQuestLOCAL _array_element)
            (goto _label Break)))
        (:Completed
          (return (LocalVariables|GetHasFinishableQuestsLOCAL) (LocalVariables|GetFinishableQuestLOCAL)))))))

(fn GetFinishableQuests
  (params (QuestsManager :type AC%20RPG%20Quests%20Manager%20Object%20Reference))
  (bind _output_get (LocalVariables|SetQuestsManagerLOCAL QuestsManager))
  (Utilities|IsValid _output_get
    (:Is%20Valid
      (bind _result (Utilities|Set|ToArray (Variables|Default|GetQuestsToFinish)))
      (for _array_element _result
        (bind _canbedisplayed (Default|CanQuestbeDisplayedtoFinish (LocalVariables|GetQuestsManagerLOCAL) _array_element))
        (if _canbedisplayed
          (Utilities|Array|Add (LocalVariables|GetFinishableQuestsLOCAL) _array_element)))
      (return (LocalVariables|GetFinishableQuestsLOCAL)))))

(fn GetHighestPriorityAvailableAction
  (params (QuestsManager :type AC%20RPG%20Quests%20Manager%20Object%20Reference))
  (LocalVariables|SetQuestsManagerLOCAL QuestsManager)
  (bind _array_element (Utilities|Array|ForEachLoopwithBreak (Variables|Default|GetQuestIndicatorDisplayPriority) :!label _label)
    (:LoopBody
      (switch Utilities|FlowControl|Switch|SwitchonE_RPG_QuestIndicatorState _array_element
        (:NewEnumerator1
          (bind _hasfinishablequests (Conditions|HasAnyFinishableQuests (LocalVariables|GetQuestsManagerLOCAL)))
          (if _hasfinishablequests
            (LocalVariables|SetHighestPriorityActionLOCAL "NewEnumerator1")
            (goto _label Break)))
        (:NewEnumerator2
          (bind _hasobjectivestoprogress (Conditions|HasAnyObjectivetoProgress (LocalVariables|GetQuestsManagerLOCAL)))
          (if _hasobjectivestoprogress
            (LocalVariables|SetHighestPriorityActionLOCAL "NewEnumerator2")
            (goto _label Break)))
        (:NewEnumerator0
          (bind _hasacceptablequests (Conditions|HasAnyAcceptableQuests (LocalVariables|GetQuestsManagerLOCAL)))
          (if _hasacceptablequests
            (LocalVariables|SetHighestPriorityActionLOCAL "NewEnumerator0")
            (goto _label Break)))
        (:NewEnumerator3
          (LocalVariables|SetHighestPriorityActionLOCAL "NewEnumerator3"))))
    (:Completed
      (return (LocalVariables|GetHighestPriorityActionLOCAL)))))