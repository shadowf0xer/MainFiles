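; Client-side component that queues and displays on-screen pop-up notifications with text, color, sound, image and animations.
; QueueNewNotification fills a queue that ShowNotification drains into slot widgets, reused from a pool capped at MaxNotificationsQueueAmount.
; ReleaseNotificationSlot frees a slot and shows the next queued message.
; Slots go into the container for the configured screen position, optionally reordered newest-on-top by re-adding children and reapplying their layout.
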(event Custom|QueueNewNotification
  (params (MessageText :type Text) (IndicatorColor :type Linear%20Color%20Structure) (Sound :type Sound%20Wave%20Object%20Reference) (Image :type Texture%202D%20Object%20Reference) (CanBeClickedToDismiss? :type Boolean) (Duration :type Float%20%28single-precision%29) (OverrideFillingColor? :type Boolean) (FillingColor :type Linear%20Color%20Structure))
  ;[0.1 0.1 0.1 1 14] Always executed on client.
  ;;[1 1 1] Add new notification to queue and try to show it.
  (Utilities|Array|Add (Variables|Notifications|GetQueuedNotifications) (Utilities|Struct|MakeS_RPG_Notification MessageText IndicatorColor Sound Image CanBeClickedToDismiss? Duration OverrideFillingColor? FillingColor))
  (CallFunction|ShowNotification))

(event Custom|ShowNotification
  ;[0.1 0.1 0.1 1 14] Always executed on client.
  (bind (_popupslot _canshownewmessage_) (WidgetsManagement|GetProperNotificationSlot))
  (if _canshownewmessage_
    (bind (_istheretexttoshow_ _messagestruct) (Notifications|GetNextNotificationfromQueuedNotifications)) ; Check if there is message queued and get its structure.
    (if _istheretexttoshow_
      (Rendering|Components|TextRender|SetText (Variables|/Game/SuperiorRPGKit/Widgets/Notifications/WBP_RPG_NotificationSlot.WBP_RPG_NotificationSlot_C|GetTextBlock_Message _popupslot) (.MessageText (Utilities|Struct|BreakS_RPG_Notification _messagestruct))) ; Set message text
      (Default|SetupIndicators _popupslot (Variables|VisualSettings|SlotSettings|GetColorIndicatorsSize) (.IndicatorColor (Utilities|Struct|BreakS_RPG_Notification _messagestruct))) ; Update slot indicators.
      (Audio|PlaySound2D (.Sound (Utilities|Struct|BreakS_RPG_Notification _messagestruct))) ; Play message sound
      (Default|SetupImage _popupslot (.Image (Utilities|Struct|BreakS_RPG_Notification _messagestruct)) (Variables|VisualSettings|SlotSettings|GetImagePosition)) ; set message image
      (Variables|/Game/SuperiorRPGKit/Widgets/Notifications/WBP_RPG_NotificationSlot.WBP_RPG_NotificationSlot_C|SetCanBeClickedToDismiss? _popupslot (.CanBeClickedToDismiss? (Utilities|Struct|BreakS_RPG_Notification _messagestruct))) ; Determine if can be clicked to dismiss
      (Widget|SetVisibility _popupslot (select (.CanBeClickedToDismiss? (Utilities|Struct|BreakS_RPG_Notification _messagestruct)) "SelfHitTestInvisible" "HitTestInvisible")) ; Make slot visible again
      (Variables|/Game/SuperiorRPGKit/Widgets/Notifications/WBP_RPG_NotificationSlot.WBP_RPG_NotificationSlot_C|SetIsInUse? _popupslot true) ; "Occupy" slot
      (Layout|BorderSlot|SetPadding _popupslot (Variables|VisualSettings|SlotSettings|GetSlotsPadding) :!class /Script/UMG.UserWidget)
      (Default|SetupFilling _popupslot (Variables|VisualSettings|SlotFilling|GetSlotFillingType) (Variables|VisualSettings|SlotFilling|GetSlotFillingOpacityBoost) (Math|Color|SelectColor (.FillingColor (Utilities|Struct|BreakS_RPG_Notification _messagestruct)) (Variables|VisualSettings|SlotFilling|GetSlotFillingColor) (.OverrideFillingColor? (Utilities|Struct|BreakS_RPG_Notification _messagestruct)))) ; Set slot background.
      (Default|ShowNotificationSlot _popupslot (Variables|VisualSettings|TransitionIn|GetInAnimationTime) (.Duration (Utilities|Struct|BreakS_RPG_Notification _messagestruct)) (Variables|VisualSettings|TransitionOut|GetOutAnimationTime) (Variables|VisualSettings|TransitionIn|GetPlayFadeInEffect?) (Variables|VisualSettings|TransitionIn|GetPlaySlideInEffect?) (Variables|VisualSettings|TransitionIn|GetSlideInEffectDirection) (Variables|VisualSettings|TransitionIn|GetPlayPopInEffect?) (Variables|VisualSettings|TransitionIn|GetPopInEffectAnchors) (Variables|VisualSettings|TransitionIn|GetPlayFloatInEffect?) (Variables|VisualSettings|TransitionOut|GetPlayFadeOutEffect?) (Variables|VisualSettings|TransitionOut|GetPlaySlideOutEffect?) (Variables|VisualSettings|TransitionOut|GetSlideOutEffectDirection) (Variables|VisualSettings|TransitionOut|GetPlayPopOutEffect?) (Variables|VisualSettings|TransitionOut|GetPopOutEffectAnchors) (Variables|VisualSettings|TransitionOut|GetPlayFloatOutEffect?)) ; Set up transition animations
      (Default|SetupSizeOverride _popupslot (Variables|VisualSettings|SlotSettings|GetOverrideSlotWidth) (Variables|VisualSettings|SlotSettings|GetOverrideSlotHeight) (Variables|VisualSettings|SlotSettings|GetMinSlotWidth) (Variables|VisualSettings|SlotSettings|GetMinSlotHeight)) ; set up slot size
      (if (Variables|GeneralSettings|GetDisplayNewestNotificationOnTop) ; If newest message should be displayed on top\nreverse all slots position in container.
        (WidgetsManagement|ReverseSlotsPosition)))))

(event EventBeginPlay)

(fn GetProperNotificationSlot
  ;[1 1 1] If there is unused notification slot in the pool of already created slots, pick it to reuse.
  (bind _array_element (Utilities|Array|ForEachLoopwithBreak (Variables|References|GetNotificationSlotsReference) :!label _label)
    (:LoopBody
      (if (not (Variables|/Game/SuperiorRPGKit/Widgets/Notifications/WBP_RPG_NotificationSlot.WBP_RPG_NotificationSlot_C|GetIsInUse? _array_element))
        (LocalVariables|SetFoundFreeSlot?LOCAL true)
        (LocalVariables|SetFreeSlotLOCAL _array_element)
        (goto _label Break)))
    (:Completed
      (if (LocalVariables|GetFoundFreeSlot?LOCAL)
        (WidgetsManagement|AddSlottoContainer (LocalVariables|GetFreeSlotLOCAL))
        (return (LocalVariables|GetFreeSlotLOCAL) true)
        (else
          ;[1 1 1] If there is no unused slots, create new one and add it to pool.
          (if (< (Utilities|Array|Length (Variables|References|GetNotificationSlotsReference)) (Variables|GeneralSettings|GetMaxNotificationsQueueAmount))
            (bind _returnvalue (UserInterface|CreateWidget "/Game/SuperiorRPGKit/Widgets/Notifications/WBP_RPG_NotificationSlot.WBP_RPG_NotificationSlot_C" 0 self))
            (Utilities|Array|Add (Variables|References|GetNotificationSlotsReference) _returnvalue)
            (Default|SetMessageFont _returnvalue (Variables|VisualSettings|Font|GetFontFamily) (Variables|VisualSettings|Font|GetFontSize))
            (WidgetsManagement|AddSlottoContainer _returnvalue)
            (return _returnvalue true)
            (else
              (return 0 false))))))))

(fn ReleaseNotificationSlot
  (params (PopUpSlot :type WBP%20RPG%20Notification%20Slot%20Object%20Reference))
  (LocalVariables|SetPopUpSlotLOCAL PopUpSlot)
  (Utilities|Array|RemoveItem (Variables|References|GetNotificationSlotsReference) (LocalVariables|GetPopUpSlotLOCAL))
  (Utilities|Array|Add (Variables|References|GetNotificationSlotsReference) (LocalVariables|GetPopUpSlotLOCAL))
  (WidgetsManagement|AddSlottoContainer (LocalVariables|GetPopUpSlotLOCAL))
  (Variables|/Game/SuperiorRPGKit/Widgets/Notifications/WBP_RPG_NotificationSlot.WBP_RPG_NotificationSlot_C|SetIsInUse? (LocalVariables|GetPopUpSlotLOCAL) false)
  (Widget|SetVisibility (LocalVariables|GetPopUpSlotLOCAL) "Collapsed")
  (CallFunction|ShowNotification) ; When slots is released, check if there are any messages queued.
)

(fn AddSlottoContainer
  (params (PopUpSlot :type WBP%20RPG%20Notification%20Slot%20Object%20Reference))
  (LocalVariables|SetPopUpSlotLOCAL PopUpSlot)
  (bind _returnvalue (Widget|Panel|AddChild (Utilities|GetProperNotificationContainer) (LocalVariables|GetPopUpSlotLOCAL)))
  (Utilities|FlowControl|Sequence
    (:then_0
      (if (== (Variables|VisualSettings|SlotSettings|GetOverrideSlotWidth) 0.0)
        (switch Utilities|FlowControl|Switch|SwitchonE_RPG_WindowPosition (Variables|GeneralSettings|GetWindowPosition) ; Set alignment for slots, but only if their width will \nadjust message text length. (no point to adjust alignment \nwhen all slots have the same width)
          (:NewEnumerator3
            (bind _asvertical_box_slot (Utilities|Casting|CastToVerticalBoxSlot _returnvalue :!label _label))
            (Layout|GridSlot|SetHorizontalAlignment _asvertical_box_slot "HAlign_Left"))
          (:NewEnumerator1
            (goto _label))
          (:NewEnumerator4
            (goto _label))
          (:NewEnumerator7
            (bind _asvertical_box_slot_2 (Utilities|Casting|CastToVerticalBoxSlot _returnvalue :!label _label_2))
            (Layout|GridSlot|SetHorizontalAlignment _asvertical_box_slot_2 "HAlign_Right"))
          (:NewEnumerator2
            (goto _label_2))
          (:NewEnumerator8
            (goto _label_2)))))
    (:then_1
      ;[1 1 1] Show hide image depending on selected option.
      (Widget|SetVisibility (Variables|/Game/SuperiorRPGKit/Widgets/Notifications/WBP_RPG_NotificationSlot.WBP_RPG_NotificationSlot_C|GetImage_Left (LocalVariables|GetPopUpSlotLOCAL)) (Utilities|Select :Index (Variables|VisualSettings|SlotSettings|GetImagePosition) :NewEnumerator2 "Collapsed" :NewEnumerator0 "HitTestInvisible" :NewEnumerator1 "Collapsed"))
      (Widget|SetVisibility (Variables|/Game/SuperiorRPGKit/Widgets/Notifications/WBP_RPG_NotificationSlot.WBP_RPG_NotificationSlot_C|GetImage_Right (LocalVariables|GetPopUpSlotLOCAL)) (Utilities|Select :Index (Variables|VisualSettings|SlotSettings|GetImagePosition) :NewEnumerator2 "Collapsed" :NewEnumerator0 "Collapsed" :NewEnumerator1 "HitTestInvisible")))))

(fn GetNextNotificationfromQueuedNotifications
  (bind _queuednotifications (Variables|Notifications|GetQueuedNotifications))
  (if (Utilities|Array|IsValidIndex _queuednotifications)
    (LocalVariables|SetMessageStructLOCAL (Utilities|Array|Get(acopy) _queuednotifications))
    (Utilities|Array|RemoveIndex (Variables|Notifications|GetQueuedNotifications))
    (return true (LocalVariables|GetMessageStructLOCAL))
    (else
      (return false ""))))

(fn ReverseSlotsPosition
  (bind _returnvalue (Utilities|GetProperNotificationContainer))
  (for _index (range 0 (- (Class|PanelWidget|GetChildrenCount (Utilities|GetProperNotificationContainer)) 2)) ; Get all notification slots, except newly added\nand store them locally.
    (bind _aswbp_rpg_notification_slot (Utilities|Casting|CastToWBP_RPG_NotificationSlot (Class|PanelWidget|GetChildat _returnvalue _index)))
    (Utilities|Array|Add (LocalVariables|GetTemporaryArrayLOCAL) _aswbp_rpg_notification_slot))
  (for _array_element (LocalVariables|GetTemporaryArrayLOCAL) ; get all locally stored slots and re-add them\nto container
    (bind _returnvalue_2 (Widget|Panel|AddChild _returnvalue _array_element))
    (Default|SetupFilling _array_element (Variables|VisualSettings|SlotFilling|GetSlotFillingType) (Variables|VisualSettings|SlotFilling|GetSlotFillingOpacityBoost) (Variables|/Game/SuperiorRPGKit/Widgets/Notifications/WBP_RPG_NotificationSlot.WBP_RPG_NotificationSlot_C|GetFillingColor _array_element)) ; When slot is re-added its options are reset\nso we need to reapply them as well.
    (if (== (Variables|VisualSettings|SlotSettings|GetOverrideSlotWidth) 0.0)
      (switch Utilities|FlowControl|Switch|SwitchonE_RPG_WindowPosition (Variables|GeneralSettings|GetWindowPosition) ; Set alignment for slots, but only if their width will \nadjust message text length. (no point to adjust alignment \nwhen all slots have the same width)
        (:NewEnumerator3
          (bind _asvertical_box_slot (Utilities|Casting|CastToVerticalBoxSlot _returnvalue_2 :!label _label))
          (Layout|GridSlot|SetHorizontalAlignment _asvertical_box_slot "HAlign_Left"))
        (:NewEnumerator1
          (goto _label))
        (:NewEnumerator4
          (goto _label))
        (:NewEnumerator7
          (bind _asvertical_box_slot_2 (Utilities|Casting|CastToVerticalBoxSlot _returnvalue_2 :!label _label_2))
          (Layout|GridSlot|SetHorizontalAlignment _asvertical_box_slot_2 "HAlign_Right"))
        (:NewEnumerator2
          (goto _label_2))
        (:NewEnumerator8
          (goto _label_2))))))

(fn InitializeNotificationsContainer
  (params (NotificationsContainer :type WBP%20RPG%20Notification%20Container%20Object%20Reference))
  (Variables|References|SetNotificationsContainerReference NotificationsContainer)
  (Widget|Panel|ClearChildren (Variables|/Game/SuperiorRPGKit/Widgets/Notifications/WBP_RPG_NotificationContainer.WBP_RPG_NotificationContainer_C|GetContainer_Center (Variables|References|GetNotificationsContainerReference)))
  (LocalVariables|SetAlignmentYLOCAL (Math|Float|SelectFloat (Math|Float|SelectFloat 0.0 1.0 (Variables|GeneralSettings|GetDisplayNewestNotificationOnTop)) (Math|Float|SelectFloat 1.0 0.0 (Variables|GeneralSettings|GetDisplayNewestNotificationOnTop)) (Variables|GeneralSettings|GetWhenNewNotificationIsAddedPushOtherSlots)))
  (switch Utilities|FlowControl|Switch|SwitchonE_RPG_WindowPosition (Variables|GeneralSettings|GetWindowPosition)
    (:NewEnumerator3
      (Class|CanvasPanelSlot|SetAlignment (Class|WidgetLayoutLibrary|SlotasCanvasSlot (Variables|/Game/SuperiorRPGKit/Widgets/Notifications/WBP_RPG_NotificationContainer.WBP_RPG_NotificationContainer_C|GetContainer_TopLeft (Variables|References|GetNotificationsContainerReference))) (Math|Vector2D|MakeVector2D 0.0 (LocalVariables|GetAlignmentYLOCAL))))
    (:NewEnumerator1
      (Class|CanvasPanelSlot|SetAlignment (Class|WidgetLayoutLibrary|SlotasCanvasSlot (Variables|/Game/SuperiorRPGKit/Widgets/Notifications/WBP_RPG_NotificationContainer.WBP_RPG_NotificationContainer_C|GetContainer_Left (Variables|References|GetNotificationsContainerReference))) (Math|Vector2D|MakeVector2D 0.0 (LocalVariables|GetAlignmentYLOCAL))))
    (:NewEnumerator4
      (Class|CanvasPanelSlot|SetAlignment (Class|WidgetLayoutLibrary|SlotasCanvasSlot (Variables|/Game/SuperiorRPGKit/Widgets/Notifications/WBP_RPG_NotificationContainer.WBP_RPG_NotificationContainer_C|GetContainer_BottomLeft (Variables|References|GetNotificationsContainerReference))) (Math|Vector2D|MakeVector2D 0.0 (LocalVariables|GetAlignmentYLOCAL))))
    (:NewEnumerator5
      (Class|CanvasPanelSlot|SetAlignment (Class|WidgetLayoutLibrary|SlotasCanvasSlot (Variables|/Game/SuperiorRPGKit/Widgets/Notifications/WBP_RPG_NotificationContainer.WBP_RPG_NotificationContainer_C|GetContainer_Top (Variables|References|GetNotificationsContainerReference))) (Math|Vector2D|MakeVector2D 0.0 (LocalVariables|GetAlignmentYLOCAL))))
    (:NewEnumerator0
      (Class|CanvasPanelSlot|SetAlignment (Class|WidgetLayoutLibrary|SlotasCanvasSlot (Variables|/Game/SuperiorRPGKit/Widgets/Notifications/WBP_RPG_NotificationContainer.WBP_RPG_NotificationContainer_C|GetContainer_Center (Variables|References|GetNotificationsContainerReference))) (Math|Vector2D|MakeVector2D 0.0 (LocalVariables|GetAlignmentYLOCAL))))
    (:NewEnumerator6
      (Class|CanvasPanelSlot|SetAlignment (Class|WidgetLayoutLibrary|SlotasCanvasSlot (Variables|/Game/SuperiorRPGKit/Widgets/Notifications/WBP_RPG_NotificationContainer.WBP_RPG_NotificationContainer_C|GetContainer_Bottom (Variables|References|GetNotificationsContainerReference))) (Math|Vector2D|MakeVector2D 1.0 (LocalVariables|GetAlignmentYLOCAL))))
    (:NewEnumerator7
      (Class|CanvasPanelSlot|SetAlignment (Class|WidgetLayoutLibrary|SlotasCanvasSlot (Variables|/Game/SuperiorRPGKit/Widgets/Notifications/WBP_RPG_NotificationContainer.WBP_RPG_NotificationContainer_C|GetContainer_TopRight (Variables|References|GetNotificationsContainerReference))) (Math|Vector2D|MakeVector2D 1.0 (LocalVariables|GetAlignmentYLOCAL))))
    (:NewEnumerator2
      (Class|CanvasPanelSlot|SetAlignment (Class|WidgetLayoutLibrary|SlotasCanvasSlot (Variables|/Game/SuperiorRPGKit/Widgets/Notifications/WBP_RPG_NotificationContainer.WBP_RPG_NotificationContainer_C|GetContainer_Right (Variables|References|GetNotificationsContainerReference))) (Math|Vector2D|MakeVector2D 1.0 (LocalVariables|GetAlignmentYLOCAL))))
    (:NewEnumerator8
      (Class|CanvasPanelSlot|SetAlignment (Class|WidgetLayoutLibrary|SlotasCanvasSlot (Variables|/Game/SuperiorRPGKit/Widgets/Notifications/WBP_RPG_NotificationContainer.WBP_RPG_NotificationContainer_C|GetContainer_BottomRight (Variables|References|GetNotificationsContainerReference))) (Math|Vector2D|MakeVector2D 1.0 (LocalVariables|GetAlignmentYLOCAL))))))