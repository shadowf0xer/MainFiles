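; Equipment component for the RPG kit that tracks equipped items by slot and drives equipment meshes and combat stance.
; A multicast event looks up meshes and sockets in the items data table and broadcasts them, updating stance when either hand slot changes.
; Stance derives from hand item subtypes, including shield and unarmed cases.
; Save/load flattens and rebuilds the slot map, with loading reapplying bonuses and refreshing widgets and meshes.
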(event Custom|ChangeEquipmentMesh_MULTICAST
  (params (EquipmentSlot :type Integer) (ItemID :type Name))
  ;[0.1 0.1 0.1 1 14] Calls OnEquipmentMeshChanged on server and clients (so everybody sees updated item mesh)
  (bind _returnvalue (Utilities|GetDataTableRow "/Game/SuperiorRPGKit/Datatables/DT_RPG_Items.DT_RPG_Items" ItemID)
    (:then
      (Default|CallOnEquipmentMeshChanged EquipmentSlot (.SkeletalMeshEquip (Utilities|Struct|BreakS_RPG_Item_Static _returnvalue)) (.Value (Utilities|Map|Find (.SkeletalMeshEquipSockets (Utilities|Struct|BreakS_RPG_Item_Static _returnvalue)) EquipmentSlot)) (.StaticMeshEquip (Utilities|Struct|BreakS_RPG_Item_Static _returnvalue)) (.Value (Utilities|Map|Find (.StaticMeshEquipSockets (Utilities|Struct|BreakS_RPG_Item_Static _returnvalue)) EquipmentSlot))))
    (:RowNotFound
      (Default|CallOnEquipmentMeshChanged EquipmentSlot)))
  (if (or (== EquipmentSlot 1) (== EquipmentSlot 2)) ; We update stance only when equipment\nchanges in slot 1 (right hand) or slot 2 (left hand).\nOther slots doesn't affect stance.
    (bind _stance (CallFunction|GetCombatStance))
    (Default|CallOnCombatStanceChanged _stance)))

(fn LoadEquipmentData
  (params (EquippedItemsSlots :type Array%20of%20Integers) (EquippedItemsData :type Array%20of%20S%20RPG%20Item%20Dynamic%20Structures))
  (bind _equippeditems (Variables|Config|GetEquippedItems))
  (bind _equippeditems_2 (Variables|Config|GetEquippedItems))
  (Utilities|FlowControl|Sequence
    (:then_1
      ;[0.1 0.1 0.1 1 12] Reconstruct equipped items map.
      (for (_array_element _array_index) EquippedItemsSlots
        (Utilities|Map|Add (Variables|Config|GetEquippedItems) _array_element (Utilities|Array|Get(acopy) EquippedItemsData _array_index))
        ;[0.1 0.1 0.1 1 12] Reapply equipment stats to hero.
        (if (Utilities|Name|NotEqual(Name) (.ID (Utilities|Struct|BreakS_RPG_Item_Dynamic (Utilities|Array|Get(acopy) EquippedItemsData _array_index))) "None")
          (bind _bonusesvalues (CallFunction|CalculateItemBonusesValues (Utilities|Array|Get(acopy) EquippedItemsData _array_index)))
          (CallFunction|ApplyBonuses (Utilities|Array|Get(acopy) (Variables|Default|GetActorsAccessingContainer)) _bonusesvalues))))
    (:then_2
      ;[0.1 0.1 0.1 1 14] Update equipment widget.
      (for _array_element_2 (Variables|Default|GetActorsAccessingContainer)
        (Utilities|IsValid (Actor|GetComponentbyClass _array_element_2 "/Game/SuperiorRPGKit/Blueprints/Components/AC_RPG_ItemsManager.AC_RPG_ItemsManager_C")
          (:Is%20Valid
            (bind _keys (Utilities|Map|Keys _equippeditems_2))
            (bind _values (Utilities|Map|Values _equippeditems_2))
            (Default|RefreshEquipmentSlotsGroupCLIENT (Actor|GetComponentbyClass _array_element_2 "/Game/SuperiorRPGKit/Blueprints/Components/AC_RPG_ItemsManager.AC_RPG_ItemsManager_C") _keys _values)))))
    (:then_3
      ;[0.1 0.1 0.1 1 14] Update meshes equipped to character.
      (bind _keys_2 (Utilities|Map|Keys _equippeditems))
      (for _array_element_3 _keys_2
        (CallFunction|ChangeEquipmentMeshMULTICAST _array_element_3 (.ID (Utilities|Struct|BreakS_RPG_Item_Dynamic (.Value (Utilities|Map|Find _equippeditems _array_element_3)))))))))

(fn GetEquipmentDatatoSave
  (bind _equippeditems (Variables|Config|GetEquippedItems))
  (bind _values (Utilities|Map|Values _equippeditems))
  (bind _keys (Utilities|Map|Keys _equippeditems))
  (return _keys _values))

(fn GetCombatStance
  (bind _returnvalue (Utilities|GetDataTableRow "/Game/SuperiorRPGKit/Datatables/DT_RPG_Items.DT_RPG_Items" (.ID (Utilities|Struct|BreakS_RPG_Item_Dynamic (.Value (Utilities|Map|Find (Variables|Config|GetEquippedItems) 1)))))
    (:then
      (switch Utilities|FlowControl|Switch|SwitchonE_RPG_ItemSubtype (Utilities|Struct|BreakS_RPG_Item_Static _returnvalue) ; Return stances only for items that are equipped to hands.
        (:NewEnumerator0
          _)
        (:NewEnumerator1
          _)
        (:NewEnumerator2
          (return "NewEnumerator4"))
        (:NewEnumerator3
          (return "NewEnumerator5"))
        (:NewEnumerator24
          (return "NewEnumerator1"))
        (:NewEnumerator25
          _)
        (:NewEnumerator30
          (return "NewEnumerator1")))
      (bind _returnvalue_2 (Utilities|GetDataTableRow "/Game/SuperiorRPGKit/Datatables/DT_RPG_Items.DT_RPG_Items" (.ID (Utilities|Struct|BreakS_RPG_Item_Dynamic (.Value (Utilities|Map|Find (Variables|Config|GetEquippedItems) 2)))))
        (:then
          (if (Utilities|Enum|Equal(Enum) (Utilities|Struct|BreakS_RPG_Item_Static _returnvalue_2) "NewEnumerator5")
            (return "NewEnumerator3") ; If there is a shield equipped we use OneHanded with Shield stance.
            (else
              _)))
        (:RowNotFound
          _))
      (return "NewEnumerator2") ; If there is no shield equipped we use OneHanded weapon stance.
    )
    (:RowNotFound
      (return "NewEnumerator0") ; If there is no item equipped to slot 1 (right hand slot)\nuse Unarmed stance.
    )))