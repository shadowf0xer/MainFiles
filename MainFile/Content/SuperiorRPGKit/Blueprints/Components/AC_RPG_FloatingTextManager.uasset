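; Floating text manager component that shows damage pop-ups at given locations, with a flag for critical hits.
; The client-named display event truncates damage to an integer and passes the text to a pop-up actor.
; Pop-ups are pooled: it takes one from the free list or spawns a new one holding a manager reference.
; Nothing in this graph returns pop-ups to the free list.
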(event Custom|DisplayDamagePopUp_CLIENT
  (params (Damage :type Float%20%28single-precision%29) (Location :type Vector) (Critical :type Boolean))
  (bind _damagepopup (CallFunction|GetAvailableDamagePopUp))
  (Default|DisplayText _damagepopup (Utilities|Text|ToText(Integer) (Math|Float|Truncate Damage) false false) Location Critical false))

(event EventBeginPlay)

(event EventTick
  (params (DeltaSeconds :type Float%20%28single-precision%29)))

(fn GetAvailableDamagePopUp
  (bind _freedamagepopups (Variables|Default|GetFreeDamagePopUps))
  (if (Utilities|Array|IsValidIndex _freedamagepopups)
    (bind _output_get (LocalVariables|SetDamagePopUpLOCAL (Utilities|Array|Get(acopy) _freedamagepopups)))
    (Utilities|Array|RemoveItem (Variables|Default|GetFreeDamagePopUps) _output_get)
    (return (LocalVariables|GetDamagePopUpLOCAL))
    (else
      (bind _returnvalue (Game|SpawnActorfromClass "/Game/SuperiorRPGKit/Blueprints/Basics/BP_RPG_PopUp_Damage.BP_RPG_PopUp_Damage_C" (Math|Transform|MakeTransform "0, 0, 0" "0, 0, 0" "1,1,1") "Undefined" 0 self 0))
      (return _returnvalue))))