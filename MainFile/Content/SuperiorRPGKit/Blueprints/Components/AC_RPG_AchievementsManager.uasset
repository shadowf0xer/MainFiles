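; Actor component that tracks RPG achievements per objective type and pays out gold and XP through the owner's items and stats managers.
; A map built from DT_RPG_Achievements sorts achievements into unfinished, finishable and claimed lists; added progress promotes them to finishable.
; A server event validates claims, while client events push progress and visibility to registered widgets, revealing follow-up achievements.
; Save and load functions export the map and rebuild the window.
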(event Custom|InitializeAchievementsWindow_CLIENT
  ;[0.1 0.1 0.1 1 14] Add all achievements to achievements window.
  (for _array_element (Variables|Default|GetWidgetsToRefresh)
    (bind _outrownames (DataTable|GetDataTableRowNames "/Game/SuperiorRPGKit/Datatables/DT_RPG_Achievements.DT_RPG_Achievements"))
    (for _array_element_2 _outrownames
      (bind _returnvalue (Utilities|GetDataTableRow "/Game/SuperiorRPGKit/Datatables/DT_RPG_Achievements.DT_RPG_Achievements" _array_element_2)
        (:then
          (Class|BPIRPGAchievementsUpdater|AddAchievementtoWindow(Message) _array_element _returnvalue))))))

(event Custom|ReloadAchievementsWindow_CLIENT
  (params (AchievementsObjectives :type Array%20of%20E_RPG_AchievementObjective%20Enums :default "NewEnumerator4") (AchievementsData :type Array%20of%20S%20RPG%20Achievement%20Dynamic%20Structures))
  (for (_array_element _array_index) AchievementsObjectives
    ;[0.1 0.1 0.1 1 14] Update displayed achievements progress.
    (CallFunction|RefreshAchievementProgressCLIENT _array_element (.CurrentProgress (Utilities|Struct|BreakS_RPG_Achievement_Dynamic (Utilities|Array|Get(acopy) AchievementsData _array_index))))
    (CallFunction|SetAchievementsStateCLIENT (.UnfinishedAchievements (Utilities|Struct|BreakS_RPG_Achievement_Dynamic (Utilities|Array|Get(acopy) AchievementsData _array_index))) "NewEnumerator0") ; Hide all unfished achievements.
    (Utilities|FlowControl|Sequence
      (:then_0
        ;[0.1 0.1 0.1 1 14] Show these unfinished achievements that are visible by default.
        (for _array_element_2 (.UnfinishedAchievements (Utilities|Struct|BreakS_RPG_Achievement_Dynamic (Utilities|Array|Get(acopy) AchievementsData _array_index)))
          (bind _returnvalue (Utilities|GetDataTableRow "/Game/SuperiorRPGKit/Datatables/DT_RPG_Achievements.DT_RPG_Achievements" _array_element_2)
            (:then
              (if (.VisibleByDefault (Utilities|Struct|BreakS_RPG_Achievement_Static _returnvalue))
                (CallFunction|SetAchievementsStateCLIENT (Utilities|Array|MakeArray _array_element_2) "NewEnumerator1"))))))
      (:then_1
        ;[0.1 0.1 0.1 1 14] Show all finishable achievements and these which are unlocked by them
        (CallFunction|SetAchievementsStateCLIENT (.FinishableAchievements (Utilities|Struct|BreakS_RPG_Achievement_Dynamic (Utilities|Array|Get(acopy) AchievementsData _array_index))) "NewEnumerator2")
        (for _array_element_3 (.FinishableAchievements (Utilities|Struct|BreakS_RPG_Achievement_Dynamic (Utilities|Array|Get(acopy) AchievementsData _array_index)))
          (bind _returnvalue_2 (Utilities|GetDataTableRow "/Game/SuperiorRPGKit/Datatables/DT_RPG_Achievements.DT_RPG_Achievements" _array_element_3)
            (:then
              (bind _result (Utilities|Set|ToArray (Utilities|Struct|BreakS_RPG_Achievement_Static _returnvalue_2)))
              (CallFunction|SetAchievementsStateCLIENT _result "NewEnumerator1")))))
      (:then_2
        ;[0.1 0.1 0.1 1 14] Show all finished achievements and these which are unlocked by them.
        (CallFunction|SetAchievementsStateCLIENT (.ClaimedAchievements (Utilities|Struct|BreakS_RPG_Achievement_Dynamic (Utilities|Array|Get(acopy) AchievementsData _array_index))) "NewEnumerator3")
        (for _array_element_4 (.ClaimedAchievements (Utilities|Struct|BreakS_RPG_Achievement_Dynamic (Utilities|Array|Get(acopy) AchievementsData _array_index)))
          (bind _returnvalue_3 (Utilities|GetDataTableRow "/Game/SuperiorRPGKit/Datatables/DT_RPG_Achievements.DT_RPG_Achievements" _array_element_4)
            (:then
              (bind _result_2 (Utilities|Set|ToArray (Utilities|Struct|BreakS_RPG_Achievement_Static _returnvalue_3)))
              (CallFunction|SetAchievementsStateCLIENT _result_2 "NewEnumerator1"))))))))

(event Custom|RefreshAchievementProgress_CLIENT
  (params (ObjectiveType :type E_RPG_AchievementObjective%20Enum :default "NewEnumerator4") (Progress :type Integer))
  ;[0.1 0.1 0.1 1 12] Update displayed achievement progress.
  (for _array_element (Variables|Default|GetWidgetsToRefresh)
    (Class|BPIRPGAchievementsUpdater|UpdateAchievementsProgressinWindow(Message) _array_element ObjectiveType Progress)))

(event Custom|SetAchievementsState_CLIENT
  (params (Achievements :type Array%20of%20Names) (State :type E_RPG_AchievementState%20Enum :default "NewEnumerator0"))
  ;[0.1 0.1 0.1 1 12] Set visibility for achievement slot.
  (for _array_element (Variables|Default|GetWidgetsToRefresh)
    (for _array_element_2 Achievements
      (Class|BPIRPGAchievementsUpdater|SetAchievementStateinWindow(Message) _array_element _array_element_2 State))))

(event Custom|ClaimAchievementReward_SERVER
  (params (ObjectiveGroup :type E_RPG_AchievementObjective%20Enum%20%28by%20ref%29 :default "NewEnumerator4") (AchievementID :type Name))
  ;[0.1 0.1 0.1 1 14] Finish achievement and get its reward.
  (if (Utilities|Array|ContainsItem (.FinishableAchievements (Utilities|Struct|BreakS_RPG_Achievement_Dynamic (.Value (Utilities|Map|Find (Variables|Default|GetAchievementsProgress) ObjectiveGroup)))) AchievementID) ; Check fi achievement can be finished
    (Management|FinishAchievement AchievementID)))

(fn AddAchievementsProgress
  (params (ObjectiveType :type E_RPG_AchievementObjective%20Enum :default "NewEnumerator4") (Progress :type Integer))
  ;[0.1 0.1 0.1 1 14] Increase progress of given achievement objective.
  (LocalVariables|SetObjectiveTypeLOCAL ObjectiveType)
  (bind _output_get (LocalVariables|SetNewProgressLOCAL (+ (.CurrentProgress (Utilities|Struct|BreakS_RPG_Achievement_Dynamic (.Value (Utilities|Map|Find (Variables|Default|GetAchievementsProgress) (LocalVariables|GetObjectiveTypeLOCAL))))) Progress)))
  (bind _structout (Utilities|Struct|SetmembersinS_RPG_Achievement_Dynamic (.Value (Utilities|Map|Find (Variables|Default|GetAchievementsProgress) (LocalVariables|GetObjectiveTypeLOCAL))) _output_get))
  (Utilities|Map|Add (Variables|Default|GetAchievementsProgress) (LocalVariables|GetObjectiveTypeLOCAL) _structout)
  ;[0.1 0.1 0.1 1 14] Check if any of unfinished achievements has been completed after new progress increment.
  (for _array_element (.UnfinishedAchievements (Utilities|Struct|BreakS_RPG_Achievement_Dynamic (.Value (Utilities|Map|Find (Variables|Default|GetAchievementsProgress) (LocalVariables|GetObjectiveTypeLOCAL)))))
    (bind _returnvalue (Utilities|GetDataTableRow "/Game/SuperiorRPGKit/Datatables/DT_RPG_Achievements.DT_RPG_Achievements" _array_element)
      (:then
        (if (<= (.RequiredProgress (Utilities|Struct|BreakS_RPG_Achievement_Static _returnvalue)) (LocalVariables|GetNewProgressLOCAL))
          (Management|MarkAchievementasFinishable _array_element)
          (CallFunction|RefreshAchievementProgressCLIENT (LocalVariables|GetObjectiveTypeLOCAL) (LocalVariables|GetNewProgressLOCAL))
          (else
            (CallFunction|RefreshAchievementProgressCLIENT (LocalVariables|GetObjectiveTypeLOCAL) (LocalVariables|GetNewProgressLOCAL))))))))

(fn FinishAchievement
  (params (AchievementID :type Name))
  (LocalVariables|SetAchievementLOCAL AchievementID)
  (bind _returnvalue (Utilities|GetDataTableRow "/Game/SuperiorRPGKit/Datatables/DT_RPG_Achievements.DT_RPG_Achievements" (LocalVariables|GetAchievementLOCAL))
    (:then
      (LocalVariables|SetAchievementProgressLOCAL (.Value (Utilities|Map|Find (Variables|Default|GetAchievementsProgress) (.ObjectiveType (Utilities|Struct|BreakS_RPG_Achievement_Static _returnvalue)))))
      (LocalVariables|SetFinishableAchievementsLOCAL (.FinishableAchievements (Utilities|Struct|BreakS_RPG_Achievement_Dynamic (LocalVariables|GetAchievementProgressLOCAL))))
      (LocalVariables|SetCompletedAchievementsLOCAL (.ClaimedAchievements (Utilities|Struct|BreakS_RPG_Achievement_Dynamic (LocalVariables|GetAchievementProgressLOCAL))))
      (CallFunction|SetAchievementsStateCLIENT (Utilities|Array|MakeArray (LocalVariables|GetAchievementLOCAL)) "NewEnumerator3")
      (Utilities|Array|RemoveItem (LocalVariables|GetFinishableAchievementsLOCAL) (LocalVariables|GetAchievementLOCAL))
      (Utilities|Array|AddUnique (LocalVariables|GetCompletedAchievementsLOCAL) (LocalVariables|GetAchievementLOCAL))
      (bind _structout (Utilities|Struct|SetmembersinS_RPG_Achievement_Dynamic (LocalVariables|GetAchievementProgressLOCAL) (LocalVariables|GetFinishableAchievementsLOCAL) (LocalVariables|GetCompletedAchievementsLOCAL)))
      (Utilities|Map|Add (Variables|Default|GetAchievementsProgress) (.ObjectiveType (Utilities|Struct|BreakS_RPG_Achievement_Static _returnvalue)) _structout)
      (Management|ReceiveAchievementReward (LocalVariables|GetAchievementLOCAL)))))

(fn ReceiveAchievementReward
  (params (AchievementID :type Name))
  (bind _returnvalue (Components|GetOwner))
  (bind _returnvalue_2 (Actor|GetComponentbyClass _returnvalue "/Game/SuperiorRPGKit/Blueprints/Components/AC_RPG_ItemsManager.AC_RPG_ItemsManager_C"))
  (bind _returnvalue_3 (Utilities|GetDataTableRow "/Game/SuperiorRPGKit/Datatables/DT_RPG_Achievements.DT_RPG_Achievements" AchievementID)
    (:then
      (Utilities|FlowControl|Sequence
        (:then_0
          ;[0.1 0.1 0.1 1 14] Grant gold.
          (if (> (.Gold (Utilities|Struct|BreakS_RPG_AchievementReward (.Reward (Utilities|Struct|BreakS_RPG_Achievement_Static _returnvalue_3)))) 0)
            (Default|ModifyGoldAmount _returnvalue_2 (Variables|/Game/SuperiorRPGKit/Blueprints/Components/AC_RPG_ItemsManager.AC_RPG_ItemsManager_C|GetInventoryContainer _returnvalue_2) (.Gold (Utilities|Struct|BreakS_RPG_AchievementReward (.Reward (Utilities|Struct|BreakS_RPG_Achievement_Static _returnvalue_3)))))))
        (:then_1
          ;[0.1 0.1 0.1 1 14] Grant XP.
          (if (> (.XP (Utilities|Struct|BreakS_RPG_AchievementReward (.Reward (Utilities|Struct|BreakS_RPG_Achievement_Static _returnvalue_3)))) 0)
            (Default|ReceiveExperience (Actor|GetComponentbyClass (Components|GetOwner) "/Game/SuperiorRPGKit/Blueprints/Components/AC_RPG_StatsManager.AC_RPG_StatsManager_C") (.XP (Utilities|Struct|BreakS_RPG_AchievementReward (.Reward (Utilities|Struct|BreakS_RPG_Achievement_Static _returnvalue_3)))))))))))

(fn InitializeAchievementsManager
  ;[0.1 0.1 0.1 1 14] Add all achievements to AchievementsProgress map.
  (bind _outrownames (DataTable|GetDataTableRowNames "/Game/SuperiorRPGKit/Datatables/DT_RPG_Achievements.DT_RPG_Achievements"))
  (for _array_element _outrownames
    (bind _returnvalue (Utilities|GetDataTableRow "/Game/SuperiorRPGKit/Datatables/DT_RPG_Achievements.DT_RPG_Achievements" _array_element)
      (:then
        (LocalVariables|SetUnfinishedQuestsLOCAL (.UnfinishedAchievements (Utilities|Struct|BreakS_RPG_Achievement_Dynamic (.Value (Utilities|Map|Find (Variables|Default|GetAchievementsProgress) (.ObjectiveType (Utilities|Struct|BreakS_RPG_Achievement_Static _returnvalue)))))))
        (Utilities|Array|Add (LocalVariables|GetUnfinishedQuestsLOCAL) _array_element)
        (bind _structout (Utilities|Struct|SetmembersinS_RPG_Achievement_Dynamic (.Value (Utilities|Map|Find (Variables|Default|GetAchievementsProgress) (.ObjectiveType (Utilities|Struct|BreakS_RPG_Achievement_Static _returnvalue)))) (LocalVariables|GetUnfinishedQuestsLOCAL)))
        (Utilities|Map|Add (Variables|Default|GetAchievementsProgress) (.ObjectiveType (Utilities|Struct|BreakS_RPG_Achievement_Static _returnvalue)) _structout))))
  (CallFunction|InitializeAchievementsWindowCLIENT) ; Updates widgets on client.
)

(fn AddWidgetstoRefresh
  (params (WidgetsToRefresh :type Array%20of%20User%20Widget%20Object%20References))
  (for _array_element WidgetsToRefresh
    (Utilities|Array|AddUnique (Variables|Default|GetWidgetsToRefresh) _array_element)
    (Class|BPIRPGAchievementsUpdater|SetAchievementsManagerReference(Message) _array_element self)))

(fn GetAchievementsDatatoSave
  (bind _achievementsprogress (Variables|Default|GetAchievementsProgress))
  (bind _values (Utilities|Map|Values _achievementsprogress))
  (bind _keys (Utilities|Map|Keys _achievementsprogress))
  (return _keys _values))

(fn LoadAchievementsData
  (params (Achievements :type Array%20of%20E_RPG_AchievementObjective%20Enums :default "NewEnumerator4") (AchievementsProgress :type Array%20of%20S%20RPG%20Achievement%20Dynamic%20Structures))
  (for (_array_element _array_index) Achievements
    (Utilities|Map|Add (Variables|Default|GetAchievementsProgress) _array_element (Utilities|Array|Get(acopy) AchievementsProgress _array_index)))
  (CallFunction|ReloadAchievementsWindowCLIENT Achievements AchievementsProgress))

(fn MarkAchievementasFinishable
  (params (AchievementID :type Name))
  (bind _output_get (LocalVariables|SetAchievementLOCAL AchievementID))
  (bind _returnvalue (Utilities|GetDataTableRow "/Game/SuperiorRPGKit/Datatables/DT_RPG_Achievements.DT_RPG_Achievements" _output_get)
    (:then
      (LocalVariables|SetAchievementProgressLOCAL (.Value (Utilities|Map|Find (Variables|Default|GetAchievementsProgress) (.ObjectiveType (Utilities|Struct|BreakS_RPG_Achievement_Static _returnvalue)))))
      (LocalVariables|SetUnfinishedAchievementsLOCAL (.UnfinishedAchievements (Utilities|Struct|BreakS_RPG_Achievement_Dynamic (LocalVariables|GetAchievementProgressLOCAL))))
      (LocalVariables|SetFinishableAchievementsLOCAL (.FinishableAchievements (Utilities|Struct|BreakS_RPG_Achievement_Dynamic (LocalVariables|GetAchievementProgressLOCAL))))
      (bind _result (Utilities|Set|ToArray (.AchievementsToShowOnFinished (Utilities|Struct|BreakS_RPG_Achievement_Static _returnvalue))))
      (CallFunction|SetAchievementsStateCLIENT _result "NewEnumerator1")
      (CallFunction|SetAchievementsStateCLIENT (Utilities|Array|MakeArray (LocalVariables|GetAchievementLOCAL)) "NewEnumerator2")
      (Utilities|Array|RemoveItem (LocalVariables|GetUnfinishedAchievementsLOCAL) (LocalVariables|GetAchievementLOCAL))
      (Utilities|Array|AddUnique (LocalVariables|GetFinishableAchievementsLOCAL) (LocalVariables|GetAchievementLOCAL))
      (bind _structout (Utilities|Struct|SetmembersinS_RPG_Achievement_Dynamic (LocalVariables|GetAchievementProgressLOCAL) (LocalVariables|GetUnfinishedAchievementsLOCAL) (LocalVariables|GetFinishableAchievementsLOCAL)))
      (Utilities|Map|Add (Variables|Default|GetAchievementsProgress) (.ObjectiveType (Utilities|Struct|BreakS_RPG_Achievement_Static _returnvalue)) _structout))))