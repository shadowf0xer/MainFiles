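; AC_RPG_Container is an RPG item container component for inventory, vendor or stash, with functions to save and load its contents.
; GetContainerDataToSave returns the ItemsList map as slot and item arrays, plus gold.
; LoadContainerData sets gold, then for each accessing actor's ItemsManager refreshes gold, blanks displayed slots, adds loaded items to the map and resends them by container type.
; The map is filled inside that actor loop and never cleared.
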(fn LoadContainerData
  (params (ItemSlots :type Array%20of%20Integers) (ItemsData :type Array%20of%20S%20RPG%20Item%20Dynamic%20Structures) (Gold :type Integer))
  (bind _itemslist (Variables|Default|GetItemsList))
  (bind _itemslist_2 (Variables|Default|GetItemsList))
  (bind _itemslist_3 (Variables|Default|GetItemsList))
  (Variables|Default|SetGold Gold)
  (for _array_element (Variables|Default|GetActorsAccessingContainer)
    (Utilities|IsValid (Actor|GetComponentbyClass _array_element "/Game/SuperiorRPGKit/Blueprints/Components/AC_RPG_ItemsManager.AC_RPG_ItemsManager_C")
      (:Is%20Valid
        (Default|ModifyGoldAmount (Actor|GetComponentbyClass _array_element "/Game/SuperiorRPGKit/Blueprints/Components/AC_RPG_ItemsManager.AC_RPG_ItemsManager_C") self) ; (FORCED) Update gold amount displayed on client side
        (Utilities|FlowControl|Sequence
          (:then_0
            ;[0.1 0.1 0.1 1 12] Clear displayed items in container before new list is sent.
            (switch Utilities|FlowControl|Switch|SwitchonE_RPG_ContainerType (Variables|Config|GetContainerType)
              (:NewEnumerator0
                (bind _keys (Utilities|Map|Keys (Variables|Default|GetItemsList)))
                (Default|RefreshInventoryItemSlotsGroupCLIENT (Actor|GetComponentbyClass _array_element "/Game/SuperiorRPGKit/Blueprints/Components/AC_RPG_ItemsManager.AC_RPG_ItemsManager_C") _keys (Utilities|Array|MakeArray)))
              (:NewEnumerator3
                (bind _keys_2 (Utilities|Map|Keys (Variables|Default|GetItemsList)))
                (Default|RefreshVendorItemSlotsGroupCLIENT (Actor|GetComponentbyClass _array_element "/Game/SuperiorRPGKit/Blueprints/Components/AC_RPG_ItemsManager.AC_RPG_ItemsManager_C") _keys_2 (Utilities|Array|MakeArray)))
              (:NewEnumerator4
                (bind _keys_3 (Utilities|Map|Keys (Variables|Default|GetItemsList)))
                (Default|RefreshStashItemSlotsGroupCLIENT (Actor|GetComponentbyClass _array_element "/Game/SuperiorRPGKit/Blueprints/Components/AC_RPG_ItemsManager.AC_RPG_ItemsManager_C") _keys_3 (Utilities|Array|MakeArray)))))
          (:then_1
            ;[0.1 0.1 0.1 1 14] Reconstruct items map.
            (for (_array_element_2 _array_index) ItemSlots
              (Utilities|Map|Add (Variables|Default|GetItemsList) _array_element_2 (Utilities|Array|Get(acopy) ItemsData _array_index))))
          (:then_2
            ;[0.1 0.1 0.1 1 14] Update containers widgets.
            (switch Utilities|FlowControl|Switch|SwitchonE_RPG_ContainerType (Variables|Config|GetContainerType)
              (:NewEnumerator0
                (bind _keys_4 (Utilities|Map|Keys _itemslist))
                (bind _values (Utilities|Map|Values _itemslist))
                (Default|RefreshInventoryItemSlotsGroupCLIENT (Actor|GetComponentbyClass _array_element "/Game/SuperiorRPGKit/Blueprints/Components/AC_RPG_ItemsManager.AC_RPG_ItemsManager_C") _keys_4 _values))
              (:NewEnumerator3
                (bind _keys_5 (Utilities|Map|Keys _itemslist_3))
                (bind _values_2 (Utilities|Map|Values _itemslist_3))
                (Default|RefreshVendorItemSlotsGroupCLIENT (Actor|GetComponentbyClass _array_element "/Game/SuperiorRPGKit/Blueprints/Components/AC_RPG_ItemsManager.AC_RPG_ItemsManager_C") _keys_5 _values_2))
              (:NewEnumerator4
                (bind _keys_6 (Utilities|Map|Keys _itemslist_2))
                (bind _values_3 (Utilities|Map|Values _itemslist_2))
                (Default|RefreshStashItemSlotsGroupCLIENT (Actor|GetComponentbyClass _array_element "/Game/SuperiorRPGKit/Blueprints/Components/AC_RPG_ItemsManager.AC_RPG_ItemsManager_C") _keys_6 _values_3)))))))))

(fn GetContainerDatatoSave
  (bind _itemslist (Variables|Default|GetItemsList))
  (bind _values (Utilities|Map|Values _itemslist))
  (bind _keys (Utilities|Map|Keys _itemslist))
  (return _keys _values (Variables|Default|GetGold)))