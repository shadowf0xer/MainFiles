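; Crafting manager component that lets players craft unlocked items defined in DT_RPG_Craftables from inventory materials.
; A server event checks unlock state, space and materials, then swaps materials for the crafted item with rolled quality through the linked items manager.
; Non-dedicated instances build grouped slot widgets in the crafting canvas, collapsing locked ones until a client event reveals them.
; Unlocked craftables start from table defaults and support save and load.
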(event Custom|RefreshCraftableItem_CLIENT
  (params (CraftableID :type Name))
  ;[0.1 0.1 0.1 1 12] Make Craftable Item visible in crafting window.
  (Utilities|Array|AddUnique (Variables|Default|GetUnlockedCraftables) CraftableID)
  (bind _array_element (Utilities|Array|ForEachLoopwithBreak (Variables|References|GetCraftingSlots) :!label _label)
    (:LoopBody
      (if (Utilities|Name|Equal(Name) (Variables|/Game/SuperiorRPGKit/Widgets/Crafting/WBP_RPG_CraftingSlot.WBP_RPG_CraftingSlot_C|GetAssignedCraftable _array_element) CraftableID)
        (Widget|SetVisibility _array_element "Visible")
        (goto _label Break)))))

(event Custom|CraftItem_SERVER
  (params (CraftableID :type Name))
  (bind _associateditemsmanager (Variables|References|GetAssociatedItemsManager))
  (bind _associateditemsmanager_2 (Variables|References|GetAssociatedItemsManager))
  ;[0.1 0.1 0.1 1 12] Inform the server that client wants to craft item.
  (if (Conditions|CanCraftItem CraftableID)
    (bind _returnvalue (Utilities|GetDataTableRow "/Game/SuperiorRPGKit/Datatables/DT_RPG_Craftables.DT_RPG_Craftables" CraftableID)
      (:then
        (bind _keys (Utilities|Map|Keys (.RequiredMaterials (Utilities|Struct|BreakS_RPG_Craftable_Static _returnvalue))))
        (for _array_element _keys
          (Default|RemoveItemfromContainer _associateditemsmanager_2 (Variables|/Game/SuperiorRPGKit/Blueprints/Components/AC_RPG_ItemsManager.AC_RPG_ItemsManager_C|GetInventoryContainer _associateditemsmanager_2) _array_element (.Value (Utilities|Map|Find (.RequiredMaterials (Utilities|Struct|BreakS_RPG_Craftable_Static _returnvalue)) _array_element)) false false))
        (Default|AddItemtoContainer(byID) _associateditemsmanager (Variables|/Game/SuperiorRPGKit/Blueprints/Components/AC_RPG_ItemsManager.AC_RPG_ItemsManager_C|GetInventoryContainer _associateditemsmanager) CraftableID (CallFunction|RollItemQuality CraftableID) (.CraftedAmount (Utilities|Struct|BreakS_RPG_Craftable_Static _returnvalue)) true)))))

(fn InitializeCraftingWindow
  (params (ItemsManager :type AC%20RPG%20Items%20Manager%20Object%20Reference))
  (Variables|References|SetAssociatedItemsManager ItemsManager)
  ;[0.1 0.1 0.1 1 14] Add all craftables unlocked by default to athe pool of unlocked craftables.
  (bind _outrownames (DataTable|GetDataTableRowNames "/Game/SuperiorRPGKit/Datatables/DT_RPG_Craftables.DT_RPG_Craftables"))
  (for _array_element _outrownames
    (bind _returnvalue (Utilities|GetDataTableRow "/Game/SuperiorRPGKit/Datatables/DT_RPG_Craftables.DT_RPG_Craftables" _array_element)
      (:then
        (if (Utilities|Struct|BreakS_RPG_Craftable_Static _returnvalue)
          (Utilities|Array|AddUnique (Variables|Default|GetUnlockedCraftables) _array_element)))))
  (if (not (Networking|IsDedicatedServer)) ; Widgets part is executed\nonly on listen server(host) or clients.
    (Utilities|FlowControl|Sequence
      (:then_0
        ;[0.1 0.1 0.1 1 14] Set initial CraftingCanvas widget reference.
        (bind _foundwidgets (Widget|GetAllWidgetsOfClass "/Game/SuperiorRPGKit/Widgets/Crafting/WBP_RPG_CraftingCanvas.WBP_RPG_CraftingCanvas_C" false))
        (Variables|References|SetCraftingCanvas (Utilities|Array|Get(acopy) _foundwidgets))
        (Utilities|IsValid (Variables|References|GetCraftingCanvas)
          (:Is%20Valid
            ;[0.1 0.1 0.1 1 14] Create slot for each craftable item and add it to crafting window. Craftables that are not unlocked by default are hidden.
            (bind _outrownames_2 (DataTable|GetDataTableRowNames "/Game/SuperiorRPGKit/Datatables/DT_RPG_Craftables.DT_RPG_Craftables"))
            (for _array_element_2 _outrownames_2
              (bind _returnvalue_2 (Utilities|GetDataTableRow "/Game/SuperiorRPGKit/Datatables/DT_RPG_Craftables.DT_RPG_Craftables" _array_element_2)
                (:then
                  (bind _slot (Getters|GetProperCraftingGroupSlot (.CraftingGroup (Utilities|Struct|BreakS_RPG_Craftable_Static _returnvalue_2))))
                  (bind _returnvalue_3 (UserInterface|CreateWidget "/Game/SuperiorRPGKit/Widgets/Crafting/WBP_RPG_CraftingSlot.WBP_RPG_CraftingSlot_C" 0 self))
                  (Utilities|Array|Add (Variables|References|GetCraftingSlots) _returnvalue_3)
                  (Default|SetCraftableData _returnvalue_3 (.ID (Utilities|Struct|BreakS_RPG_Craftable_Static _returnvalue_2)))
                  (Widget|Panel|AddChild (Variables|/Game/SuperiorRPGKit/Widgets/Crafting/WBP_RPG_CraftingGroupSlot.WBP_RPG_CraftingGroupSlot_C|GetContainer_CraftingSlots _slot) _returnvalue_3)
                  (Layout|BorderSlot|SetPadding _returnvalue_3 (Utilities|Struct|MakeMargin 0.0 2.0 0.0 0.0) :!class /Script/UMG.UserWidget)
                  (Widget|SetVisibility _returnvalue_3 (select (.UnlockedByDefault (Utilities|Struct|BreakS_RPG_Craftable_Static _returnvalue_2)) "SelfHitTestInvisible" "Collapsed"))))))
          (:Is%20Not%20Valid
            (Development|PrintString "Couldn't find CraftingCanvas widget. Make sure you added one to you UI." true true "(R=1.000000,G=0.500000,B=0.000000,A=1.000000)" 4.0))))
      (:then_1
        ;[0.1 0.1 0.1 1 14] Set initial CraftingInfo widget references.
        (bind _foundwidgets_2 (Widget|GetAllWidgetsOfClass "/Game/SuperiorRPGKit/Widgets/Crafting/WBP_RPG_CraftingInfo.WBP_RPG_CraftingInfo_C" false))
        (Variables|References|SetCraftingInfo (Utilities|Array|Get(acopy) _foundwidgets_2))
        (Utilities|IsValid (Variables|References|GetCraftingCanvas)
          (:Is%20Valid
            (Variables|/Game/SuperiorRPGKit/Widgets/Crafting/WBP_RPG_CraftingInfo.WBP_RPG_CraftingInfo_C|SetCraftingManager (Variables|References|GetCraftingInfo) self))
          (:Is%20Not%20Valid
            (Development|PrintString "Couldn't find CraftingInfo widget. Make sure you added one to you UI." true true "(R=1.000000,G=0.500000,B=0.000000,A=1.000000)" 4.0)))))))

(fn GetProperCraftingGroupSlot
  (params (CraftingGroup :type E_RPG_CraftingGroup%20Enum :default "NewEnumerator0"))
  (bind _craftinggroupslots (Variables|References|GetCraftingGroupSlots))
  (bind (_value _returnvalue) (Utilities|Map|Find _craftinggroupslots CraftingGroup))
  (if _returnvalue
    (return _value)
    (else
      ;[0.1 0.1 0.1 1 12] If is not created then add it to CraftingCanvas widget.
      (bind _returnvalue_2 (UserInterface|CreateWidget "/Game/SuperiorRPGKit/Widgets/Crafting/WBP_RPG_CraftingGroupSlot.WBP_RPG_CraftingGroupSlot_C" 0 CraftingGroup self))
      (Utilities|Map|Add (Variables|References|GetCraftingGroupSlots) CraftingGroup _returnvalue_2)
      (bind _returnvalue_3 (Class|VerticalBox|AddChildtoVerticalBox (Variables|/Game/SuperiorRPGKit/Widgets/Crafting/WBP_RPG_CraftingCanvas.WBP_RPG_CraftingCanvas_C|GetContainer_CraftingGroups (Variables|References|GetCraftingCanvas)) _returnvalue_2))
      (Layout|BorderSlot|SetPadding _returnvalue_3 (Utilities|Struct|MakeMargin 0.0 4.0 0.0 0.0) :!class /Script/UMG.VerticalBoxSlot)
      (return _returnvalue_2))))

(fn InitializeCraftingManager
  (params (AssociatedItemsManager :type AC%20RPG%20Items%20Manager%20Object%20Reference))
  (Variables|References|SetAssociatedItemsManager AssociatedItemsManager) ; Store ItemsManager reference.
  ;[0.1 0.1 0.1 1 14] Add all craftables unlocked by default to athe pool of unlocked craftables.
  (bind _outrownames (DataTable|GetDataTableRowNames "/Game/SuperiorRPGKit/Datatables/DT_RPG_Craftables.DT_RPG_Craftables"))
  (for _array_element _outrownames
    (bind _returnvalue (Utilities|GetDataTableRow "/Game/SuperiorRPGKit/Datatables/DT_RPG_Craftables.DT_RPG_Craftables" _array_element)
      (:then
        (if (Utilities|Struct|BreakS_RPG_Craftable_Static _returnvalue)
          (Utilities|Array|AddUnique (Variables|Default|GetUnlockedCraftables) _array_element))))))

(fn ShowCraftingInfo
  (params (CraftableID :type Name))
  (bind _returnvalue (Utilities|GetDataTableRow "/Game/SuperiorRPGKit/Datatables/DT_RPG_Craftables.DT_RPG_Craftables" CraftableID)
    (:then
      (Default|SetCraftableData (Variables|References|GetCraftingInfo) (.ID (Utilities|Struct|BreakS_RPG_Craftable_Static _returnvalue)) (.RequiredMaterials (Utilities|Struct|BreakS_RPG_Craftable_Static _returnvalue)))
      (Widget|SetVisibility (Variables|References|GetCraftingInfo) "SelfHitTestInvisible"))))

(fn CanCraftItem
  (params (ItemID :type Name))
  (bind _associateditemsmanager (Variables|References|GetAssociatedItemsManager))
  (bind _associateditemsmanager_2 (Variables|References|GetAssociatedItemsManager))
  (if (Utilities|Array|ContainsItem (Variables|Default|GetUnlockedCraftables) ItemID) ; Is craftable unlocked?
    (bind _enoughspace_ (Default|IsThereEnoughSpaceinContainerforItems _associateditemsmanager_2 (Variables|/Game/SuperiorRPGKit/Blueprints/Components/AC_RPG_ItemsManager.AC_RPG_ItemsManager_C|GetInventoryContainer _associateditemsmanager_2) (Utilities|Array|MakeArray ItemID)))
    (if _enoughspace_
      (bind _returnvalue (Utilities|GetDataTableRow "/Game/SuperiorRPGKit/Datatables/DT_RPG_Craftables.DT_RPG_Craftables" ItemID)
        (:then
          (bind _keys (Utilities|Map|Keys (Utilities|Struct|BreakS_RPG_Craftable_Static _returnvalue)))
          ;[0.1 0.1 0.1 1 12] Check if any required material is missing.
          (bind _array_element (Utilities|Array|ForEachLoopwithBreak _keys :!label _label)
            (:LoopBody
              (bind _totalamount (Default|GetTotalAmountOfIteminContainer _associateditemsmanager (Variables|/Game/SuperiorRPGKit/Blueprints/Components/AC_RPG_ItemsManager.AC_RPG_ItemsManager_C|GetInventoryContainer _associateditemsmanager) _array_element))
              (if (< _totalamount (.Value (Utilities|Map|Find (Utilities|Struct|BreakS_RPG_Craftable_Static _returnvalue) _array_element)))
                (LocalVariables|SetResultLOCAL false)
                (Development|PrintString (Utilities|String|Append "Can't craft." "Lack of material: " (Utilities|String|ToString(Name) _array_element)) true true "(R=1.000000,G=0.500000,B=0.000000,A=1.000000)" 4.0)
                (goto _label Break)))
            (:Completed
              (return (LocalVariables|GetResultLOCAL))))))
      (else
        (Development|PrintString "Can't craft. Not enough space in inventory." true true "(R=1.000000,G=0.500000,B=0.000000,A=1.000000)" 4.0)
        (return false)))
    (else
      (Development|PrintString "Can't craft. Craftable is not unlocked." true true "(R=1.000000,G=0.500000,B=0.000000,A=1.000000)" 4.0)
      (return false))))

(fn UnlockCraftable
  (params (CraftableID :type Name))
  (if (not (Utilities|Array|ContainsItem (Variables|Default|GetUnlockedCraftables) CraftableID))
    (Utilities|Array|Add (Variables|Default|GetUnlockedCraftables) CraftableID)
    (CallFunction|RefreshCraftableItemCLIENT CraftableID)))

(fn GetCraftingDatatoSave
  (return (Variables|Default|GetUnlockedCraftables)))

(fn LoadCraftingData
  (params (UnlockedCraftables :type Array%20of%20Names))
  (for _array_element UnlockedCraftables
    (Utilities|Array|AddUnique (Variables|Default|GetUnlockedCraftables) _array_element)
    (CallFunction|RefreshCraftableItemCLIENT _array_element)))