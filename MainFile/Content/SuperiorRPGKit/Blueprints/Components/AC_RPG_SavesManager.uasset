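; Actor component that saves and loads an RPG hero's progression and tracks the active respawn point.
; SaveHero gathers data from the owner's manager components, plus map and respawn ID, into a save slot.
; LoadHero reads the slot and uploads each category through server events, optionally grants data-table starter items, then recalculates stats.
; Respawn activation refreshes the client and records a global spawn ID in the GameInstance for joining players.
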(event Custom|UploadEquipmentSaveData_SERVER
  (params (EquippedItemSlots :type Array%20of%20Integers) (EquippedItemsData :type Array%20of%20S%20RPG%20Item%20Dynamic%20Structures))
  (Default|LoadEquipmentData (Variables|/Game/SuperiorRPGKit/Blueprints/Components/AC_RPG_ItemsManager.AC_RPG_ItemsManager_C|GetEquipment (Actor|GetComponentbyClass (Components|GetOwner) "/Game/SuperiorRPGKit/Blueprints/Components/AC_RPG_ItemsManager.AC_RPG_ItemsManager_C")) EquippedItemSlots EquippedItemsData))

(event Custom|UploadStatsSaveData_SERVER
  (params (CurrentStats :type Array%20of%20E_RPG_StatType%20Enums :default "NewEnumerator0") (CurrentStatsValues :type Array%20of%20Floats%20%28single-precision%29) (Attributes :type Array%20of%20E_RPG_AttributeType%20Enums :default "NewEnumerator4") (AttributesInvestedPoints :type Array%20of%20Integers) (TotalAttributePointsSpent :type Integer) (AvailableAttributePoints :type Integer) (CurrentLevel :type Integer) (CurrentExperience :type Integer))
  (Default|LoadStatsData (Actor|GetComponentbyClass (Components|GetOwner) "/Game/SuperiorRPGKit/Blueprints/Components/AC_RPG_StatsManager.AC_RPG_StatsManager_C") CurrentStats CurrentStatsValues Attributes AttributesInvestedPoints TotalAttributePointsSpent AvailableAttributePoints CurrentLevel CurrentExperience))

(event Custom|UploadAchievementsSaveData_SERVER
  (params (Achievements :type Array%20of%20E_RPG_AchievementObjective%20Enums :default "NewEnumerator4") (AchievementsProgress :type Array%20of%20S%20RPG%20Achievement%20Dynamic%20Structures))
  (Default|LoadAchievementsData (Actor|GetComponentbyClass (Components|GetOwner) "/Game/SuperiorRPGKit/Blueprints/Components/AC_RPG_AchievementsManager.AC_RPG_AchievementsManager_C") Achievements AchievementsProgress))

(event Custom|UploadPerksSaveData_SERVER
  (params (Perks :type Array%20of%20E_RPG_PerkType%20Enums :default "NewEnumerator4") (PerksLevels :type Array%20of%20Integers) (TotalPerkPointsSpent :type Integer) (AvailablePerkPoints :type Integer))
  (Default|LoadPerksData (Actor|GetComponentbyClass (Components|GetOwner) "/Game/SuperiorRPGKit/Blueprints/Components/AC_RPG_StatsManager.AC_RPG_StatsManager_C") Perks PerksLevels TotalPerkPointsSpent AvailablePerkPoints))

(event Custom|AddStarterStuff_SERVER
  (params (Add :type Boolean) (HeroID :type Name))
  (bind _returnvalue (Components|GetOwner))
  (bind _returnvalue_2 (Components|GetOwner))
  (bind _returnvalue_3 (Components|GetOwner))
  (bind _returnvalue_4 (Actor|GetComponentbyClass _returnvalue "/Game/SuperiorRPGKit/Blueprints/Components/AC_RPG_ItemsManager.AC_RPG_ItemsManager_C"))
  (bind _returnvalue_5 (Actor|GetComponentbyClass _returnvalue_2 "/Game/SuperiorRPGKit/Blueprints/Components/AC_RPG_ItemsManager.AC_RPG_ItemsManager_C"))
  (bind _returnvalue_6 (Actor|GetComponentbyClass _returnvalue_3 "/Game/SuperiorRPGKit/Blueprints/Components/AC_RPG_ItemsManager.AC_RPG_ItemsManager_C"))
  (if Add
    (bind _returnvalue_7 (Utilities|GetDataTableRow "/Game/SuperiorRPGKit/Datatables/DT_RPG_Heroes.DT_RPG_Heroes" HeroID)
      (:then
        (Utilities|FlowControl|Sequence
          (:then_0
            ;[0.1 0.1 0.1 1 14] Add starter equipment.
            (bind _keys (Utilities|Map|Keys (.StarterEquipment (Utilities|Struct|BreakS_RPG_Hero_Static _returnvalue_7))))
            (for _array_element _keys
              (Default|EquipItem _returnvalue_6 _array_element (.Value (Utilities|Map|Find (.StarterEquipment (Utilities|Struct|BreakS_RPG_Hero_Static _returnvalue_7)) _array_element)) (Variables|/Game/SuperiorRPGKit/Blueprints/Components/AC_RPG_ItemsManager.AC_RPG_ItemsManager_C|GetEquipment _returnvalue_6) false)))
          (:then_1
            ;[0.1 0.1 0.1 1 14] Add starter inventory items.
            (for _array_element_2 (.StarterItems (Utilities|Struct|BreakS_RPG_Hero_Static _returnvalue_7))
              (Default|AddItemtoContainer(byStruct) _returnvalue_5 (Variables|/Game/SuperiorRPGKit/Blueprints/Components/AC_RPG_ItemsManager.AC_RPG_ItemsManager_C|GetInventoryContainer _returnvalue_5) _array_element_2 true (Utilities|Struct|BreakS_RPG_Item_Dynamic _array_element_2))))
          (:then_2
            ;[0.1 0.1 0.1 1 14] Add starter storage items.
            (for _array_element_3 (.StarterStashItems (Utilities|Struct|BreakS_RPG_Hero_Static _returnvalue_7))
              (Default|AddItemtoContainer(byStruct) _returnvalue_4 (Variables|/Game/SuperiorRPGKit/Blueprints/Components/AC_RPG_ItemsManager.AC_RPG_ItemsManager_C|GetPersonalStashContainer _returnvalue_4) _array_element_3 true (Utilities|Struct|BreakS_RPG_Item_Dynamic _array_element_3)))))))))

(event Custom|UploadSkillsSaveData_SERVER
  (params (AcquiredSkills :type Array%20of%20Names) (AcquiredSkillsData :type Array%20of%20S%20RPG%20Skill%20Dynamic%20Structures) (SkillsOnCooldown :type Array%20of%20Names) (CooldownData :type Array%20of%20S%20RPG%20Cooldown%20Structures) (AvailableSkillPoints :type Integer) (TotalSkillPointsSpent :type Integer))
  (Default|LoadSkillsData (Actor|GetComponentbyClass (Components|GetOwner) "/Game/SuperiorRPGKit/Blueprints/Components/AC_RPG_SkillsManager.AC_RPG_SkillsManager_C") AcquiredSkills AcquiredSkillsData SkillsOnCooldown CooldownData AvailableSkillPoints TotalSkillPointsSpent))

(event Custom|UploadQuestsSaveData_SERVER
  (params (FinishedQuests :type Array%20of%20Names) (FinishedQuestsCount :type Array%20of%20Integers) (OngoingQuests :type Array%20of%20Names) (OngoingQuestsData :type Array%20of%20S%20RPG%20Quest%20Dynamic%20Structures) (UnlockedQuests :type Array%20of%20Names) (OngoingObjectives :type Array%20of%20Names))
  (Default|LoadQuestsData (Actor|GetComponentbyClass (Components|GetOwner) "/Game/SuperiorRPGKit/Blueprints/Components/AC_RPG_QuestsManager.AC_RPG_QuestsManager_C") FinishedQuests FinishedQuestsCount OngoingQuests OngoingQuestsData UnlockedQuests OngoingObjectives))

(event Custom|UploadInventorySaveData_SERVER
  (params (InventoryItemSlots :type Array%20of%20Integers) (InventoryItemsData :type Array%20of%20S%20RPG%20Item%20Dynamic%20Structures) (InventoryGold :type Integer))
  (Default|LoadContainerData (Variables|/Game/SuperiorRPGKit/Blueprints/Components/AC_RPG_ItemsManager.AC_RPG_ItemsManager_C|GetInventoryContainer (Actor|GetComponentbyClass (Components|GetOwner) "/Game/SuperiorRPGKit/Blueprints/Components/AC_RPG_ItemsManager.AC_RPG_ItemsManager_C")) InventoryItemSlots InventoryItemsData InventoryGold))

(event Custom|UploadQuickAccessSaveData_SERVER
  (params (QuickAccessSlots :type Array%20of%20Integers) (QuickAccessSlotsData :type Array%20of%20S%20RPG%20Quick%20Slot%20Structures))
  (Default|LoadQuickAccessData (Actor|GetComponentbyClass (Components|GetOwner) "/Game/SuperiorRPGKit/Blueprints/Components/AC_RPG_QuickAccessManager.AC_RPG_QuickAccessManager_C") QuickAccessSlots QuickAccessSlotsData))

(event Custom|FinalizeLoad_SERVER
  (params (HeroName :type String))
  (Variables|Default|SetHeroName HeroName)
  (Default|PerformFullAttributesandStatsRecalculation (Actor|GetComponentbyClass (Components|GetOwner) "/Game/SuperiorRPGKit/Blueprints/Components/AC_RPG_StatsManager.AC_RPG_StatsManager_C"))
  (Default|CallOnLoadFinished))

(event Custom|UploadCraftingSaveData_SERVER
  (params (UnlockedCraftables :type Array%20of%20Names))
  (Default|LoadCraftingData (Actor|GetComponentbyClass (Components|GetOwner) "/Game/SuperiorRPGKit/Blueprints/Components/AC_RPG_CraftingManager.AC_RPG_CraftingManager_C") UnlockedCraftables))

(event Custom|UploadPersonalStashSaveData_SERVER
  (params (PersonalStashItemSlots :type Array%20of%20Integers) (PersonalStashItemsData :type Array%20of%20S%20RPG%20Item%20Dynamic%20Structures) (PersonalStashGold :type Integer))
  (Default|LoadContainerData (Variables|/Game/SuperiorRPGKit/Blueprints/Components/AC_RPG_ItemsManager.AC_RPG_ItemsManager_C|GetPersonalStashContainer (Actor|GetComponentbyClass (Components|GetOwner) "/Game/SuperiorRPGKit/Blueprints/Components/AC_RPG_ItemsManager.AC_RPG_ItemsManager_C")) PersonalStashItemSlots PersonalStashItemsData PersonalStashGold))

(event Custom|UploadBuffsSaveData_SERVER
  (params (Effects :type Array%20of%20E_RPG_EffectType%20Enums :default "NewEnumerator0") (EffectsData :type Array%20of%20S%20RPG%20Effect%20Dynamic%20Structures) (Buffs :type Array%20of%20E_RPG_BuffType%20Enums :default "NewEnumerator0") (BuffsData :type Array%20of%20S%20RPG%20Buff%20Dynamic%20Structures))
  (Default|LoadBuffsData (Actor|GetComponentbyClass (Components|GetOwner) "/Game/SuperiorRPGKit/Blueprints/Components/AC_RPG_StatsManager.AC_RPG_StatsManager_C") Effects EffectsData Buffs BuffsData))

(event Custom|RefreshActiveRespawn_CLIENT
  (params (ActiveRespawn :type BP%20RPG%20Hero%20Respawn%20Object%20Reference))
  (Utilities|IsValid ActiveRespawn
    (:Is%20Valid
      (Utilities|FlowControl|Sequence
        (:then_0
          (bind _activerespawn (Variables|Default|GetActiveRespawn)
            (:then
              (Default|Deactivate _activerespawn))
            (:else)))
        (:then_1
          (bind _output_get (Variables|Default|SetActiveRespawn ActiveRespawn))
          (Default|Activate _output_get))))))

(event Custom|ActivateRespawn_SERVER
  (params (HeroRespawn :type BP%20RPG%20Hero%20Respawn%20Object%20Reference))
  (if (and (Utilities|IsValid HeroRespawn) (!= HeroRespawn (Variables|Default|GetActiveRespawn)))
    (bind _output_get (Variables|Default|SetActiveRespawn HeroRespawn))
    (CallFunction|RefreshActiveRespawnCLIENT _output_get)
    ;[0.1 0.1 0.1 1 14] Every time respawn point is activated set is as global respawn point.
    ; This is used in case new player joins game and his last map was different than current server map, he got different map so spawn point ID also will be different. In this case player that joins the game will be respawned at last Global Spawn point (perhaps closest to other players).
    (bind _activerespawn (Variables|Default|GetActiveRespawn)
      (:then
        (bind _asbp_rpg_game_instance (Utilities|Casting|CastToBP_RPG_GameInstance (Game|GetGameInstance)))
        (Variables|/Game/SuperiorRPGKit/Blueprints/Basics/BP_RPG_GameInstance.BP_RPG_GameInstance_C|SetGlobalSpawnPointID _asbp_rpg_game_instance (Variables|/Game/SuperiorRPGKit/Blueprints/Basics/BP_RPG_HeroRespawn.BP_RPG_HeroRespawn_C|GetRespawnID _activerespawn)))
      (:else))))

(fn SaveHero
  (params (HeroSaveName :type String))
  (bind _returnvalue (SaveGame|LoadGamefromSlot HeroSaveName))
  (bind _asbp_rpg_save_hero (Utilities|Casting|CastToBP_RPG_SAVE_Hero _returnvalue)
    (:then
      (LocalVariables|SetSaveLOCAL _asbp_rpg_save_hero))
    (:CastFailed
      (bind _returnvalue_2 (SaveGame|CreateSaveGameObject "/Game/SuperiorRPGKit/Blueprints/Saves/BP_RPG_SAVE_Hero.BP_RPG_SAVE_Hero_C"))
      (LocalVariables|SetSaveLOCAL _returnvalue_2)))
  (Utilities|FlowControl|Sequence
    (:then_0
      ;[0.1 0.1 0.1 1 14] Save quests data.
      (bind (_finishedquests _finishedquestscount _ongoingquests _ongoingquestsdata _unlockedquests _ongoingobjectives) (Default|GetQuestsDatatoSave (Actor|GetComponentbyClass (Components|GetOwner) "/Game/SuperiorRPGKit/Blueprints/Components/AC_RPG_QuestsManager.AC_RPG_QuestsManager_C")))
      (Variables|/Game/SuperiorRPGKit/Blueprints/Saves/BP_RPG_SAVE_Hero.BP_RPG_SAVE_Hero_C|SetFinishedQuests (LocalVariables|GetSaveLOCAL) _finishedquests)
      (Variables|/Game/SuperiorRPGKit/Blueprints/Saves/BP_RPG_SAVE_Hero.BP_RPG_SAVE_Hero_C|SetFinishedQuestsCount (LocalVariables|GetSaveLOCAL) _finishedquestscount)
      (Variables|/Game/SuperiorRPGKit/Blueprints/Saves/BP_RPG_SAVE_Hero.BP_RPG_SAVE_Hero_C|SetOngoingQuests (LocalVariables|GetSaveLOCAL) _ongoingquests)
      (Variables|/Game/SuperiorRPGKit/Blueprints/Saves/BP_RPG_SAVE_Hero.BP_RPG_SAVE_Hero_C|SetOngoingQuestsData (LocalVariables|GetSaveLOCAL) _ongoingquestsdata)
      (Variables|/Game/SuperiorRPGKit/Blueprints/Saves/BP_RPG_SAVE_Hero.BP_RPG_SAVE_Hero_C|SetUnlockedQuests (LocalVariables|GetSaveLOCAL) _unlockedquests)
      (Variables|/Game/SuperiorRPGKit/Blueprints/Saves/BP_RPG_SAVE_Hero.BP_RPG_SAVE_Hero_C|SetOngoingObjectives (LocalVariables|GetSaveLOCAL) _ongoingobjectives)
      ;[0.1 0.1 0.1 1 14] Save achievements data.
      (bind (_acievements _achievementsprogress) (Default|GetAchievementsDatatoSave (Actor|GetComponentbyClass (Components|GetOwner) "/Game/SuperiorRPGKit/Blueprints/Components/AC_RPG_AchievementsManager.AC_RPG_AchievementsManager_C")))
      (Variables|/Game/SuperiorRPGKit/Blueprints/Saves/BP_RPG_SAVE_Hero.BP_RPG_SAVE_Hero_C|SetAchievements (LocalVariables|GetSaveLOCAL) _acievements)
      (Variables|/Game/SuperiorRPGKit/Blueprints/Saves/BP_RPG_SAVE_Hero.BP_RPG_SAVE_Hero_C|SetAchievementsProgress (LocalVariables|GetSaveLOCAL) _achievementsprogress))
    (:then_1
      ;[0.1 0.1 0.1 1 14] Save stats data.
      (bind (_currentstats _currentstatsvalues _attributes _attributesinvestedpoints _totalattributepointsspent _availableattributepoints _currentlevel _currentexperience) (Default|GetStatsDatatoSave (Actor|GetComponentbyClass (Components|GetOwner) "/Game/SuperiorRPGKit/Blueprints/Components/AC_RPG_StatsManager.AC_RPG_StatsManager_C")))
      (Variables|/Game/SuperiorRPGKit/Blueprints/Saves/BP_RPG_SAVE_Hero.BP_RPG_SAVE_Hero_C|SetCurrentStats (LocalVariables|GetSaveLOCAL) _currentstats)
      (Variables|/Game/SuperiorRPGKit/Blueprints/Saves/BP_RPG_SAVE_Hero.BP_RPG_SAVE_Hero_C|SetCurrentStatsValues (LocalVariables|GetSaveLOCAL) _currentstatsvalues)
      (Variables|/Game/SuperiorRPGKit/Blueprints/Saves/BP_RPG_SAVE_Hero.BP_RPG_SAVE_Hero_C|SetAttributes (LocalVariables|GetSaveLOCAL) _attributes)
      (Variables|/Game/SuperiorRPGKit/Blueprints/Saves/BP_RPG_SAVE_Hero.BP_RPG_SAVE_Hero_C|SetAttributesInvestedPoints (LocalVariables|GetSaveLOCAL) _attributesinvestedpoints)
      (Variables|/Game/SuperiorRPGKit/Blueprints/Saves/BP_RPG_SAVE_Hero.BP_RPG_SAVE_Hero_C|SetTotalAttributePointsSpent (LocalVariables|GetSaveLOCAL) _totalattributepointsspent)
      (Variables|/Game/SuperiorRPGKit/Blueprints/Saves/BP_RPG_SAVE_Hero.BP_RPG_SAVE_Hero_C|SetAvailableAttributePoints (LocalVariables|GetSaveLOCAL) _availableattributepoints)
      (Variables|/Game/SuperiorRPGKit/Blueprints/Saves/BP_RPG_SAVE_Hero.BP_RPG_SAVE_Hero_C|SetCurrentLevel (LocalVariables|GetSaveLOCAL) _currentlevel)
      (Variables|/Game/SuperiorRPGKit/Blueprints/Saves/BP_RPG_SAVE_Hero.BP_RPG_SAVE_Hero_C|SetCurrentExperience (LocalVariables|GetSaveLOCAL) _currentexperience)
      ;[0.1 0.1 0.1 1 14] Save buffs and effects data.
      (bind (_effects _effectsdata _buffs _buffsdata) (Default|GetBuffsDatatoSave (Actor|GetComponentbyClass (Components|GetOwner) "/Game/SuperiorRPGKit/Blueprints/Components/AC_RPG_StatsManager.AC_RPG_StatsManager_C")))
      (Variables|/Game/SuperiorRPGKit/Blueprints/Saves/BP_RPG_SAVE_Hero.BP_RPG_SAVE_Hero_C|SetEffects (LocalVariables|GetSaveLOCAL) _effects)
      (Variables|/Game/SuperiorRPGKit/Blueprints/Saves/BP_RPG_SAVE_Hero.BP_RPG_SAVE_Hero_C|SetEffectsData (LocalVariables|GetSaveLOCAL) _effectsdata)
      (Variables|/Game/SuperiorRPGKit/Blueprints/Saves/BP_RPG_SAVE_Hero.BP_RPG_SAVE_Hero_C|SetBuffs (LocalVariables|GetSaveLOCAL) _buffs)
      (Variables|/Game/SuperiorRPGKit/Blueprints/Saves/BP_RPG_SAVE_Hero.BP_RPG_SAVE_Hero_C|SetBuffsData (LocalVariables|GetSaveLOCAL) _buffsdata)
      ;[0.1 0.1 0.1 1 14] Save perks data.
      (bind (_perks _perkslevels _totalperkpointsspent _availableperkpoints) (Default|GetPerksDatatoSave (Actor|GetComponentbyClass (Components|GetOwner) "/Game/SuperiorRPGKit/Blueprints/Components/AC_RPG_StatsManager.AC_RPG_StatsManager_C")))
      (Variables|/Game/SuperiorRPGKit/Blueprints/Saves/BP_RPG_SAVE_Hero.BP_RPG_SAVE_Hero_C|SetPerks (LocalVariables|GetSaveLOCAL) _perks)
      (Variables|/Game/SuperiorRPGKit/Blueprints/Saves/BP_RPG_SAVE_Hero.BP_RPG_SAVE_Hero_C|SetPerksLevels (LocalVariables|GetSaveLOCAL) _perkslevels)
      (Variables|/Game/SuperiorRPGKit/Blueprints/Saves/BP_RPG_SAVE_Hero.BP_RPG_SAVE_Hero_C|SetTotalPerkPointsSpent (LocalVariables|GetSaveLOCAL) _totalperkpointsspent)
      (Variables|/Game/SuperiorRPGKit/Blueprints/Saves/BP_RPG_SAVE_Hero.BP_RPG_SAVE_Hero_C|SetAvailablePerkPoints (LocalVariables|GetSaveLOCAL) _availableperkpoints))
    (:then_2
      ;[0.1 0.1 0.1 1 14] Save inventory data.
      (bind (_itemsslots _itemsdata _gold) (Default|GetContainerDatatoSave (Variables|/Game/SuperiorRPGKit/Blueprints/Components/AC_RPG_ItemsManager.AC_RPG_ItemsManager_C|GetInventoryContainer (Actor|GetComponentbyClass (Components|GetOwner) "/Game/SuperiorRPGKit/Blueprints/Components/AC_RPG_ItemsManager.AC_RPG_ItemsManager_C"))))
      (Variables|/Game/SuperiorRPGKit/Blueprints/Saves/BP_RPG_SAVE_Hero.BP_RPG_SAVE_Hero_C|SetInventoryItemSlots (LocalVariables|GetSaveLOCAL) _itemsslots)
      (Variables|/Game/SuperiorRPGKit/Blueprints/Saves/BP_RPG_SAVE_Hero.BP_RPG_SAVE_Hero_C|SetInventoryItemsData (LocalVariables|GetSaveLOCAL) _itemsdata)
      (Variables|/Game/SuperiorRPGKit/Blueprints/Saves/BP_RPG_SAVE_Hero.BP_RPG_SAVE_Hero_C|SetInventoryGold (LocalVariables|GetSaveLOCAL) _gold)
      ;[0.1 0.1 0.1 1 14] Save personal storage data.
      (bind (_itemsslots_2 _itemsdata_2 _gold_2) (Default|GetContainerDatatoSave (Variables|/Game/SuperiorRPGKit/Blueprints/Components/AC_RPG_ItemsManager.AC_RPG_ItemsManager_C|GetPersonalStashContainer (Actor|GetComponentbyClass (Components|GetOwner) "/Game/SuperiorRPGKit/Blueprints/Components/AC_RPG_ItemsManager.AC_RPG_ItemsManager_C"))))
      (Variables|/Game/SuperiorRPGKit/Blueprints/Saves/BP_RPG_SAVE_Hero.BP_RPG_SAVE_Hero_C|SetPersonalStashItemSlots (LocalVariables|GetSaveLOCAL) _itemsslots_2)
      (Variables|/Game/SuperiorRPGKit/Blueprints/Saves/BP_RPG_SAVE_Hero.BP_RPG_SAVE_Hero_C|SetPersonalStashItemsData (LocalVariables|GetSaveLOCAL) _itemsdata_2)
      (Variables|/Game/SuperiorRPGKit/Blueprints/Saves/BP_RPG_SAVE_Hero.BP_RPG_SAVE_Hero_C|SetPersonalStashGold (LocalVariables|GetSaveLOCAL) _gold_2)
      ;[0.1 0.1 0.1 1 14] Save equipment data.
      (bind (_equippeditemsslots _equippeditemsdata) (Default|GetEquipmentDatatoSave (Variables|/Game/SuperiorRPGKit/Blueprints/Components/AC_RPG_ItemsManager.AC_RPG_ItemsManager_C|GetEquipment (Actor|GetComponentbyClass (Components|GetOwner) "/Game/SuperiorRPGKit/Blueprints/Components/AC_RPG_ItemsManager.AC_RPG_ItemsManager_C"))))
      (Variables|/Game/SuperiorRPGKit/Blueprints/Saves/BP_RPG_SAVE_Hero.BP_RPG_SAVE_Hero_C|SetEquippedItemSlots (LocalVariables|GetSaveLOCAL) _equippeditemsslots)
      (Variables|/Game/SuperiorRPGKit/Blueprints/Saves/BP_RPG_SAVE_Hero.BP_RPG_SAVE_Hero_C|SetEquippedItemsData (LocalVariables|GetSaveLOCAL) _equippeditemsdata)
      ;[0.1 0.1 0.1 1 14] Save crafting data.
      (bind _unlockedcraftables (Default|GetCraftingDatatoSave (Actor|GetComponentbyClass (Components|GetOwner) "/Game/SuperiorRPGKit/Blueprints/Components/AC_RPG_CraftingManager.AC_RPG_CraftingManager_C")))
      (Variables|/Game/SuperiorRPGKit/Blueprints/Saves/BP_RPG_SAVE_Hero.BP_RPG_SAVE_Hero_C|SetUnlockedCraftables (LocalVariables|GetSaveLOCAL) _unlockedcraftables))
    (:then_3
      ;[0.1 0.1 0.1 1 14] Save quick access bar data.
      (bind (_quickaccessslots _quickaccessslotsdata) (Default|GetQuickAccessDatatoSave (Actor|GetComponentbyClass (Components|GetOwner) "/Game/SuperiorRPGKit/Blueprints/Components/AC_RPG_QuickAccessManager.AC_RPG_QuickAccessManager_C")))
      (Variables|/Game/SuperiorRPGKit/Blueprints/Saves/BP_RPG_SAVE_Hero.BP_RPG_SAVE_Hero_C|SetQuickAccessSlots (LocalVariables|GetSaveLOCAL) _quickaccessslots)
      (Variables|/Game/SuperiorRPGKit/Blueprints/Saves/BP_RPG_SAVE_Hero.BP_RPG_SAVE_Hero_C|SetQuickAccessSlotsData (LocalVariables|GetSaveLOCAL) _quickaccessslotsdata)
      ;[0.1 0.1 0.1 1 14] Save skills data.
      (bind (_acquiredskills _acquiredskillsdata _skillsoncooldown _cooldowndata _availableskillpoints _totalskillpointsspent) (Default|GetSkillsDatatoSave (Actor|GetComponentbyClass (Components|GetOwner) "/Game/SuperiorRPGKit/Blueprints/Components/AC_RPG_SkillsManager.AC_RPG_SkillsManager_C") true))
      (Variables|/Game/SuperiorRPGKit/Blueprints/Saves/BP_RPG_SAVE_Hero.BP_RPG_SAVE_Hero_C|SetAcquiredSkills (LocalVariables|GetSaveLOCAL) _acquiredskills)
      (Variables|/Game/SuperiorRPGKit/Blueprints/Saves/BP_RPG_SAVE_Hero.BP_RPG_SAVE_Hero_C|SetAcquiredSkillsData (LocalVariables|GetSaveLOCAL) _acquiredskillsdata)
      (Variables|/Game/SuperiorRPGKit/Blueprints/Saves/BP_RPG_SAVE_Hero.BP_RPG_SAVE_Hero_C|SetSkillsOnCooldown (LocalVariables|GetSaveLOCAL) _skillsoncooldown)
      (Variables|/Game/SuperiorRPGKit/Blueprints/Saves/BP_RPG_SAVE_Hero.BP_RPG_SAVE_Hero_C|SetCooldownData (LocalVariables|GetSaveLOCAL) _cooldowndata)
      (Variables|/Game/SuperiorRPGKit/Blueprints/Saves/BP_RPG_SAVE_Hero.BP_RPG_SAVE_Hero_C|SetAvailableSkillPoints (LocalVariables|GetSaveLOCAL) _availableskillpoints)
      (Variables|/Game/SuperiorRPGKit/Blueprints/Saves/BP_RPG_SAVE_Hero.BP_RPG_SAVE_Hero_C|SetTotalSkillPointsSpent (LocalVariables|GetSaveLOCAL) _totalskillpointsspent))
    (:then_4
      ;[0.1 0.1 0.1 1 14] Save hero basic data, map and respawn point.
      (Variables|/Game/SuperiorRPGKit/Blueprints/Saves/BP_RPG_SAVE_Hero.BP_RPG_SAVE_Hero_C|SetHeroID (LocalVariables|GetSaveLOCAL) (Variables|/Game/SuperiorRPGKit/Blueprints/Components/AC_RPG_StatsManager.AC_RPG_StatsManager_C|GetCharacterID (Actor|GetComponentbyClass (Components|GetOwner) "/Game/SuperiorRPGKit/Blueprints/Components/AC_RPG_StatsManager.AC_RPG_StatsManager_C")))
      (Variables|/Game/SuperiorRPGKit/Blueprints/Saves/BP_RPG_SAVE_Hero.BP_RPG_SAVE_Hero_C|SetAddStarterStuff (LocalVariables|GetSaveLOCAL) false)
      (bind _activerespawn (Variables|Default|GetActiveRespawn)
        (:then
          (Variables|/Game/SuperiorRPGKit/Blueprints/Saves/BP_RPG_SAVE_Hero.BP_RPG_SAVE_Hero_C|SetSpawnID (LocalVariables|GetSaveLOCAL) (Variables|/Game/SuperiorRPGKit/Blueprints/Basics/BP_RPG_HeroRespawn.BP_RPG_HeroRespawn_C|GetRespawnID _activerespawn))
          (bind _returnvalue_3 (Game|GetCurrentLevelName true))
          (Variables|/Game/SuperiorRPGKit/Blueprints/Saves/BP_RPG_SAVE_Hero.BP_RPG_SAVE_Hero_C|SetMapName (LocalVariables|GetSaveLOCAL) (Utilities|String|StringToName _returnvalue_3)))
        (:else)))
    (:then_5
      (SaveGame|SaveGametoSlot (LocalVariables|GetSaveLOCAL) HeroSaveName) ; Save to file.
    )))

(fn LoadHero
  (params (HeroSaveName :type String))
  (bind _returnvalue (SaveGame|LoadGamefromSlot HeroSaveName))
  (bind _asbp_rpg_save_hero (Utilities|Casting|CastToBP_RPG_SAVE_Hero _returnvalue)
    (:then
      (LocalVariables|SetSaveLOCAL _asbp_rpg_save_hero))
    (:CastFailed
      ;[0.1 0.1 0.1 1 14] Create placeholder save in case it failed to load. This is mainly for development purposes because proper save will be loaded only if you select hero from main menu and it would be tedious to start from main menu each time we want to test small thing on the map.
      ; In this case if we start on the map directly it will fail to load and create empty hero data.
      (bind _returnvalue_2 (SaveGame|CreateSaveGameObject "/Game/SuperiorRPGKit/Blueprints/Saves/BP_RPG_SAVE_Hero.BP_RPG_SAVE_Hero_C"))
      (LocalVariables|SetSaveLOCAL _returnvalue_2)))
  (Utilities|FlowControl|Sequence
    (:then_0
      ;[0.1 0.1 0.1 1 14] Send quests data to server.
      (CallFunction|UploadQuestsSaveDataSERVER (Variables|/Game/SuperiorRPGKit/Blueprints/Saves/BP_RPG_SAVE_Hero.BP_RPG_SAVE_Hero_C|GetFinishedQuests (LocalVariables|GetSaveLOCAL)) (Variables|/Game/SuperiorRPGKit/Blueprints/Saves/BP_RPG_SAVE_Hero.BP_RPG_SAVE_Hero_C|GetFinishedQuestsCount (LocalVariables|GetSaveLOCAL)) (Variables|/Game/SuperiorRPGKit/Blueprints/Saves/BP_RPG_SAVE_Hero.BP_RPG_SAVE_Hero_C|GetOngoingQuests (LocalVariables|GetSaveLOCAL)) (Variables|/Game/SuperiorRPGKit/Blueprints/Saves/BP_RPG_SAVE_Hero.BP_RPG_SAVE_Hero_C|GetOngoingQuestsData (LocalVariables|GetSaveLOCAL)) (Variables|/Game/SuperiorRPGKit/Blueprints/Saves/BP_RPG_SAVE_Hero.BP_RPG_SAVE_Hero_C|GetUnlockedQuests (LocalVariables|GetSaveLOCAL)) (Variables|/Game/SuperiorRPGKit/Blueprints/Saves/BP_RPG_SAVE_Hero.BP_RPG_SAVE_Hero_C|GetOngoingObjectives (LocalVariables|GetSaveLOCAL)))
      ;[0.1 0.1 0.1 1 14] Send achievements data to server
      (CallFunction|UploadAchievementsSaveDataSERVER (Variables|/Game/SuperiorRPGKit/Blueprints/Saves/BP_RPG_SAVE_Hero.BP_RPG_SAVE_Hero_C|GetAchievements (LocalVariables|GetSaveLOCAL)) (Variables|/Game/SuperiorRPGKit/Blueprints/Saves/BP_RPG_SAVE_Hero.BP_RPG_SAVE_Hero_C|GetAchievementsProgress (LocalVariables|GetSaveLOCAL))))
    (:then_1
      ;[0.1 0.1 0.1 1 14] Send inventory data to server.
      (CallFunction|UploadInventorySaveDataSERVER (Variables|/Game/SuperiorRPGKit/Blueprints/Saves/BP_RPG_SAVE_Hero.BP_RPG_SAVE_Hero_C|GetInventoryItemSlots (LocalVariables|GetSaveLOCAL)) (Variables|/Game/SuperiorRPGKit/Blueprints/Saves/BP_RPG_SAVE_Hero.BP_RPG_SAVE_Hero_C|GetInventoryItemsData (LocalVariables|GetSaveLOCAL)) (Variables|/Game/SuperiorRPGKit/Blueprints/Saves/BP_RPG_SAVE_Hero.BP_RPG_SAVE_Hero_C|GetInventoryGold (LocalVariables|GetSaveLOCAL)))
      ;[0.1 0.1 0.1 1 14] Send personal storage data to server.
      (CallFunction|UploadPersonalStashSaveDataSERVER (Variables|/Game/SuperiorRPGKit/Blueprints/Saves/BP_RPG_SAVE_Hero.BP_RPG_SAVE_Hero_C|GetPersonalStashItemSlots (LocalVariables|GetSaveLOCAL)) (Variables|/Game/SuperiorRPGKit/Blueprints/Saves/BP_RPG_SAVE_Hero.BP_RPG_SAVE_Hero_C|GetPersonalStashItemsData (LocalVariables|GetSaveLOCAL)) (Variables|/Game/SuperiorRPGKit/Blueprints/Saves/BP_RPG_SAVE_Hero.BP_RPG_SAVE_Hero_C|GetPersonalStashGold (LocalVariables|GetSaveLOCAL)))
      ;[0.1 0.1 0.1 1 14] Send equipment data to server.
      (CallFunction|UploadEquipmentSaveDataSERVER (Variables|/Game/SuperiorRPGKit/Blueprints/Saves/BP_RPG_SAVE_Hero.BP_RPG_SAVE_Hero_C|GetEquippedItemSlots (LocalVariables|GetSaveLOCAL)) (Variables|/Game/SuperiorRPGKit/Blueprints/Saves/BP_RPG_SAVE_Hero.BP_RPG_SAVE_Hero_C|GetEquippedItemsData (LocalVariables|GetSaveLOCAL)))
      ;[0.1 0.1 0.1 1 14] Send crafting data to server.
      (CallFunction|UploadCraftingSaveDataSERVER (Variables|/Game/SuperiorRPGKit/Blueprints/Saves/BP_RPG_SAVE_Hero.BP_RPG_SAVE_Hero_C|GetUnlockedCraftables (LocalVariables|GetSaveLOCAL))))
    (:then_2
      ;[0.1 0.1 0.1 1 14] Send quick access bar data to server.
      (CallFunction|UploadQuickAccessSaveDataSERVER (Variables|/Game/SuperiorRPGKit/Blueprints/Saves/BP_RPG_SAVE_Hero.BP_RPG_SAVE_Hero_C|GetQuickAccessSlots (LocalVariables|GetSaveLOCAL)) (Variables|/Game/SuperiorRPGKit/Blueprints/Saves/BP_RPG_SAVE_Hero.BP_RPG_SAVE_Hero_C|GetQuickAccessSlotsData (LocalVariables|GetSaveLOCAL)))
      ;[0.1 0.1 0.1 1 14] Send skills data to server.
      (CallFunction|UploadSkillsSaveDataSERVER (Variables|/Game/SuperiorRPGKit/Blueprints/Saves/BP_RPG_SAVE_Hero.BP_RPG_SAVE_Hero_C|GetAcquiredSkills (LocalVariables|GetSaveLOCAL)) (Variables|/Game/SuperiorRPGKit/Blueprints/Saves/BP_RPG_SAVE_Hero.BP_RPG_SAVE_Hero_C|GetAcquiredSkillsData (LocalVariables|GetSaveLOCAL)) (Variables|/Game/SuperiorRPGKit/Blueprints/Saves/BP_RPG_SAVE_Hero.BP_RPG_SAVE_Hero_C|GetSkillsOnCooldown (LocalVariables|GetSaveLOCAL)) (Variables|/Game/SuperiorRPGKit/Blueprints/Saves/BP_RPG_SAVE_Hero.BP_RPG_SAVE_Hero_C|GetCooldownData (LocalVariables|GetSaveLOCAL)) (Variables|/Game/SuperiorRPGKit/Blueprints/Saves/BP_RPG_SAVE_Hero.BP_RPG_SAVE_Hero_C|GetAvailableSkillPoints (LocalVariables|GetSaveLOCAL)) (Variables|/Game/SuperiorRPGKit/Blueprints/Saves/BP_RPG_SAVE_Hero.BP_RPG_SAVE_Hero_C|GetTotalSkillPointsSpent (LocalVariables|GetSaveLOCAL))))
    (:then_3
      ;[0.1 0.1 0.1 1 14] Send buffs and effects data to server.
      (CallFunction|UploadBuffsSaveDataSERVER (Variables|/Game/SuperiorRPGKit/Blueprints/Saves/BP_RPG_SAVE_Hero.BP_RPG_SAVE_Hero_C|GetEffects (LocalVariables|GetSaveLOCAL)) (Variables|/Game/SuperiorRPGKit/Blueprints/Saves/BP_RPG_SAVE_Hero.BP_RPG_SAVE_Hero_C|GetEffectsData (LocalVariables|GetSaveLOCAL)) (Variables|/Game/SuperiorRPGKit/Blueprints/Saves/BP_RPG_SAVE_Hero.BP_RPG_SAVE_Hero_C|GetBuffs (LocalVariables|GetSaveLOCAL)) (Variables|/Game/SuperiorRPGKit/Blueprints/Saves/BP_RPG_SAVE_Hero.BP_RPG_SAVE_Hero_C|GetBuffsData (LocalVariables|GetSaveLOCAL)))
      ;[0.1 0.1 0.1 1 14] Send stats data to server.
      (CallFunction|UploadStatsSaveDataSERVER (Variables|/Game/SuperiorRPGKit/Blueprints/Saves/BP_RPG_SAVE_Hero.BP_RPG_SAVE_Hero_C|GetCurrentStats (LocalVariables|GetSaveLOCAL)) (Variables|/Game/SuperiorRPGKit/Blueprints/Saves/BP_RPG_SAVE_Hero.BP_RPG_SAVE_Hero_C|GetCurrentStatsValues (LocalVariables|GetSaveLOCAL)) (Variables|/Game/SuperiorRPGKit/Blueprints/Saves/BP_RPG_SAVE_Hero.BP_RPG_SAVE_Hero_C|GetAttributes (LocalVariables|GetSaveLOCAL)) (Variables|/Game/SuperiorRPGKit/Blueprints/Saves/BP_RPG_SAVE_Hero.BP_RPG_SAVE_Hero_C|GetAttributesInvestedPoints (LocalVariables|GetSaveLOCAL)) (Variables|/Game/SuperiorRPGKit/Blueprints/Saves/BP_RPG_SAVE_Hero.BP_RPG_SAVE_Hero_C|GetTotalAttributePointsSpent (LocalVariables|GetSaveLOCAL)) (Variables|/Game/SuperiorRPGKit/Blueprints/Saves/BP_RPG_SAVE_Hero.BP_RPG_SAVE_Hero_C|GetAvailableAttributePoints (LocalVariables|GetSaveLOCAL)) (Variables|/Game/SuperiorRPGKit/Blueprints/Saves/BP_RPG_SAVE_Hero.BP_RPG_SAVE_Hero_C|GetCurrentLevel (LocalVariables|GetSaveLOCAL)) (Variables|/Game/SuperiorRPGKit/Blueprints/Saves/BP_RPG_SAVE_Hero.BP_RPG_SAVE_Hero_C|GetCurrentExperience (LocalVariables|GetSaveLOCAL)))
      ;[0.1 0.1 0.1 1 14] Send perks data to server.
      (CallFunction|UploadPerksSaveDataSERVER (Variables|/Game/SuperiorRPGKit/Blueprints/Saves/BP_RPG_SAVE_Hero.BP_RPG_SAVE_Hero_C|GetPerks (LocalVariables|GetSaveLOCAL)) (Variables|/Game/SuperiorRPGKit/Blueprints/Saves/BP_RPG_SAVE_Hero.BP_RPG_SAVE_Hero_C|GetPerksLevels (LocalVariables|GetSaveLOCAL)) (Variables|/Game/SuperiorRPGKit/Blueprints/Saves/BP_RPG_SAVE_Hero.BP_RPG_SAVE_Hero_C|GetTotalAttributePointsSpent (LocalVariables|GetSaveLOCAL)) (Variables|/Game/SuperiorRPGKit/Blueprints/Saves/BP_RPG_SAVE_Hero.BP_RPG_SAVE_Hero_C|GetAvailablePerkPoints (LocalVariables|GetSaveLOCAL))))
    (:then_4
      ;[0.1 0.1 0.1 1 14] Tell server to add (or to not) starter items to hero.
      (CallFunction|AddStarterStuffSERVER (Variables|/Game/SuperiorRPGKit/Blueprints/Saves/BP_RPG_SAVE_Hero.BP_RPG_SAVE_Hero_C|GetAddStarterStuff (LocalVariables|GetSaveLOCAL)) (Variables|/Game/SuperiorRPGKit/Blueprints/Components/AC_RPG_StatsManager.AC_RPG_StatsManager_C|GetCharacterID (Actor|GetComponentbyClass (Components|GetOwner) "/Game/SuperiorRPGKit/Blueprints/Components/AC_RPG_StatsManager.AC_RPG_StatsManager_C"))))
    (:then_5
      ;[0.1 0.1 0.1 1 14] Finalize hero load.
      (CallFunction|FinalizeLoadSERVER (Variables|/Game/SuperiorRPGKit/Blueprints/Saves/BP_RPG_SAVE_Hero.BP_RPG_SAVE_Hero_C|GetHeroName (LocalVariables|GetSaveLOCAL))))))

(fn FindRespawnwithID
  (params (RespawnID :type Name))
  (bind _outactors (Actor|GetAllActorsOfClass "/Game/SuperiorRPGKit/Blueprints/Basics/BP_RPG_HeroRespawn.BP_RPG_HeroRespawn_C"))
  (bind _array_element (Utilities|Array|ForEachLoopwithBreak _outactors :!label _label)
    (:LoopBody
      (if (Utilities|Name|Equal(Name) (Variables|/Game/SuperiorRPGKit/Blueprints/Basics/BP_RPG_HeroRespawn.BP_RPG_HeroRespawn_C|GetRespawnID _array_element) RespawnID)
        (LocalVariables|SetRespawnLOCAL _array_element)
        (LocalVariables|SetSuccessLOCAL true)
        (goto _label Break)))
    (:Completed
      (return (LocalVariables|GetSuccessLOCAL) (LocalVariables|GetRespawnLOCAL)))))